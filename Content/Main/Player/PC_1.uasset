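; Player controller for a mouse-driven game with a pannable camera, where right click sets a move target and left click sets a shooting location.
; Clicks trace WorldStatic under the cursor, store the hit point and spawn a marker actor there; BeginPlay seeds the move target from BP_PlayerPawn's location.
; An axis event blends axis input with depth-scaled screen-edge scrolling, smooths it exponentially and feeds it to the controlled pawn as movement input.
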(event EventBeginPlay
  ;[1 1 1] Коэффициенты
  (Variables|Default|SetViewportEdgeThreshold 0.1)
  (Variables|Default|SetMouseLeftScale 1.0)
  (Variables|Default|SetMouseForwardScale 1.0)
  (bind _returnvalue (Actor|GetActorOfClass "/Game/Main/Player/BP_PlayerPawn.BP_PlayerPawn_C"))
  (bind _asbp_player_pawn (Utilities|Casting|CastToBP_PlayerPawn _returnvalue)
    (:then
      (Development|PrintString (Utilities|String|ToString(Vector) (Transformation|GetActorLocation _returnvalue)))
      (Variables|Default|SetMoveTargetLocation (Transformation|GetActorLocation _returnvalue)))
    (:CastFailed
      (Development|PrintString "Kill me"))))

(event Input|AxisEvents|InputAxisCameraMoveForward
  (params (AxisValue :type Float%20%28single-precision%29))
  ;[1 1 1] Управление камерой с помощью мыши
)

(event Input|AxisEvents|InputAxisCameraMoveLeft
  (params (AxisValue :type Float%20%28single-precision%29))
  ;[1 1 1] Управление камерой с клавиатуры WASD
)

(event Input|AxisEvents|InputAxisCameraMoveMouse
  (params (AxisValue :type Float%20%28single-precision%29))
  (bind (_locationx _locationy) (Game|Player|GetMousePosition))
  (bind _returnvalue (Viewport|GetViewportSize))
  (bind _returnvalue_2 (Pawn|GetControlledPawn))
  (bind _mouseforwardscale (Variables|Default|GetMouseForwardScale))
  (bind _mouseleftscale (Variables|Default|GetMouseLeftScale))
  (bind _viewportedgethreshold (Variables|Default|GetViewportEdgeThreshold))
  (bind _camerasmoothkoeff (Variables|Default|GetCameraSmoothKoeff))
  (bind _returnvalue_3 (/ _locationy (.y _returnvalue)))
  (bind _returnvalue_4 (- 1.0 _viewportedgethreshold))
  (bind _returnvalue_5 (/ _locationx (.x _returnvalue)))
  ;[1 1 1] Управление камерой с помощью мыши
  (CallFunction|SmoothMovenentCamera)
  ;[1 1 1] Фильр сглаживания камеры
  (bind _output_get (Variables|Default|SetCameraSmoothX (+ (* (Variables|Default|GetCameraSmoothX) (- 1.0 _camerasmoothkoeff)) (* (+ (stale Input|AxisEvents|InputAxisCameraMoveForward AxisValue) (Math|Float|SelectFloat (* _mouseforwardscale -1.0) (Math|Float|SelectFloat _mouseforwardscale 0.0 (< _returnvalue_3 _viewportedgethreshold)) (> _returnvalue_3 _returnvalue_4))) _camerasmoothkoeff))))
  (bind _output_get_2 (Variables|Default|SetCameraSmoothY (+ (* (Variables|Default|GetCameraSmoothY) (- 1.0 _camerasmoothkoeff)) (* (+ (* (stale Input|AxisEvents|InputAxisCameraMoveLeft AxisValue) -1.0) (Math|Float|SelectFloat _mouseleftscale (Math|Float|SelectFloat (* _mouseleftscale -1.0) 0.0 (< _returnvalue_5 _viewportedgethreshold)) (> _returnvalue_5 _returnvalue_4))) _camerasmoothkoeff))))
  ;[1 1 1] Движение камеры
  (Pawn|Input|AddMovementInput _returnvalue_2 "0.000000,1.000000,0.000000" _output_get_2 false)
  (Pawn|Input|AddMovementInput _returnvalue_2 "1.000000,0.000000,0.000000" _output_get false))

(event Input|MouseEvents|MouseWheelDown
  (params (Key :type Key%20Structure :default "None"))
  ;[1 1 1] Управление камерой с помощью колёсика мыши
)

(event Input|MouseEvents|RightMouseButton
  (params (Key :type Key%20Structure :default "None"))
  (bind _array (Utilities|Array|MakeArray "ObjectTypeQuery1"))
  (bind _hitresult (Class|PlayerController|GetHitResultUnderCursorforObjects _array true))
  (bind _location (Collision|BreakHitResult _hitresult))
  ;[1 1 1] Управление персонажем правой кнопкой мыши
  (:Pressed
    (CallFunction|SpawnMousePosition (Math|Conversions|ToTransform(Vector) _location))
    (Variables|Default|SetMoveTargetLocation _location)))

(event Input|MouseEvents|LeftMouseButton
  (params (Key :type Key%20Structure :default "None"))
  (bind _array (Utilities|Array|MakeArray "ObjectTypeQuery1"))
  (bind _hitresult (Class|PlayerController|GetHitResultUnderCursorforObjects _array true))
  (bind _location (Collision|BreakHitResult _hitresult))
  ;[1 1 1] Управление персонажем левой кнопкой мыши
  (:Pressed
    (CallFunction|SpawnMousePosition2 (Math|Conversions|ToTransform(Vector) _location))
    (Variables|Default|SetShootingLocation _location)))

(event Input|MouseEvents|MouseWheelUp
  (params (Key :type Key%20Structure :default "None"))
  ;[1 1 1] Управление камерой с помощью колёсика мыши
)

(fn ConstructionScript)

(fn SmoothMovenentCamera
  (bind (_locationx _locationy) (Game|Player|GetMousePosition))
  (bind _returnvalue (Viewport|GetViewportSize))
  (bind _viewportedgethreshold (Variables|Default|GetViewportEdgeThreshold))
  (bind _viewportedgethreshold_2 (Variables|Default|GetViewportEdgeThreshold))
  (bind _viewportedgethreshold_3 (Variables|Default|GetViewportEdgeThreshold))
  (bind _returnvalue_2 (/ _locationx (.x _returnvalue)))
  (bind _returnvalue_3 (/ _locationy (.y _returnvalue)))
  (bind _returnvalue_4 (- 1.0 _viewportedgethreshold))
  (bind _output_get (Variables|Default|SetMouseLeftScale (Math|Float|SelectFloat (/ (- _returnvalue_2 _returnvalue_4) _viewportedgethreshold_3) (Math|Float|SelectFloat (* (/ (- _returnvalue_2 _viewportedgethreshold_3) _viewportedgethreshold_3) -1.0) 0.0 (< _returnvalue_2 _viewportedgethreshold)) (> _returnvalue_2 _returnvalue_4))))
  (bind _output_get_2 (Variables|Default|SetMouseForwardScale (Math|Float|SelectFloat (/ (- _returnvalue_3 _returnvalue_4) _viewportedgethreshold_2) (Math|Float|SelectFloat (* (/ (- _returnvalue_3 _viewportedgethreshold_2) _viewportedgethreshold_2) -1.0) 0.0 (< _returnvalue_3 _viewportedgethreshold)) (> _returnvalue_3 _returnvalue_4)))))

(fn SpawnMousePosition
  (params (SpawnTransform :type Transform))
  (Game|SpawnActorfromClass "/Game/Main/Player/BP_MousePosition.BP_MousePosition_C" SpawnTransform "AlwaysSpawn" "MultiplyWithRoot" 0 0))

(fn SpawnMousePosition2
  (params (SpawnTransform :type Transform))
  (Game|SpawnActorfromClass "/Game/Main/Player/BP_MousePosition2.BP_MousePosition2_C" SpawnTransform "Undefined" "MultiplyWithRoot" 0 0))