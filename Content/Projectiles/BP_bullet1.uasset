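; Bullet projectile actor that flies forward and damages whatever it overlaps.
; Tick moves it along its local X axis by BulletVelocity scaled with delta time, without sweeping.
; When its Sphere overlaps an actor, it applies Damage with its owner as causer, spawns a small explosion effect and sound, then destroys itself.
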(event OnComponentBeginOverlap(Sphere)
  (params (OverlappedComponent :type Primitive%20Component%20Object%20Reference) (OtherActor :type Actor%20Object%20Reference) (OtherComp :type Primitive%20Component%20Object%20Reference) (OtherBodyIndex :type Integer) (bFromSweep :type Boolean) (SweepResult :type Hit%20Result%20Structure%20%28by%20ref%29))
  (bind _returnvalue (Transformation|GetActorLocation))
  (Game|Damage|ApplyDamage OtherActor (Variables|Default|GetDamage) 0 (Components|GetOwner))
  (Effects|SpawnEmitteratLocation "/Game/StarterContent/Particles/P_Explosion.P_Explosion" _returnvalue "0, 0, 0" "0.300000,0.300000,0.300000")
  (Audio|SpawnSoundatLocation "/Game/StarterContent/Audio/Explosion_Cue.Explosion_Cue" _returnvalue "0, 0, 0" 2.0 2.0 0.0 0 0)
  (Actor|DestroyActor))

(event EventBeginPlay)

(event Collision|EventActorBeginOverlap
  (params (OtherActor :type Actor%20Object%20Reference)))

(event EventTick
  (params (DeltaSeconds :type Float%20%28single-precision%29))
  (Transformation|AddActorLocalOffset (Math|Vector|MakeVector (* (Variables|Default|GetBulletVelocity) DeltaSeconds) 0.0 0.0) false false))

(fn ConstructionScript)