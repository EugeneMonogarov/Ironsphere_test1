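; BP_CrateObjective is a child Blueprint in the mission destruction set, apparently a destructible crate used as an objective.
; It relies on its parent for all behavior, as its event graph holds only disabled default events.
; The SoundDamage override always passes a fixed enum value to the parent.
; The Destruction override forwards damage, radius and sound, but leaves its IsBlow input unconnected.
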(event EventBeginPlay
  (|CallParentFunction) ; This node is disabled and will not be called.\nDrag off pins to build functionality.
)

(event Collision|EventActorBeginOverlap
  (params (OtherActor :type Actor%20Object%20Reference))
  (|CallParentFunction OtherActor) ; This node is disabled and will not be called.\nDrag off pins to build functionality.
)

(event EventTick
  (params (DeltaSeconds :type Float%20%28single-precision%29))
  (|CallParentFunction DeltaSeconds) ; This node is disabled and will not be called.\nDrag off pins to build functionality.
)

(fn ConstructionScript
  (|CallParentFunction))

(fn SoundDamage
  (params (SoundDamage :type SoundDamage%20Enum :default "NewEnumerator0"))
  (|CallParentFunction "NewEnumerator0"))

(fn Destruction
  (params (IsBlow :type Boolean) (Damage :type Float%20%28double-precision%29) (Radius :type Float%20%28double-precision%29) (Sound :type SoundDestroy%20Enum :default "NewEnumerator0"))
  (|CallParentFunction false Damage Radius Sound))