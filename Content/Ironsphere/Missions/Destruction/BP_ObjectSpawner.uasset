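; BP_ObjectSpawner is a placement point for the Destruction mission that turns itself into an objective or other mission actor.
; Each Tick, it removes itself if the player is within 300 units, otherwise randomly attempts a spawn using BP_MissionDestruction's remaining quotas.
; Objectives fill first, then dens, delayed instants or hides, with hides also spawning BP_MissionDen.
; A successful spawn decrements its quota and destroys the spawner.
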(event EventBeginPlay)

(event Collision|EventActorBeginOverlap
  (params (OtherActor :type Actor%20Object%20Reference)))

(event EventTick
  (params (DeltaSeconds :type Float%20%28single-precision%29))
  (bind _outactors (Actor|GetAllActorsOfClass "/Game/Ironsphere/Core/Player/BP_CharacterPlayer.BP_CharacterPlayer_C"))
  (if (< (Math|Vector|VectorLength (- (Transformation|GetActorLocation (Utilities|Array|Get(acopy) _outactors)) (Transformation|GetActorLocation))) 3e+02)
    (Actor|DestroyActor)
    (else
      (bind _returnvalue (Actor|GetActorOfClass "/Game/Ironsphere/Missions/Destruction/BP_MissionDestruction.BP_MissionDestruction_C"))
      (if (> (Variables|/Game/Ironsphere/Missions/Destruction/BP_MissionDestruction.BP_MissionDestruction_C|GetNumberOfObjectives _returnvalue) 0)
        (if (> (Math|Random|RandomFloatinRange 0.0 1.0) 0.9)
          (Utilities|FlowControl|Sequence
            (:then_0
              (bind _returnvalue_2 (Game|SpawnActorfromClass (Variables|/Game/Ironsphere/Missions/Destruction/BP_MissionDestruction.BP_MissionDestruction_C|GetObject _returnvalue) (Transformation|GetActorTransform) "Undefined" "MultiplyWithRoot" 0 true 1e+01 1e+01 0)))
            (:then_1
              (bind _returnvalue_3 (Actor|GetActorOfClass "/Game/Ironsphere/Missions/Destruction/BP_MissionDestruction.BP_MissionDestruction_C"))
              (Math|Integer|DecrementInt (Variables|/Game/Ironsphere/Missions/Destruction/BP_MissionDestruction.BP_MissionDestruction_C|GetNumberOfObjectives _returnvalue_3)
                (:%20%20
                  (Actor|DestroyActor))))))
        (elif (> (Math|Random|RandomFloatinRange 0.0 1.0) 0.9)
          (switch int (Math|Random|RandomIntegerinRange 0 2)
            (:0
              (bind _returnvalue_4 (Actor|GetActorOfClass "/Game/Ironsphere/Missions/Destruction/BP_MissionDestruction.BP_MissionDestruction_C"))
              (if (> (Variables|/Game/Ironsphere/Missions/Destruction/BP_MissionDestruction.BP_MissionDestruction_C|GetNumberOfDens _returnvalue_4) 0)
                (Game|SpawnActorfromClass "/Game/Ironsphere/Missions/BP_MissionDen.BP_MissionDen_C" (Transformation|GetActorTransform) "Undefined" "MultiplyWithRoot" 0 0)
                (bind _returnvalue_5 (Actor|GetActorOfClass "/Game/Ironsphere/Missions/Destruction/BP_MissionDestruction.BP_MissionDestruction_C"))
                (Math|Integer|DecrementInt (Variables|/Game/Ironsphere/Missions/Destruction/BP_MissionDestruction.BP_MissionDestruction_C|GetNumberOfDens _returnvalue_5)
                  (:%20%20
                    (Actor|DestroyActor)))))
            (:1
              (bind _returnvalue_6 (Actor|GetActorOfClass "/Game/Ironsphere/Missions/Destruction/BP_MissionDestruction.BP_MissionDestruction_C"))
              (if (> (Variables|/Game/Ironsphere/Missions/Destruction/BP_MissionDestruction.BP_MissionDestruction_C|GetNumberOfInstants _returnvalue_6) 0)
                (Game|SpawnActorfromClass "/Game/Ironsphere/Missions/BP_MissionInstant.BP_MissionInstant_C" (Transformation|GetActorTransform) "Undefined" "MultiplyWithRoot" 0 (Math|Random|RandomFloatinRange 0.5 3.0) 0)
                (bind _returnvalue_7 (Actor|GetActorOfClass "/Game/Ironsphere/Missions/Destruction/BP_MissionDestruction.BP_MissionDestruction_C"))
                (Math|Integer|DecrementInt (Variables|/Game/Ironsphere/Missions/Destruction/BP_MissionDestruction.BP_MissionDestruction_C|GetNumberOfInstants _returnvalue_7)
                  (:%20%20
                    (Actor|DestroyActor)))))
            (:2
              (bind _returnvalue_8 (Actor|GetActorOfClass "/Game/Ironsphere/Missions/Destruction/BP_MissionDestruction.BP_MissionDestruction_C"))
              (if (> (Variables|/Game/Ironsphere/Missions/Destruction/BP_MissionDestruction.BP_MissionDestruction_C|GetNumberOfHides _returnvalue_8) 0)
                (Game|SpawnActorfromClass "/Game/Ironsphere/Missions/BP_MissionDen.BP_MissionDen_C" (Transformation|GetActorTransform) "Undefined" "MultiplyWithRoot" 0 0)
                (bind _returnvalue_9 (Actor|GetActorOfClass "/Game/Ironsphere/Missions/Destruction/BP_MissionDestruction.BP_MissionDestruction_C"))
                (Math|Integer|DecrementInt (Variables|/Game/Ironsphere/Missions/Destruction/BP_MissionDestruction.BP_MissionDestruction_C|GetNumberOfHides _returnvalue_9)
                  (:%20%20
                    (Actor|DestroyActor)))))))))))

(fn ConstructionScript)