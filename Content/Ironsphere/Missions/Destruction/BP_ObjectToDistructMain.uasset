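; Destructible mission object that can serve as an objective, extending a parent that supplies damage and HP-bar logic.
; BeginPlay attaches an objective arrow to the player's mech and, for objectives, adds a minimap icon placed by scaled world position.
; The icon hides at zero HP or in Destruction, which can also explode with radial damage, effects, camera shake and a Fire debuff on nearby characters.
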(event EventBeginPlay
  (bind _returnvalue (Transformation|GetActorLocation))
  (bind (_x _y) (Math|Vector|BreakVector _returnvalue))
  (Utilities|FlowControl|Sequence
    (:then_0
      (|CallParentFunction)
      (Rendering|SetVisibility (Variables|Default|Getwidget_HPbar) true false)
      (if (Variables|Default|GetIsObjective)
        (bind _returnvalue_2 (UserInterface|CreateWidget "/Game/Ironsphere/UI/Ingame/Map/WBS_MinimapObject.WBS_MinimapObject_C" 0 "/Game/Ironsphere/UI/Ingame/Map/Objective.Objective" true))
        (Variables|Default|SetObjectMap _returnvalue_2)
        (UserInterface|Viewport|AddtoViewport _returnvalue_2 1)
        (Class|UserWidget|SetPositioninViewport _returnvalue_2 (Math|Vector2D|MakeVector2D (+ (* _x -0.1) 2e+02) (+ (* _y -0.1) 2e+02)) true)))
    (:then_1
      (bind _aspc_ingame (Utilities|Casting|CastToPC_Ingame (Game|GetPlayerController 0))
        (:then
          (bind _returnvalue_3 (Game|SpawnActorfromClass "/Game/Ironsphere/Core/Player/BP_ObjectiveArrow.BP_ObjectiveArrow_C" (Math|Transform|MakeTransform "0, 0, 0") "Undefined" "MultiplyWithRoot" (Variables|/Game/Ironsphere/Core/Framework/Battle/PC_Ingame.PC_Ingame_C|GetControlledMech _aspc_ingame) self 0))
          (Transformation|AttachActorToActor _returnvalue_3 (Variables|/Game/Ironsphere/Core/Framework/Battle/PC_Ingame.PC_Ingame_C|GetControlledMech _aspc_ingame) "None" "KeepRelative" "KeepRelative" "KeepRelative" true))
        (:CastFailed
          (Audio|SpawnSound2D "/Engine/EditorSounds/Notifications/CompileFailed.CompileFailed" 1.0 1.0 0.0 0))))))

(event Collision|EventActorBeginOverlap
  (params (OtherActor :type Actor%20Object%20Reference)))

(event EventTick
  (params (DeltaSeconds :type Float%20%28single-precision%29))
  (|CallParentFunction DeltaSeconds)
  (Utilities|FlowControl|Sequence
    (:then_0
      (CallFunction|UpdateHPbar)
      (if (<= (Variables|Default|GetCurrentHP) 0.0)
        (if (Variables|Default|GetIsObjective)
          (Widget|SetVisibility (Variables|Default|GetObjectMap) "Hidden"))))))

(event Game|Damage|EventAnyDamage
  (params (Damage :type Float%20%28single-precision%29) (DamageType :type Damage%20Type%20Object%20Reference) (InstigatedBy :type Controller%20Object%20Reference) (DamageCauser :type Actor%20Object%20Reference))
  (|CallParentFunction Damage DamageType InstigatedBy DamageCauser))

(fn ConstructionScript)

(fn UpdateHPbar
  (|CallParentFunction))

(fn SoundDamage
  (params (SoundDamage :type SoundDamage%20Enum :default "NewEnumerator0"))
  (|CallParentFunction SoundDamage))

(fn Destruction
  (params (IsBlow :type Boolean) (Damage :type Float%20%28double-precision%29) (Radius :type Float%20%28double-precision%29) (Sound :type SoundDestroy%20Enum :default "NewEnumerator0"))
  (bind _returnvalue (Transformation|GetActorLocation))
  (bind _objectmap (Variables|Default|GetObjectMap))
  (bind (_x _y) (Math|Vector|BreakVector _returnvalue))
  (if (Variables|Default|GetIsObjective)
    (if (Utilities|IsValid _objectmap)
      (Widget|SetVisibility _objectmap "Hidden")
      (Audio|SpawnSound2D "/Engine/VREditor/Sounds/UI/Click_on_Button_Cue.Click_on_Button_Cue" 2.0 1.0 0.0 0)
      (if IsBlow :!label _label
        (CallFunction|SoundDestroy "NewEnumerator2")
        (Class|GameplayStatics|ApplyRadialDamagewithFalloff Damage 0.0 (Math|Vector|MakeVector _x _y 1e+01) 0.0 Radius 0.2 "/Game/Ironsphere/Feature/Consumable/DamageTypes/BP_PhysicalDamage.BP_PhysicalDamage_C" 0 self 0 "ECC_Visibility")
        (Effects|SpawnEmitteratLocation "/Game/StarterContent/Particles/P_Explosion.P_Explosion" _returnvalue "0, 0, 0" (Math|Conversions|ToVector(Float) (/ (Math|Float|Sqrt (Math|Float|Sqrt Radius)) 3.0)))
        (Audio|SpawnSoundatLocation "/Game/Ironsphere/Sound/Explosion/explosion_4.explosion_4" _returnvalue "0, 0, 0" 1.0 1.0 0.0 0 0)
        (Class|LegacyCameraShake|StartLegacyCameraShake (Game|GetPlayerCameraManager 0) "/Game/Ironsphere/Core/Player/CamShakeBlow.CamShakeBlow_C" (/ Damage 1e+01) "CameraLocal" "0, 0, 0")
        (bind _outactors (Actor|GetAllActorsOfClass "/Game/Ironsphere/Core/Character/BP_CharacterBase.BP_CharacterBase_C"))
        (for _array_element _outactors
          (if (< (Math|Vector|VectorLength (- (Transformation|GetActorLocation _array_element) (Transformation|GetActorLocation))) 1.3e+02)
            (Default|AddBuff _array_element (Utilities|Struct|MakeST_buff "NewEnumerator7" -5.0 5.0 false "Fire" "/Game/Ironsphere/UI/Icons/Buffs/Fire.Fire"))
            (CallFunction|KillWidgets)))
        (else
          (CallFunction|SoundDestroy "NewEnumerator0" :!label _label_2)
          (CallFunction|KillWidgets)))
      (else
        (goto _label_2)))
    (else
      (goto _label))))