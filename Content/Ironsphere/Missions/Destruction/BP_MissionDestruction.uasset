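; BP_MissionDestruction is a mission Blueprint where the player destroys every instance of a randomly chosen target: fuel barrels, eggs, silos or crates.
; BeginPlay sets the objective text and scales objective, spawner and turret counts by mission number, mostly also difficulty, randomly splitting spawners into dens, hides and instants.
; Tick polls actors by class to update the UI and complete the mission, granting the timed bonus if LevelTimer remains.
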(event EventBeginPlay
  (bind _gs_battle_ref (Variables|Default|GetGS_Battle_ref))
  (bind _gi_main_ref (Variables|Default|GetGI_Main_ref))
  (bind _gi_main_ref_2 (Variables|Default|GetGI_Main_ref))
  (bind _currentmission (Variables|/Game/Ironsphere/Core/Framework/GI_Main.GI_Main_C|GetCurrentMission _gi_main_ref))
  (bind _difficultylevel (Variables|/Game/Ironsphere/Core/Framework/GI_Main.GI_Main_C|GetDifficultyLevel _gi_main_ref))
  (bind _returnvalue (+ _currentmission _difficultylevel))
  (|CallParentFunction)
  (Utilities|FlowControl|Sequence
    (:then_0
      (switch int (Math|Random|RandomIntegerinRange 0 3)
        (:0
          (Variables|Default|SetObject "/Game/Ironsphere/Missions/Destruction/BP_FuelBarrelObjective.BP_FuelBarrelObjective_C")
          (Variables|/Game/Ironsphere/Core/Framework/Battle/GS_Battle.GS_Battle_C|SetObjective _gs_battle_ref "Destroy all fuel barrels!"))
        (:1
          (Variables|Default|SetObject "/Game/Ironsphere/Missions/Destruction/BP_GiantEggObjective.BP_GiantEggObjective_C")
          (Variables|/Game/Ironsphere/Core/Framework/Battle/GS_Battle.GS_Battle_C|SetObjective _gs_battle_ref "Destroy all eggs!"))
        (:2
          (Variables|Default|SetObject "/Game/Ironsphere/Missions/Destruction/BP_SiloObjective.BP_SiloObjective_C")
          (Variables|/Game/Ironsphere/Core/Framework/Battle/GS_Battle.GS_Battle_C|SetObjective _gs_battle_ref "Destroy all silos!"))
        (:3
          (Variables|Default|SetObject "/Game/Ironsphere/Missions/Destruction/BP_CrateObjective.BP_CrateObjective_C")
          (Variables|/Game/Ironsphere/Core/Framework/Battle/GS_Battle.GS_Battle_C|SetObjective _gs_battle_ref "Destroy all crates!")))
      (Variables|/Game/Ironsphere/Core/Framework/Battle/GS_Battle.GS_Battle_C|SetBonusObjective _gs_battle_ref "Complete in 3 minutes"))
    (:then_1
      (Variables|Default|SetNumberOfObjectives (/ (+ _currentmission 20) 7))
      (Variables|Default|SetNumberOfSpawners (+ (/ _returnvalue 3) 4 (/ (* _returnvalue _returnvalue) 500)))
      (while (> (Variables|Default|GetNumberOfSpawners) 0)
        (switch int (Math|Random|RandomIntegerinRange 0 6)
          (:Default
            (Math|Integer|IncrementInt (Variables|Default|GetNumberOfDens) :!label _label
              (:%20%20
                _)))
          (:0
            (Math|Integer|IncrementInt (Variables|Default|GetNumberOfHides) :!label _label_2
              (:%20%20
                _)))
          (:1
            (goto _label_2))
          (:2
            (goto _label))
          (:3
            (goto _label))
          (:4
            (goto _label_2))
          (:5
            (goto _label))
          (:6
            (Math|Integer|IncrementInt (Variables|Default|GetNumberOfInstants)
              (:%20%20
                _))))
        (Math|Integer|DecrementInt (Variables|Default|GetNumberOfSpawners))))
    (:then_2
      (Variables|Default|SetNumberOfTurrets (+ (/ (+ (Variables|/Game/Ironsphere/Core/Framework/GI_Main.GI_Main_C|GetCurrentMission _gi_main_ref_2) (Variables|/Game/Ironsphere/Core/Framework/GI_Main.GI_Main_C|GetDifficultyLevel _gi_main_ref_2) 4) 10) 2)))
    (:then_3
      (Variables|/Game/Ironsphere/Core/Framework/Battle/GS_Battle.GS_Battle_C|SetBonusObjectivepassed (Variables|Default|GetGS_Battle_ref) true))))

(event Collision|EventActorBeginOverlap
  (params (OtherActor :type Actor%20Object%20Reference))
  (|CallParentFunction OtherActor) ; This node is disabled and will not be called.\nDrag off pins to build functionality.
)

(event EventTick
  (params (DeltaSeconds :type Float%20%28single-precision%29))
  (bind _gs_battle_ref (Variables|Default|GetGS_Battle_ref))
  (bind _gs_battle_ref_2 (Variables|Default|GetGS_Battle_ref))
  (|CallParentFunction DeltaSeconds)
  (if (Utilities|IsValid (Variables|Default|GetGS_Battle_ref))
    (Utilities|FlowControl|Sequence
      (:then_0
        (bind _outactors (Actor|GetAllActorsOfClass (Variables|Default|GetObject)))
        (if (and (<= (Utilities|Array|Length _outactors) 0) (> (Variables|/Game/Ironsphere/Core/Framework/Battle/GS_Battle.GS_Battle_C|GetStartDelay _gs_battle_ref) 1e+01))
          (if (> (Variables|Default|GetLevelTimer) 0.0)
            (Variables|/Game/Ironsphere/Core/Framework/Battle/GS_Battle.GS_Battle_C|SetBonusObjectivepassed _gs_battle_ref true)
            (else
              (Variables|/Game/Ironsphere/Core/Framework/Battle/GS_Battle.GS_Battle_C|SetBonusObjectivepassed _gs_battle_ref false)))
          (Variables|/Game/Ironsphere/Core/Framework/Battle/GS_Battle.GS_Battle_C|SetObjectivePassed _gs_battle_ref true)))
      (:then_1
        (bind _outactors_2 (Actor|GetAllActorsOfClass "/Game/Ironsphere/Missions/Destruction/BP_ObjectToDistructMain.BP_ObjectToDistructMain_C"))
        (Variables|/Game/Ironsphere/Core/Framework/Battle/GS_Battle.GS_Battle_C|SetObjectiveUI _gs_battle_ref_2 (Utilities|Text|FormatText "{x} {y} left." (Variables|/Game/Ironsphere/Core/Framework/Battle/GS_Battle.GS_Battle_C|GetObjective _gs_battle_ref_2) (Utilities|Array|Length _outactors_2)))
        (Variables|/Game/Ironsphere/Core/Framework/Battle/GS_Battle.GS_Battle_C|SetBonusObjectiveUI _gs_battle_ref_2 (Utilities|Text|FormatText "Complete in {x} seconds." (Class|KismetMathLibrary|ToInt64(Float) (Variables|Default|GetLevelTimer))))))))

(fn ConstructionScript
  (|CallParentFunction))