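; Placed mission spawner that picks an enemy type and group size from the current mission number in GI_Main.
; On BeginPlay it removes its Cube component, then rolls a mission-scaled random tier through nested branches.
; Up to mission 10 it picks creatures; later missions use small spider droids or hover units, with counts based on the squared mission number.
; The result spawns one BP_Hide at its transform, passing NPC class, count, unhide delay and Objective.
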(event EventBeginPlay
  (Components|DestroyComponent (Variables|Default|GetCube))
  (bind _asgi_main (Utilities|Casting|CastToGI_Main (Game|GetGameInstance)))
  (bind _output_get (Variables|Default|SetCurrent%20Mission (+ (Variables|/Game/Ironsphere/Core/Framework/GI_Main.GI_Main_C|GetCurrentMission _asgi_main) 0)))
  (Variables|Default|Setrandom (Math|Random|RandomIntegerinRange (- (/ _output_get 2) 1) (+ _output_get 3)))
  (if (> (Variables|/Game/Ironsphere/Core/Framework/GI_Main.GI_Main_C|GetCurrentMission _asgi_main) 10)
    (Variables|Default|SetRandom (Math|Random|RandomIntegerinRange (- (/ (- (Variables|Default|GetCurrent%20Mission) 10) 3) 2) (+ (- (Variables|Default|GetCurrent%20Mission) 10) 3)))
    (Variables|Default|SetCurrent%20Mission (/ (* (Variables|Default|GetCurrent%20Mission) (Variables|Default|GetCurrent%20Mission)) 10))
    (if (> (Variables|Default|GetRandom) 1)
      (if (> (Variables|Default|GetRandom) 5)
        (if (> (Variables|Default|GetRandom) 7)
          (Game|SpawnActorfromClass "/Game/Ironsphere/Feature/World/Spawners/BP_Hide.BP_Hide_C" (Transformation|GetActorTransform) "Undefined" "MultiplyWithRoot" 0 (Variables|Default|GetDelay) (+ (/ (+ (Variables|Default|GetCurrent%20Mission) (Math|Random|RandomIntegerinRange 0 1)) 7) 1) "/Game/Ironsphere/Feature/NPC/Hover/BP_CombatHover.BP_CombatHover_C" (Variables|Default|GetObjective) 3e+01 3e+01 0.0 0)
          (else
            (Game|SpawnActorfromClass "/Game/Ironsphere/Feature/World/Spawners/BP_Hide.BP_Hide_C" (Transformation|GetActorTransform) "Undefined" "MultiplyWithRoot" 0 (Variables|Default|GetDelay) (/ (+ (Variables|Default|GetCurrent%20Mission) (Math|Random|RandomIntegerinRange 0 1)) 3) "/Game/Ironsphere/Feature/NPC/Hover/BP_GaussHover.BP_GaussHover_C" (Variables|Default|GetObjective) 3e+01 3e+01 0.0 0)))
        (elif (Math|Random|RandomBool)
          (Game|SpawnActorfromClass "/Game/Ironsphere/Feature/World/Spawners/BP_Hide.BP_Hide_C" (Transformation|GetActorTransform) "Undefined" "MultiplyWithRoot" 0 (Variables|Default|GetDelay) (/ (+ (Variables|Default|GetCurrent%20Mission) (Math|Random|RandomIntegerinRange 0 1)) 3) "/Game/Ironsphere/Feature/NPC/Hover/BP_LaserHover.BP_LaserHover_C" (Variables|Default|GetObjective) 3e+01 3e+01 0.0 0)
          (else
            (Game|SpawnActorfromClass "/Game/Ironsphere/Feature/World/Spawners/BP_Hide.BP_Hide_C" (Transformation|GetActorTransform) "Undefined" "MultiplyWithRoot" 0 (Variables|Default|GetDelay) (/ (+ (Variables|Default|GetCurrent%20Mission) (Math|Random|RandomIntegerinRange 0 1)) 3) "/Game/Ironsphere/Feature/NPC/Hover/BP_ACHover.BP_ACHover_C" (Variables|Default|GetObjective) 3e+01 3e+01 0.0 0))))
      (else
        (Game|SpawnActorfromClass "/Game/Ironsphere/Feature/World/Spawners/BP_Hide.BP_Hide_C" (Transformation|GetActorTransform) "Undefined" "MultiplyWithRoot" 0 (Variables|Default|GetDelay) (+ (Variables|Default|GetCurrent%20Mission) (Math|Random|RandomIntegerinRange 3 6)) "/Game/Ironsphere/Feature/NPC/SpiderDroid/BP_SmallSpiderDroid.BP_SmallSpiderDroid_C" (Variables|Default|GetObjective) 3e+01 3e+01 0.0 0)))
    (elif (> (Variables|Default|GetRandom) 1)
      (if (> (Variables|Default|GetRandom) 2)
        (if (> (Variables|Default|GetRandom) 3)
          (if (> (Variables|Default|GetRandom) 4)
            (if (> (Variables|Default|GetRandom) 5)
              (if (> (Variables|Default|GetRandom) 6)
                (if (> (Variables|Default|GetRandom) 7)
                  (Game|SpawnActorfromClass "/Game/Ironsphere/Feature/World/Spawners/BP_Hide.BP_Hide_C" (Transformation|GetActorTransform) "Undefined" "MultiplyWithRoot" 0 (Variables|Default|GetDelay) (+ (* (Math|Conversions|ToFloat(Integer) (Variables|Default|GetCurrent%20Mission)) 0.5) (Math|Random|RandomIntegerinRange 2 2)) "/Game/Ironsphere/Feature/NPC/Spider/BP_RedSpider.BP_RedSpider_C" (Variables|Default|GetObjective) 3e+01 3e+01 0.0 0)
                  (else
                    (Game|SpawnActorfromClass "/Game/Ironsphere/Feature/World/Spawners/BP_Hide.BP_Hide_C" (Transformation|GetActorTransform) "Undefined" "MultiplyWithRoot" 0 (Variables|Default|GetDelay) (+ (* (Variables|Default|GetCurrent%20Mission) 0.5) (Math|Random|RandomIntegerinRange 3 5)) "/Game/Ironsphere/Feature/NPC/Worm/BP_NeedleWorm.BP_NeedleWorm_C" (Variables|Default|GetObjective) 3e+01 3e+01 0.0 0)))
                (elif (Math|Random|RandomBool)
                  (Game|SpawnActorfromClass "/Game/Ironsphere/Feature/World/Spawners/BP_Hide.BP_Hide_C" (Transformation|GetActorTransform) "Undefined" "MultiplyWithRoot" 0 (Variables|Default|GetDelay) (+ (* (Variables|Default|GetCurrent%20Mission) 2) (Math|Random|RandomIntegerinRange 2 4)) "/Game/Ironsphere/Feature/NPC/Hornet/BP_Hornet.BP_Hornet_C" (Variables|Default|GetObjective) 3e+01 3e+01 0.0 0)
                  (else
                    (Game|SpawnActorfromClass "/Game/Ironsphere/Feature/World/Spawners/BP_Hide.BP_Hide_C" (Transformation|GetActorTransform) "Undefined" "MultiplyWithRoot" 0 (Variables|Default|GetDelay) (+ (* (Variables|Default|GetCurrent%20Mission) 0.6) (Math|Random|RandomIntegerinRange 1 2)) "/Game/Ironsphere/Feature/NPC/Spider/BP_SandSpider.BP_SandSpider_C" (Variables|Default|GetObjective) 3e+01 3e+01 0.0 0))))
              (else
                (Game|SpawnActorfromClass "/Game/Ironsphere/Feature/World/Spawners/BP_Hide.BP_Hide_C" (Transformation|GetActorTransform) "Undefined" "MultiplyWithRoot" 0 (Variables|Default|GetDelay) (+ (Variables|Default|GetCurrent%20Mission) (Math|Random|RandomIntegerinRange 2 3)) "/Game/Ironsphere/Feature/NPC/Worm/BP_TigerLeech.BP_TigerLeech_C" (Variables|Default|GetObjective) 3e+01 3e+01 0.0 0)))
            (else
              (Game|SpawnActorfromClass "/Game/Ironsphere/Feature/World/Spawners/BP_Hide.BP_Hide_C" (Transformation|GetActorTransform) "Undefined" "MultiplyWithRoot" 0 (Variables|Default|GetDelay) (+ (Math|Random|RandomIntegerinRange (Variables|Default|GetCurrent%20Mission) (* (Variables|Default|GetCurrent%20Mission) 2)) (Math|Random|RandomIntegerinRange 3 5)) "/Game/Ironsphere/Feature/NPC/Hornet/BP_FlyingEye.BP_FlyingEye_C" (Variables|Default|GetObjective) 3e+01 3e+01 0.0 0)))
          (else
            (Game|SpawnActorfromClass "/Game/Ironsphere/Feature/World/Spawners/BP_Hide.BP_Hide_C" (Transformation|GetActorTransform) "Undefined" "MultiplyWithRoot" 0 (Variables|Default|GetDelay) (+ (* (Variables|Default|GetCurrent%20Mission) 6) (Math|Random|RandomIntegerinRange 10 12)) "/Game/Ironsphere/Feature/NPC/Hornet/BP_DesertWasp.BP_DesertWasp_C" (Variables|Default|GetObjective) 3e+01 3e+01 0.0 0)))
        (else
          (Game|SpawnActorfromClass "/Game/Ironsphere/Feature/World/Spawners/BP_Hide.BP_Hide_C" (Transformation|GetActorTransform) "Undefined" "MultiplyWithRoot" 0 (Variables|Default|GetDelay) (+ (* (Variables|Default|GetCurrent%20Mission) 3) (Math|Random|RandomIntegerinRange 5 6)) "/Game/Ironsphere/Feature/NPC/Spider/BP_DesertSpider.BP_DesertSpider_C" (Variables|Default|GetObjective) 3e+01 3e+01 0.0 0)))
      (else
        (Game|SpawnActorfromClass "/Game/Ironsphere/Feature/World/Spawners/BP_Hide.BP_Hide_C" (Transformation|GetActorTransform) "Undefined" "MultiplyWithRoot" 0 (Variables|Default|GetDelay) (+ (* (Variables|Default|GetCurrent%20Mission) 4) (Math|Random|RandomIntegerinRange 5 7)) "/Game/Ironsphere/Feature/NPC/Worm/BP_GreyWorm.BP_GreyWorm_C" (Variables|Default|GetObjective) 3e+01 3e+01 0.0 0)))))

(event Collision|EventActorBeginOverlap
  (params (OtherActor :type Actor%20Object%20Reference)))

(event EventTick
  (params (DeltaSeconds :type Float%20%28single-precision%29)))

(fn ConstructionScript)