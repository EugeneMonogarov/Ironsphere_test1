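; Mission placeholder that turns into an enemy spawner (den, hive or egg spawner) at its transform on BeginPlay, removing its cube.
; A random tier derived from mission number plus difficulty picks spawner and NPC type.
; Missions up to 10 draw creatures; later ones draw drones, vehicles and armed giant spiders, with quadratic level scaling.
; That level generally shortens den and hive cooldowns, raises their HP and increases hive and egg counts.
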(event EventBeginPlay
  (Components|DestroyComponent (Variables|Default|GetCube))
  (bind _asgi_main (Utilities|Casting|CastToGI_Main (Game|GetGameInstance)))
  (bind _output_get (Variables|Default|SetCurrentMission (+ (Variables|/Game/Ironsphere/Core/Framework/GI_Main.GI_Main_C|GetCurrentMission _asgi_main) (Variables|/Game/Ironsphere/Core/Framework/GI_Main.GI_Main_C|GetDifficultyLevel _asgi_main))))
  (Variables|Default|SetRandom (Math|Random|RandomIntegerinRange (- (/ _output_get 2) 3) (+ _output_get 3)))
  (if (> (Variables|/Game/Ironsphere/Core/Framework/GI_Main.GI_Main_C|GetCurrentMission _asgi_main) 10)
    (Variables|Default|SetRandom (Math|Random|RandomIntegerinRange (- (/ (- (Variables|Default|GetCurrentMission) 10) 3) 2) (+ (- (Variables|Default|GetCurrentMission) 10) 3)))
    (Variables|Default|SetCurrentMission (/ (* (Variables|Default|GetCurrentMission) (Variables|Default|GetCurrentMission)) 10))
    (if (> (Variables|Default|GetRandom) 2)
      (if (> (Variables|Default|GetRandom) 4)
        (if (> (Variables|Default|GetRandom) 6)
          (if (> (Variables|Default|GetRandom) 9)
            (if (> (Variables|Default|GetRandom) 11)
              (if (Math|Random|RandomBool)
                (Game|SpawnActorfromClass "/Game/Ironsphere/Feature/World/Spawners/BP_Den.BP_Den_C" (Transformation|GetActorTransform) "Undefined" "MultiplyWithRoot" 0 (+ (Math|Float|SafeDivide 1e+03 (+ (Math|Conversions|ToFloat(Integer) (Variables|Default|GetCurrentMission)) 3.0)) 3e+01) (/ (+ (Math|Float|SafeDivide 1e+03 (+ (Math|Conversions|ToFloat(Integer) (Variables|Default|GetCurrentMission)) 3.0)) 3e+01) 2.0) "/Game/Ironsphere/Feature/NPC/SpiderDroid/BP_GiantCannonSpider.BP_GiantCannonSpider_C" 5e+01 1 0 0.95 false (+ 5e+01 (* (Math|Conversions|ToFloat(Integer) (Variables|Default|GetCurrentMission)) 1e+01)) (+ 5e+01 (* (Math|Conversions|ToFloat(Integer) (Variables|Default|GetCurrentMission)) 1e+01)) 25.0 0)
                (else
                  (Game|SpawnActorfromClass "/Game/Ironsphere/Feature/World/Spawners/BP_Den.BP_Den_C" (Transformation|GetActorTransform) "Undefined" "MultiplyWithRoot" 0 (+ (Math|Float|SafeDivide 1e+03 (+ (Math|Conversions|ToFloat(Integer) (Variables|Default|GetCurrentMission)) 3.0)) 3e+01) (/ (+ (Math|Float|SafeDivide 1e+03 (+ (Math|Conversions|ToFloat(Integer) (Variables|Default|GetCurrentMission)) 3.0)) 3e+01) 2.0) "/Game/Ironsphere/Feature/NPC/SpiderDroid/BP_GiantLaserSpider.BP_GiantLaserSpider_C" 5e+01 1 0 0.95 false (+ 5e+01 (* (Math|Conversions|ToFloat(Integer) (Variables|Default|GetCurrentMission)) 1e+01)) (+ 5e+01 (* (Math|Conversions|ToFloat(Integer) (Variables|Default|GetCurrentMission)) 1e+01)) 25.0 0)))
              (else
                (Game|SpawnActorfromClass "/Game/Ironsphere/Feature/World/Spawners/BP_Hive.BP_Hive_C" (Transformation|GetActorTransform) "Undefined" "MultiplyWithRoot" 0 (+ (Math|Float|SafeDivide 6.5e+02 (+ (Math|Conversions|ToFloat(Integer) (Variables|Default|GetCurrentMission)) 3.0)) 8.0) (/ (+ (Math|Float|SafeDivide 6.5e+02 (+ (Math|Conversions|ToFloat(Integer) (Variables|Default|GetCurrentMission)) 3.0)) 8.0) 5.0) "/Game/Ironsphere/Feature/NPC/Drone/BP_CombatDrone.BP_CombatDrone_C" 4e+01 (+ (Variables|Default|GetCurrentMission) 5) 0 0.95 false (Math|Conversions|ToFloat(Integer) (+ (* (Variables|Default|GetCurrentMission) 8) 50)) (Math|Conversions|ToFloat(Integer) (+ (* (Variables|Default|GetCurrentMission) 8) 50)) 25.0 0)))
            (else
              (switch int (Math|Random|RandomIntegerinRange 0 1)
                (:0
                  (Game|SpawnActorfromClass "/Game/Ironsphere/Feature/World/Spawners/BP_Den.BP_Den_C" (Transformation|GetActorTransform) "Undefined" "MultiplyWithRoot" 0 (+ (Math|Float|SafeDivide 6.5e+02 (+ (Math|Conversions|ToFloat(Integer) (Variables|Default|GetCurrentMission)) 3.0)) 15.0) (/ (+ (Math|Float|SafeDivide 6.5e+02 (+ (Math|Conversions|ToFloat(Integer) (Variables|Default|GetCurrentMission)) 3.0)) 15.0) 2.0) "/Game/Ironsphere/Feature/NPC/Vehicle/BP_LargeMissileVehicle1.BP_LargeMissileVehicle1_C" 5e+01 1 0 0.95 false (+ 5e+01 (* (Math|Conversions|ToFloat(Integer) (Variables|Default|GetCurrentMission)) 1e+01)) (+ 5e+01 (* (Math|Conversions|ToFloat(Integer) (Variables|Default|GetCurrentMission)) 1e+01)) 25.0 0))
                (:1
                  (Game|SpawnActorfromClass "/Game/Ironsphere/Feature/World/Spawners/BP_Den.BP_Den_C" (Transformation|GetActorTransform) "Undefined" "MultiplyWithRoot" 0 (+ (Math|Float|SafeDivide 6.5e+02 (+ (Math|Conversions|ToFloat(Integer) (Variables|Default|GetCurrentMission)) 3.0)) 15.0) (/ (+ (Math|Float|SafeDivide 6.5e+02 (+ (Math|Conversions|ToFloat(Integer) (Variables|Default|GetCurrentMission)) 3.0)) 15.0) 2.0) "/Game/Ironsphere/Feature/NPC/Vehicle/BP_LargeGunVehicle.BP_LargeGunVehicle_C" 5e+01 1 0 0.95 false (+ 5e+01 (* (Math|Conversions|ToFloat(Integer) (Variables|Default|GetCurrentMission)) 1e+01)) (+ 5e+01 (* (Math|Conversions|ToFloat(Integer) (Variables|Default|GetCurrentMission)) 1e+01)) 25.0 0)))))
          (elif (Math|Random|RandomBool)
            (Game|SpawnActorfromClass "/Game/Ironsphere/Feature/World/Spawners/BP_Hive.BP_Hive_C" (Transformation|GetActorTransform) "Undefined" "MultiplyWithRoot" 0 (+ (Math|Float|SafeDivide 9e+01 (+ (Math|Conversions|ToFloat(Integer) (Variables|Default|GetCurrentMission)) 3.0)) 8.0) (+ (Math|Float|SafeDivide 5.0 (+ (Math|Conversions|ToFloat(Integer) (Variables|Default|GetCurrentMission)) 3.0)) 1.0) "/Game/Ironsphere/Feature/NPC/Drone/BP_LargeLaserDrone1.BP_LargeLaserDrone1_C" 4e+01 (+ (Variables|Default|GetCurrentMission) 5) 0 0.95 false (Math|Conversions|ToFloat(Integer) (+ (* (Variables|Default|GetCurrentMission) 8) 50)) (Math|Conversions|ToFloat(Integer) (+ (* (Variables|Default|GetCurrentMission) 8) 50)) 25.0 0)
            (else
              (Game|SpawnActorfromClass "/Game/Ironsphere/Feature/World/Spawners/BP_Hive.BP_Hive_C" (Transformation|GetActorTransform) "Undefined" "MultiplyWithRoot" 0 (+ (Math|Float|SafeDivide 9e+01 (+ (Math|Conversions|ToFloat(Integer) (Variables|Default|GetCurrentMission)) 3.0)) 8.0) (+ (Math|Float|SafeDivide 5.0 (+ (Math|Conversions|ToFloat(Integer) (Variables|Default|GetCurrentMission)) 3.0)) 1.0) "/Game/Ironsphere/Feature/NPC/Drone/BP_LargeMissileDron.BP_LargeMissileDron_C" 4e+01 (+ (Variables|Default|GetCurrentMission) 5) 0 0.95 false (Math|Conversions|ToFloat(Integer) (+ (* (Variables|Default|GetCurrentMission) 8) 50)) (Math|Conversions|ToFloat(Integer) (+ (* (Variables|Default|GetCurrentMission) 8) 50)) 25.0 0))))
        (else
          (switch int (Math|Random|RandomIntegerinRange 0 4)
            (:0
              (Game|SpawnActorfromClass "/Game/Ironsphere/Feature/World/Spawners/BP_Den.BP_Den_C" (Transformation|GetActorTransform) "Undefined" "MultiplyWithRoot" 0 (+ (Math|Float|SafeDivide 4.7e+02 (+ (Math|Conversions|ToFloat(Integer) (Variables|Default|GetCurrentMission)) 3.0)) 15.0) (/ (+ (Math|Float|SafeDivide 4.7e+02 (+ (Math|Conversions|ToFloat(Integer) (Variables|Default|GetCurrentMission)) 3.0)) 15.0) 2.0) "/Game/Ironsphere/Feature/NPC/Vehicle/BP_BolsterVehicle.BP_BolsterVehicle_C" 5e+01 (Math|Random|RandomIntegerinRange 1 2) 0 0.95 false (+ 5e+01 (* (Math|Conversions|ToFloat(Integer) (Variables|Default|GetCurrentMission)) 1e+01)) (+ 5e+01 (* (Math|Conversions|ToFloat(Integer) (Variables|Default|GetCurrentMission)) 1e+01)) 25.0 0))
            (:1
              (Game|SpawnActorfromClass "/Game/Ironsphere/Feature/World/Spawners/BP_Den.BP_Den_C" (Transformation|GetActorTransform) "Undefined" "MultiplyWithRoot" 0 (+ (Math|Float|SafeDivide 4.7e+02 (+ (Math|Conversions|ToFloat(Integer) (Variables|Default|GetCurrentMission)) 3.0)) 15.0) (/ (+ (Math|Float|SafeDivide 4.7e+02 (+ (Math|Conversions|ToFloat(Integer) (Variables|Default|GetCurrentMission)) 3.0)) 15.0) 2.0) "/Game/Ironsphere/Feature/NPC/Vehicle/BP_GunVehicle.BP_GunVehicle_C" 5e+01 (Math|Random|RandomIntegerinRange 1 2) 0 0.95 false (+ 5e+01 (* (Math|Conversions|ToFloat(Integer) (Variables|Default|GetCurrentMission)) 1e+01)) (+ 5e+01 (* (Math|Conversions|ToFloat(Integer) (Variables|Default|GetCurrentMission)) 1e+01)) 25.0 0))
            (:2
              (Game|SpawnActorfromClass "/Game/Ironsphere/Feature/World/Spawners/BP_Den.BP_Den_C" (Transformation|GetActorTransform) "Undefined" "MultiplyWithRoot" 0 (+ (Math|Float|SafeDivide 4.7e+02 (+ (Math|Conversions|ToFloat(Integer) (Variables|Default|GetCurrentMission)) 3.0)) 15.0) (/ (+ (Math|Float|SafeDivide 4.7e+02 (+ (Math|Conversions|ToFloat(Integer) (Variables|Default|GetCurrentMission)) 3.0)) 15.0) 2.0) "/Game/Ironsphere/Feature/NPC/Vehicle/BP_CannonVehicle.BP_CannonVehicle_C" 5e+01 (Math|Random|RandomIntegerinRange 1 2) 0 0.95 false (+ 5e+01 (* (Math|Conversions|ToFloat(Integer) (Variables|Default|GetCurrentMission)) 1e+01)) (+ 5e+01 (* (Math|Conversions|ToFloat(Integer) (Variables|Default|GetCurrentMission)) 1e+01)) 25.0 0))
            (:3
              (Game|SpawnActorfromClass "/Game/Ironsphere/Feature/World/Spawners/BP_Den.BP_Den_C" (Transformation|GetActorTransform) "Undefined" "MultiplyWithRoot" 0 (+ (Math|Float|SafeDivide 4.7e+02 (+ (Math|Conversions|ToFloat(Integer) (Variables|Default|GetCurrentMission)) 3.0)) 15.0) (/ (+ (Math|Float|SafeDivide 4.7e+02 (+ (Math|Conversions|ToFloat(Integer) (Variables|Default|GetCurrentMission)) 3.0)) 15.0) 2.0) "/Game/Ironsphere/Feature/NPC/Vehicle/BP_MissileVehicle.BP_MissileVehicle_C" 5e+01 (Math|Random|RandomIntegerinRange 1 2) 0 0.95 false (+ 5e+01 (* (Math|Conversions|ToFloat(Integer) (Variables|Default|GetCurrentMission)) 1e+01)) (+ 5e+01 (* (Math|Conversions|ToFloat(Integer) (Variables|Default|GetCurrentMission)) 1e+01)) 25.0 0))
            (:4
              (Game|SpawnActorfromClass "/Game/Ironsphere/Feature/World/Spawners/BP_Den.BP_Den_C" (Transformation|GetActorTransform) "Undefined" "MultiplyWithRoot" 0 (+ (Math|Float|SafeDivide 4.7e+02 (+ (Math|Conversions|ToFloat(Integer) (Variables|Default|GetCurrentMission)) 3.0)) 15.0) (/ (+ (Math|Float|SafeDivide 4.7e+02 (+ (Math|Conversions|ToFloat(Integer) (Variables|Default|GetCurrentMission)) 3.0)) 15.0) 2.0) "/Game/Ironsphere/Feature/NPC/Vehicle/BP_LaserVehicle.BP_LaserVehicle_C" 5e+01 (Math|Random|RandomIntegerinRange 1 2) 0 0.8 false (+ 5e+01 (* (Math|Conversions|ToFloat(Integer) (Variables|Default|GetCurrentMission)) 1e+01)) (+ 5e+01 (* (Math|Conversions|ToFloat(Integer) (Variables|Default|GetCurrentMission)) 1e+01)) 25.0 0)))))
      (elif (Math|Random|RandomBool)
        (Game|SpawnActorfromClass "/Game/Ironsphere/Feature/World/Spawners/BP_Hive.BP_Hive_C" (Transformation|GetActorTransform) "Undefined" "MultiplyWithRoot" 0 (+ (Math|Float|SafeDivide 1.5e+02 (+ (Math|Conversions|ToFloat(Integer) (Variables|Default|GetCurrentMission)) 3.0)) 8.0) (+ (Math|Float|SafeDivide 1e+01 (+ (Math|Conversions|ToFloat(Integer) (Variables|Default|GetCurrentMission)) 3.0)) 1.0) "/Game/Ironsphere/Feature/NPC/Drone/BP_SmallLaserDrone.BP_SmallLaserDrone_C" 4e+01 (+ (Variables|Default|GetCurrentMission) 5) 0 0.95 false (Math|Conversions|ToFloat(Integer) (+ (* (Variables|Default|GetCurrentMission) 8) 50)) (Math|Conversions|ToFloat(Integer) (+ (* (Variables|Default|GetCurrentMission) 8) 50)) 25.0 0)
        (else
          (Game|SpawnActorfromClass "/Game/Ironsphere/Feature/World/Spawners/BP_Hive.BP_Hive_C" (Transformation|GetActorTransform) "Undefined" "MultiplyWithRoot" 0 (+ (Math|Float|SafeDivide 4e+01 (+ (Math|Conversions|ToFloat(Integer) (Variables|Default|GetCurrentMission)) 3.0)) 8.0) (+ (Math|Float|SafeDivide 1e+01 (+ (Math|Conversions|ToFloat(Integer) (Variables|Default|GetCurrentMission)) 3.0)) 1.0) "/Game/Ironsphere/Feature/NPC/Drone/BP_SmallGunDrone.BP_SmallGunDrone_C" 4e+01 (+ (Variables|Default|GetCurrentMission) 5) 0 0.95 false (Math|Conversions|ToFloat(Integer) (+ (* (Variables|Default|GetCurrentMission) 8) 50)) (Math|Conversions|ToFloat(Integer) (+ (* (Variables|Default|GetCurrentMission) 8) 50)) 25.0 0))))
    (elif (> (Variables|Default|GetRandom) 1)
      (if (> (Variables|Default|GetRandom) 2)
        (if (> (Variables|Default|GetRandom) 3)
          (if (> (Variables|Default|GetRandom) 4)
            (if (> (Variables|Default|GetRandom) 6)
              (if (> (Variables|Default|GetRandom) 7)
                (Game|SpawnActorfromClass "/Game/Ironsphere/Feature/World/Spawners/BP_EggsSpawner.BP_EggsSpawner_C" (Transformation|GetActorTransform) "Undefined" "MultiplyWithRoot" 0 1e+01 1.8e+02 (+ (* (Variables|Default|GetCurrentMission) 1) (Math|Random|RandomIntegerinRange 0 4)) "/Game/Ironsphere/Feature/NPC/Spider/BP_DarkWidow.BP_DarkWidow_C" 5e+01 4.0 45.0 45.0 0.0 0)
                (else
                  (Game|SpawnActorfromClass "/Game/Ironsphere/Feature/World/Spawners/BP_Den.BP_Den_C" (Transformation|GetActorTransform) "Undefined" "MultiplyWithRoot" 0 (+ (Math|Float|SafeDivide 2e+02 (+ (Math|Conversions|ToFloat(Integer) (Variables|Default|GetCurrentMission)) 5.0)) 3e+01) (/ (+ (Math|Float|SafeDivide 2e+02 (+ (Math|Conversions|ToFloat(Integer) (Variables|Default|GetCurrentMission)) 5.0)) 3e+01) 2.0) "/Game/Ironsphere/Feature/NPC/Spider/BP_GiantSpider.BP_GiantSpider_C" 5e+01 1 0 0.8 false (+ 5e+01 (* (Math|Conversions|ToFloat(Integer) (Variables|Default|GetCurrentMission)) 15.0)) (+ 5e+01 (* (Math|Conversions|ToFloat(Integer) (Variables|Default|GetCurrentMission)) 15.0)) 25.0 0)))
              (elif (Math|Random|RandomBool)
                (Game|SpawnActorfromClass "/Game/Ironsphere/Feature/World/Spawners/BP_Hive.BP_Hive_C" (Transformation|GetActorTransform) "Undefined" "MultiplyWithRoot" 0 (+ (Math|Float|SafeDivide 3e+01 (Math|Conversions|ToFloat(Integer) (Variables|Default|GetCurrentMission))) 8.0) (+ (Math|Float|SafeDivide 3.0 (Math|Conversions|ToFloat(Integer) (Variables|Default|GetCurrentMission))) 1.0) "/Game/Ironsphere/Feature/NPC/Hornet/BP_Hornet.BP_Hornet_C" 4e+01 (+ (* (Variables|Default|GetCurrentMission) 2) 5) 0 0.9 false (Math|Conversions|ToFloat(Integer) (+ (* (Variables|Default|GetCurrentMission) 12) 50)) (Math|Conversions|ToFloat(Integer) (+ (* (Variables|Default|GetCurrentMission) 12) 50)) 25.0 0)
                (else
                  (Game|SpawnActorfromClass "/Game/Ironsphere/Feature/World/Spawners/BP_EggsSpawner.BP_EggsSpawner_C" (Transformation|GetActorTransform) "Undefined" "MultiplyWithRoot" 0 1e+01 1.8e+02 (+ (* (Variables|Default|GetCurrentMission) 1) (Math|Random|RandomIntegerinRange 0 5)) "/Game/Ironsphere/Feature/NPC/Spider/BP_RedSpider.BP_RedSpider_C" 45.0 4.0 0.0 0.0 0.0 0))))
            (else
              (Game|SpawnActorfromClass "/Game/Ironsphere/Feature/World/Spawners/BP_Den.BP_Den_C" (Transformation|GetActorTransform) "Undefined" "MultiplyWithRoot" 0 (+ (Math|Float|SafeDivide 7e+01 (+ (Math|Conversions|ToFloat(Integer) (Variables|Default|GetCurrentMission)) 3.0)) 15.0) (/ (+ (Math|Float|SafeDivide 7e+01 (+ (Math|Conversions|ToFloat(Integer) (Variables|Default|GetCurrentMission)) 3.0)) 15.0) 2.0) "/Game/Ironsphere/Feature/NPC/Spider/BP_SandSpider.BP_SandSpider_C" 5e+01 1 0 0.8 false (+ 5e+01 (* (Math|Conversions|ToFloat(Integer) (Variables|Default|GetCurrentMission)) 12.0)) (+ 5e+01 (* (Math|Conversions|ToFloat(Integer) (Variables|Default|GetCurrentMission)) 12.0)) 25.0 0)))
          (else
            (Game|SpawnActorfromClass "/Game/Ironsphere/Feature/World/Spawners/BP_Hive.BP_Hive_C" (Transformation|GetActorTransform) "Undefined" "MultiplyWithRoot" 0 (+ (Math|Float|SafeDivide 4e+01 (+ (Math|Conversions|ToFloat(Integer) (Variables|Default|GetCurrentMission)) 3.0)) 8.0) (+ (Math|Float|SafeDivide 5.0 (+ (Math|Conversions|ToFloat(Integer) (Variables|Default|GetCurrentMission)) 3.0)) 1.0) "/Game/Ironsphere/Feature/NPC/Hornet/BP_FlyingEye.BP_FlyingEye_C" 4e+01 (+ (* (Variables|Default|GetCurrentMission) 3) 5) 0 0.9 false (Math|Conversions|ToFloat(Integer) (+ (* (Variables|Default|GetCurrentMission) 12) 50)) (Math|Conversions|ToFloat(Integer) (+ (* (Variables|Default|GetCurrentMission) 12) 50)) 25.0 0)))
        (else
          (Game|SpawnActorfromClass "/Game/Ironsphere/Feature/World/Spawners/BP_Hive.BP_Hive_C" (Transformation|GetActorTransform) "Undefined" "MultiplyWithRoot" 0 (+ (Math|Float|SafeDivide 2e+01 (+ (Math|Conversions|ToFloat(Integer) (Variables|Default|GetCurrentMission)) 3.0)) 2.0) (+ (Math|Float|SafeDivide 5.0 (+ (Math|Conversions|ToFloat(Integer) (Variables|Default|GetCurrentMission)) 3.0)) 0.3) "/Game/Ironsphere/Feature/NPC/Hornet/BP_DesertWasp.BP_DesertWasp_C" 5e+01 (+ (* (Variables|Default|GetCurrentMission) 3) 15) 0 0.9 false (Math|Conversions|ToFloat(Integer) (+ (* (Variables|Default|GetCurrentMission) 13) 50)) (Math|Conversions|ToFloat(Integer) (+ (* (Variables|Default|GetCurrentMission) 13) 50)) 25.0 0)))
      (else
        (Game|SpawnActorfromClass "/Game/Ironsphere/Feature/World/Spawners/BP_EggsSpawner.BP_EggsSpawner_C" (Transformation|GetActorTransform) "Undefined" "MultiplyWithRoot" 0 1e+01 1.8e+02 (+ (* (Variables|Default|GetCurrentMission) 3) (Math|Random|RandomIntegerinRange 3 5)) "/Game/Ironsphere/Feature/NPC/Spider/BP_DesertSpider.BP_DesertSpider_C" 25.0 2.0 3e+01 3e+01 0.0 0)))))

(event Collision|EventActorBeginOverlap
  (params (OtherActor :type Actor%20Object%20Reference)))

(event EventTick
  (params (DeltaSeconds :type Float%20%28single-precision%29)))

(fn ConstructionScript)