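; Placeholder spawn point for the capturing mission that replaces itself with one mission object at its own transform.
; Each tick it randomly rolls to spawn a cap zone while objectives remain, then a den, instant or turret, decrementing BP_MissionCapturing's matching counter.
; The hide quota also spawns BP_MissionDen.
; It self-destructs when the player is near, or after a startup delay if objective and turret counts are zero.
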(event EventBeginPlay
  (Utilities|FlowControl|Delay 3.0 :!label _label)
  (bind _returnvalue (Actor|GetActorOfClass "/Game/Ironsphere/Missions/Capturing/BP_MissionCapturing.BP_MissionCapturing_C"))
  (if (and (== (Variables|/Game/Ironsphere/Missions/Capturing/BP_MissionCapturing.BP_MissionCapturing_C|GetNumberOfObjectives _returnvalue) 0) (== (Variables|/Game/Ironsphere/Missions/Capturing/BP_MissionCapturing.BP_MissionCapturing_C|GetNumberOfTurrets _returnvalue) 0))
    (Actor|DestroyActor)
    (goto _label)))

(event Collision|EventActorBeginOverlap
  (params (OtherActor :type Actor%20Object%20Reference)))

(event EventTick
  (params (DeltaSeconds :type Float%20%28single-precision%29))
  (bind _outactors (Actor|GetAllActorsOfClass "/Game/Ironsphere/Core/Player/BP_CharacterPlayer.BP_CharacterPlayer_C"))
  (if (< (Math|Vector|VectorLength (- (Transformation|GetActorLocation (Utilities|Array|Get(acopy) _outactors)) (Transformation|GetActorLocation))) 3e+02)
    (Actor|DestroyActor)
    (else
      (bind _returnvalue (Actor|GetActorOfClass "/Game/Ironsphere/Missions/Capturing/BP_MissionCapturing.BP_MissionCapturing_C"))
      (Utilities|FlowControl|Sequence
        (:then_0
          (if (> (Variables|/Game/Ironsphere/Missions/Capturing/BP_MissionCapturing.BP_MissionCapturing_C|GetNumberOfObjectives _returnvalue) 0)
            (if (> (Math|Random|RandomFloatinRange 0.0 1.0) 0.9)
              (Utilities|FlowControl|Sequence
                (:then_0
                  (Game|SpawnActorfromClass "/Game/Ironsphere/Missions/Capturing/BP_CapZone.BP_CapZone_C" (Transformation|GetActorTransform) "Undefined" "MultiplyWithRoot" 0 0))
                (:then_1
                  (bind _returnvalue_2 (Actor|GetActorOfClass "/Game/Ironsphere/Missions/Capturing/BP_MissionCapturing.BP_MissionCapturing_C"))
                  (Math|Integer|DecrementInt (Variables|/Game/Ironsphere/Missions/Capturing/BP_MissionCapturing.BP_MissionCapturing_C|GetNumberOfObjectives _returnvalue_2)
                    (:%20%20
                      (Actor|DestroyActor))))))
            (elif (> (Math|Random|RandomFloatinRange 0.0 1.0) 0.9)
              (switch int (Math|Random|RandomIntegerinRange 0 4)
                (:0
                  (bind _returnvalue_3 (Actor|GetActorOfClass "/Game/Ironsphere/Missions/Capturing/BP_MissionCapturing.BP_MissionCapturing_C"))
                  (if (> (Variables|/Game/Ironsphere/Missions/Capturing/BP_MissionCapturing.BP_MissionCapturing_C|GetNumberOfDens _returnvalue_3) 0)
                    (Game|SpawnActorfromClass "/Game/Ironsphere/Missions/BP_MissionDen.BP_MissionDen_C" (Transformation|GetActorTransform) "Undefined" "MultiplyWithRoot" 0 false 0)
                    (Actor|GetActorOfClass "/Game/Ironsphere/Missions/Capturing/BP_MissionCapturing.BP_MissionCapturing_C")
                    (Math|Integer|DecrementInt (Variables|/Game/Ironsphere/Missions/Capturing/BP_MissionCapturing.BP_MissionCapturing_C|GetNumberOfDens _returnvalue_3)
                      (:%20%20
                        (Actor|DestroyActor)))))
                (:1
                  (bind _returnvalue_4 (Actor|GetActorOfClass "/Game/Ironsphere/Missions/Capturing/BP_MissionCapturing.BP_MissionCapturing_C"))
                  (if (> (Variables|/Game/Ironsphere/Missions/Capturing/BP_MissionCapturing.BP_MissionCapturing_C|GetNumberOfInstants _returnvalue_4) 0)
                    (Game|SpawnActorfromClass "/Game/Ironsphere/Missions/BP_MissionInstant.BP_MissionInstant_C" (Transformation|GetActorTransform) "Undefined" "MultiplyWithRoot" 0 (Math|Random|RandomFloatinRange 0.5 3.0) false 0)
                    (bind _returnvalue_5 (Actor|GetActorOfClass "/Game/Ironsphere/Missions/Capturing/BP_MissionCapturing.BP_MissionCapturing_C"))
                    (Math|Integer|DecrementInt (Variables|/Game/Ironsphere/Missions/Capturing/BP_MissionCapturing.BP_MissionCapturing_C|GetNumberOfInstants _returnvalue_5)
                      (:%20%20
                        (Actor|DestroyActor)))))
                (:2
                  (bind _returnvalue_6 (Actor|GetActorOfClass "/Game/Ironsphere/Missions/Capturing/BP_MissionCapturing.BP_MissionCapturing_C"))
                  (if (> (Variables|/Game/Ironsphere/Missions/Capturing/BP_MissionCapturing.BP_MissionCapturing_C|GetNumberOfHides _returnvalue_6) 0)
                    (Game|SpawnActorfromClass "/Game/Ironsphere/Missions/BP_MissionDen.BP_MissionDen_C" (Transformation|GetActorTransform) "Undefined" "MultiplyWithRoot" 0 false 0)
                    (bind _returnvalue_7 (Actor|GetActorOfClass "/Game/Ironsphere/Missions/Capturing/BP_MissionCapturing.BP_MissionCapturing_C"))
                    (Math|Integer|DecrementInt (Variables|/Game/Ironsphere/Missions/Capturing/BP_MissionCapturing.BP_MissionCapturing_C|GetNumberOfHides _returnvalue_7)
                      (:%20%20
                        (Actor|DestroyActor)))))
                (:3
                  (bind _returnvalue_8 (Actor|GetActorOfClass "/Game/Ironsphere/Missions/Capturing/BP_MissionCapturing.BP_MissionCapturing_C"))
                  (if (> (Variables|/Game/Ironsphere/Missions/Capturing/BP_MissionCapturing.BP_MissionCapturing_C|GetNumberOfTurrets _returnvalue_8) 0)
                    (Game|SpawnActorfromClass "/Game/Ironsphere/Missions/BP_MissionTurret.BP_MissionTurret_C" (Transformation|GetActorTransform) "Undefined" "MultiplyWithRoot" 0 0)
                    (bind _returnvalue_9 (Actor|GetActorOfClass "/Game/Ironsphere/Missions/Capturing/BP_MissionCapturing.BP_MissionCapturing_C"))
                    (Math|Integer|DecrementInt (Variables|/Game/Ironsphere/Missions/Capturing/BP_MissionCapturing.BP_MissionCapturing_C|GetNumberOfTurrets _returnvalue_9)
                      (:%20%20
                        (Actor|DestroyActor)))))))))))))

(fn ConstructionScript)