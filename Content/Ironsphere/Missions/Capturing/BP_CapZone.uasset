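; Capture zone objective that fills a progress bar while the first player character stands close to it, then awards experience on completion.
; BeginPlay snaps it to ground height zero, adds a minimap icon and attaches an objective arrow to the player's mech.
; Tick runs the distance-based capture, removing the arrow and announcing success when full.
; It also spawns rotating lights on a timer, red until captured, and collapses the minimap icon afterwards.
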(event EventBeginPlay
  (bind _returnvalue (Transformation|GetActorLocation))
  (bind _returnvalue_2 (Transformation|GetActorLocation))
  (bind (_x _y) (Math|Vector|BreakVector _returnvalue))
  (bind (_x_2 _y_2) (Math|Vector|BreakVector _returnvalue_2))
  (Transformation|SetActorLocation (Math|Vector|MakeVector _x _y 0.0) false false)
  (Rendering|SetVisibility (Variables|Default|GetWidgetProgressBar) true false)
  (bind _returnvalue_3 (UserInterface|CreateWidget "/Game/Ironsphere/UI/Ingame/Map/WBS_MinimapObject.WBS_MinimapObject_C" 0 "/Game/Ironsphere/UI/Ingame/Map/Objective.Objective" true))
  (Variables|Default|SetObject%20Map _returnvalue_3)
  (UserInterface|Viewport|AddtoViewport _returnvalue_3 1)
  (Class|UserWidget|SetPositioninViewport _returnvalue_3 (Math|Vector2D|MakeVector2D (+ (* _x_2 -0.1) 2e+02) (+ (* _y_2 -0.1) 2e+02)) true)
  (bind _aswbc_progress_bar (Utilities|Casting|CastToWBC_ProgressBar (UserInterface|GetWidget (Variables|Default|GetWidgetProgressBar))))
  (Default|UpdateProgress _aswbc_progress_bar (Variables|Default|GetCapturingPercent))
  (bind _aspc_ingame (Utilities|Casting|CastToPC_Ingame (Game|GetPlayerController 0))
    (:then
      (bind _returnvalue_4 (Game|SpawnActorfromClass "/Game/Ironsphere/Core/Player/BP_ObjectiveArrow.BP_ObjectiveArrow_C" (Math|Transform|MakeTransform "0, 0, 0") "Undefined" "MultiplyWithRoot" (Variables|/Game/Ironsphere/Core/Framework/Battle/PC_Ingame.PC_Ingame_C|GetControlledMech _aspc_ingame) self 0))
      (Transformation|AttachActorToActor _returnvalue_4 (Variables|/Game/Ironsphere/Core/Framework/Battle/PC_Ingame.PC_Ingame_C|GetControlledMech _aspc_ingame) "None" "KeepRelative" "KeepWorld" "KeepRelative" true)
      (Variables|Default|SetArrow _returnvalue_4))
    (:CastFailed
      (Audio|SpawnSound2D "/Engine/EditorSounds/Notifications/CompileFailed.CompileFailed" 1.0 1.0 0.0 0))))

(event Collision|EventActorBeginOverlap
  (params (OtherActor :type Actor%20Object%20Reference)))

(event EventTick
  (params (DeltaSeconds :type Float%20%28single-precision%29))
  (bind _returnvalue (Transformation|GetActorTransform))
  (bind (_location _rotation _scale) (Math|Transform|BreakTransform _returnvalue))
  (Utilities|FlowControl|Sequence
    (:then_0
      (if (Variables|Default|GetCaptured)
        (Rendering|SetVisibility (Variables|Default|GetWidgetProgressBar) false false)
        (else
          (bind _outactors (Actor|GetAllActorsOfClass "/Game/Ironsphere/Core/Player/BP_CharacterPlayer.BP_CharacterPlayer_C"))
          (if (< (Math|Vector|VectorLength (- (Transformation|GetActorLocation (Utilities|Array|Get(acopy) _outactors)) (Transformation|GetActorLocation))) 7e+01)
            (Variables|Default|SetCapturingPercent (+ (Variables|Default|GetCapturingPercent) (* DeltaSeconds 0.2)))
            (bind _aswbc_progress_bar (Utilities|Casting|CastToWBC_ProgressBar (UserInterface|GetWidget (Variables|Default|GetWidgetProgressBar))))
            (Default|UpdateProgress _aswbc_progress_bar (Variables|Default|GetCapturingPercent))
            (if (>= (Variables|Default|GetCapturingPercent) 1.0)
              (Variables|Default|SetCaptured true)
              (bind _asgi_main (Utilities|Casting|CastToGI_Main (Game|GetGameInstance)))
              (Variables|/Game/Ironsphere/Core/Framework/GI_Main.GI_Main_C|SetExperience _asgi_main (+ (Variables|/Game/Ironsphere/Core/Framework/GI_Main.GI_Main_C|GetExperience _asgi_main) 3e+01))
              (Audio|SpawnSound2D "/Engine/VREditor/Sounds/UI/Click_on_Button.Click_on_Button" 1.0 1.0 0.0 0)
              (bind _returnvalue_2 (UserInterface|CreateWidget "/Game/Ironsphere/UI/Ingame/WBC_ObjectiveOnStart.WBC_ObjectiveOnStart_C" 0 "Zone captured!"))
              (UserInterface|Viewport|AddtoViewport _returnvalue_2 0)
              (Actor|DestroyActor (Variables|Default|GetArrow)))))))
    (:then_1
      (if (> (Variables|Default|GetTimerSpawnLight) 0.1)
        (Variables|Default|SetTimerSpawnLight 0.0)
        (bind _output_get (Variables|Default|SetLightAngle (+ (Variables|Default|GetLightAngle) 15.0)))
        (if (>= _output_get 3.6e+02)
          (Variables|Default|SetLightAngle 0.0))
        (if (Variables|Default|GetCaptured)
          (Game|SpawnActorfromClass "/Game/Ironsphere/Missions/Capturing/BP_CapZoneLight.BP_CapZoneLight_C" (Math|Transform|MakeTransform _location (Math|Rotator|MakeRotator 0.0 0.0 (Variables|Default|GetLightAngle)) _scale) "Undefined" "MultiplyWithRoot" 0 false 0)
          (Utilities|FlowControl|DoOnce false
            (:Completed
              (Widget|SetVisibility (Variables|Default|GetObject%20Map) "Collapsed")))
          (else
            (Game|SpawnActorfromClass "/Game/Ironsphere/Missions/Capturing/BP_CapZoneLight.BP_CapZoneLight_C" (Math|Transform|MakeTransform _location (Math|Rotator|MakeRotator 0.0 0.0 (Variables|Default|GetLightAngle)) _scale) "Undefined" "MultiplyWithRoot" 0 true 0)))
        (else
          (Variables|Default|SetTimerSpawnLight (+ (Variables|Default|GetTimerSpawnLight) DeltaSeconds)))))))

(fn ConstructionScript)