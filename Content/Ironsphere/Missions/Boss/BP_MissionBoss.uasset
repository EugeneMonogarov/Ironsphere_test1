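; Boss mission Blueprint that sets a "Kill the boss!" objective, a level timer and a den count scaled by the square root of the current mission number.
; Tick passes the objective once BossKilled is set, and until then permanently fails the bonus if the player mech drops below half HP.
; UI text mismatches this logic, showing a survival timer and cargo ship HP; neither the timer countdown nor BossKilled trigger is here.
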(event EventBeginPlay
  (bind _gs_battle_ref (Variables|Default|GetGS_Battle_ref))
  (|CallParentFunction)
  (Utilities|FlowControl|Sequence
    (:then_0
      (Variables|/Game/Ironsphere/Core/Framework/Battle/GS_Battle.GS_Battle_C|SetObjective (Variables|Default|GetGS_Battle_ref) "Kill the boss!"))
    (:then_1
      (Variables|Default|SetNumberOfDens (+ (* (Math|Float|Sqrt (Math|Conversions|ToFloat(Integer) (Variables|/Game/Ironsphere/Core/Framework/GI_Main.GI_Main_C|GetCurrentMission (Variables|Default|GetGI_Main_ref)))) 2.0) 3)))
    (:then_2
      (Variables|/Game/Ironsphere/Core/Framework/Battle/GS_Battle.GS_Battle_C|SetObjectivePassed _gs_battle_ref false)
      (Variables|Default|SetLevelTimer 1.8e+02)
      (Variables|/Game/Ironsphere/Core/Framework/Battle/GS_Battle.GS_Battle_C|SetBonusObjectivepassed _gs_battle_ref true)
      (Variables|Default|SetBossKilled false))))

(event Collision|EventActorBeginOverlap
  (params (OtherActor :type Actor%20Object%20Reference))
  (|CallParentFunction OtherActor) ; This node is disabled and will not be called.\nDrag off pins to build functionality.
)

(event EventTick
  (params (DeltaSeconds :type Float%20%28single-precision%29))
  (bind _pc_ingame_ref (Variables|Default|GetPC_Ingame_ref))
  (bind _gs_battle_ref (Variables|Default|GetGS_Battle_ref))
  (bind _controlledmech (Variables|/Game/Ironsphere/Core/Framework/Battle/PC_Ingame.PC_Ingame_C|GetControlledMech _pc_ingame_ref))
  (|CallParentFunction DeltaSeconds)
  (if (Utilities|IsValid (Variables|Default|GetGS_Battle_ref))
    (Utilities|FlowControl|Sequence
      (:then_0
        (if (Variables|Default|GetBossKilled)
          (Variables|/Game/Ironsphere/Core/Framework/Battle/GS_Battle.GS_Battle_C|SetObjectivePassed (Variables|Default|GetGS_Battle_ref) true)
          (elif (< (/ (Variables|/Game/Ironsphere/Core/Character/BP_CharacterBase.BP_CharacterBase_C|GetCurrentHP _controlledmech) (Variables|/Game/Ironsphere/Core/Character/BP_CharacterBase.BP_CharacterBase_C|GetMaxHP _controlledmech)) 0.5)
            (Variables|/Game/Ironsphere/Core/Framework/Battle/GS_Battle.GS_Battle_C|SetBonusObjectivepassed (Variables|Default|GetGS_Battle_ref) false))))
      (:then_1
        (Variables|/Game/Ironsphere/Core/Framework/Battle/GS_Battle.GS_Battle_C|SetObjectiveUI _gs_battle_ref (Utilities|Text|FormatText "Survive for {x} srconds." (Utilities|Text|ToText(String) (Class|KismetMathLibrary|ToInt64(Float) (Variables|Default|GetLevelTimer)))))
        (if (Variables|/Game/Ironsphere/Core/Framework/Battle/GS_Battle.GS_Battle_C|GetBonusObjectivepassed _gs_battle_ref)
          (Variables|/Game/Ironsphere/Core/Framework/Battle/GS_Battle.GS_Battle_C|SetBonusObjectiveUI _gs_battle_ref "Maintain 50% HP of cargo ship")
          (else
            (Variables|/Game/Ironsphere/Core/Framework/Battle/GS_Battle.GS_Battle_C|SetBonusObjectiveUI _gs_battle_ref "Maintain 50% HP of cargo ship(failed)")))))))

(fn ConstructionScript
  (|CallParentFunction))