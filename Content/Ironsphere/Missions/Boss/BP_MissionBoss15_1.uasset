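; Boss mission 15_1, where the player protects a cargo ship, with a bonus for keeping it at 50% HP.
; BeginPlay sets objectives, a timer, random wave count and a spawner count scaled by the mission number's square root.
; Tick polls actors by class: no giant cannon or laser spiders late in the timer passes the mission, otherwise a missing ship after the start delay fails it.
; Tick also updates bonus status and objective UI text.
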(event EventBeginPlay
  (bind _gs_battle_ref (Variables|Default|GetGS_Battle_ref))
  (bind _gs_battle_ref_2 (Variables|Default|GetGS_Battle_ref))
  (|CallParentFunction)
  (Utilities|FlowControl|Sequence
    (:then_0
      (Variables|/Game/Ironsphere/Core/Framework/Battle/GS_Battle.GS_Battle_C|SetObjective _gs_battle_ref_2 "Protect the cargo ship!")
      (Variables|/Game/Ironsphere/Core/Framework/Battle/GS_Battle.GS_Battle_C|SetBonusObjective _gs_battle_ref_2 "Maintain 50% HP of cargo ship"))
    (:then_1
      (Variables|Default|SetNumberOfSpawners (+ (* (Math|Float|Sqrt (Math|Conversions|ToFloat(Integer) (Variables|/Game/Ironsphere/Core/Framework/GI_Main.GI_Main_C|GetCurrentMission (Variables|Default|GetGI_Main_ref)))) 0.5) 4 0))
      (Variables|Default|SetNumberOfWaves (Math|Random|RandomIntegerinRange 4 5))
      (while (> (Variables|Default|GetNumberOfSpawners) 0)
        (Math|Integer|IncrementInt (Variables|Default|GetNumberOfInstants)
          (:%20%20
            (Math|Integer|DecrementInt (Variables|Default|GetNumberOfSpawners)))))
      (Variables|Default|SetMaximalSpawnersInWave 0))
    (:then_2
      (Variables|/Game/Ironsphere/Core/Framework/Battle/GS_Battle.GS_Battle_C|SetObjectivePassed _gs_battle_ref false)
      (Variables|Default|SetLevelTimer 1.8e+02)
      (Variables|/Game/Ironsphere/Core/Framework/Battle/GS_Battle.GS_Battle_C|SetBonusObjectivepassed _gs_battle_ref true))))

(event Collision|EventActorBeginOverlap
  (params (OtherActor :type Actor%20Object%20Reference))
  (|CallParentFunction OtherActor) ; This node is disabled and will not be called.\nDrag off pins to build functionality.
)

(event EventTick
  (params (DeltaSeconds :type Float%20%28single-precision%29))
  (bind _gs_battle_ref (Variables|Default|GetGS_Battle_ref))
  (bind _gs_battle_ref_2 (Variables|Default|GetGS_Battle_ref))
  (|CallParentFunction DeltaSeconds)
  (if (Utilities|IsValid (Variables|Default|GetGS_Battle_ref))
    (Utilities|FlowControl|Sequence
      (:then_0
        (bind _outactors (Actor|GetAllActorsOfClass "/Game/Ironsphere/Feature/NPC/SpiderDroid/BP_GiantCannonSpider.BP_GiantCannonSpider_C"))
        (bind _outactors_2 (Actor|GetAllActorsOfClass "/Game/Ironsphere/Feature/NPC/SpiderDroid/BP_GiantLaserSpider.BP_GiantLaserSpider_C"))
        (if (and (< (Variables|Default|GetLevelTimer) 9e+01) (== (+ (Utilities|Array|Length _outactors_2) (Utilities|Array|Length _outactors)) 0))
          (Variables|/Game/Ironsphere/Core/Framework/Battle/GS_Battle.GS_Battle_C|SetObjectivePassed (Variables|Default|GetGS_Battle_ref) true)
          (else
            (bind _outactors_3 (Actor|GetAllActorsOfClass "/Game/Ironsphere/Feature/World/LevelObjectives/BP_CargoShip.BP_CargoShip_C"))
            (if (and (== (Utilities|Array|Length _outactors_3) 0) (> (Variables|/Game/Ironsphere/Core/Framework/Battle/GS_Battle.GS_Battle_C|GetStartDelay _gs_battle_ref) 5.0))
              (Variables|/Game/Ironsphere/Core/Framework/Battle/GS_Battle.GS_Battle_C|SetMissionFailed _gs_battle_ref true))
            (if (Utilities|IsValid (Utilities|Array|Get(acopy) _outactors_3))
              (if (< (/ (Variables|/Game/Ironsphere/Feature/World/BP_WorldObjectDistructable.BP_WorldObjectDistructable_C|GetCurrentHP (Utilities|Array|Get(acopy) _outactors_3)) (Variables|/Game/Ironsphere/Feature/World/BP_WorldObjectDistructable.BP_WorldObjectDistructable_C|GetMaxHP (Utilities|Array|Get(acopy) _outactors_3))) 0.5)
                (Variables|/Game/Ironsphere/Core/Framework/Battle/GS_Battle.GS_Battle_C|SetBonusObjectivepassed (Variables|Default|GetGS_Battle_ref) false))))))
      (:then_1
        (Variables|/Game/Ironsphere/Core/Framework/Battle/GS_Battle.GS_Battle_C|SetObjectiveUI _gs_battle_ref_2 (Utilities|Text|FormatText "Protect the cargo ship for {x} srconds." (Utilities|Text|ToText(String) (Class|KismetMathLibrary|ToInt64(Float) (Variables|Default|GetLevelTimer)))))
        (if (Variables|/Game/Ironsphere/Core/Framework/Battle/GS_Battle.GS_Battle_C|GetBonusObjectivepassed _gs_battle_ref_2)
          (Variables|/Game/Ironsphere/Core/Framework/Battle/GS_Battle.GS_Battle_C|SetBonusObjectiveUI _gs_battle_ref_2 "Maintain 50% HP of cargo ship")
          (else
            (Variables|/Game/Ironsphere/Core/Framework/Battle/GS_Battle.GS_Battle_C|SetBonusObjectiveUI _gs_battle_ref_2 "Maintain 50% HP of cargo ship(failed)")))))))

(fn ConstructionScript
  (|CallParentFunction))