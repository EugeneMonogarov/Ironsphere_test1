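; BP_CargoTrack is the convoy mission's cargo objective, a destructible vehicle that creeps forward unless a forward sphere trace finds an obstacle.
; On spawn it scales max HP by mission number, attaches objective arrows to the player's mech (in two separate branches) and places a minimap icon.
; While the mech is close, it regains HP at a mission-scaled rate.
; Its Destruction override only clears IsAlive, bypassing the parent logic.
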(event EventBeginPlay
  (bind _returnvalue (Transformation|GetActorLocation))
  (bind (_x _y) (Math|Vector|BreakVector _returnvalue))
  (|CallParentFunction)
  (Utilities|FlowControl|Sequence
    (:then_0
      (bind _asgi_main (Utilities|Casting|CastToGI_Main (Game|GetGameInstance)))
      (Variables|Default|SetAs%20GI%20Main _asgi_main)
      (bind _output_get (Variables|Default|SetMaxHP (Math|Conversions|ToFloat(Integer) (+ (* (Variables|/Game/Ironsphere/Core/Framework/GI_Main.GI_Main_C|GetCurrentMission _asgi_main) 25) 100))))
      (Variables|Default|SetCurrentHP _output_get)
      (bind _aspc_ingame (Utilities|Casting|CastToPC_Ingame (Game|GetPlayerController 0)))
      (Variables|Default|SetMech (Variables|/Game/Ironsphere/Core/Framework/Battle/PC_Ingame.PC_Ingame_C|GetControlledMech _aspc_ingame))
      (bind _returnvalue_2 (Game|SpawnActorfromClass "/Game/Ironsphere/Core/Player/BP_ObjectiveArrow.BP_ObjectiveArrow_C" (Math|Transform|MakeTransform "0, 0, 0") "Undefined" "MultiplyWithRoot" (Variables|/Game/Ironsphere/Core/Framework/Battle/PC_Ingame.PC_Ingame_C|GetControlledMech _aspc_ingame) self 0))
      (Transformation|AttachActorToActor _returnvalue_2 (Variables|/Game/Ironsphere/Core/Framework/Battle/PC_Ingame.PC_Ingame_C|GetControlledMech _aspc_ingame) "None" "KeepRelative" "KeepRelative" "KeepRelative" true))
    (:then_1
      (bind _aspc_ingame_2 (Utilities|Casting|CastToPC_Ingame (Game|GetPlayerController 0))
        (:then
          (bind _returnvalue_3 (Game|SpawnActorfromClass "/Game/Ironsphere/Core/Player/BP_ObjectiveArrow.BP_ObjectiveArrow_C" (Math|Transform|MakeTransform "0, 0, 0") "Undefined" "MultiplyWithRoot" (Variables|/Game/Ironsphere/Core/Framework/Battle/PC_Ingame.PC_Ingame_C|GetControlledMech _aspc_ingame_2) self 0))
          (Transformation|AttachActorToActor _returnvalue_3 (Variables|/Game/Ironsphere/Core/Framework/Battle/PC_Ingame.PC_Ingame_C|GetControlledMech _aspc_ingame_2) "None" "KeepRelative" "KeepRelative" "KeepRelative" true))
        (:CastFailed
          (Audio|SpawnSound2D "/Engine/EditorSounds/Notifications/CompileFailed.CompileFailed" 1.0 1.0 0.0 0))))
    (:then_2
      (bind _returnvalue_4 (UserInterface|CreateWidget "/Game/Ironsphere/UI/Ingame/Map/WBS_MinimapObject.WBS_MinimapObject_C" 0 "/Game/Ironsphere/UI/Ingame/Map/Objective.Objective" true))
      (bind _output_get_2 (Variables|Default|SetObject%20Map _returnvalue_4))
      (UserInterface|Viewport|AddtoViewport _returnvalue_4 1)
      (Class|UserWidget|SetPositioninViewport _returnvalue_4 (Math|Vector2D|MakeVector2D (+ (* _x -0.1) 2e+02) (+ (* _y -0.1) 2e+02)) true))))

(event Collision|EventActorBeginOverlap
  (params (OtherActor :type Actor%20Object%20Reference)))

(event EventTick
  (params (DeltaSeconds :type Float%20%28single-precision%29))
  (|CallParentFunction DeltaSeconds)
  (Utilities|FlowControl|Sequence
    (:then_0
      (CallFunction|UpdateHPbar)
      (if (< (Variables|Default|GetCurrentHP) (Variables|Default|GetMaxHP))
        (if (< (Math|Vector|VectorLength (- (Transformation|GetActorLocation (Variables|Default|GetMech)) (Transformation|GetActorLocation))) 1.5e+02)
          (Variables|Default|SetCurrentHP (+ (* DeltaSeconds 3.0) (* DeltaSeconds (/ (Variables|/Game/Ironsphere/Core/Framework/GI_Main.GI_Main_C|GetCurrentMission (stale EventBeginPlay _asgi_main)) 4)) (Variables|Default|GetCurrentHP)))
          (if (> (Variables|Default|GetCurrentHP) (Variables|Default|GetMaxHP))
            (Variables|Default|SetCurrentHP (Variables|Default|GetMaxHP))))))
    (:then_1
      (bind _returnvalue (Collision|SphereTraceForObjects (Transformation|GetActorLocation) (+ (Transformation|GetActorLocation) (* (Math|Vector|Normalize (Transformation|GetActorForwardVector)) 1.2e+02)) 22.0 (Utilities|Array|MakeArray "ObjectTypeQuery6" "ObjectTypeQuery7" "ObjectTypeQuery8") false 0 "ForOneFrame" true "(R=1.000000,G=0.000000,B=0.000000,A=1.000000)" "(R=0.000000,G=1.000000,B=0.000000,A=1.000000)" 0.25))
      (if (not _returnvalue)
        (Transformation|AddActorLocalOffset (Math|Vector|MakeVector (* DeltaSeconds 25.0) 0.0 0.0) false false)))))

(fn ConstructionScript)

(fn UpdateHPbar
  (|CallParentFunction))

(fn Destruction
  (params (IsBlow :type Boolean) (Damage :type Float%20%28double-precision%29) (Radius :type Float%20%28double-precision%29) (Sound :type SoundDestroy%20Enum :default "NewEnumerator0"))
  (Variables|Default|SetIsAlive false))