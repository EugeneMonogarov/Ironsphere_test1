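; Candidate spawn point for the Convoy mission that randomly becomes an ambush or a turret.
; After a short startup delay, each Tick it removes itself if the first player character is very close, otherwise rolls chances to spawn either type at its transform.
; Spawns draw down shared counters on BP_MissionConvoy and destroy the spawner.
; A delayed BeginPlay check also destroys it if both counters are empty.
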(event EventBeginPlay
  (Variables|Default|SetLetAmbushesAdd false)
  (Utilities|FlowControl|Delay 1.0)
  (Variables|Default|SetLetAmbushesAdd true)
  (Utilities|FlowControl|Delay 1.0 :!label _label)
  (bind _returnvalue (Actor|GetActorOfClass "/Game/Ironsphere/Missions/Convoy/BP_MissionConvoy.BP_MissionConvoy_C"))
  (if (== (+ (Variables|/Game/Ironsphere/Missions/Convoy/BP_MissionConvoy.BP_MissionConvoy_C|GetNumberOfAmbushes _returnvalue) (Variables|/Game/Ironsphere/Missions/Convoy/BP_MissionConvoy.BP_MissionConvoy_C|GetNumberOfTurrets _returnvalue)) 0)
    (Actor|DestroyActor)
    (goto _label)))

(event Collision|EventActorBeginOverlap
  (params (OtherActor :type Actor%20Object%20Reference)))

(event EventTick
  (params (DeltaSeconds :type Float%20%28single-precision%29))
  (if (Variables|Default|GetLetAmbushesAdd)
    (bind _outactors (Actor|GetAllActorsOfClass "/Game/Ironsphere/Core/Player/BP_CharacterPlayer.BP_CharacterPlayer_C"))
    (if (< (Math|Vector|VectorLength (- (Transformation|GetActorLocation (Utilities|Array|Get(acopy) _outactors)) (Transformation|GetActorLocation))) 2e+02)
      (Actor|DestroyActor)
      (else
        (Utilities|FlowControl|Sequence
          (:then_0
            (bind _returnvalue (Actor|GetActorOfClass "/Game/Ironsphere/Missions/Convoy/BP_MissionConvoy.BP_MissionConvoy_C"))
            (if (> (Variables|/Game/Ironsphere/Missions/Convoy/BP_MissionConvoy.BP_MissionConvoy_C|GetNumberOfAmbushes _returnvalue) 0)
              (if (> (Math|Random|RandomFloatinRange 0.0 1.0) 0.96)
                (Game|SpawnActorfromClass "/Game/Ironsphere/Missions/BP_MissionAmbush.BP_MissionAmbush_C" (Transformation|GetActorTransform) "Undefined" "MultiplyWithRoot" 0 0.0 0)
                (bind _returnvalue_2 (Actor|GetActorOfClass "/Game/Ironsphere/Missions/Convoy/BP_MissionConvoy.BP_MissionConvoy_C"))
                (Math|Integer|DecrementInt (Variables|/Game/Ironsphere/Missions/Convoy/BP_MissionConvoy.BP_MissionConvoy_C|GetNumberOfAmbushes _returnvalue_2)
                  (:%20%20
                    (Actor|DestroyActor))))))
          (:then_1
            (bind _returnvalue_3 (Actor|GetActorOfClass "/Game/Ironsphere/Missions/Convoy/BP_MissionConvoy.BP_MissionConvoy_C"))
            (if (> (Variables|/Game/Ironsphere/Missions/Convoy/BP_MissionConvoy.BP_MissionConvoy_C|GetNumberOfTurrets _returnvalue_3) 0)
              (if (> (Math|Random|RandomFloatinRange 0.0 1.0) 0.9)
                (Game|SpawnActorfromClass "/Game/Ironsphere/Missions/BP_MissionTurret.BP_MissionTurret_C" (Transformation|GetActorTransform) "Undefined" "MultiplyWithRoot" 0 0)
                (bind _returnvalue_4 (Actor|GetActorOfClass "/Game/Ironsphere/Missions/Convoy/BP_MissionConvoy.BP_MissionConvoy_C"))
                (Math|Integer|DecrementInt (Variables|/Game/Ironsphere/Missions/Convoy/BP_MissionConvoy.BP_MissionConvoy_C|GetNumberOfTurrets _returnvalue_4)
                  (:%20%20
                    (Actor|DestroyActor)))))))))))

(fn ConstructionScript)