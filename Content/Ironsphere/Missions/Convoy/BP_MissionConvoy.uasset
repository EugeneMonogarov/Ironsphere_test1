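; Convoy mission Blueprint for protecting the cargo track until the level timer expires, with a bonus objective to keep it at 50% HP.
; BeginPlay sets objectives and scales spawner and turret counts from mission number, turrets also by difficulty; a loop converts spawners into an ambush count.
; Tick polls for BP_CargoTrack actors to update pass, fail and bonus flags on GSBattleRef, then refreshes objective UI text.
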(event EventBeginPlay
  (bind _gs_battle_ref (Variables|Default|GetGS_Battle_ref))
  (bind _gi_main_ref (Variables|Default|GetGI_Main_ref))
  (|CallParentFunction)
  (Utilities|FlowControl|Sequence
    (:then_0
      (Variables|/Game/Ironsphere/Core/Framework/Battle/GS_Battle.GS_Battle_C|SetObjective _gs_battle_ref "Protect the cargo track!")
      (Variables|/Game/Ironsphere/Core/Framework/Battle/GS_Battle.GS_Battle_C|SetBonusObjective _gs_battle_ref "Maintain 50% HP of cargo track"))
    (:then_1
      (Variables|Default|SetNumberOfSpawners (+ (/ (Math|Float|Sqrt (Math|Conversions|ToFloat(Integer) (Variables|/Game/Ironsphere/Core/Framework/GI_Main.GI_Main_C|GetCurrentMission (Variables|Default|GetGI_Main_ref)))) 2.0) 4))
      (Variables|Default|SetNumberOfAmbushes 0)
      (while (> (Variables|Default|GetNumberOfSpawners) 0)
        (Math|Integer|IncrementInt (Variables|Default|GetNumberOfAmbushes)
          (:%20%20
            (Math|Integer|DecrementInt (Variables|Default|GetNumberOfSpawners))))))
    (:then_2
      (Variables|/Game/Ironsphere/Core/Framework/Battle/GS_Battle.GS_Battle_C|SetBonusObjectivepassed (Variables|Default|GetGS_Battle_ref) true))
    (:then_3
      (Variables|Default|SetNumberOfTurrets (+ (/ (Variables|/Game/Ironsphere/Core/Framework/GI_Main.GI_Main_C|GetCurrentMission _gi_main_ref) 3) (Variables|/Game/Ironsphere/Core/Framework/GI_Main.GI_Main_C|GetDifficultyLevel _gi_main_ref) 2)))))

(event Collision|EventActorBeginOverlap
  (params (OtherActor :type Actor%20Object%20Reference))
  (|CallParentFunction OtherActor) ; This node is disabled and will not be called.\nDrag off pins to build functionality.
)

(event EventTick
  (params (DeltaSeconds :type Float%20%28single-precision%29))
  (bind _gs_battle_ref (Variables|Default|GetGS_Battle_ref))
  (bind _gs_battle_ref_2 (Variables|Default|GetGS_Battle_ref))
  (|CallParentFunction DeltaSeconds)
  (if (Utilities|IsValid (Variables|Default|GetGS_Battle_ref))
    (Utilities|FlowControl|Sequence
      (:then_0
        (if (<= (Variables|Default|GetLevelTimer) 0.0)
          (Variables|/Game/Ironsphere/Core/Framework/Battle/GS_Battle.GS_Battle_C|SetObjectivePassed (Variables|Default|GetGS_Battle_ref) true))
        (bind _outactors (Actor|GetAllActorsOfClass "/Game/Ironsphere/Missions/Convoy/BP_CargoTrack.BP_CargoTrack_C"))
        (if (and (== (Utilities|Array|Length _outactors) 0) (> (Variables|/Game/Ironsphere/Core/Framework/Battle/GS_Battle.GS_Battle_C|GetStartDelay _gs_battle_ref) 5.0))
          (Variables|/Game/Ironsphere/Core/Framework/Battle/GS_Battle.GS_Battle_C|SetMissionFailed _gs_battle_ref true)
          (elif (and (<= (Variables|Default|GetLevelTimer) 175.0) (< (/ (Variables|/Game/Ironsphere/Feature/World/BP_WorldObjectDistructable.BP_WorldObjectDistructable_C|GetCurrentHP (Utilities|Array|Get(acopy) _outactors)) (Variables|/Game/Ironsphere/Feature/World/BP_WorldObjectDistructable.BP_WorldObjectDistructable_C|GetMaxHP (Utilities|Array|Get(acopy) _outactors))) 0.5))
            (Variables|/Game/Ironsphere/Core/Framework/Battle/GS_Battle.GS_Battle_C|SetBonusObjectivepassed (Variables|Default|GetGS_Battle_ref) false))))
      (:then_1
        (Variables|/Game/Ironsphere/Core/Framework/Battle/GS_Battle.GS_Battle_C|SetObjectiveUI _gs_battle_ref_2 (Utilities|Text|FormatText "Protect the cargo track"))
        (if (Variables|/Game/Ironsphere/Core/Framework/Battle/GS_Battle.GS_Battle_C|GetBonusObjectivepassed _gs_battle_ref_2)
          (Variables|/Game/Ironsphere/Core/Framework/Battle/GS_Battle.GS_Battle_C|SetBonusObjectiveUI _gs_battle_ref_2 "Maintain 50% HP of cargo track")
          (else
            (Variables|/Game/Ironsphere/Core/Framework/Battle/GS_Battle.GS_Battle_C|SetBonusObjectiveUI _gs_battle_ref_2 "Maintain 50% HP of cargo track(failed)")))))))

(fn ConstructionScript
  (|CallParentFunction))