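; Survival mission spawn point that may turn into a BP_MissionDen at its own location.
; Each tick it destroys itself if the first player character found is within 300 units.
; Otherwise, while BP_MissionSurvival has NumberOfDens left, it has a roughly 10% chance per tick to spawn a den, decrement that shared count and destroy itself.
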(event EventBeginPlay)

(event Collision|EventActorBeginOverlap
  (params (OtherActor :type Actor%20Object%20Reference)))

(event EventTick
  (params (DeltaSeconds :type Float%20%28single-precision%29))
  (bind _outactors (Actor|GetAllActorsOfClass "/Game/Ironsphere/Core/Player/BP_CharacterPlayer.BP_CharacterPlayer_C"))
  (if (< (Math|Vector|VectorLength (- (Transformation|GetActorLocation (Utilities|Array|Get(acopy) _outactors)) (Transformation|GetActorLocation))) 3e+02)
    (Actor|DestroyActor)
    (else
      (bind _returnvalue (Actor|GetActorOfClass "/Game/Ironsphere/Missions/Survival/BP_MissionSurvival.BP_MissionSurvival_C"))
      (if (> (Variables|/Game/Ironsphere/Missions/Survival/BP_MissionSurvival.BP_MissionSurvival_C|GetNumberOfDens _returnvalue) 0)
        (if (> (Math|Random|RandomFloatinRange 0.0 1.0) 0.9)
          (Utilities|FlowControl|Sequence
            (:then_0
              (Game|SpawnActorfromClass "/Game/Ironsphere/Missions/BP_MissionDen.BP_MissionDen_C" (Transformation|GetActorTransform) "Undefined" "MultiplyWithRoot" 0 0))
            (:then_1
              (bind _returnvalue_2 (Actor|GetActorOfClass "/Game/Ironsphere/Missions/Survival/BP_MissionSurvival.BP_MissionSurvival_C"))
              (Math|Integer|DecrementInt (Variables|/Game/Ironsphere/Missions/Survival/BP_MissionSurvival.BP_MissionSurvival_C|GetNumberOfDens _returnvalue_2)
                (:%20%20
                  (Actor|DestroyActor))))))))))

(fn ConstructionScript)