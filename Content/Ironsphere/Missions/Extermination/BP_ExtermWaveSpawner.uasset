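; One-shot wave spawn point for the Extermination mission, which creates a BP_ExtermWave at its own transform.
; After a one-second wait it caches the mission's wave count, then destroys itself if the player is too near or no waves remain.
; Otherwise a random per-tick roll spawns a wave, decrements the shared counter and destroys the spawner.
; Each wave's Delay grows with waves already claimed, staggering them over roughly two minutes.
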(event EventBeginPlay
  (Variables|Default|SetLetWavesAdd false)
  (Utilities|FlowControl|Delay 1.0)
  (bind _returnvalue (Actor|GetActorOfClass "/Game/Ironsphere/Missions/Extermination/BP_MissionExtermination.BP_MissionExtermination_C"))
  (bind _output_get (Variables|Default|SetWavesSumm (Variables|/Game/Ironsphere/Missions/Extermination/BP_MissionExtermination.BP_MissionExtermination_C|GetNumberOfWaves _returnvalue)))
  (Variables|Default|SetLetWavesAdd true))

(event Collision|EventActorBeginOverlap
  (params (OtherActor :type Actor%20Object%20Reference)))

(event EventTick
  (params (DeltaSeconds :type Float%20%28single-precision%29))
  (bind _wavessumm (Variables|Default|GetWavesSumm))
  (if (Variables|Default|GetLetWavesAdd)
    (bind _outactors (Actor|GetAllActorsOfClass "/Game/Ironsphere/Core/Player/BP_CharacterPlayer.BP_CharacterPlayer_C"))
    (if (< (Math|Vector|VectorLength (- (Transformation|GetActorLocation (Utilities|Array|Get(acopy) _outactors)) (Transformation|GetActorLocation))) 2e+02)
      (Actor|DestroyActor)
      (else
        (bind _returnvalue (Actor|GetActorOfClass "/Game/Ironsphere/Missions/Extermination/BP_MissionExtermination.BP_MissionExtermination_C"))
        (if (> (Variables|/Game/Ironsphere/Missions/Extermination/BP_MissionExtermination.BP_MissionExtermination_C|GetNumberOfWaves _returnvalue) 0)
          (if (> (Math|Random|RandomFloatinRange 0.0 1.0) 0.98)
            (Game|SpawnActorfromClass "/Game/Ironsphere/Missions/Extermination/BP_ExtermWave.BP_ExtermWave_C" (Transformation|GetActorTransform) "Undefined" "MultiplyWithRoot" 0 (+ 1.0 (* (* (/ 120 _wavessumm) (- _wavessumm (Variables|/Game/Ironsphere/Missions/Extermination/BP_MissionExtermination.BP_MissionExtermination_C|GetNumberOfWaves _returnvalue))) 1.0)) 0)
            (bind _returnvalue_2 (Actor|GetActorOfClass "/Game/Ironsphere/Missions/Extermination/BP_MissionExtermination.BP_MissionExtermination_C"))
            (Math|Integer|DecrementInt (Variables|/Game/Ironsphere/Missions/Extermination/BP_MissionExtermination.BP_MissionExtermination_C|GetNumberOfWaves _returnvalue_2)
              (:%20%20
                (Actor|DestroyActor))))
          (else
            (Actor|DestroyActor)))))))

(fn ConstructionScript)