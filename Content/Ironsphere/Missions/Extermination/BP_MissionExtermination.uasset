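; Extermination mission that requires killing all enemies, with a bonus objective to spare fuel barrels.
; BeginPlay sets objectives and a 60-second timer, scales spawner count by mission number and difficulty, and randomizes wave count.
; Once the timer reaches 30 or below, Tick scans all NPCs every frame and passes the objective when none are hostile.
; Tick also refreshes objective text, showing bonus failure from a game state flag.
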(event EventBeginPlay
  (bind _gi_main_ref (Variables|Default|GetGI_Main_ref))
  (bind _gs_battle_ref (Variables|Default|GetGS_Battle_ref))
  (bind _gs_battle_ref_2 (Variables|Default|GetGS_Battle_ref))
  (|CallParentFunction)
  (Utilities|FlowControl|Sequence
    (:then_0
      (Variables|/Game/Ironsphere/Core/Framework/Battle/GS_Battle.GS_Battle_C|SetObjective _gs_battle_ref_2 "Exterminate all enemies!")
      (Variables|/Game/Ironsphere/Core/Framework/Battle/GS_Battle.GS_Battle_C|SetBonusObjective _gs_battle_ref_2 "Do not destroy fuel barrels!"))
    (:then_1
      (Variables|Default|SetNumberOfSpawners (+ (* (Math|Float|Sqrt (Math|Conversions|ToFloat(Integer) (Variables|/Game/Ironsphere/Core/Framework/GI_Main.GI_Main_C|GetCurrentMission _gi_main_ref))) 0.5) 3 (Variables|/Game/Ironsphere/Core/Framework/GI_Main.GI_Main_C|GetDifficultyLevel _gi_main_ref)))
      (Variables|Default|SetNumberOfWaves (Math|Random|RandomIntegerinRange 4 5))
      (while (> (Variables|Default|GetNumberOfSpawners) 0)
        (Math|Integer|IncrementInt (Variables|Default|GetNumberOfInstants)
          (:%20%20
            (Math|Integer|DecrementInt (Variables|Default|GetNumberOfSpawners)))))
      (Variables|Default|SetMaximalSpawnersInWave 0))
    (:then_2
      (Variables|/Game/Ironsphere/Core/Framework/Battle/GS_Battle.GS_Battle_C|SetObjectivePassed _gs_battle_ref false)
      (Variables|Default|SetLevelTimer 6e+01)
      (Variables|/Game/Ironsphere/Core/Framework/Battle/GS_Battle.GS_Battle_C|SetBonusObjectivepassed _gs_battle_ref true))))

(event Collision|EventActorBeginOverlap
  (params (OtherActor :type Actor%20Object%20Reference))
  (|CallParentFunction OtherActor) ; This node is disabled and will not be called.\nDrag off pins to build functionality.
)

(event EventTick
  (params (DeltaSeconds :type Float%20%28single-precision%29))
  (bind _gs_battle_ref (Variables|Default|GetGS_Battle_ref))
  (|CallParentFunction DeltaSeconds)
  (if (Utilities|IsValid (Variables|Default|GetGS_Battle_ref))
    (Utilities|FlowControl|Sequence
      (:then_0
        (if (<= (Variables|Default|GetLevelTimer) 3e+01)
          (Variables|Default|SetEnemyNotDestroyed false)
          (bind _outactors (Actor|GetAllActorsOfClass "/Game/Ironsphere/Feature/NPC/BP_NPC_Base.BP_NPC_Base_C"))
          (for _array_element _outactors
            (if (not (Variables|/Game/Ironsphere/Feature/NPC/BP_NPC_Base.BP_NPC_Base_C|GetAllied _array_element))
              (Variables|Default|SetEnemyNotDestroyed true)))
          (if (not (Variables|Default|GetEnemyNotDestroyed))
            (Variables|/Game/Ironsphere/Core/Framework/Battle/GS_Battle.GS_Battle_C|SetObjectivePassed (Variables|Default|GetGS_Battle_ref) true))))
      (:then_1
        (Variables|/Game/Ironsphere/Core/Framework/Battle/GS_Battle.GS_Battle_C|SetObjectiveUI _gs_battle_ref (Utilities|Text|FormatText "Exterminate all enemies."))
        (if (Variables|/Game/Ironsphere/Core/Framework/Battle/GS_Battle.GS_Battle_C|GetBonusObjectivepassed _gs_battle_ref)
          (Variables|/Game/Ironsphere/Core/Framework/Battle/GS_Battle.GS_Battle_C|SetBonusObjectiveUI _gs_battle_ref "Do not destroy fuel barrels")
          (else
            (Variables|/Game/Ironsphere/Core/Framework/Battle/GS_Battle.GS_Battle_C|SetBonusObjectiveUI _gs_battle_ref "Do not destroy fuel barrels(failed)")))))))

(fn ConstructionScript
  (|CallParentFunction))