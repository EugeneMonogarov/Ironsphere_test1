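; BP_ExtermWave is a wave actor for the Extermination mission that spawns BP_MissionInstant actors near itself, drawing on the mission's remaining NumberOfInstants.
; Each Tick it looks up BP_MissionExtermination and spawns while its count is below the shared MaximalSpawnersInWave, otherwise only on a rare random roll.
; Each spawn passes on Delay, decrements the pool and raises the shared maximum if exceeded.
; Both X/Y random ranges have equal bounds, so the offset is fixed.
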(event EventBeginPlay
  (Variables|Default|SetInstantsInWave 0))

(event Collision|EventActorBeginOverlap
  (params (OtherActor :type Actor%20Object%20Reference)))

(event EventTick
  (params (DeltaSeconds :type Float%20%28single-precision%29))
  (bind _returnvalue (Transformation|GetActorTransform))
  (bind _instantsinwave (Variables|Default|GetInstantsInWave))
  (bind (_location _rotation _scale) (Math|Transform|BreakTransform _returnvalue))
  (bind (_x _y _z) (Math|Vector|BreakVector _location))
  (bind _outactors (Actor|GetAllActorsOfClass "/Game/Ironsphere/Missions/Extermination/BP_MissionExtermination.BP_MissionExtermination_C"))
  (if (> (Variables|/Game/Ironsphere/Missions/Extermination/BP_MissionExtermination.BP_MissionExtermination_C|GetNumberOfInstants (Utilities|Array|Get(acopy) _outactors)) 0)
    (if (< (Variables|Default|GetInstantsInWave) (Variables|/Game/Ironsphere/Missions/Extermination/BP_MissionExtermination.BP_MissionExtermination_C|GetMaximalSpawnersInWave (Utilities|Array|Get(acopy) _outactors)))
      (Game|SpawnActorfromClass "/Game/Ironsphere/Missions/BP_MissionInstant.BP_MissionInstant_C" (Math|Transform|MakeTransform (Math|Vector|MakeVector (+ _x (Math|Random|RandomFloatinRange 33.0 33.0)) (+ _y (Math|Random|RandomFloatinRange 33.0 33.0)) _z) _rotation _scale) "Undefined" "MultiplyWithRoot" 0 (Variables|Default|Getdelay) 0 :!label _label)
      (Math|Integer|IncrementInt _instantsinwave
        (:%20%20
          (bind _outactors_2 (Actor|GetAllActorsOfClass "/Game/Ironsphere/Missions/Extermination/BP_MissionExtermination.BP_MissionExtermination_C"))
          (if (> _instantsinwave (Variables|/Game/Ironsphere/Missions/Extermination/BP_MissionExtermination.BP_MissionExtermination_C|GetMaximalSpawnersInWave (Utilities|Array|Get(acopy) _outactors_2)))
            (Variables|/Game/Ironsphere/Missions/Extermination/BP_MissionExtermination.BP_MissionExtermination_C|SetMaximalSpawnersInWave (Utilities|Array|Get(acopy) _outactors_2) (Variables|Default|GetInstantsInWave)))
          (Math|Integer|DecrementInt (Variables|/Game/Ironsphere/Missions/Extermination/BP_MissionExtermination.BP_MissionExtermination_C|GetNumberOfInstants (Utilities|Array|Get(acopy) _outactors_2)))))
      (elif (> (Math|Random|RandomFloatinRange 0.0 1.0) 0.99)
        (goto _label)))))

(fn ConstructionScript)