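; Wave spawn point for the defending mission that creates at most one BP_Wave, then destroys itself.
; One second after BeginPlay it caches the mission's wave total, then rolls a small random chance each tick while waves remain.
; A successful spawn decrements the mission counter and passes a Delay that staggers waves across roughly 180 seconds.
; It removes itself without spawning if the player is within 200 units or no waves remain.
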(event EventBeginPlay
  (Variables|Default|SetLetWavesAdd false)
  (Utilities|FlowControl|Delay 1.0)
  (bind _returnvalue (Actor|GetActorOfClass "/Game/Ironsphere/Missions/Defending/BP_MissionDefending.BP_MissionDefending_C"))
  (bind _output_get (Variables|Default|SetWavesSumm (Variables|/Game/Ironsphere/Missions/Defending/BP_MissionDefending.BP_MissionDefending_C|GetNumberOfWaves _returnvalue)))
  (Variables|Default|SetLetWavesAdd true))

(event Collision|EventActorBeginOverlap
  (params (OtherActor :type Actor%20Object%20Reference)))

(event EventTick
  (params (DeltaSeconds :type Float%20%28single-precision%29))
  (bind _wavessumm (Variables|Default|GetWavesSumm))
  (if (Variables|Default|GetLetWavesAdd)
    (bind _outactors (Actor|GetAllActorsOfClass "/Game/Ironsphere/Core/Player/BP_CharacterPlayer.BP_CharacterPlayer_C"))
    (if (< (Math|Vector|VectorLength (- (Transformation|GetActorLocation (Utilities|Array|Get(acopy) _outactors)) (Transformation|GetActorLocation))) 2e+02)
      (Actor|DestroyActor)
      (else
        (bind _returnvalue (Actor|GetActorOfClass "/Game/Ironsphere/Missions/Defending/BP_MissionDefending.BP_MissionDefending_C"))
        (if (> (Variables|/Game/Ironsphere/Missions/Defending/BP_MissionDefending.BP_MissionDefending_C|GetNumberOfWaves _returnvalue) 0)
          (if (> (Math|Random|RandomFloatinRange 0.0 1.0) 0.96)
            (Game|SpawnActorfromClass "/Game/Ironsphere/Missions/Defending/BP_Wave.BP_Wave_C" (Transformation|GetActorTransform) "Undefined" "MultiplyWithRoot" 0 (+ 1.0 (* (/ 180 _wavessumm) (- _wavessumm (Variables|/Game/Ironsphere/Missions/Defending/BP_MissionDefending.BP_MissionDefending_C|GetNumberOfWaves _returnvalue)))) 0)
            (Development|PrintString (Utilities|String|ToString(Float) (+ 1.0 (* (/ 180 _wavessumm) (- _wavessumm (Variables|/Game/Ironsphere/Missions/Defending/BP_MissionDefending.BP_MissionDefending_C|GetNumberOfWaves _returnvalue))))) true true "(R=0.000000,G=0.660000,B=1.000000,A=1.000000)" (+ 1.0 (* (/ 180 _wavessumm) (- _wavessumm (Variables|/Game/Ironsphere/Missions/Defending/BP_MissionDefending.BP_MissionDefending_C|GetNumberOfWaves _returnvalue)))))
            (bind _returnvalue_2 (Actor|GetActorOfClass "/Game/Ironsphere/Missions/Defending/BP_MissionDefending.BP_MissionDefending_C"))
            (Math|Integer|DecrementInt (Variables|/Game/Ironsphere/Missions/Defending/BP_MissionDefending.BP_MissionDefending_C|GetNumberOfWaves _returnvalue_2)
              (:%20%20
                (Actor|DestroyActor))))
          (else
            (Actor|DestroyActor)))))))

(fn ConstructionScript)