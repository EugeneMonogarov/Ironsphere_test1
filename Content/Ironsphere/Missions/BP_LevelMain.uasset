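; BP_LevelMain is a mission-level actor for Ironsphere that provides a level countdown and an objective display.
; BeginPlay caches the game instance, battle game state and in-game player controller, playing an error sound if any cast fails.
; Tick decrements LevelTimer while it is positive, with no action on expiry.
; LevelObjectivesPrint, not called here, shows an objective widget with hardcoded barrel-destruction and time-limit text, ignoring its text inputs.
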(event EventBeginPlay
  (CallFunction|Casts))

(event Collision|EventActorBeginOverlap
  (params (OtherActor :type Actor%20Object%20Reference)))

(event EventTick
  (params (DeltaSeconds :type Float%20%28single-precision%29))
  (CallFunction|Timers DeltaSeconds))

(fn ConstructionScript
  (|CallParentFunction))

(fn Timers
  (params (B :type Float%20%28double-precision%29))
  (if (> (Variables|Default|GetLevelTimer) 0.0)
    (Variables|Default|SetLevelTimer (- (Variables|Default|GetLevelTimer) B))))

(fn LevelObjectivesPrint
  (params (Text1 :type Text) (Text2 :type Text))
  (bind _returnvalue (UserInterface|CreateWidget "/Game/Ironsphere/UI/Ingame/WBC_ObjectiveOnStart.WBC_ObjectiveOnStart_C" 0 "Destroy red oil barrels!" "Complete in 3 minutes"))
  (UserInterface|Viewport|AddtoViewport _returnvalue 0))

(fn Casts
  (bind _asgi_main (Utilities|Casting|CastToGI_Main (Game|GetGameInstance))
    (:then
      (Variables|Default|SetGI_Main_ref _asgi_main)
      (bind _asgs_battle (Utilities|Casting|CastToGS_Battle (Game|GetGameState))
        (:then
          (Variables|Default|SetGS_Battle_ref _asgs_battle)
          (bind _aspc_ingame (Utilities|Casting|CastToPC_Ingame (Game|GetPlayerController 0))
            (:then
              (Variables|Default|SetPC_Ingame_ref _aspc_ingame))
            (:CastFailed
              (Audio|PlaySound2D "/Engine/EditorSounds/Notifications/CompileFailed.CompileFailed" 1.0 1.0 0.0 0 0 :!label _label))))
        (:CastFailed
          (goto _label))))
    (:CastFailed
      (goto _label))))