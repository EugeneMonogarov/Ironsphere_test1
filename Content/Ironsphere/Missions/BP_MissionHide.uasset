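; BP_MissionHide is a mission placement marker that spawns BP_Hide worm hideouts at its transform, removing its Cube component on BeginPlay.
; Tick sums current mission and difficulty from GI_Main, then rolls to pick grey worm, tiger leech or needle worm, with scaled counts and random unhide times.
; Spawning repeats every Tick, with no guard or self-destroy.
; Disconnected branches hold unused egg spawner, den and hive variants.
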(event EventBeginPlay
  (Components|DestroyComponent (Variables|Default|GetCube)))

(event Collision|EventActorBeginOverlap
  (params (OtherActor :type Actor%20Object%20Reference)))

(event EventTick
  (params (DeltaSeconds :type Float%20%28single-precision%29))
  (bind _asgi_main (Utilities|Casting|CastToGI_Main (Game|GetGameInstance)))
  (bind _output_get (Variables|Default|SetCurrentMission (+ (Variables|/Game/Ironsphere/Core/Framework/GI_Main.GI_Main_C|GetCurrentMission _asgi_main) (Variables|/Game/Ironsphere/Core/Framework/GI_Main.GI_Main_C|GetDifficultyLevel _asgi_main))))
  (Variables|Default|SetRandom (Math|Random|RandomIntegerinRange (- (/ _output_get 2) 3) (+ _output_get 3)))
  (if (> (Variables|Default|GetRandom) 3)
    (if (> (Variables|Default|GetRandom) 5)
      (if (> (Variables|Default|GetRandom) 7)
        (Game|SpawnActorfromClass "/Game/Ironsphere/Feature/World/Spawners/BP_Hide.BP_Hide_C" (Transformation|GetActorTransform) "Undefined" "MultiplyWithRoot" 0 (Math|Random|RandomFloatinRange 5.0 1.5e+02) (+ (* (Variables|Default|GetCurrentMission) 1) 3) "/Game/Ironsphere/Feature/NPC/Worm/BP_NeedleWorm.BP_NeedleWorm_C" 3e+01 3e+01 0.0 0)
        (else
          (Game|SpawnActorfromClass "/Game/Ironsphere/Feature/World/Spawners/BP_Hide.BP_Hide_C" (Transformation|GetActorTransform) "Undefined" "MultiplyWithRoot" 0 (Math|Random|RandomFloatinRange 5.0 1.5e+02) (+ (* (Variables|Default|GetCurrentMission) 1) 2) "/Game/Ironsphere/Feature/NPC/Worm/BP_NeedleWorm.BP_NeedleWorm_C" 3e+01 3e+01 0.0 0)))
      (else
        (Game|SpawnActorfromClass "/Game/Ironsphere/Feature/World/Spawners/BP_Hide.BP_Hide_C" (Transformation|GetActorTransform) "Undefined" "MultiplyWithRoot" 0 (Math|Random|RandomFloatinRange 5.0 1.5e+02) (+ (* (Variables|Default|GetCurrentMission) 2) 2) "/Game/Ironsphere/Feature/NPC/Worm/BP_TigerLeech.BP_TigerLeech_C" 3e+01 3e+01 0.0 0)))
    (else
      (Game|SpawnActorfromClass "/Game/Ironsphere/Feature/World/Spawners/BP_Hide.BP_Hide_C" (Transformation|GetActorTransform) "Undefined" "MultiplyWithRoot" 0 (Math|Random|RandomFloatinRange 5.0 1.5e+02) (+ (* (Variables|Default|GetCurrentMission) 5) 3) "/Game/Ironsphere/Feature/NPC/Worm/BP_GreyWorm.BP_GreyWorm_C" 3e+01 3e+01 0.0 0))))

(fn ConstructionScript)