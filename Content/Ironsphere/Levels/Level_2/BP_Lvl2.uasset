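; BP_Lvl2 runs the Level 2 objectives: destroy all hives, with a bonus for killing 100 desert wasps.
; BeginPlay retries until the battle game state is ready, sets the level index and shows the objective intro widget.
; Tick infers kills from drops in the wasp actor count and updates objective text on GS_Battle.
; When no hives remain, it flags objectives passed and records the bonus result; timed bonus failure is disconnected.
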(event EventBeginPlay
  (Utilities|FlowControl|Sequence
    (:then_0
      (bind _asgs_battle (Utilities|Casting|CastToGS_Battle (Game|GetGameState) :!label _label)
        (:then
          (Variables|Default|SetGS_Battle_ref _asgs_battle)
          (bind _asgi_main (Utilities|Casting|CastToGI_Main (Game|GetGameInstance)))
          (bind _output_get (Variables|Default|SetGI_Main_ref _asgi_main))
          (Variables|/Game/Ironsphere/Core/Framework/GI_Main.GI_Main_C|SetCurrentLevelIndex _output_get 2)
          (bind _aspc_ingame (Utilities|Casting|CastToPC_Ingame (Game|GetPlayerController 0)))
          (Variables|Default|SetPC%20Ref _aspc_ingame)
          (Variables|Default|SetBonusFailed false))
        (:CastFailed
          (Utilities|FlowControl|Delay 0.2)
          (goto _label))))
    (:then_1
      (bind _outactors (Actor|GetAllActorsOfClass "/Game/Ironsphere/Feature/NPC/Hornet/BP_DesertWasp.BP_DesertWasp_C"))
      (Variables|Default|SetNumberOfWasps (Utilities|Array|Length _outactors)))
    (:then_2
      (bind _returnvalue (UserInterface|CreateWidget "/Game/Ironsphere/UI/Ingame/WBC_ObjectiveOnStart.WBC_ObjectiveOnStart_C" 0 "Destroy the hives!" "Bonus: Kill 100 desert wasps"))
      (UserInterface|Viewport|AddtoViewport _returnvalue 0))))

(event Collision|EventActorBeginOverlap
  (params (OtherActor :type Actor%20Object%20Reference)))

(event EventTick
  (params (DeltaSeconds :type Float%20%28single-precision%29))
  (bind _gs_battle_ref (Variables|Default|GetGS_Battle_ref))
  (bind _gs_battle_ref_2 (Variables|Default|GetGS_Battle_ref))
  (Utilities|FlowControl|Sequence
    (:then_0
      (bind _outactors (Actor|GetAllActorsOfClass "/Game/Ironsphere/Feature/NPC/Hornet/BP_DesertWasp.BP_DesertWasp_C"))
      (if (< (Utilities|Array|Length _outactors) (Variables|Default|GetNumberOfWasps))
        (Variables|Default|SetKilledWasps (+ (Variables|Default|GetKilledWasps) (- (Variables|Default|GetNumberOfWasps) (Utilities|Array|Length _outactors)))))
      (Variables|Default|SetNumberOfWasps (Utilities|Array|Length _outactors)))
    (:then_1
      (Variables|Default|SetTimer (- (Variables|Default|GetTimer) DeltaSeconds))
      (if (> (- 100 (Variables|Default|GetKilledWasps)) 0)
        (Variables|/Game/Ironsphere/Core/Framework/Battle/GS_Battle.GS_Battle_C|SetObjective2 _gs_battle_ref (Utilities|Text|FormatText "Bonus: Kill 100 desert wasps.({sec} left." (Utilities|Text|ToText(String) (Class|KismetMathLibrary|ToInt64(Integer) (- 100 (Variables|Default|GetKilledWasps))))))
        (else
          (Variables|/Game/Ironsphere/Core/Framework/Battle/GS_Battle.GS_Battle_C|SetObjective2 _gs_battle_ref (Utilities|Text|FormatText "Bonus: Kill 100 desert wasps.Completed."))))
      (bind _outactors_2 (Actor|GetAllActorsOfClass "/Game/Ironsphere/Feature/World/Spawners/BP_Hive.BP_Hive_C"))
      (Variables|/Game/Ironsphere/Core/Framework/Battle/GS_Battle.GS_Battle_C|SetObjective1 (Variables|Default|GetGS_Battle_ref) (Utilities|Text|FormatText "Destroy the hives({count} left)" (Utilities|Array|Length _outactors_2)))
      (if (== (Utilities|Array|Length _outactors_2) 0)
        (if (>= (Variables|Default|GetKilledWasps) 100)
          (Variables|/Game/Ironsphere/Core/Framework/Battle/GS_Battle.GS_Battle_C|SetBonusObjectivepassed _gs_battle_ref_2 true)
          (else
            (Variables|/Game/Ironsphere/Core/Framework/Battle/GS_Battle.GS_Battle_C|SetBonusObjectivepassed _gs_battle_ref_2 false)))
        (Variables|/Game/Ironsphere/Core/Framework/Battle/GS_Battle.GS_Battle_C|SetObjective1passed _gs_battle_ref_2 true)
        (Variables|/Game/Ironsphere/Core/Framework/Battle/GS_Battle.GS_Battle_C|SetObjective2passed _gs_battle_ref_2 true)
        (Variables|/Game/Ironsphere/Core/Framework/Battle/GS_Battle.GS_Battle_C|SetObjective3passed _gs_battle_ref_2 true)))))

(fn ConstructionScript
  (|CallParentFunction))