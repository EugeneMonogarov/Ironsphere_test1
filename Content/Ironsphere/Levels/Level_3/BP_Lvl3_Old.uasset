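; Level 3 objective controller: the player must destroy all spider dens, with a bonus for sparing the fuel barrels.
; BeginPlay retries until GS_Battle is available, then caches references, sets the level index and writes objective text.
; Tick polls actor counts, updating dens left and failing the bonus with a sound if barrels drop below a fixed count.
; With no dens left, it flags objectives passed and records the bonus result; a survival countdown remains as unused leftover.
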(event EventBeginPlay
  (bind _asgs_battle (Utilities|Casting|CastToGS_Battle (Game|GetGameState) :!label _label)
    (:then
      (Variables|Default|SetGS_Battle_ref _asgs_battle)
      (Variables|/Game/Ironsphere/Core/Framework/Battle/GS_Battle.GS_Battle_C|SetObjective2 (Variables|Default|GetGS_Battle_ref) "Bonus: Dont destroy fuel barrels")
      (bind _asgi_main (Utilities|Casting|CastToGI_Main (Game|GetGameInstance)))
      (bind _output_get (Variables|Default|SetGI_Main_ref _asgi_main))
      (Variables|/Game/Ironsphere/Core/Framework/GI_Main.GI_Main_C|SetCurrentLevelIndex _output_get 3)
      (bind _aspc_ingame (Utilities|Casting|CastToPC_Ingame (Game|GetPlayerController 0)))
      (Variables|Default|SetPC%20Ref _aspc_ingame)
      (Variables|Default|SetBonusFailed false)
      (Variables|/Game/Ironsphere/Core/Framework/Battle/GS_Battle.GS_Battle_C|SetObjective1 (Variables|Default|GetGS_Battle_ref) "Destroy all spider's dens"))
    (:CastFailed
      (Utilities|FlowControl|Delay 0.2)
      (goto _label))))

(event Collision|EventActorBeginOverlap
  (params (OtherActor :type Actor%20Object%20Reference)))

(event EventTick
  (params (DeltaSeconds :type Float%20%28single-precision%29))
  (bind _gs_battle_ref (Variables|Default|GetGS_Battle_ref))
  (if (> (Variables|Default|GetTimer) 0.0)
    (Variables|Default|SetTimer (- (Variables|Default|GetTimer) DeltaSeconds))
    (else
      (Variables|Default|SetTimer 0.0)))
  (bind _outactors (Actor|GetAllActorsOfClass "/Game/Ironsphere/Feature/World/Spawners/BP_Den.BP_Den_C"))
  (if (== (Utilities|Array|Length _outactors) 0)
    (if (Variables|Default|GetBonusFailed)
      (Variables|/Game/Ironsphere/Core/Framework/Battle/GS_Battle.GS_Battle_C|SetBonusObjectivepassed _gs_battle_ref false)
      (else
        (Variables|/Game/Ironsphere/Core/Framework/Battle/GS_Battle.GS_Battle_C|SetBonusObjectivepassed _gs_battle_ref true)))
    (Variables|/Game/Ironsphere/Core/Framework/Battle/GS_Battle.GS_Battle_C|SetObjective1passed _gs_battle_ref true)
    (Variables|/Game/Ironsphere/Core/Framework/Battle/GS_Battle.GS_Battle_C|SetObjective2passed _gs_battle_ref true)
    (Variables|/Game/Ironsphere/Core/Framework/Battle/GS_Battle.GS_Battle_C|SetObjective3passed _gs_battle_ref true)
    (else
      (Variables|/Game/Ironsphere/Core/Framework/Battle/GS_Battle.GS_Battle_C|SetObjective1 (Variables|Default|GetGS_Battle_ref) (Utilities|Text|FormatText "Bonus Destroy all spider dens({x} left)" (Utilities|Array|Length _outactors)))
      (if (not (Variables|Default|GetBonusFailed))
        (bind _outactors_2 (Actor|GetAllActorsOfClass "/Game/Ironsphere/Feature/World/LevelObjectives/BP_FuelBarrel_objective.BP_FuelBarrel_objective_C"))
        (if (< (Utilities|Array|Length _outactors_2) 10)
          (Variables|Default|SetBonusFailed true)
          (Audio|SpawnSound2D "/Engine/VREditor/Sounds/UI/Dockable_Window_Close.Dockable_Window_Close" 1.0 1.0 0.0 0)
          (Variables|/Game/Ironsphere/Core/Framework/Battle/GS_Battle.GS_Battle_C|SetObjective2 (Variables|Default|GetGS_Battle_ref) "Bonus: Dont destroy fuel barrels(failed)"))))))

(fn ConstructionScript
  (|CallParentFunction))