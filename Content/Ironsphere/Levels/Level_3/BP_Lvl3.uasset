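; BP_Lvl3 runs the objectives for Level 3: survive a countdown, with a bonus for protecting the cargo ship.
; BeginPlay retries until GS_Battle is available, then caches game references and sets the level index.
; Tick counts down, updates objective text and permanently fails the bonus if the player's pawn strays too far from BP_CargoShip.
; At zero, it plays a sound and flags objectives passed on every tick, recording the bonus result.
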(event EventBeginPlay
  (bind _asgs_battle (Utilities|Casting|CastToGS_Battle (Game|GetGameState) :!label _label)
    (:then
      (Variables|Default|SetGS_Battle_ref _asgs_battle)
      (bind _asgi_main (Utilities|Casting|CastToGI_Main (Game|GetGameInstance)))
      (bind _output_get (Variables|Default|SetGI_Main_ref _asgi_main))
      (Variables|/Game/Ironsphere/Core/Framework/GI_Main.GI_Main_C|SetCurrentLevelIndex _output_get 3)
      (bind _aspc_ingame (Utilities|Casting|CastToPC_Ingame (Game|GetPlayerController 0)))
      (Variables|Default|SetPC%20Ref _aspc_ingame)
      (Variables|Default|SetBonusFailed false))
    (:CastFailed
      (Utilities|FlowControl|Delay 0.2)
      (goto _label))))

(event Collision|EventActorBeginOverlap
  (params (OtherActor :type Actor%20Object%20Reference)))

(event EventTick
  (params (DeltaSeconds :type Float%20%28single-precision%29))
  (bind _gs_battle_ref (Variables|Default|GetGS_Battle_ref))
  (if (> (Variables|Default|GetTimer) 0.0)
    (Variables|Default|SetTimer (- (Variables|Default|GetTimer) DeltaSeconds))
    (else
      (Variables|Default|SetTimer 0.0)))
  (if (Variables|Default|GetBonusFailed)
    (Variables|/Game/Ironsphere/Core/Framework/Battle/GS_Battle.GS_Battle_C|SetObjective2 (Variables|Default|GetGS_Battle_ref) "Bonus: Protect the cargo ship (failed)")
    (else
      (Variables|/Game/Ironsphere/Core/Framework/Battle/GS_Battle.GS_Battle_C|SetObjective2 (Variables|Default|GetGS_Battle_ref) "Bonus: Protect the cargo ship")
      (bind _returnvalue (Actor|GetActorOfClass "/Game/Ironsphere/Feature/World/LevelObjectives/BP_CargoShip.BP_CargoShip_C"))
      (if (> (Math|Vector|VectorLength (- (Transformation|GetActorLocation _returnvalue) (Transformation|GetActorLocation (Pawn|GetControlledPawn (Variables|Default|GetPC%20Ref))))) 2.5e+02)
        (Variables|Default|SetBonusFailed true)
        (Audio|PlaySound2D "/Engine/VREditor/Sounds/UI/Leave_Simulate.Leave_Simulate" 1.0 1.0 0.0 0 0))))
  (Variables|/Game/Ironsphere/Core/Framework/Battle/GS_Battle.GS_Battle_C|SetObjective1 (Variables|Default|GetGS_Battle_ref) (Utilities|Text|FormatText "Survive {count} seconds" (Class|KismetMathLibrary|ToInt64(Float) (Variables|Default|GetTimer))))
  (if (<= (Variables|Default|GetTimer) 0.0)
    (Audio|SpawnSound2D "/Engine/VREditor/Sounds/VR_confirm_Cue.VR_confirm_Cue" 1.0 1.0 0.0 0)
    (if (Variables|Default|GetBonusFailed)
      (Variables|/Game/Ironsphere/Core/Framework/Battle/GS_Battle.GS_Battle_C|SetBonusObjectivepassed _gs_battle_ref false)
      (else
        (Variables|/Game/Ironsphere/Core/Framework/Battle/GS_Battle.GS_Battle_C|SetBonusObjectivepassed _gs_battle_ref true)))
    (Variables|/Game/Ironsphere/Core/Framework/Battle/GS_Battle.GS_Battle_C|SetObjective1passed _gs_battle_ref true)
    (Variables|/Game/Ironsphere/Core/Framework/Battle/GS_Battle.GS_Battle_C|SetObjective2passed _gs_battle_ref true)
    (Variables|/Game/Ironsphere/Core/Framework/Battle/GS_Battle.GS_Battle_C|SetObjective3passed _gs_battle_ref true)))

(fn ConstructionScript
  (|CallParentFunction))