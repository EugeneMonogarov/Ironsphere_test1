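; Mission logic actor for the Initiation level: destroy the objective oil barrels, then return to the cargo ship, with a timed bonus.
; BeginPlay retries until the battle GameState exists, resets the level index and shows the objective popup.
; Tick counts down the timer and, every few frames, polls remaining barrels and mech-to-ship distance, writing objective text and pass flags to GS_Battle.
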(event EventBeginPlay
  (bind _asgs_battle (Utilities|Casting|CastToGS_Battle (Game|GetGameState) :!label _label)
    (:then
      (Variables|Default|SetGS_Battle_ref _asgs_battle)
      (bind _asgi_main (Utilities|Casting|CastToGI_Main (Game|GetGameInstance)))
      (Variables|/Game/Ironsphere/Core/Framework/GI_Main.GI_Main_C|SetCurrentLevelIndex _asgi_main 0)
      (bind _aspc_ingame (Utilities|Casting|CastToPC_Ingame (Game|GetPlayerController 0)))
      (Variables|Default|SetPC_Ingame_ref _aspc_ingame)
      (bind _returnvalue (UserInterface|CreateWidget "/Game/Ironsphere/UI/Ingame/WBC_ObjectiveOnStart.WBC_ObjectiveOnStart_C" 0 "Destroy red oil barrels!" "Complete in 3 minutes"))
      (UserInterface|Viewport|AddtoViewport _returnvalue 0))
    (:CastFailed
      (Utilities|FlowControl|Delay 0.2)
      (goto _label))))

(event Collision|EventActorBeginOverlap
  (params (OtherActor :type Actor%20Object%20Reference)))

(event EventTick
  (params (DeltaSeconds :type Float%20%28single-precision%29))
  (bind _gs_battle_ref (Variables|Default|GetGS_Battle_ref))
  (bind _gs_battle_ref_2 (Variables|Default|GetGS_Battle_ref))
  (bind _gs_battle_ref_3 (Variables|Default|GetGS_Battle_ref))
  (if (> (Variables|Default|GetTimer) 0.0)
    (Variables|Default|SetTimer (- (Variables|Default|GetTimer) DeltaSeconds)))
  (if (>= (Variables|Default|GetTickCount) 10)
    (Variables|Default|SetTickCount 0)
    (if (> (Variables|Default|GetTimer) 0.0)
      (bind _outactors (Actor|GetAllActorsOfClass "/Game/Ironsphere/Feature/World/LevelObjectives/BP_FuelBarrel_objective.BP_FuelBarrel_objective_C"))
      (if (> (Utilities|Array|Length _outactors) 0)
        (Variables|/Game/Ironsphere/Core/Framework/Battle/GS_Battle.GS_Battle_C|SetObjective1 _gs_battle_ref_2 (Utilities|Text|ToText(String) (Utilities|String|Append (Utilities|String|ToString(Text) (Utilities|Text|FormatText "1. Destroy oil barrels")) " (" (Utilities|String|ToString(Integer) (Utilities|Array|Length _outactors)) " left" ")")))
        (else
          (Variables|/Game/Ironsphere/Core/Framework/Battle/GS_Battle.GS_Battle_C|SetObjective1 _gs_battle_ref_2 "1. Destroy oil barrels. (Completed)")))
      (Variables|/Game/Ironsphere/Core/Framework/Battle/GS_Battle.GS_Battle_C|SetObjective2 _gs_battle_ref_2 "2. Return to ship")
      (Variables|/Game/Ironsphere/Core/Framework/Battle/GS_Battle.GS_Battle_C|SetObjective3 _gs_battle_ref_2 (Utilities|Text|FormatText "Bonus: Complete in {sec} seconds" (Utilities|Text|ToText(String) (Class|KismetMathLibrary|ToInt64(Float) (Variables|Default|GetTimer)))))
      (else
        (Variables|Default|SetTimer 0.0)
        (if (Variables|Default|GetBonusFailed)
          _
          (else
            (Variables|Default|SetBonusFailed true)
            (Audio|PlaySound2D "/Engine/VREditor/Sounds/UI/Leave_Simulate.Leave_Simulate" 1.0 1.0 0.0 0 0)
            (Variables|/Game/Ironsphere/Core/Framework/Battle/GS_Battle.GS_Battle_C|SetObjective3 (Variables|Default|GetGS_Battle_ref) "Bonus: failed")))))
    (bind _outactors_2 (Actor|GetAllActorsOfClass "/Game/Ironsphere/Feature/World/LevelObjectives/BP_FuelBarrel_objective.BP_FuelBarrel_objective_C"))
    (if (== (Utilities|Array|Length _outactors_2) 0)
      (if (Variables|/Game/Ironsphere/Core/Framework/Battle/GS_Battle.GS_Battle_C|GetObjective1passed _gs_battle_ref)
        (bind _outactors_3 (Actor|GetAllActorsOfClass "/Game/Ironsphere/Feature/World/LevelObjectives/BP_CargoShip_Initiation.BP_CargoShip_Initiation_C"))
        (if (< (Math|Vector|VectorLength (- (Transformation|GetActorLocation (Utilities|Array|Get(acopy) _outactors_3)) (Transformation|GetActorLocation (Variables|/Game/Ironsphere/Core/Framework/Battle/PC_Ingame.PC_Ingame_C|GetControlledMech (Variables|Default|GetPC_Ingame_ref))))) 2e+02)
          (if (<= (Variables|Default|GetTimer) 0.0)
            (Variables|/Game/Ironsphere/Core/Framework/Battle/GS_Battle.GS_Battle_C|SetBonusObjectivepassed _gs_battle_ref_3 false)
            (else
              (Variables|/Game/Ironsphere/Core/Framework/Battle/GS_Battle.GS_Battle_C|SetBonusObjectivepassed _gs_battle_ref_3 true)))
          (Variables|/Game/Ironsphere/Core/Framework/Battle/GS_Battle.GS_Battle_C|SetObjective2passed _gs_battle_ref_3 true)
          (Variables|/Game/Ironsphere/Core/Framework/Battle/GS_Battle.GS_Battle_C|SetObjective3passed _gs_battle_ref_3 true))
        (else
          (Variables|/Game/Ironsphere/Core/Framework/Battle/GS_Battle.GS_Battle_C|SetObjective1passed _gs_battle_ref true)
          (bind _returnvalue (UserInterface|CreateWidget "/Game/Ironsphere/UI/Ingame/WBC_ObjectiveOnStart.WBC_ObjectiveOnStart_C" 0 "Oil barrels destroyed!" "Return to Cargoship"))
          (UserInterface|Viewport|AddtoViewport _returnvalue 0))))
    (else
      (Math|Integer|IncrementInt (Variables|Default|GetTickCount)))))

(fn ConstructionScript
  (|CallParentFunction))