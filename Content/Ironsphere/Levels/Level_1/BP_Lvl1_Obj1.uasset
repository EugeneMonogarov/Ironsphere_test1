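; BP_Lvl1_Obj1 is the first objective actor for Level 1, a timed survival goal.
; On BeginPlay it caches the GS_Battle game state, retrying every 0.2 seconds until the cast succeeds.
; Tick counts a timer down and writes the remaining seconds into the game state's Objective1 text.
; When the timer runs out, it plays a 2D confirm sound and destroys itself.
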(event EventBeginPlay
  (bind _asgs_battle (Utilities|Casting|CastToGS_Battle (Game|GetGameState) :!label _label)
    (:then
      (Variables|Default|SetGS_Battle_ref _asgs_battle))
    (:CastFailed
      (Utilities|FlowControl|Delay 0.2)
      (goto _label))))

(event Collision|EventActorBeginOverlap
  (params (OtherActor :type Actor%20Object%20Reference)))

(event EventTick
  (params (DeltaSeconds :type Float%20%28single-precision%29))
  (Variables|Default|SetTimer (- (Variables|Default|GetTimer) DeltaSeconds))
  (if (<= (Variables|Default|GetTimer) 0.0)
    (Audio|SpawnSound2D "/Engine/VREditor/Sounds/VR_confirm_Cue.VR_confirm_Cue" 1.0 1.0 0.0 0)
    (Actor|DestroyActor)
    (else
      (Variables|/Game/Ironsphere/Core/Framework/Battle/GS_Battle.GS_Battle_C|SetObjective1 (Variables|Default|GetGS_Battle_ref) (Utilities|Text|FormatText "1: Survive {0} seconds" (Utilities|Text|ToText(String) (Class|KismetMathLibrary|ToInt64(Float) (Variables|Default|GetTimer))))))))

(fn ConstructionScript
  (|CallParentFunction))