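; Level 1 objective actor that tracks the second objective, destroying all dens.
; On BeginPlay it caches the GS_Battle game state, retrying after a short delay until the cast succeeds.
; Each Tick it counts remaining BP_Den actors and writes the objective text with that count to the game state.
; When none remain, it plays a confirmation sound and destroys itself.
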(event EventBeginPlay
  (bind _asgs_battle (Utilities|Casting|CastToGS_Battle (Game|GetGameState) :!label _label)
    (:then
      (Variables|Default|SetGS_Battle_ref _asgs_battle))
    (:CastFailed
      (Utilities|FlowControl|Delay 0.2)
      (goto _label))))

(event Collision|EventActorBeginOverlap
  (params (OtherActor :type Actor%20Object%20Reference)))

(event EventTick
  (params (DeltaSeconds :type Float%20%28single-precision%29))
  (bind _outactors (Actor|GetAllActorsOfClass "/Game/Ironsphere/Feature/World/Spawners/BP_Den.BP_Den_C"))
  (if (== (Utilities|Array|Length _outactors) 0)
    (Audio|SpawnSound2D "/Engine/VREditor/Sounds/VR_confirm_Cue.VR_confirm_Cue" 1.0 1.0 0.0 0)
    (Actor|DestroyActor)
    (else
      (Variables|Default|SetDensCount 0)
      (for _array_element _outactors
        (Variables|Default|SetDensCount (+ (Variables|Default|GetDensCount) 1)))
      (Variables|/Game/Ironsphere/Core/Framework/Battle/GS_Battle.GS_Battle_C|SetObjective2 (Variables|Default|GetGS_Battle_ref) (Utilities|Text|FormatText "2: Destroy all dens. {0} left " (Variables|Default|GetDensCount))))))

(fn ConstructionScript
  (|CallParentFunction))