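; BP_Level6 is the objective controller for Level 6, with a timed bonus for killing all enemies.
; On BeginPlay it caches the GS_Battle game state, retrying the cast after a short delay until it succeeds.
; Tick counts down the timer and polls for remaining BP_DarkWidowMother actors, setting objective and bonus results when none remain.
; Timer expiry plays a one-time failure sound while polling continues; bonus text updates are disconnected.
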(event EventBeginPlay
  (bind _asgs_battle (Utilities|Casting|CastToGS_Battle (Game|GetGameState) :!label _label)
    (:then
      (Variables|Default|SetGS_Battle_ref _asgs_battle))
    (:CastFailed
      (Utilities|FlowControl|Delay 0.2)
      (goto _label))))

(event Collision|EventActorBeginOverlap
  (params (OtherActor :type Actor%20Object%20Reference)))

(event EventTick
  (params (DeltaSeconds :type Float%20%28single-precision%29))
  (bind _gs_battle_ref (Variables|Default|GetGS_Battle_ref))
  (if (> (Variables|Default|GetTimer) 0.0)
    (Variables|/Game/Ironsphere/Core/Framework/Battle/GS_Battle.GS_Battle_C|SetObjective (Variables|Default|GetGS_Battle_ref) (Utilities|Text|FormatText "Kill all enemies"))
    (Variables|Default|SetTimer (- (Variables|Default|GetTimer) DeltaSeconds))
    (bind _outactors (Actor|GetAllActorsOfClass "/Game/Ironsphere/Feature/NPC/Spider/BP_DarkWidowMother.BP_DarkWidowMother_C" :!label _label))
    (if (== (Utilities|Array|Length _outactors) 0)
      (if (<= (Variables|Default|GetTimer) 0.0)
        (Variables|/Game/Ironsphere/Core/Framework/Battle/GS_Battle.GS_Battle_C|SetBonusObjectivepassed _gs_battle_ref false)
        (else
          (Variables|/Game/Ironsphere/Core/Framework/Battle/GS_Battle.GS_Battle_C|SetBonusObjectivepassed _gs_battle_ref true)))
      (Variables|/Game/Ironsphere/Core/Framework/Battle/GS_Battle.GS_Battle_C|SetObjectivePassed _gs_battle_ref true))
    (else
      (Variables|Default|SetTimer 0.0)
      (if (Variables|Default|GetBonusFailed)
        (goto _label)
        (else
          (Variables|Default|SetBonusFailed true)
          (Audio|PlaySound2D "/Engine/VREditor/Sounds/UI/Leave_Simulate.Leave_Simulate" 1.0 1.0 0.0 0 0))))))

(fn ConstructionScript
  (|CallParentFunction))