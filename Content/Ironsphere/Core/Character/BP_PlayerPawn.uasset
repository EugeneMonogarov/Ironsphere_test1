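; Player tank-style pawn with WASD-style driving, a rotating turret and a reloading gun.
; Tick integrates PC_1's move and turn inputs into clamped velocity with slower reverse and coasting deceleration, moves and yaws the actor, and spins two markers.
; UpdateTowerDirection steps turret yaw toward a given direction, snapping when close.
; Shooting spawns BP_bullet1 at AmmoSpawn, then Reload re-arms after an AttackRate-based delay; click-to-move logic remains unconnected.
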(event Custom|Reload
  (Utilities|FlowControl|Delay (/ 1.0 (Variables|Default|GetAttackRate)))
  (Variables|Default|SetWeaponLoaded true))

(event EventBeginPlay
  ;[1 1 1] Управление персонажем WASD
  (Variables|Default|SetWeaponLoaded true)
  (bind _aspc_1 (Utilities|Casting|CastToPC_1 (Game|GetPlayerController 0))))

(event Collision|EventActorBeginOverlap
  (params (OtherActor :type Actor%20Object%20Reference)))

(event EventTick
  (params (DeltaSeconds :type Float%20%28single-precision%29))
  (bind _maxvelocity (Variables|Default|GetMaxVelocity))
  (bind _backwardspeedmultiplyer (Variables|Default|GetBackwardSpeedMultiplyer))
  (bind _maxvelocity_2 (Variables|Default|GetMaxVelocity))
  (bind _returnvalue (* _maxvelocity_2 -1.0 _backwardspeedmultiplyer))
  ;[1 1 1] Управление персонажем WASD
  (bind _output_get (Variables|Default|SetCurrentVelocity (+ (* (Variables|Default|GetMaxVelocity) DeltaSeconds (Variables|/Game/Ironsphere/Core/Player/PC_1.PC_1_C|GetCharacterMove (stale EventBeginPlay _aspc_1))) (Variables|Default|GetCurrentVelocity))))
  (if (> (Variables|Default|GetCurrentVelocity) _maxvelocity)
    (Variables|Default|SetCurrentVelocity _maxvelocity))
  (if (> _returnvalue (Variables|Default|GetCurrentVelocity))
    (Variables|Default|SetCurrentVelocity _returnvalue))
  (if (== (Variables|/Game/Ironsphere/Core/Player/PC_1.PC_1_C|GetCharacterMove (stale EventBeginPlay _aspc_1)) 0.0)
    (Variables|Default|SetCurrentVelocity (- (Variables|Default|GetCurrentVelocity) (* (Math|Float|Absolute(Float) (Variables|Default|GetMaxVelocity)) DeltaSeconds (Math|Float|Sign(Float) (Variables|Default|GetCurrentVelocity))))))
  (Transformation|SetActorRelativeRotation (Math|Rotator|Delta(Rotator) (Transformation|GetActorRotation) (Math|Rotator|MakeRotator 0.0 0.0 (Variables|/Game/Ironsphere/Core/Player/PC_1.PC_1_C|GetCharacterTurn (stale EventBeginPlay _aspc_1)))))
  (if (> (Math|Float|Absolute(Float) (Variables|Default|GetCurrentVelocity)) (* (Math|Float|Absolute(Float) (Variables|Default|GetMaxVelocity)) DeltaSeconds))
    (Transformation|AddActorLocalOffset (* (Math|Vector|MakeVector (* _output_get DeltaSeconds) 0.0 0.0) "1.000000,0.000000,0.000000") false false))
  (Transformation|AddWorldRotation (Variables|Default|GetMarker_inner) "0.000000,0.500000,0.000000" false false)
  (Transformation|AddWorldRotation (Variables|Default|GetMarker_outer) "0.000000,-0.500000,0.000000" false false))

(fn ConstructionScript)

(fn UpdateTowerDirection
  (params (Direction :type Vector))
  (bind _returnvalue (Math|Vector|Normalize Direction))
  (bind _towerroot (Variables|Default|GetTowerRoot))
  (bind _returnvalue_2 (Math|Conversions|RotationFromXVector _returnvalue))
  (bind _returnvalue_3 (Transformation|GetWorldRotation _towerroot))
  (bind _yaw (Math|Rotator|BreakRotator _returnvalue_2))
  (bind _returnvalue_4 (Math|Rotator|MakeRotator 0.0 0.0 _yaw))
  (bind _returnvalue_5 (Math|Rotator|Delta(Rotator) _returnvalue_3 _returnvalue_4))
  (bind _yaw_2 (Math|Rotator|BreakRotator _returnvalue_5))
  (if (> (Math|Float|Absolute(Float) _yaw_2) (Variables|Default|GetdeltaTowerDirection))
    (Transformation|AddWorldRotation (Variables|Default|GetTowerRoot) (Math|Rotator|MakeRotator 0.0 0.0 (* (Variables|Default|GetdeltaTowerDirection) (Math|Float|Sign(Float) _yaw_2) -1.0)) false false)
    (else
      (Transformation|SetWorldRotation (Variables|Default|GetTowerRoot) _returnvalue_4 false false))))

(fn Shooting
  (if (Variables|Default|GetWeaponLoaded)
    (Game|SpawnActorfromClass "/Game/Projectiles/BP_bullet1.BP_bullet1_C" (Transformation|GetWorldTransform (Variables|Default|GetAmmoSpawn)) "Undefined" "MultiplyWithRoot" self 0)
    (CallFunction|Reload)
    (Variables|Default|SetWeaponLoaded false)
    (else
      (Development|PrintString "Not ready"))))