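; BP_CharacterBase is a base pawn for characters, providing health, movement, yaw rotation and death.
; Damage lowers CurrentHP; at zero, a living character spawns an explosion, is marked dead and is destroyed after a delay.
; Movement feeds FloatingPawnMovement, rotation scales input by speed and delta time, and Tick pins the actor to world Z zero.
; Shooting, Reloading and GetShootTransform are placeholders, with Shooting marked abstract.
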(event EventBeginPlay
  (Variables|Default|SetCurrentHP (Variables|Default|GetMaxHP)))

(event Collision|EventActorBeginOverlap
  (params (OtherActor :type Actor%20Object%20Reference)))

(event EventTick
  (params (DeltaSeconds :type Float%20%28single-precision%29))
  (bind _returnvalue (Transformation|GetActorLocation))
  (bind (_x _y _z) (Math|Vector|BreakVector _returnvalue))
  (if (!= _z 0.0)
    (Transformation|SetActorLocation (Math|Vector|MakeVector _x _y 0.0) false false)))

(event Game|Damage|EventAnyDamage
  (params (Damage :type Float%20%28single-precision%29) (DamageType :type Damage%20Type%20Object%20Reference) (InstigatedBy :type Controller%20Object%20Reference) (DamageCauser :type Actor%20Object%20Reference))
  (Variables|Default|SetCurrentHP (- (Variables|Default|GetCurrentHP) Damage))
  (if (<= (Variables|Default|GetCurrentHP) 0.0)
    (if (Variables|Default|GetAlive)
      (CallFunction|Death)
      (Utilities|FlowControl|Delay 5.0)
      (Actor|DestroyActor))))

(fn ConstructionScript)

(fn UpdateMovement
  (params (Direction :type Vector))
  (Class|PawnMovementComponent|AddInputVector (Variables|Default|GetFloatingPawnMovement) Direction false))

(fn Shooting
  (params (Active :type Boolean) (SelectedWeapon :type WeaponActiveSlot%20Enum :default "NewEnumerator0"))
  ;[1 1 1] Abstract FUnction
)

(fn GetShootTransform
  (return (Math|Transform|MakeTransform "0, 0, 0")))

(fn UpdateRotation
  (params (Rotation :type Float%20%28single-precision%29))
  (Transformation|AddActorLocalRotation (Math|Rotator|MakeRotator 0.0 0.0 (* Rotation -1.0 (Variables|Default|GetRotationSpeed) (Utilities|Time|GetWorldDeltaSeconds))) false false))

(fn Reloading
  (params (Active :type Boolean)))

(fn Death
  (params (DeathAnim :type Anim%20Montage%20Object%20Reference))
  (Effects|SpawnEmitteratLocation "/Game/StarterContent/Particles/P_Explosion.P_Explosion" (Transformation|GetActorLocation))
  (Variables|Default|SetAlive false))