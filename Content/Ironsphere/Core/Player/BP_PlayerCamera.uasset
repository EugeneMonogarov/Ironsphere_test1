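; BP_PlayerCamera is the player camera, with a zoomable spring arm and a camera-frame marker for the minimap.
; BeginPlay sets the starting arm length and adds a minimap object widget with the CameraFrame icon to the viewport.
; Tick repositions that widget by mapping the camera's world X/Y to screen coordinates with an inverted scale and fixed offset.
; CameraZoom adjusts arm length from its input, clamped between minimum and maximum limits.
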(event EventBeginPlay
  (bind _output_get (Variables|Default|SetTargetArmL 1.2e+03))
  (Variables|/Script/Engine.SpringArmComponent|SetTargetArmLength (Variables|Default|GetSpringArm01) _output_get)
  (bind _returnvalue (UserInterface|CreateWidget "/Game/Ironsphere/UI/Ingame/Map/WBS_MinimapObject.WBS_MinimapObject_C" 0 "/Game/Ironsphere/UI/Ingame/Map/CameraFrame.CameraFrame"))
  (UserInterface|Viewport|AddtoViewport _returnvalue 0))

(event Collision|EventActorBeginOverlap
  (params (OtherActor :type Actor%20Object%20Reference)))

(event EventTick
  (params (DeltaSeconds :type Float%20%28single-precision%29))
  (bind _returnvalue (Transformation|GetActorLocation))
  (bind (_x _y) (Math|Vector|BreakVector _returnvalue))
  (Class|UserWidget|SetPositioninViewport (stale EventBeginPlay _returnvalue) (Math|Vector2D|MakeVector2D (+ (* _x -0.1) 2e+02) (+ (* _y -0.1) 2e+02)) true))

(fn ConstructionScript)

(fn CameraZoom
  (params (ZoomCamera :type Float%20%28double-precision%29))
  (bind _springarm01 (Variables|Default|GetSpringArm01))
  (bind _minarmlenght (Variables|Default|GetMinArmLenght))
  (bind _output_get (Variables|Default|SetTargetArmL (+ (Variables|/Script/Engine.SpringArmComponent|GetTargetArmLength (Variables|Default|GetSpringArm01)) (* ZoomCamera 2.0))))
  (if (<= (Variables|Default|GetTargetArmL) (Variables|Default|GetMaxArmLenght))
    (if (>= (Variables|Default|GetTargetArmL) (Variables|Default|GetMinArmLenght))
      (Variables|/Script/Engine.SpringArmComponent|SetTargetArmLength _springarm01 _output_get)
      (else
        (Variables|Default|SetTargetArmL _minarmlenght)
        (Variables|/Script/Engine.SpringArmComponent|SetTargetArmLength _springarm01 _minarmlenght)))
    (else
      (Variables|/Script/Engine.SpringArmComponent|SetTargetArmLength _springarm01 (Variables|Default|GetMaxArmLenght)))))