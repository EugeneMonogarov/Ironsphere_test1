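; BP_ObjectiveArrow is an indicator actor that points horizontally toward its assigned Objective.
; BeginPlay moves it to world X/Y zero at a slightly randomized negative Z.
; Each Tick stores the objective distance, sets yaw toward it, and permanently enlarges the arrow if that distance is shorter than any other arrow's.
; The arrow destroys itself once its Objective is invalid.
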(event EventBeginPlay
  (Transformation|SetActorLocation (Math|Vector|MakeVector 0.0 0.0 (Math|Random|RandomFloatinRange -22.0 -2e+01)) false false))

(event Collision|EventActorBeginOverlap
  (params (OtherActor :type Actor%20Object%20Reference)))

(event EventTick
  (params (DeltaSeconds :type Float%20%28single-precision%29))
  (bind _returnvalue (Transformation|GetActorLocation))
  (bind _objective (Variables|Default|GetObjective))
  (bind _returnvalue_2 (Transformation|GetActorLocation _objective))
  (bind _returnvalue_3 (- _returnvalue_2 _returnvalue))
  (if (Utilities|IsValid _objective)
    (Variables|Default|SetLenght (Math|Vector|VectorLength _returnvalue_3))
    (Transformation|SetActorRotation (Math|Rotator|MakeRotator 0.0 0.0 (.Yaw (Math|Rotator|BreakRotator (Math|Conversions|RotationFromXVector (Math|Vector|Normalize _returnvalue_3))))))
    (bind _outactors (Actor|GetAllActorsOfClass "BP_ObjectiveArrow_C"))
    (bind _array_element (Utilities|Array|ForEachLoopwithBreak _outactors)
      (:LoopBody
        (if (< (Variables|Default|GetLenght) (Variables|BP_ObjectiveArrow_C|GetLenght _array_element))
          (Transformation|SetActorScale3D "1.200000,1.200000,1.200000"))))
    (else
      (Actor|DestroyActor)
      (Variables|Default|SetLenght 1e+04))))

(fn ConstructionScript)