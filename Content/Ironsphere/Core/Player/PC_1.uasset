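; Player controller that drives a separate camera pawn and relays mouse aim and fire to the BP_PlayerPawn found in the level.
; Tick stores move/turn axes, points the tower at the cursor's ground hit, snaps the camera to the player while CameraFix is held and applies zoom-scaled right-drag panning.
; BeginPlay creates the in-game widget; the wheel zooms the camera.
; Smoothed screen-edge scrolling is present but never runs.
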(event EventBeginPlay
  ;[1 1 1] Коэффициенты
  (Variables|Default|SetViewportEdgeThreshold 0.1)
  (Variables|Default|SetMouseLeftScale 1.0)
  (Variables|Default|SetMouseForwardScale 1.0)
  ;[1 1 1] Фиксация камеры на перонаже в начале игры
  (bind _returnvalue (Actor|GetActorOfClass "/Game/Ironsphere/Feature/Character/BP_PlayerPawn.BP_PlayerPawn_C"))
  (Variables|Default|SetPlayerPawn_var _returnvalue)
  (Variables|Default|SetMoveTargetLocation (Transformation|GetActorLocation _returnvalue))
  (bind _asbp_player_camera (Utilities|Casting|CastToBP_PlayerCamera (Pawn|GetControlledPawn)))
  (Variables|Default|SetAs%20BP%20Player%20Camera_var _asbp_player_camera)
  (bind _returnvalue_2 (UserInterface|CreateWidget "/Game/Ironsphere/UI/WBS_ingame.WBS_ingame_C"))
  (bind _output_get (Variables|Default|SetIngameWindow _returnvalue_2))
  (UserInterface|Viewport|AddtoViewport _output_get 0))

(event EventTick
  (params (DeltaSeconds :type Float%20%28single-precision%29))
  (bind (_locationx _locationy) (Game|Player|GetMousePosition))
  (bind _array (Utilities|Array|MakeArray "ObjectTypeQuery1"))
  (bind _hitresult (Class|PlayerController|GetHitResultUnderCursorforObjects _array true))
  (bind _returnvalue (Math|Vector|MakeVector _locationx _locationy 0.0))
  (bind _location (Collision|BreakHitResult _hitresult))
  (bind (_x _y) (Math|Vector|BreakVector _location))
  ;[1 1 1] Управление движением персонажа WASD
  (Variables|Default|SetCharacterMove (stale Input|AxisEvents|InputAxisCharacterMove AxisValue))
  (Variables|Default|SetCharacterTurn (stale Input|AxisEvents|InputAxisCharacterTurn AxisValue))
  ;[1 1 1] Поворот башни
  (Default|UpdateTowerDirection (Variables|Default|GetPlayerPawn_var) (- (Math|Vector|MakeVector _x _y 0.0) (Math|Vector|MakeVector (.X (Math|Vector|BreakVector (Transformation|GetWorldLocation (Variables|/Game/Ironsphere/Feature/Character/BP_PlayerPawn.BP_PlayerPawn_C|GetTowerRoot (Variables|Default|GetPlayerPawn_var))))) (.Y (Math|Vector|BreakVector (Transformation|GetWorldLocation (Variables|/Game/Ironsphere/Feature/Character/BP_PlayerPawn.BP_PlayerPawn_C|GetTowerRoot (Variables|Default|GetPlayerPawn_var))))) 0.0)))
  ;[1 1 1] Фиксация камеры на персонаже при нажатии ПРОБЕЛ
  (bind _returnvalue_2 (Actor|GetActorOfClass "/Game/Ironsphere/Feature/Character/BP_PlayerPawn.BP_PlayerPawn_C"))
  (Variables|Default|SetPlayerPawn_var _returnvalue_2)
  (if (== (Input|AxisValues|GetCameraFix) 1.0)
    (Transformation|SetActorLocation (Pawn|GetControlledPawn) (Transformation|GetActorLocation _returnvalue_2) false false))
  ;[1 1 1] Слайд камеры
  (if (Variables|Default|GetMouseSliding)
    (Pawn|Input|AddMovementInput (Pawn|GetControlledPawn) (- _returnvalue (Variables|Default|GetMouseSlidingOld)) (* (Variables|/Game/Ironsphere/Core/Player/BP_PlayerCamera.BP_PlayerCamera_C|GetTargetArmL (Variables|Default|GetAs%20BP%20Player%20Camera_var)) 2e-05) false)
    (Variables|Default|SetMouseSlidingOld (* _returnvalue "1.000000,1.000000,0.000000"))))

(event Input|AxisEvents|InputAxisCameraMoveMouse
  (params (AxisValue :type Float%20%28single-precision%29))
  ;[1 1 1] Управление камерой с помощью мыши (край экрана)
)

(event Input|AxisEvents|InputAxisCharacterTurn
  (params (AxisValue :type Float%20%28single-precision%29))
  ;[1 1 1] Управление движением персонажа WASD
)

(event Input|AxisEvents|InputAxisCharacterMove
  (params (AxisValue :type Float%20%28single-precision%29))
  ;[1 1 1] Управление движением персонажа WASD
)

(event Input|MouseEvents|MouseWheelDown
  (params (Key :type Key%20Structure))
  ;[1 1 1] Приближение-удаление с помощью колёсика мыши
  (:Pressed
    (Default|CameraZoom (Variables|Default|GetAs%20BP%20Player%20Camera_var) 122.0)))

(event Input|MouseEvents|RightMouseButton
  (params (Key :type Key%20Structure))
  ;[0 0 0] Управление правой кнопкой мыши
)

(event Input|MouseEvents|LeftMouseButton
  (params (Key :type Key%20Structure))
  ;[1 1 1] Стрельба
  (:Pressed
    (Default|Shooting (Variables|Default|GetPlayerPawn_var))))

(event Input|MouseEvents|MouseWheelUp
  (params (Key :type Key%20Structure))
  ;[1 1 1] Приближение-удаление с помощью колёсика мыши
  (:Pressed
    (Default|CameraZoom (Variables|Default|GetAs%20BP%20Player%20Camera_var) -122.0)))

(event Input|MouseEvents|MiddleMouseButton
  (params (Key :type Key%20Structure))
  ;[1 1 1] Приближение-удаление с помощью колёсика мыши
  (:Pressed
    (Variables|Default|SetMidMouse true)
    (Pawn|Input|AddMovementInput (Pawn|GetControlledPawn) "1.000000,1.000000,0.000000" (* (stale Input|AxisEvents|InputAxisCameraMoveMouse AxisValue) 1999.0) false)))

(event Input|MouseEvents|RightMouseButton
  (params (Key :type Key%20Structure))
  (bind (_locationx _locationy) (Game|Player|GetMousePosition))
  ;[1 1 1] Слайд камеры
  (:Pressed
    (if (not (Variables|Default|GetMouseSliding))
      (Variables|Default|SetMouseSliding true)
      (Variables|Default|SetMouseSlidingOld (Math|Vector|MakeVector _locationx _locationy 0.0))))
  (:Released
    (Variables|Default|SetMouseSliding false)))

(fn ConstructionScript)

(fn SmoothMovenentCamera
  (bind (_locationx _locationy) (Game|Player|GetMousePosition))
  (bind _returnvalue (Viewport|GetViewportSize))
  (bind _viewportedgethreshold (Variables|Default|GetViewportEdgeThreshold))
  (bind _viewportedgethreshold_2 (Variables|Default|GetViewportEdgeThreshold))
  (bind _viewportedgethreshold_3 (Variables|Default|GetViewportEdgeThreshold))
  (bind _returnvalue_2 (/ _locationx (.x _returnvalue)))
  (bind _returnvalue_3 (/ _locationy (.y _returnvalue)))
  (bind _returnvalue_4 (- 1.0 _viewportedgethreshold))
  (bind _output_get (Variables|Default|SetMouseLeftScale (Math|Float|SelectFloat (/ (- _returnvalue_2 _returnvalue_4) _viewportedgethreshold_3) (Math|Float|SelectFloat (* (/ (- _returnvalue_2 _viewportedgethreshold_3) _viewportedgethreshold_3) -1.0) 0.0 (< _returnvalue_2 _viewportedgethreshold)) (> _returnvalue_2 _returnvalue_4))))
  (bind _output_get_2 (Variables|Default|SetMouseForwardScale (Math|Float|SelectFloat (/ (- _returnvalue_3 _returnvalue_4) _viewportedgethreshold_2) (Math|Float|SelectFloat (* (/ (- _returnvalue_3 _viewportedgethreshold_2) _viewportedgethreshold_2) -1.0) 0.0 (< _returnvalue_3 _viewportedgethreshold)) (> _returnvalue_3 _returnvalue_4)))))

(fn SpawnMousePosition
  (params (SpawnTransform :type Transform))
  (Game|SpawnActorfromClass "/Game/Ironsphere/Core/Player/BP_MousePosition.BP_MousePosition_C" SpawnTransform "AlwaysSpawn" "MultiplyWithRoot" 0 0))

(fn SpawnMousePosition2
  (params (SpawnTransform :type Transform))
  (Game|SpawnActorfromClass "/Game/Ironsphere/Core/Player/BP_MousePosition2.BP_MousePosition2_C" SpawnTransform "Undefined" "MultiplyWithRoot" 0 0))