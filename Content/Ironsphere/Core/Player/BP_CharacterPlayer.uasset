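; Player mech pawn with a rotating tower and two weapon slots.
; SetMech and SetWeapon pull mesh, speed, HP, armor and weapon classes from data tables, attaching spawned weapons to mount points.
; Shooting and reloading go to the selected slot's weapon, while the tower yaws toward a given direction in capped steps.
; Tick plays random footstep sounds when either foot marker drops below a fixed world height.
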(event EventBeginPlay
  (|CallParentFunction))

(event Collision|EventActorBeginOverlap
  (params (OtherActor :type Actor%20Object%20Reference)))

(event EventTick
  (params (DeltaSeconds :type Float%20%28single-precision%29))
  (bind _returnvalue (Transformation|GetActorLocation))
  (bind _stepsoundr (Variables|Default|GetStepSoundR))
  (Utilities|FlowControl|Sequence
    (:then_0
      (if (> (.Z (Math|Vector|BreakVector (Transformation|GetWorldLocation (Variables|Default|GetStepSoundL)))) 7.0)
        (Variables|Default|SetLeftLegDown false))
      (if (and (not (Variables|Default|GetLeftLegDown)) (> 7.0 (.Z (Math|Vector|BreakVector (Transformation|GetWorldLocation (Variables|Default|GetStepSoundL))))))
        (Variables|Default|SetLeftLegDown true)
        (switch int (Math|Random|RandomInteger 4) :!label _label
          (:0
            (Audio|SpawnSoundatLocation "/Game/Ironsphere/Sound/Step/mech_step_4.mech_step_4" _returnvalue "0, 0, 0" 0.4 1.0 0.0 0 0))
          (:1
            (Audio|SpawnSoundatLocation "/Game/Ironsphere/Sound/Step/mech_step_1.mech_step_1" _returnvalue "0, 0, 0" 0.4 1.0 0.0 0 0))
          (:2
            (Audio|SpawnSoundatLocation "/Game/Ironsphere/Sound/Step/mech_step_2.mech_step_2" _returnvalue "0, 0, 0" 0.4 1.0 0.0 0 0))
          (:3
            (Audio|SpawnSoundatLocation "/Game/Ironsphere/Sound/Step/mech_step_3.mech_step_3" _returnvalue "0, 0, 0" 0.4 1.0 0.0 0 0)))))
    (:then_1
      (if (> (.Z (Math|Vector|BreakVector (Transformation|GetWorldLocation _stepsoundr))) 7.0)
        (Variables|Default|SetRightLegDown false))
      (if (and (not (Variables|Default|GetRightLegDown)) (> 7.0 (.Z (Math|Vector|BreakVector (Transformation|GetWorldLocation _stepsoundr)))))
        (Variables|Default|SetRightLegDown true)
        (goto _label)))))

(fn ConstructionScript
  (|CallParentFunction))

(fn UpdateTowerDirection
  (params (TowerDirection :type Vector))
  (bind _returnvalue (Math|Vector|Normalize TowerDirection))
  (bind _towerroot1 (Variables|Default|GetTowerRoot1))
  (bind _returnvalue_2 (Math|Conversions|RotationFromXVector _returnvalue))
  (bind _returnvalue_3 (Transformation|GetWorldRotation _towerroot1))
  (bind _yaw (Math|Rotator|BreakRotator _returnvalue_2))
  (bind _returnvalue_4 (Math|Rotator|MakeRotator 0.0 0.0 _yaw))
  (bind _returnvalue_5 (Math|Rotator|Delta(Rotator) _returnvalue_3 _returnvalue_4))
  (bind _yaw_2 (Math|Rotator|BreakRotator _returnvalue_5))
  (if (> (Math|Float|Absolute(Float) _yaw_2) (Variables|Default|GetdeltaTowerDirection))
    (Transformation|AddWorldRotation (Variables|Default|GetTowerRoot1) (Math|Rotator|MakeRotator 0.0 0.0 (* (Variables|Default|GetdeltaTowerDirection) (Math|Float|Sign(Float) _yaw_2) -1.0)) false false)
    (else
      (Transformation|SetWorldRotation (Variables|Default|GetTowerRoot1) _returnvalue_4 false false))))

(fn GetShootTransform
  (return (Transformation|GetWorldTransform (Variables|Default|GetProjectileSpawnPoint))))

(fn Shooting
  (params (Active :type Boolean))
  (switch Utilities|FlowControl|Switch|SwitchonWeaponActiveSlot (Variables|Default|GetSelectedWeapon)
    (:NewEnumerator0
      (if (Utilities|IsValid (Variables|Default|GetWeapon1_reference))
        (Default|WeaponShot (Variables|Default|GetWeapon1_reference) Active)
        (elif Active
          (Audio|SpawnSoundatLocation "/Engine/VREditor/Sounds/UI/Flashlight_Switch.Flashlight_Switch" (Transformation|GetActorLocation) "0, 0, 0" 1.0 1.0 0.0 0 0))))
    (:NewEnumerator1
      (if (Utilities|IsValid (Variables|Default|GetWeapon2_reference))
        (Default|WeaponShot (Variables|Default|GetWeapon2_reference) Active)
        (elif Active
          (Audio|SpawnSoundatLocation "/Engine/VREditor/Sounds/UI/Flashlight_Switch.Flashlight_Switch" "0, 0, 0" "0, 0, 0" 1.0 1.0 0.0 0 0))))))

(fn SetActiveSlot
  (params (SelectedWeapon :type WeaponActiveSlot%20Enum :default "NewEnumerator0"))
  (Variables|Default|SetSelectedWeapon SelectedWeapon))

(fn SetMech
  (params (MechID :type Name))
  (Variables|Default|SetMechId (Utilities|String|ToString(Name) MechID))
  (bind _returnvalue (Utilities|GetDataTableRow "/Game/Ironsphere/Feature/Mechs/DT_Mechs.DT_Mechs" MechID)
    (:then
      (Components|SkeletalMesh|SetSkeletalMeshAsset (Variables|Default|GetMesh) (.SkeletalMeshAsset (Utilities|Struct|BreakST_Mechs _returnvalue)))
      (Utilities|FlowControl|Sequence
        (:then_0
          (Variables|/Script/Engine.FloatingPawnMovement|SetMaxSpeed (Variables|Default|GetFloatingPawnMovement) (Math|Conversions|ToFloat(Integer) (.Speed (Utilities|Struct|BreakST_Mechs _returnvalue)))))
        (:then_1
          (Variables|Default|SetMaxHP (Math|Conversions|ToFloat(Integer) (.HP (Utilities|Struct|BreakST_Mechs _returnvalue)))))
        (:then_2
          (Variables|Default|SetPhysicalArmor (Math|Conversions|ToFloat(Integer) (.PhysicalArmor (Utilities|Struct|BreakST_Mechs _returnvalue)))))
        (:then_3
          (Variables|Default|SetLaserArmor (Math|Conversions|ToFloat(Integer) (.LaserArmor (Utilities|Struct|BreakST_Mechs _returnvalue)))))))))

(fn SetWeapon
  (params (Slot :type WeaponActiveSlot%20Enum :default "NewEnumerator0") (WeaponID :type String))
  (bind _returnvalue (Utilities|String|StringToName WeaponID))
  (switch Utilities|FlowControl|Switch|SwitchonWeaponActiveSlot Slot
    (:NewEnumerator0
      (if (Utilities|IsValid (Variables|Default|GetWeapon1_reference))
        (Actor|DestroyActor (Variables|Default|GetWeapon1_reference)))
      (bind _returnvalue_2 (Utilities|GetDataTableRow "/Game/Ironsphere/Feature/Weapon/DT_Weapon.DT_Weapon" _returnvalue)
        (:then
          (bind _returnvalue_3 (Game|SpawnActorfromClass (.WeaponBP (Utilities|Struct|BreakST_Weapon _returnvalue_2)) (Transformation|GetWorldTransform (Variables|Default|GetWeaponPlace1)) "AlwaysSpawn" "MultiplyWithRoot" self 0))
          (bind _output_get (Variables|Default|SetWeapon1_reference _returnvalue_3))
          (Transformation|AttachComponentToComponent _output_get (Variables|Default|GetWeaponPlace1) "None" "SnapToTarget" "SnapToTarget" "SnapToTarget" true))
        (:RowNotFound
          (Development|PrintString (Utilities|String|Append "Not Found Weapon:" WeaponID)))))
    (:NewEnumerator1
      (if (Utilities|IsValid (Variables|Default|GetWeapon2_reference))
        (Actor|DestroyActor (Variables|Default|GetWeapon2_reference)))
      (bind _returnvalue_4 (Utilities|GetDataTableRow "/Game/Ironsphere/Feature/Weapon/DT_Weapon.DT_Weapon" _returnvalue)
        (:then
          (bind _returnvalue_5 (Game|SpawnActorfromClass (.WeaponBP (Utilities|Struct|BreakST_Weapon _returnvalue_4)) (Transformation|GetWorldTransform (Variables|Default|GetWeaponPlace2)) "AlwaysSpawn" "MultiplyWithRoot" self 0))
          (bind _output_get_2 (Variables|Default|SetWeapon2_reference _returnvalue_5))
          (Transformation|AttachComponentToComponent _output_get_2 (Variables|Default|GetWeaponPlace2) "None" "SnapToTarget" "SnapToTarget" "SnapToTarget" true))))))

(fn Reloading
  (params (Active :type Boolean))
  (switch Utilities|FlowControl|Switch|SwitchonWeaponActiveSlot (Variables|Default|GetSelectedWeapon)
    (:NewEnumerator0
      (if (Utilities|IsValid (Variables|Default|GetWeapon1_reference))
        (Default|WeaponReload (Variables|Default|GetWeapon1_reference))
        (elif Active
          _)))
    (:NewEnumerator1
      (if (Utilities|IsValid (Variables|Default|GetWeapon2_reference))
        (Default|WeaponReload (Variables|Default|GetWeapon2_reference))
        (elif Active
          _)))))