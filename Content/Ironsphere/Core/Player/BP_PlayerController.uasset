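; Player controller for a mech game that possesses a separate camera pawn while driving the BP_CharacterPlayer mech found in the level.
; Input axes move and turn the mech, mouse buttons and number keys handle firing and weapon slots, and Tick aims the tower at the cursor trace.
; The camera snaps to the mech, drag-slides and wheel-zooms; edge scrolling is disconnected.
; BeginPlay creates the mech-selection and in-game widgets.
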(event EventBeginPlay
  ;[1 1 1] Коэффициенты
  (Variables|Default|SetViewportEdgeThreshold 0.1)
  (Variables|Default|SetMouseLeftScale 1.0)
  (Variables|Default|SetMouseForwardScale 1.0)
  ;[1 1 1 1 44] Фиксация камеры на перонаже в начале игры
  (CallFunction|InitializePlayer)
  (bind _asbp_player_camera (Utilities|Casting|CastToBP_PlayerCamera (Pawn|GetControlledPawn)))
  (Variables|Default|SetAs%20BP%20Player%20Camera_var _asbp_player_camera)
  ;[1 1 1 1 44] Интерйфейс выбора меха
  (bind _returnvalue (UserInterface|CreateWidget "/Game/Ironsphere/UI/SelectMech/SelectMech.SelectMech_C"))
  (UserInterface|Viewport|AddtoViewport _returnvalue 0)
  ;[1 1 1 1 44] Загрузка игрового интерфейса
  (bind _returnvalue_2 (UserInterface|CreateWidget "/Game/Ironsphere/UI/Ingame/WBS_ingame.WBS_ingame_C"))
  (bind _output_get (Variables|Default|SetIngameWindow _returnvalue_2))
  (UserInterface|Viewport|AddtoViewport _output_get 0)
  (Variables|/Game/Ironsphere/UI/Ingame/WBS_ingame.WBS_ingame_C|SetMech _output_get (Variables|Default|GetControlledMech)))

(event EventTick
  (params (DeltaSeconds :type Float%20%28single-precision%29))
  (bind (_locationx _locationy) (Game|Player|GetMousePosition))
  (bind _array (Utilities|Array|MakeArray "ObjectTypeQuery1"))
  (bind _controlledmech (Variables|Default|GetControlledMech))
  (bind _hitresult (Class|PlayerController|GetHitResultUnderCursorforObjects _array true))
  (bind _returnvalue (Math|Vector|MakeVector _locationx _locationy 0.0))
  (bind _towerroot1 (Variables|/Game/Ironsphere/Core/Player/BP_CharacterPlayer.BP_CharacterPlayer_C|GetTowerRoot1 _controlledmech))
  (bind _location (Collision|BreakHitResult _hitresult))
  (bind _returnvalue_2 (Transformation|GetWorldLocation _towerroot1))
  (bind (_x _y) (Math|Vector|BreakVector _location))
  (bind (_x_2 _y_2) (Math|Vector|BreakVector _returnvalue_2))
  ;[0 0 0 1 44] Управление движением персонажа WASD
  (Variables|Default|SetCharacterMove 0.0)
  (Variables|Default|SetCharacterTurn 0.0)
  ;[1 1 1 1 44] Поворот башни
  (Default|UpdateTowerDirection (Variables|Default|GetControlledMech) (- (Math|Vector|MakeVector _x _y 0.0) (Math|Vector|MakeVector _x_2 _y_2 0.0)))
  ;[1 1 1 1 44] Фиксация камеры на персонаже при нажатии ПРОБЕЛ
  (if (== (Input|AxisValues|GetCameraFix) 1.0)
    (Transformation|SetActorLocation (Pawn|GetControlledPawn) (Transformation|GetActorLocation (Variables|Default|GetControlledMech)) false false))
  ;[1 1 1 1 44] Слайд камеры
  (if (Variables|Default|GetMouseSliding)
    (Pawn|Input|AddMovementInput (Pawn|GetControlledPawn) (- _returnvalue (Variables|Default|GetMouseSlidingOld)) (* (Variables|/Game/Ironsphere/Core/Player/BP_PlayerCamera.BP_PlayerCamera_C|GetTargetArmL (Variables|Default|GetAs%20BP%20Player%20Camera_var)) 2e-05) false)
    (Variables|Default|SetMouseSlidingOld (* _returnvalue "1.000000,1.000000,0.000000"))))

(event Input|AxisEvents|InputAxisCameraMoveMouse
  (params (AxisValue :type Float%20%28single-precision%29))
  ;[1 1 1] Управление камерой с помощью мыши (край экрана)
)

(event Input|AxisEvents|InputAxisCharacterTurn
  (params (AxisValue :type Float%20%28single-precision%29))
  (Default|UpdateRotation (Variables|Default|GetControlledMech) AxisValue))

(event Input|AxisEvents|InputAxisCharacterMove
  (params (AxisValue :type Float%20%28single-precision%29))
  (bind _controlledmech (Variables|Default|GetControlledMech))
  (Default|UpdateMovement _controlledmech (* AxisValue (Transformation|GetActorForwardVector _controlledmech))))

(event Input|MouseEvents|MouseWheelDown
  (params (Key :type Key%20Structure :default "None"))
  ;[1 1 1] Приближение-удаление с помощью колёсика мыши
  (:Pressed
    (Default|CameraZoom (Variables|Default|GetAs%20BP%20Player%20Camera_var) 122.0)))

(event Input|KeyboardEvents|Q
  (params (Key :type Key%20Structure :default "None"))
  ;[0 0 0] ОТЛАДКА ОРУЖИЯ
)

(event Input|KeyboardEvents|E
  (params (Key :type Key%20Structure :default "None"))
  ;[0 0 0] ОТЛАДКА ОРУЖИЯ
)

(event Input|KeyboardEvents|F
  (params (Key :type Key%20Structure :default "None"))
  ;[0 0 0] ОТЛАДКА ОРУЖИЯ
)

(event Input|KeyboardEvents|D
  (params (Key :type Key%20Structure :default "None"))
  ;[0 0 0] ОТЛАДКА ОРУЖИЯ
)

(event Input|MouseEvents|LeftMouseButton
  (params (Key :type Key%20Structure :default "None"))
  (bind _controlledmech (Variables|Default|GetControlledMech))
  ;[1 1 1 1 44] Стрельба
  (:Pressed
    (Default|Shooting _controlledmech true))
  (:Released
    (Default|Shooting _controlledmech false)))

(event Input|MouseEvents|MouseWheelUp
  (params (Key :type Key%20Structure :default "None"))
  ;[1 1 1] Приближение-удаление с помощью колёсика мыши
  (:Pressed
    (Default|CameraZoom (Variables|Default|GetAs%20BP%20Player%20Camera_var) -122.0)))

(event Input|MouseEvents|MiddleMouseButton
  (params (Key :type Key%20Structure :default "None"))
  ;[1 1 1] Приближение-удаление с помощью колёсика мыши
  (:Pressed
    (Variables|Default|SetMidMouse true)
    (Pawn|Input|AddMovementInput (Pawn|GetControlledPawn) "1.000000,1.000000,0.000000" (* (stale Input|AxisEvents|InputAxisCameraMoveMouse AxisValue) 1999.0) false)))

(event Input|MouseEvents|RightMouseButton
  (params (Key :type Key%20Structure :default "None"))
  (bind (_locationx _locationy) (Game|Player|GetMousePosition))
  ;[1 1 1 1 44] Слайд камеры
  (:Pressed
    (if (not (Variables|Default|GetMouseSliding))
      (Variables|Default|SetMouseSliding true)
      (Variables|Default|SetMouseSlidingOld (Math|Vector|MakeVector _locationx _locationy 0.0))))
  (:Released
    (Variables|Default|SetMouseSliding false)))

(event Input|KeyboardEvents|1
  (params (Key :type Key%20Structure :default "None"))
  ;[1 1 1 1 44] Выбор оружия
  (:Pressed
    (Default|SetActiveSlot (Variables|Default|GetControlledMech) "NewEnumerator0")
    (Default|WeaponShot (Variables|/Game/Ironsphere/Core/Player/BP_CharacterPlayer.BP_CharacterPlayer_C|GetWeapon2_reference (Variables|Default|GetControlledMech)) false)))

(event Input|KeyboardEvents|2
  (params (Key :type Key%20Structure :default "None"))
  ;[1 1 1 1 44] Выбор оружия
  (:Pressed
    (Default|SetActiveSlot (Variables|Default|GetControlledMech) "NewEnumerator1")
    (Default|WeaponShot (Variables|/Game/Ironsphere/Core/Player/BP_CharacterPlayer.BP_CharacterPlayer_C|GetWeapon1_reference (Variables|Default|GetControlledMech)) false)))

(event Input|KeyboardEvents|3
  (params (Key :type Key%20Structure :default "None"))
  ;[1 1 1 1 44] Выбор оружия
  (:Pressed
    (Default|SetActiveSlot (Variables|Default|GetControlledMech) "NewEnumerator2")))

(fn ConstructionScript)

(fn SmoothMovenentCamera
  (bind (_locationx _locationy) (Game|Player|GetMousePosition))
  (bind _returnvalue (Viewport|GetViewportSize))
  (bind _viewportedgethreshold (Variables|Default|GetViewportEdgeThreshold))
  (bind _viewportedgethreshold_2 (Variables|Default|GetViewportEdgeThreshold))
  (bind _viewportedgethreshold_3 (Variables|Default|GetViewportEdgeThreshold))
  (bind _returnvalue_2 (/ _locationx (.x _returnvalue)))
  (bind _returnvalue_3 (/ _locationy (.y _returnvalue)))
  (bind _returnvalue_4 (- 1.0 _viewportedgethreshold))
  (bind _output_get (Variables|Default|SetMouseLeftScale (Math|Float|SelectFloat (/ (- _returnvalue_2 _returnvalue_4) _viewportedgethreshold_3) (Math|Float|SelectFloat (* (/ (- _returnvalue_2 _viewportedgethreshold_3) _viewportedgethreshold_3) -1.0) 0.0 (< _returnvalue_2 _viewportedgethreshold)) (> _returnvalue_2 _returnvalue_4))))
  (bind _output_get_2 (Variables|Default|SetMouseForwardScale (Math|Float|SelectFloat (/ (- _returnvalue_3 _returnvalue_4) _viewportedgethreshold_2) (Math|Float|SelectFloat (* (/ (- _returnvalue_3 _viewportedgethreshold_2) _viewportedgethreshold_2) -1.0) 0.0 (< _returnvalue_3 _viewportedgethreshold)) (> _returnvalue_3 _returnvalue_4)))))

(fn InitializePlayer
  (Actor|GetAllActorsOfClass "/Script/Engine.PlayerStart")
  (bind _returnvalue (Actor|GetActorOfClass "/Game/Ironsphere/Core/Player/BP_CharacterPlayer.BP_CharacterPlayer_C"))
  (Variables|Default|SetControlledMech _returnvalue))