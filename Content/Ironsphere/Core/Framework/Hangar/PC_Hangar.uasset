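; Player controller for the mech hangar menu: creates the hangar widget, plays music and ambience, and handles inventory and save state.
; On the session's first visit it loads the single save slot or starts a new game with a starter loadout.
; Move functions edit inventory arrays, stacking consumables by DataTable limits with Shift/Ctrl setting amounts, then refresh widgets.
; Hotkeys trigger new/save/load, a money cheat and a test map.
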(event EventBeginPlay
  ;[1 1 1] Begin Play
  (Variables|Default|SetbShowMouseCursor true)
  (bind _asgi_main (Utilities|Casting|CastToGI_Main (Game|GetGameInstance)))
  (bind _output_get (Variables|Default|SetGI_Main_ref _asgi_main))
  (Variables|/Game/Ironsphere/Core/Framework/GI_Main.GI_Main_C|SetCurrentLevelIndex _output_get -1)
  (Utilities|FlowControl|Sequence
    (:then_0
      (bind _returnvalue (UserInterface|CreateWidget "/Game/Ironsphere/UI/Hangar/WBC_Hangar.WBC_Hangar_C"))
      (Default|UpdateMechParameters (Variables|Default|GetGI_Main_ref))
      (while (not (Utilities|IsValid _returnvalue))
        (Utilities|FlowControl|Delay 0.1))
      (UserInterface|Viewport|AddtoViewport _returnvalue 0)
      (Variables|Default|SetHangarWidget_reference _returnvalue)
      (Default|ShowMechParameters (Variables|/Game/Ironsphere/UI/Hangar/WBC_Hangar.WBC_Hangar_C|GetWBC_HangarMech (Variables|Default|GetHangarWidget_reference)))
      (Default|UpdateHangarStorage (Variables|/Game/Ironsphere/UI/Hangar/WBC_Hangar.WBC_Hangar_C|GetWBC_HangarStorage (Variables|Default|GetHangarWidget_reference)))
      (Default|UpdateMechInventory (Variables|/Game/Ironsphere/UI/Hangar/WBC_Hangar.WBC_Hangar_C|GetWBC_Consumable (Variables|Default|GetHangarWidget_reference)))
      (CallFunction|UpdateAllWidgets)
      (Utilities|FlowControl|Sequence
        (:then_0
          (switch int (Math|Random|RandomInteger 5)
            (:0
              (Audio|SpawnSound2D "/Game/Ironsphere/Sound/Music/Hangar5.Hangar5" 0.3 1.0 0.0 0 :!label _label))
            (:1
              (Audio|SpawnSound2D "/Game/Ironsphere/Sound/Music/Hangar2.Hangar2" 0.3 1.0 0.0 0))
            (:2
              (Audio|SpawnSound2D "/Game/Ironsphere/Sound/Music/Hangar1.Hangar1" 0.3 1.0 0.0 0))
            (:3
              (Audio|SpawnSound2D "/Game/Ironsphere/Sound/Music/Hangar3.Hangar3" 0.3 1.0 0.0 0))
            (:4
              (goto _label))
            (:5
              (goto _label))))
        (:then_1
          (Audio|SpawnSound2D "/Game/Ironsphere/Sound/Music/MenuAmbient.MenuAmbient" 0.05 1.0 0.0 0))))
    (:then_1
      (if (not (Variables|/Game/Ironsphere/Core/Framework/GI_Main.GI_Main_C|GetGameStarted _output_get))
        ;[1 1 1] Запуск игры (загрузка или новая игра)
        (Variables|/Game/Ironsphere/Core/Framework/GI_Main.GI_Main_C|SetGameStarted _output_get true)
        (bind _returnvalue_2 (SaveGame|DoesSaveGameExist "1"))
        (if _returnvalue_2
          (bind _returnvalue_3 (SaveGame|LoadGamefromSlot "1"))
          (Audio|SpawnSound2D "/Engine/VREditor/Sounds/UI/Dockable_Window_Pick_Up.Dockable_Window_Pick_Up" 1.0 1.0 0.0 0)
          (bind _asbp_save_game (Utilities|Casting|CastToBP_SaveGame _returnvalue_3))
          (Variables|Default|SetSaveGame_ref _asbp_save_game)
          (CallFunction|LoadGame)
          (else
            (bind _returnvalue_4 (SaveGame|CreateSaveGameObject "/Game/Ironsphere/Core/SaveGame/BP_SaveGame.BP_SaveGame_C"))
            (Variables|Default|SetSaveGame_ref _returnvalue_4)
            (CallFunction|NewGame)))))))

(event EventTick
  (params (DeltaSeconds :type Float%20%28single-precision%29))
  (if (Variables|Default|GetisShiftPressed)
    (Variables|Default|SetItemsMoveAmount 10)
    (elif (Variables|Default|GetisCtrlPressed)
      (Variables|Default|SetItemsMoveAmount 1)
      (else
        (Variables|Default|SetItemsMoveAmount 0)))))

(event Input|KeyboardEvents|LeftCtrl
  (params (Key :type Key%20Structure :default "None"))
  (:Pressed
    (Variables|Default|SetisCtrlPressed true)
    (Utilities|FlowControl|Delay 0.1 :!label _label))
  (:Released
    (Variables|Default|SetisCtrlPressed false)
    (goto _label)))

(event Input|KeyboardEvents|O
  (params (Key :type Key%20Structure :default "None"))
  ;[1 1 1] Load Game
  (:Pressed
    (if (Variables|Default|GetisCtrlPressed)
      (CallFunction|LoadGame))))

(event Input|KeyboardEvents|N
  (params (Key :type Key%20Structure :default "None"))
  ;[1 1 1] Save Game
  (:Pressed
    (if (Variables|Default|GetisCtrlPressed)
      (CallFunction|NewGame))))

(event Input|KeyboardEvents|T
  (params (Key :type Key%20Structure :default "None"))
  ;[1 1 1] TestLevel
  (:Pressed
    (if (and (Variables|Default|GetisShiftPressed) (Variables|Default|GetisCtrlPressed))
      (if (not (Variables|Default|GetLoadingLevel))
        (Variables|Default|SetLoadingLevel true)
        (Game|OpenLevel(byName) "TestMap")))))

(event Input|KeyboardEvents|S
  (params (Key :type Key%20Structure :default "None"))
  ;[1 1 1] Save Game
  (:Pressed
    (if (Variables|Default|GetisCtrlPressed)
      (CallFunction|SaveGame))))

(event Input|KeyboardEvents|M
  (params (Key :type Key%20Structure :default "None"))
  (bind _gi_main_ref (Variables|Default|GetGI_Main_ref))
  ;[1 1 1] Чит на деньги
  (:Pressed
    (if (and (Variables|Default|GetisCtrlPressed) (Variables|Default|GetisShiftPressed))
      (Variables|/Game/Ironsphere/Core/Framework/GI_Main.GI_Main_C|SetMoney _gi_main_ref (+ (Variables|/Game/Ironsphere/Core/Framework/GI_Main.GI_Main_C|GetMoney _gi_main_ref) 1e+04)))))

(event Input|KeyboardEvents|LeftShift
  (params (Key :type Key%20Structure :default "None"))
  (:Pressed
    (Variables|Default|SetisShiftPressed true)
    (Utilities|FlowControl|Delay 0.1 :!label _label))
  (:Released
    (Variables|Default|SetisShiftPressed false)
    (goto _label)))

(event Input|KeyboardEvents|LeftAlt
  (params (Key :type Key%20Structure :default "None"))
  (:Pressed
    (Variables|Default|SetisAltPressed true)
    (Audio|SpawnSound2D "/Engine/VREditor/Sounds/UI/Dockable_Window_Open.Dockable_Window_Open" 1.0 1.0 0.0 0)
    (Utilities|FlowControl|Delay 0.1 :!label _label))
  (:Released
    (Variables|Default|SetisAltPressed false)
    (goto _label)))

(fn ConstructionScript)

(fn MoveItemfromto
  (params (Elem :type Integer) (From :type Array%20of%20ST%20Item%20Structures) (To :type Array%20of%20ST%20Item%20Structures))
  (bind _output (Utilities|Array|Get(acopy) From Elem))
  (if (Utilities|Array|IsEmpty (.ID (Utilities|Struct|BreakST_ItemTemplate (.ItemTemplate (Utilities|Struct|BreakST_Item _output)))))
    (Audio|SpawnSound2D "/Engine/VREditor/Sounds/UI/Click_on_Button.Click_on_Button" 1.0 1.0 0.0 0)
    (else
      (bind _invfull (CallFunction|AddItemtoInventory _output To))
      (if _invfull
        (Audio|SpawnSound2D "/Engine/VREditor/Sounds/VR_click1.VR_click1" 1.0 1.0 0.0 0)
        (else
          (CallFunction|RemoveItemfromInventory Elem From)
          (CallFunction|UpdateAllWidgets)
          (Audio|SpawnSound2D "/Engine/VREditor/Sounds/UI/Gizmo_Handle_Clicked.Gizmo_Handle_Clicked" 1.0 1.0 0.0 0))))))

(fn GetFirstEmptySlot
  (params (Ivnentory :type Array%20of%20ST%20Item%20Structures))
  (for (_array_element _array_index) Ivnentory
    (if (Utilities|Array|IsEmpty (.ID (Utilities|Struct|BreakST_ItemTemplate (.ItemTemplate (Utilities|Struct|BreakST_Item _array_element)))))
      (return _array_index)))
  (return -1))

(fn AddItemtoInventory
  (params (Item :type ST%20Item%20Structure) (Inventory :type Array%20of%20ST%20Item%20Structures))
  (bind _newparam (CallFunction|GetFirstEmptySlot Inventory))
  (if (>= _newparam 0)
    (if true
      (Utilities|Array|SetArrayElem Inventory _newparam Item)
      (Default|UpdateHangarStorage (Variables|/Game/Ironsphere/UI/Hangar/WBC_Hangar.WBC_Hangar_C|GetWBC_HangarStorage (Variables|Default|GetHangarWidget_reference)))
      (return false))
    (else
      (return true))))

(fn RemoveItemfromInventory
  (params (Index :type Integer) (Inventory :type Array%20of%20ST%20Item%20Structures))
  (Utilities|Array|SetArrayElem Inventory Index (Utilities|Struct|MakeST_Item (Utilities|Struct|MakeST_ItemTemplate "" "NewEnumerator7" "None")))
  (Default|UpdateHangarStorage (Variables|/Game/Ironsphere/UI/Hangar/WBC_Hangar.WBC_Hangar_C|GetWBC_HangarStorage (Variables|Default|GetHangarWidget_reference))))

(fn MoveConsumablefromto
  (params (From :type Array%20of%20ST%20Item%20Structures) (To :type Array%20of%20ST%20Item%20Structures) (Index :type Integer) (Device :type Boolean))
  (bind _output (Utilities|Array|Get(acopy) From Index))
  (bind (_itemtemplate _count) (Utilities|Struct|BreakST_Item _output))
  (bind _output_2 (Utilities|Array|Get(acopy) From Index))
  (bind _output_3 (Utilities|Array|Get(acopy) From Index))
  (bind (_itemtemplate_2 _count_2) (Utilities|Struct|BreakST_Item _output_3))
  (bind _itemtemplate_3 (Utilities|Struct|BreakST_Item _output_2))
  (bind _id (Utilities|Struct|BreakST_ItemTemplate _itemtemplate_3))
  (bind _returnvalue (Utilities|String|StringToName _id))
  (if (Variables|Default|GetisShiftPressed)
    (Variables|Default|SetAmount 10)
    (elif (Variables|Default|GetisCtrlPressed)
      (Variables|Default|SetAmount 1)
      (else
        (Variables|Default|SetAmount _count))))
  (if (Utilities|Array|IsEmpty (.ID (Utilities|Struct|BreakST_ItemTemplate _itemtemplate)))
    (Audio|SpawnSound2D "/Engine/VREditor/Sounds/UI/Click_on_Button.Click_on_Button" 1.0 1.0 0.0 0)
    (else
      (Utilities|FlowControl|Sequence
        (:then_0
          ;[1 1 1] Поиск целевого слота (куда)
          (for (_array_element _array_index) To
            (if Device
              (bind _returnvalue_2 (Utilities|GetDataTableRow "/Game/Ironsphere/Feature/Device/DT_Device.DT_Device" _returnvalue)
                (:then
                  (Variables|Default|SetStack (.Stack (Utilities|Struct|BreakST_Device _returnvalue_2)))))
              (else
                (bind _returnvalue_3 (Utilities|GetDataTableRow "/Game/Ironsphere/Feature/Consumable/DT_Consumable.DT_Consumable" _returnvalue)
                  (:then
                    (bind _output_get (Variables|Default|SetStack (.Stack (Utilities|Struct|BreakST_Consumable _returnvalue_3))))))))
            (if (and (Utilities|Enum|Equal(Enum) (.ID (Utilities|Struct|BreakST_ItemTemplate (.ItemTemplate (Utilities|Struct|BreakST_Item _array_element)))) _id) (< (.Count (Utilities|Struct|BreakST_Item _array_element)) _output_get))
              (LocalVariables|SetL_TargetSlot _array_index)))
          (if (< (LocalVariables|GetL_TargetSlot) 0)
            (LocalVariables|SetL_TargetSlot (CallFunction|GetFirstEmptySlot To))))
        (:then_1
          ;[1 1 1] Кол-во предметов, которые мы можем переместить
          (if (> (Variables|Default|GetAmount) _count)
            (LocalVariables|SetL_Count _count)
            (else
              (bind _output_get_2 (LocalVariables|SetL_Count (Variables|Default|GetAmount)))))
          (if (not (Utilities|Array|IsEmpty (.ID (Utilities|Struct|BreakST_ItemTemplate (.ItemTemplate (Utilities|Struct|BreakST_Item (Utilities|Array|Get(acopy) To (LocalVariables|GetL_TargetSlot))))))))
            (if (not (< _output_get_2 (- (Variables|Default|GetStack) (.Count (Utilities|Struct|BreakST_Item (Utilities|Array|Get(acopy) To (LocalVariables|GetL_TargetSlot)))))))
              (LocalVariables|Setreminder (- (LocalVariables|GetL_Count) (- (Variables|Default|GetStack) (.Count (Utilities|Struct|BreakST_Item (Utilities|Array|Get(acopy) To (LocalVariables|GetL_TargetSlot)))))))
              (LocalVariables|SetL_Count (- (Variables|Default|GetStack) (.Count (Utilities|Struct|BreakST_Item (Utilities|Array|Get(acopy) To (LocalVariables|GetL_TargetSlot)))))))))
        (:then_2
          ;[1 1 1] Добавление предмета в целевой слот
          (Utilities|Array|SetArrayElem To (LocalVariables|GetL_TargetSlot) (Utilities|Struct|MakeST_Item (.ItemTemplate (Utilities|Struct|BreakST_Item (Utilities|Array|Get(acopy) From Index))) (+ (.Count (Utilities|Struct|BreakST_Item (Utilities|Array|Get(acopy) To (LocalVariables|GetL_TargetSlot)))) (LocalVariables|GetL_Count)))))
        (:then_3
          ;[1 1 1] Удаление предметов
          (Utilities|Array|SetArrayElem From Index (Utilities|Struct|MakeST_Item _itemtemplate_2 (- _count_2 (LocalVariables|GetL_Count))))
          (if (== (.Count (Utilities|Struct|BreakST_Item (Utilities|Array|Get(acopy) From Index))) 0)
            (CallFunction|RemoveItemfromInventory Index From)))
        (:then_4
          (CallFunction|UpdateAllWidgets)
          (Audio|SpawnSound2D "/Engine/VREditor/Sounds/UI/Gizmo_Handle_Clicked.Gizmo_Handle_Clicked" 1.0 1.0 0.0 0))))))

(fn UpdateAllWidgets
  (bind _hangarwidget_reference (Variables|Default|GetHangarWidget_reference))
  (Default|UpdateHangarStorage (Variables|/Game/Ironsphere/UI/Hangar/WBC_Hangar.WBC_Hangar_C|GetWBC_HangarStorage _hangarwidget_reference))
  (Default|UpdateMechInventory (Variables|/Game/Ironsphere/UI/Hangar/WBC_Hangar.WBC_Hangar_C|GetWBC_Consumable _hangarwidget_reference))
  (Default|UpdateMechInventory (Variables|/Game/Ironsphere/UI/Hangar/WBC_Hangar.WBC_Hangar_C|GetWBC_Gear _hangarwidget_reference))
  (Default|UpdateMechInventory (Variables|/Game/Ironsphere/UI/Hangar/WBC_Hangar.WBC_Hangar_C|GetWBC_Devices _hangarwidget_reference))
  (Default|UpdateMechInventory (Variables|/Game/Ironsphere/UI/Hangar/WBC_Hangar.WBC_Hangar_C|GetWBC_Armor _hangarwidget_reference))
  (Default|UpdateMechInventory (Variables|/Game/Ironsphere/UI/Hangar/WBC_Hangar.WBC_Hangar_C|GetWBC_WeaponArm _hangarwidget_reference))
  (Default|UpdateMechInventory (Variables|/Game/Ironsphere/UI/Hangar/WBC_Hangar.WBC_Hangar_C|GetWBC_SelectedMech _hangarwidget_reference))
  (Default|UpdateMechInventory (Variables|/Game/Ironsphere/UI/Hangar/WBC_Hangar.WBC_Hangar_C|GetWBC_WeaponBoarding _hangarwidget_reference))
  (Default|UpdateMechParameters (Variables|Default|GetGI_Main_ref))
  (Default|ShowMechParameters (Variables|/Game/Ironsphere/UI/Hangar/WBC_Hangar.WBC_Hangar_C|GetWBC_HangarMech (Variables|Default|GetHangarWidget_reference))))

(fn LoadGame
  (bind _savegame_ref (Variables|Default|GetSaveGame_ref))
  (bind _gi_main_ref (Variables|Default|GetGI_Main_ref))
  (Audio|SpawnSound2D "/Engine/VREditor/Sounds/UI/Dockable_Window_Pick_Up.Dockable_Window_Pick_Up" 1.0 1.0 0.0 0)
  (SaveGame|LoadGamefromSlot "1")
  (Variables|/Game/Ironsphere/Core/Framework/GI_Main.GI_Main_C|SetProgress _gi_main_ref (Variables|/Game/Ironsphere/Core/SaveGame/BP_SaveGame.BP_SaveGame_C|GetProgressSave _savegame_ref))
  (Variables|/Game/Ironsphere/Core/Framework/GI_Main.GI_Main_C|SetPlayTime _gi_main_ref (Variables|/Game/Ironsphere/Core/SaveGame/BP_SaveGame.BP_SaveGame_C|GetPlayTimeSave _savegame_ref))
  (Variables|/Game/Ironsphere/Core/Framework/GI_Main.GI_Main_C|SetMoney _gi_main_ref (Variables|/Game/Ironsphere/Core/SaveGame/BP_SaveGame.BP_SaveGame_C|GetMoneySave _savegame_ref))
  (Variables|/Game/Ironsphere/Core/Framework/GI_Main.GI_Main_C|SetHangarItems _gi_main_ref (Variables|/Game/Ironsphere/Core/SaveGame/BP_SaveGame.BP_SaveGame_C|GetHangarItems _savegame_ref))
  (Variables|/Game/Ironsphere/Core/Framework/GI_Main.GI_Main_C|SetMech _gi_main_ref (Variables|/Game/Ironsphere/Core/SaveGame/BP_SaveGame.BP_SaveGame_C|GetMech _savegame_ref))
  (Variables|/Game/Ironsphere/Core/Framework/GI_Main.GI_Main_C|SetWeaponArm _gi_main_ref (Variables|/Game/Ironsphere/Core/SaveGame/BP_SaveGame.BP_SaveGame_C|GetWeaponArm _savegame_ref))
  (Variables|/Game/Ironsphere/Core/Framework/GI_Main.GI_Main_C|SetWeaponOnboard _gi_main_ref (Variables|/Game/Ironsphere/Core/SaveGame/BP_SaveGame.BP_SaveGame_C|GetWeaponOnboard _savegame_ref))
  (Variables|/Game/Ironsphere/Core/Framework/GI_Main.GI_Main_C|SetDevices _gi_main_ref (Variables|/Game/Ironsphere/Core/SaveGame/BP_SaveGame.BP_SaveGame_C|GetDevices _savegame_ref))
  (Variables|/Game/Ironsphere/Core/Framework/GI_Main.GI_Main_C|SetGear _gi_main_ref (Variables|/Game/Ironsphere/Core/SaveGame/BP_SaveGame.BP_SaveGame_C|GetGear _savegame_ref))
  (Variables|/Game/Ironsphere/Core/Framework/GI_Main.GI_Main_C|SetConsumable _gi_main_ref (Variables|/Game/Ironsphere/Core/SaveGame/BP_SaveGame.BP_SaveGame_C|GetConsumable _savegame_ref))
  (Variables|/Game/Ironsphere/Core/Framework/GI_Main.GI_Main_C|SetArmor _gi_main_ref (Variables|/Game/Ironsphere/Core/SaveGame/BP_SaveGame.BP_SaveGame_C|GetArmor _savegame_ref))
  (CallFunction|UpdateAllWidgets))

(fn SaveGame
  (bind _gi_main_ref (Variables|Default|GetGI_Main_ref))
  (bind _savegame_ref (Variables|Default|GetSaveGame_ref))
  (Audio|SpawnSound2D "/Engine/VREditor/Sounds/UI/Drop_Item_From_ContentBrowser.Drop_Item_From_ContentBrowser" 1.0 1.0 0.0 0)
  (Variables|/Game/Ironsphere/Core/SaveGame/BP_SaveGame.BP_SaveGame_C|SetMoneySave _savegame_ref (Variables|/Game/Ironsphere/Core/Framework/GI_Main.GI_Main_C|GetMoney _gi_main_ref))
  (Variables|/Game/Ironsphere/Core/SaveGame/BP_SaveGame.BP_SaveGame_C|SetProgressSave _savegame_ref (Variables|/Game/Ironsphere/Core/Framework/GI_Main.GI_Main_C|GetProgress _gi_main_ref))
  (Variables|/Game/Ironsphere/Core/SaveGame/BP_SaveGame.BP_SaveGame_C|SetMech _savegame_ref (Variables|/Game/Ironsphere/Core/Framework/GI_Main.GI_Main_C|GetMech _gi_main_ref))
  (Variables|/Game/Ironsphere/Core/SaveGame/BP_SaveGame.BP_SaveGame_C|SetHangarItems _savegame_ref (Variables|/Game/Ironsphere/Core/Framework/GI_Main.GI_Main_C|GetHangarItems _gi_main_ref))
  (Variables|/Game/Ironsphere/Core/SaveGame/BP_SaveGame.BP_SaveGame_C|SetWeaponArm _savegame_ref (Variables|/Game/Ironsphere/Core/Framework/GI_Main.GI_Main_C|GetWeaponArm _gi_main_ref))
  (Variables|/Game/Ironsphere/Core/SaveGame/BP_SaveGame.BP_SaveGame_C|SetWeaponOnboard _savegame_ref (Variables|/Game/Ironsphere/Core/Framework/GI_Main.GI_Main_C|GetWeaponOnboard _gi_main_ref))
  (Variables|/Game/Ironsphere/Core/SaveGame/BP_SaveGame.BP_SaveGame_C|SetDevices _savegame_ref (Variables|/Game/Ironsphere/Core/Framework/GI_Main.GI_Main_C|GetDevices _gi_main_ref))
  (Variables|/Game/Ironsphere/Core/SaveGame/BP_SaveGame.BP_SaveGame_C|SetGear _savegame_ref (Variables|/Game/Ironsphere/Core/Framework/GI_Main.GI_Main_C|GetGear _gi_main_ref))
  (Variables|/Game/Ironsphere/Core/SaveGame/BP_SaveGame.BP_SaveGame_C|SetConsumable _savegame_ref (Variables|/Game/Ironsphere/Core/Framework/GI_Main.GI_Main_C|GetConsumable _gi_main_ref))
  (Variables|/Game/Ironsphere/Core/SaveGame/BP_SaveGame.BP_SaveGame_C|SetArmor _savegame_ref (Variables|/Game/Ironsphere/Core/Framework/GI_Main.GI_Main_C|GetArmor _gi_main_ref))
  (Variables|/Game/Ironsphere/Core/SaveGame/BP_SaveGame.BP_SaveGame_C|SetPlayTimeSave _savegame_ref (Variables|/Game/Ironsphere/Core/Framework/GI_Main.GI_Main_C|GetPlayTime _gi_main_ref))
  (SaveGame|SaveGametoSlot _savegame_ref "1"))

(fn NewGame
  (bind _gi_main_ref (Variables|Default|GetGI_Main_ref))
  (bind _gi_main_ref_2 (Variables|Default|GetGI_Main_ref))
  (bind _gi_main_ref_3 (Variables|Default|GetGI_Main_ref))
  (bind _gi_main_ref_4 (Variables|Default|GetGI_Main_ref))
  (bind _progress (Variables|/Game/Ironsphere/Core/Framework/GI_Main.GI_Main_C|GetProgress _gi_main_ref_3))
  (bind _weaponarm (Variables|/Game/Ironsphere/Core/Framework/GI_Main.GI_Main_C|GetWeaponArm _gi_main_ref_4))
  (Utilities|FlowControl|Sequence
    (:then_0
      (SaveGame|LoadGamefromSlot "1")
      (for (_ _array_index) _progress
        (Utilities|Array|SetArrayElem _progress _array_index (Utilities|Struct|MakeST_Progress false false))
        (Utilities|Array|SetArrayElem _progress 0 (Utilities|Struct|MakeST_Progress true false)))
      (Variables|/Game/Ironsphere/Core/Framework/GI_Main.GI_Main_C|SetPlayTime _gi_main_ref 0.0)
      (Variables|/Game/Ironsphere/Core/Framework/GI_Main.GI_Main_C|SetMoney _gi_main_ref 1e+02)
      (CallFunction|ClearInventory (Variables|/Game/Ironsphere/Core/Framework/GI_Main.GI_Main_C|GetHangarItems _gi_main_ref_2) "NewEnumerator7")
      (CallFunction|ClearInventory (Variables|/Game/Ironsphere/Core/Framework/GI_Main.GI_Main_C|GetMech _gi_main_ref_2) "NewEnumerator7")
      (CallFunction|ClearInventory (Variables|/Game/Ironsphere/Core/Framework/GI_Main.GI_Main_C|GetWeaponArm _gi_main_ref_2) "NewEnumerator7")
      (CallFunction|ClearInventory (Variables|/Game/Ironsphere/Core/Framework/GI_Main.GI_Main_C|GetWeaponOnboard _gi_main_ref_2) "NewEnumerator7")
      (CallFunction|ClearInventory (Variables|/Game/Ironsphere/Core/Framework/GI_Main.GI_Main_C|GetDevices _gi_main_ref_2) "NewEnumerator7")
      (CallFunction|ClearInventory (Variables|/Game/Ironsphere/Core/Framework/GI_Main.GI_Main_C|GetGear _gi_main_ref_2) "NewEnumerator7")
      (CallFunction|ClearInventory (Variables|/Game/Ironsphere/Core/Framework/GI_Main.GI_Main_C|GetConsumable _gi_main_ref_2) "NewEnumerator7")
      (CallFunction|ClearInventory (Variables|/Game/Ironsphere/Core/Framework/GI_Main.GI_Main_C|GetArmor _gi_main_ref_2) "NewEnumerator7"))
    (:then_1
      (Utilities|Array|SetArrayElem (Variables|/Game/Ironsphere/Core/Framework/GI_Main.GI_Main_C|GetMech _gi_main_ref_4) 0 (Utilities|Struct|MakeST_Item (Utilities|Struct|MakeST_ItemTemplate "Mech_S_T1_Crow" "NewEnumerator1" "None") 1))
      (Utilities|Array|SetArrayElem _weaponarm 0 (Utilities|Struct|MakeST_Item (Utilities|Struct|MakeST_ItemTemplate "Wpn_L_Engraver" "NewEnumerator0" "None") 1))
      (Utilities|Array|SetArrayElem _weaponarm 1 (Utilities|Struct|MakeST_Item (Utilities|Struct|MakeST_ItemTemplate "Wpn_B_HandRooster" "NewEnumerator0" "None") 1))
      (Utilities|Array|SetArrayElem (Variables|/Game/Ironsphere/Core/Framework/GI_Main.GI_Main_C|GetConsumable _gi_main_ref_4) 0 (Utilities|Struct|MakeST_Item (Utilities|Struct|MakeST_ItemTemplate "Cns_B_15mmShell" "NewEnumerator2" "None") 200))
      (CallFunction|UpdateAllWidgets))
    (:then_2
      (Default|AddItemstoShop (Variables|Default|GetGI_Main_ref)))))

(fn ClearInventory
  (params (Inventory :type Array%20of%20ST%20Item%20Structures) (Type :type SlotType%20Enum :default "NewEnumerator1"))
  (for (_ _array_index) Inventory
    (Utilities|Array|SetArrayElem Inventory _array_index (Utilities|Struct|MakeST_Item (Utilities|Struct|MakeST_ItemTemplate "" Type "None")))))