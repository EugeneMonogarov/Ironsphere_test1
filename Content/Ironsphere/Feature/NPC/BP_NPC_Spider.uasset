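; Spider NPC Blueprint that tracks enemies, passes damage to its parent class and refreshes its health bar widget every tick.
; The enemy list starts with the player's controlled mech, and the detection sensor adds any other pawns it overlaps.
; The attack range volume toggles TargetInRange on the AI controller, only for the first listed enemy.
; NPC_Shot plays just a sound when melee, otherwise drives the weapon; weapon init is empty.
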(event OnComponentBeginOverlap(sensorDetect)
  (params (OverlappedComponent :type Primitive%20Component%20Object%20Reference) (OtherActor :type Actor%20Object%20Reference) (OtherComp :type Primitive%20Component%20Object%20Reference) (OtherBodyIndex :type Integer) (bFromSweep :type Boolean) (SweepResult :type Hit%20Result%20Structure%20%28by%20ref%29))
  (bind _aspawn (Utilities|Casting|CastToPawn OtherActor))
  (if (!= OtherActor self)
    (Utilities|Array|AddUnique (Variables|Default|GetEnemy) _aspawn)))

(event OnComponentEndOverlap(sensorDetect)
  (params (OverlappedComponent :type Primitive%20Component%20Object%20Reference) (OtherActor :type Actor%20Object%20Reference) (OtherComp :type Primitive%20Component%20Object%20Reference) (OtherBodyIndex :type Integer)))

(event OnComponentBeginOverlap(AttackRange)
  (params (OverlappedComponent :type Primitive%20Component%20Object%20Reference) (OtherActor :type Actor%20Object%20Reference) (OtherComp :type Primitive%20Component%20Object%20Reference) (OtherBodyIndex :type Integer) (bFromSweep :type Boolean) (SweepResult :type Hit%20Result%20Structure%20%28by%20ref%29))
  (if (!= OtherActor self)
    (if (== OtherActor (Utilities|Array|Get(acopy) (Variables|Default|GetEnemy)))
      (bind _asbp_aicontroller_old (Utilities|Casting|CastToBP_AIController_Old (AI|GetAIController self)))
      (Variables|/Game/Ironsphere/Feature/NPC/BP_AIController_Old.BP_AIController_Old_C|SetTargetInRange _asbp_aicontroller_old true))))

(event OnComponentEndOverlap(AttackRange)
  (params (OverlappedComponent :type Primitive%20Component%20Object%20Reference) (OtherActor :type Actor%20Object%20Reference) (OtherComp :type Primitive%20Component%20Object%20Reference) (OtherBodyIndex :type Integer))
  (if (!= OtherActor self)
    (if (== OtherActor (Utilities|Array|Get(acopy) (Variables|Default|GetEnemy)))
      (bind _asbp_aicontroller_old (Utilities|Casting|CastToBP_AIController_Old (AI|GetAIController self)))
      (Variables|/Game/Ironsphere/Feature/NPC/BP_AIController_Old.BP_AIController_Old_C|SetTargetInRange _asbp_aicontroller_old false))))

(event EventBeginPlay
  (bind _asbp_player_controller (Utilities|Casting|CastToBP_PlayerController (Game|GetPlayerController 0)))
  (Variables|Default|SetEnemy (Utilities|Array|MakeArray (Variables|/Game/Ironsphere/Core/Player/BP_PlayerController.BP_PlayerController_C|GetControlledMech _asbp_player_controller))))

(event Collision|EventActorBeginOverlap
  (params (OtherActor :type Actor%20Object%20Reference)))

(event EventTick
  (params (DeltaSeconds :type Float%20%28single-precision%29))
  (bind _aswbc_hehth_bar (Utilities|Casting|CastToWBC_HehthBar (UserInterface|GetWidget (Variables|Default|Getwidget_HPbar))))
  (Default|UpdateHP _aswbc_hehth_bar (/ (Variables|Default|GetCurrentHP) (Variables|Default|GetMaxHP))))

(event Game|Damage|EventAnyDamage
  (params (Damage :type Float%20%28single-precision%29) (DamageType :type Damage%20Type%20Object%20Reference) (InstigatedBy :type Controller%20Object%20Reference) (DamageCauser :type Actor%20Object%20Reference))
  (|CallParentFunction Damage DamageType InstigatedBy DamageCauser))

(fn ConstructionScript)

(fn InitNPCWeapon)

(fn NPCShot
  (params (Active :type Boolean))
  (if (Variables|Default|GetIsMelee)
    (Audio|SpawnSoundatLocation "/Engine/VREditor/Sounds/VR_grab.VR_grab" (Transformation|GetActorLocation) "0, 0, 0" 1.0 1.0 0.0 0 0)
    (else
      (Default|WeaponShot (Variables|Default|GetWeaponNPCReference) Active))))