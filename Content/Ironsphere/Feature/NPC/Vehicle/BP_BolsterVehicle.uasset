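; BP_BolsterVehicle is a vehicle NPC that sets up its parameters from the NPC_BolsterVehicle ID on BeginPlay.
; Its shot alternates between two weapon arrows, firing a shotgun-style volley with accuracy-based yaw spread, randomized speed and range, and divided damage.
; Death passes a spider death montage to the parent, while leftover logic flagging a mission boss kill is never executed.
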(event EventBeginPlay
  (|CallParentFunction)
  (CallFunction|SetNPCParameters "NPC_BolsterVehicle" (Variables|Default|GetScaleFactor)))

(event Collision|EventActorBeginOverlap
  (params (OtherActor :type Actor%20Object%20Reference))
  (|CallParentFunction OtherActor) ; This node is disabled and will not be called.\nDrag off pins to build functionality.
)

(event EventTick
  (params (DeltaSeconds :type Float%20%28single-precision%29))
  (|CallParentFunction DeltaSeconds) ; This node is disabled and will not be called.\nDrag off pins to build functionality.
)

(fn ConstructionScript
  (|CallParentFunction))

(fn SetNPCParameters
  (params (ID :type Name :default "None") (ScaleFactor :type Float%20%28double-precision%29))
  (|CallParentFunction ID ScaleFactor))

(fn Death
  (params (DeathAnim :type Anim%20Montage%20Object%20Reference))
  (|CallParentFunction "/Game/Ironsphere/3D/Animations/Spider/SpiderDeath_Montage.SpiderDeath_Montage"))

(fn NPCShot
  (bind _returnvalue (Math|Random|RandomFloatinRange 0.8 1.2))
  (bind _npcaccuracy (Variables|Default|GetNPCAccuracy))
  (bind _returnvalue_2 (- 1.0 _npcaccuracy))
  (bind _returnvalue_3 (* _returnvalue_2 45.0))
  (Audio|SpawnSoundatLocation "/Game/Ironsphere/Sound/Step/shot_3.shot_3" (Transformation|GetActorLocation self) "0, 0, 0" 0.5 1.0 0.0 0 0)
  (if (Variables|Default|GetDoubleWeaponToggle)
    (Variables|Default|SetBulletSpawnTransform (Transformation|GetWorldTransform (Variables|Default|GetWeaponArrow)))
    (Variables|Default|SetDoubleWeaponToggle false)
    (else
      (Variables|Default|SetBulletSpawnTransform (Transformation|GetWorldTransform (Variables|Default|GetWeaponArrowSecond)))
      (Variables|Default|SetDoubleWeaponToggle true)))
  (for _index (range 0 8)
    (Game|SpawnActorfromClass :Class (Variables|Default|GetProjectile) :SpawnTransform (Math|Transform|MakeTransform (.Location (Math|Transform|BreakTransform (Variables|Default|GetBulletSpawnTransform))) (Math|Rotator|MakeRotator (.Roll (Math|Rotator|BreakRotator (.Rotation (Math|Transform|BreakTransform (Variables|Default|GetBulletSpawnTransform))))) (.Pitch (Math|Rotator|BreakRotator (.Rotation (Math|Transform|BreakTransform (Variables|Default|GetBulletSpawnTransform))))) (+ (.Yaw (Math|Rotator|BreakRotator (.Rotation (Math|Transform|BreakTransform (Variables|Default|GetBulletSpawnTransform))))) (Math|Random|RandomFloatinRange (* _returnvalue_3 -1.0) _returnvalue_3))) (.Scale (Math|Transform|BreakTransform (Variables|Default|GetBulletSpawnTransform)))) :CollisionHandlingOverride "AlwaysSpawn" :TransformScaleMethod "MultiplyWithRoot" :Owner self :ProjectileVelocity (* (Variables|Default|GetProjectileVelocity) _returnvalue) :ProjectileRange (* (Variables|Default|GetAttackRange) _returnvalue) :ProjectileDamage (/ (Variables|Default|GetDamage) 8.0) :ProjectileArmorPenetration (Variables|Default|GetNPCArmorPenetration) :Instigator self)))