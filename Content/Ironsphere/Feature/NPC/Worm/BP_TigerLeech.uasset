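; Tiger Leech NPC Blueprint in the Worm feature, a thin child class that relies on its parent for NPC behavior.
; On BeginPlay it registers the NPC_TigerLeech ID with a slightly randomized scale factor through SetNPCParameters.
; Shot and parameter overrides just call the parent, while Death always passes the worm death montage instead of the incoming animation.
; A custom event plays a supplied montage on the skeletal mesh.
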(event Custom|CustomEvent
  (params (AnimMontage :type Anim%20Montage%20Object%20Reference))
  (Animation|Montage|PlayMontage (Variables|Default|GetSkeletalMesh) AnimMontage))

(event EventBeginPlay
  (|CallParentFunction)
  (CallFunction|SetNPCParameters "NPC_TigerLeech" (Math|Random|RandomFloatinRange 0.9 1.1)))

(event Collision|EventActorBeginOverlap
  (params (OtherActor :type Actor%20Object%20Reference))
  (|CallParentFunction OtherActor) ; This node is disabled and will not be called.\nDrag off pins to build functionality.
)

(event EventTick
  (params (DeltaSeconds :type Float%20%28single-precision%29))
  (|CallParentFunction DeltaSeconds) ; This node is disabled and will not be called.\nDrag off pins to build functionality.
)

(fn ConstructionScript
  (|CallParentFunction))

(fn NPCShot
  (|CallParentFunction))

(fn SetNPCParameters
  (params (ID :type Name :default "None") (ScaleFactor :type Float%20%28double-precision%29))
  (|CallParentFunction ID ScaleFactor))

(fn Death
  (params (DeathAnim :type Anim%20Montage%20Object%20Reference))
  (|CallParentFunction "/Game/Ironsphere/3D/Animations/Worm/WormDeathMontage.WormDeathMontage"))