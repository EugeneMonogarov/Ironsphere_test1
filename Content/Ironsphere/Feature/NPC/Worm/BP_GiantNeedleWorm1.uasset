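; Giant needle worm boss NPC that reports its kill to the BP_MissionBoss5_1_ mission actor.
; BeginPlay loads its NPC parameters and attaches an objective arrow to the player's mech, pointing to the worm.
; The NPCShot override deals typed melee damage or fires three spike projectiles with randomized yaw, speed, range and damage, plus random sounds.
; Death sets BossKilled and calls parent death twice, with worm then spider montages.
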(event Custom|CustomEvent
  (params (AnimMontage :type Anim%20Montage%20Object%20Reference))
  (Animation|Montage|PlayMontage (Variables|Default|GetSkeletalMesh) AnimMontage))

(event EventBeginPlay
  (|CallParentFunction)
  (bind _asgi_main (Utilities|Casting|CastToGI_Main (Game|GetGameInstance)))
  (CallFunction|SetNPCParameters "NPC_GiantNeddleWorm" 1.2)
  (bind _aspc_ingame (Utilities|Casting|CastToPC_Ingame (Game|GetPlayerController 0)))
  (bind _returnvalue (Game|SpawnActorfromClass "/Game/Ironsphere/Core/Player/BP_ObjectiveArrow.BP_ObjectiveArrow_C" (Math|Transform|MakeTransform "0, 0, 0") "Undefined" "MultiplyWithRoot" (Variables|/Game/Ironsphere/Core/Framework/Battle/PC_Ingame.PC_Ingame_C|GetControlledMech _aspc_ingame) self 0))
  (Transformation|AttachActorToActor _returnvalue (Variables|/Game/Ironsphere/Core/Framework/Battle/PC_Ingame.PC_Ingame_C|GetControlledMech _aspc_ingame) "None" "KeepRelative" "KeepRelative" "KeepRelative" true))

(event Collision|EventActorBeginOverlap
  (params (OtherActor :type Actor%20Object%20Reference))
  (|CallParentFunction OtherActor) ; This node is disabled and will not be called.\nDrag off pins to build functionality.
)

(event EventTick
  (params (DeltaSeconds :type Float%20%28single-precision%29))
  (|CallParentFunction DeltaSeconds) ; This node is disabled and will not be called.\nDrag off pins to build functionality.
)

(fn ConstructionScript
  (|CallParentFunction))

(fn NPCShot
  (bind _returnvalue (Transformation|GetActorLocation))
  (bind _returnvalue_2 (Math|Random|RandomFloatinRange 0.75 1.0))
  (bind _returnvalue_3 (Math|Random|RandomFloatinRange 0.5 1.5))
  (bind _returnvalue_4 (Math|Random|RandomFloatinRange 0.1 0.8))
  (bind _returnvalue_5 (Transformation|GetActorTransform))
  (bind _returnvalue_6 (Transformation|GetActorLocation))
  (bind _returnvalue_7 (Math|Random|RandomFloatinRange 0.8 1.2))
  (bind _damage (Variables|Default|GetDamage))
  (bind (_location _rotation) (Math|Transform|BreakTransform _returnvalue_5))
  (bind (_roll _pitch _yaw) (Math|Rotator|BreakRotator _rotation))
  (Utilities|FlowControl|Sequence
    (:then_0
      (if (Variables|Default|GetAlive)
        (if (Variables|Default|GetMelee)
          (switch Utilities|FlowControl|Switch|SwitchonE_DamageTypes (Variables|Default|GetDamageType)
            (:NewEnumerator0
              (Game|Damage|ApplyDamage (Utilities|Array|Get(acopy) (Variables|Default|GetEnemy)) _damage 0 self "/Game/Ironsphere/Feature/Consumable/DamageTypes/BP_PhysicalDamage.BP_PhysicalDamage_C"))
            (:NewEnumerator1
              (Game|Damage|ApplyDamage 0 _damage 0 0 "/Game/Ironsphere/Feature/Consumable/DamageTypes/BP_LaserDamage.BP_LaserDamage_C"))
            (:NewEnumerator2
              (Game|Damage|ApplyDamage 0 0.0 0 0 "/Game/Ironsphere/Feature/Consumable/DamageTypes/BP_LaserDamage.BP_LaserDamage_C")))
          (else
            (Utilities|FlowControl|Sequence
              (:then_0
                _)
              (:then_1
                _)
              (:then_2
                _))
            (Game|SpawnActorfromClass :Class "/Game/Ironsphere/Feature/NPC/Ammo/Spikes.Spikes_C" :SpawnTransform (Math|Transform|MakeTransform _location (Math|Rotator|MakeRotator _roll _pitch (+ _yaw (Math|Random|RandomFloatinRange -3e+01 3e+01))) "2.000000,2.000000,2.000000") :CollisionHandlingOverride "AlwaysSpawn" :TransformScaleMethod "MultiplyWithRoot" :Owner self :ProjectileVelocity (* (Variables|Default|GetProjectileVelocity) _returnvalue_7) :ProjectileRange (* (Variables|Default|GetAttackRange) _returnvalue_7) :ProjectileDamage (* (Variables|Default|GetDamage) (Math|Random|RandomFloatinRange 0.8 1.2)) :ProjectileArmorPenetration (Variables|Default|GetNPCArmorPenetration) :Instigator self)))))
    (:then_1
      (switch int (Math|Random|RandomInteger 3)
        (:Default
          (Audio|SpawnSoundatLocation "/Game/Ironsphere/Sound/NPC/SpyderAttack3.SpyderAttack3" _returnvalue "0, 0, 0" 0.5 _returnvalue_2 0.0 0 0 :!label _label))
        (:0
          (Audio|SpawnSoundatLocation "/Game/Ironsphere/Sound/NPC/SpyderAttack1.SpyderAttack1" _returnvalue "0, 0, 0" 0.5 _returnvalue_2 0.0 0 0))
        (:1
          (Audio|SpawnSoundatLocation "/Game/Ironsphere/Sound/NPC/SpyderAttack2.SpyderAttack2" _returnvalue "0, 0, 0" 0.5 _returnvalue_2 0.0 0 0))
        (:2
          (goto _label)))
      (switch int (Math|Random|RandomInteger 3)
        (:0
          (Audio|SpawnSoundatLocation "/Game/Ironsphere/Sound/NPC/gui_006.gui_006" _returnvalue_6 "0, 0, 0" _returnvalue_4 _returnvalue_3 0.0 0 0))
        (:1
          (Audio|SpawnSoundatLocation "/Game/Ironsphere/Sound/NPC/gui_005.gui_005" _returnvalue_6 "0, 0, 0" _returnvalue_4 _returnvalue_3 0.0 0 0))))))

(fn SetNPCParameters
  (params (ID :type Name :default "None") (ScaleFactor :type Float%20%28double-precision%29))
  (|CallParentFunction ID ScaleFactor))

(fn Death
  (params (DeathAnim :type Anim%20Montage%20Object%20Reference))
  (|CallParentFunction "/Game/Ironsphere/3D/Animations/Worm/WormDeathMontage.WormDeathMontage")
  (bind _outactors (Actor|GetAllActorsOfClass "/Game/Ironsphere/Missions/Boss/BP_MissionBoss5_1_.BP_MissionBoss5_1__C"))
  (if (Utilities|IsValid (Utilities|Array|Get(acopy) _outactors))
    (Variables|/Game/Ironsphere/Missions/Boss/BP_MissionBoss5_1_.BP_MissionBoss5_1__C|SetBossKilled (Utilities|Array|Get(acopy) _outactors) true))
  (|CallParentFunction "/Game/Ironsphere/3D/Animations/Spider/SpiderDeath_Montage.SpiderDeath_Montage"))