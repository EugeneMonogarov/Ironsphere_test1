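; Giant laser spider NPC that extends a parent NPC class, adding minion spawning and a reactive shield.
; On Tick it periodically spawns a small spider droid, or less often a blow droid, at a random navigable point nearby.
; Taking damage can trigger a timed shield buff with sound, with odds rising with damage relative to max HP and gated by a cooldown.
; Death passes a spider-specific montage to the parent.
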(event EventBeginPlay
  (|CallParentFunction)
  (CallFunction|SetNPCParameters "NPC_GiantLaserSpider" 1.0))

(event Collision|EventActorBeginOverlap
  (params (OtherActor :type Actor%20Object%20Reference))
  (|CallParentFunction OtherActor) ; This node is disabled and will not be called.\nDrag off pins to build functionality.
)

(event EventTick
  (params (DeltaSeconds :type Float%20%28single-precision%29))
  (|CallParentFunction DeltaSeconds)
  (Utilities|FlowControl|Sequence
    (:then_0
      (if (> (Variables|Default|GetSpawnDroidCooldown) 0.0)
        (Variables|Default|SetSpawnDroidCooldown (- (Variables|Default|GetSpawnDroidCooldown) DeltaSeconds))
        (else
          (bind _randomlocation (Class|NavigationSystemV1|GetRandomLocationinNavigableRadius (Transformation|GetActorLocation) 2e+02 0 0))
          (if (== (Math|Random|RandomIntegerinRange 1 3) 3)
            (bind _returnvalue (AI|SpawnAIFromClass "/Game/Ironsphere/Feature/NPC/SpiderDroid/BP_SmallBlowDroid.BP_SmallBlowDroid_C" 0 _randomlocation "0, 0, 0" false 0))
            (if (Utilities|IsValid _returnvalue)
              (Variables|Default|SetSpawnDroidCooldown 1e+01))
            (else
              (bind _returnvalue_2 (AI|SpawnAIFromClass "/Game/Ironsphere/Feature/NPC/SpiderDroid/BP_SmallSpiderDroid.BP_SmallSpiderDroid_C" 0 _randomlocation "0, 0, 0" false 0))
              (if (Utilities|IsValid _returnvalue_2)
                (Variables|Default|SetSpawnDroidCooldown 1e+01)))))))
    (:then_1
      (if (> (Variables|Default|GetSpawnShieldCooldown) 0.0)
        (Variables|Default|SetSpawnShieldCooldown (- (Variables|Default|GetSpawnShieldCooldown) DeltaSeconds))))))

(event Game|Damage|EventAnyDamage
  (params (Damage :type Float%20%28single-precision%29) (DamageType :type Damage%20Type%20Object%20Reference) (InstigatedBy :type Controller%20Object%20Reference) (DamageCauser :type Actor%20Object%20Reference))
  (|CallParentFunction Damage DamageType InstigatedBy DamageCauser)
  (if (and (> (* Damage 15.0) (Math|Random|RandomFloatinRange 0.0 (Variables|Default|GetMaxHP))) (<= (Variables|Default|GetSpawnShieldCooldown) 0.0))
    (CallFunction|AddBuff (Utilities|Struct|MakeST_buff "NewEnumerator4" 8e+01 7.0 false "DarkWidowShield" 0))
    (Variables|Default|SetCurrentShield 8e+01)
    (Audio|SpawnSoundatLocation "/Game/Ironsphere/Sound/Devices/shield_boost.shield_boost" (Transformation|GetActorLocation) "0, 0, 0" 0.15 1.0 0.0 0 0)
    (Variables|Default|SetSpawnShieldCooldown 15.0)))

(fn ConstructionScript
  (|CallParentFunction))

(fn SetNPCParameters
  (params (ID :type Name :default "None") (ScaleFactor :type Float%20%28double-precision%29))
  (|CallParentFunction ID ScaleFactor))

(fn Death
  (params (DeathAnim :type Anim%20Montage%20Object%20Reference))
  (|CallParentFunction "/Game/Ironsphere/3D/Animations/Spider/SpiderDeath_Montage.SpiderDeath_Montage"))

(fn NPCShot
  (|CallParentFunction))