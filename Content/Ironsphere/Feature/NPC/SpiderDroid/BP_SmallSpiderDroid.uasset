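; BP_SmallSpiderDroid is the small spider droid NPC, built as a thin child of a parent NPC Blueprint.
; On BeginPlay it runs the parent logic, then sets its NPC parameters using its own ID and an unscaled size factor.
; Death overrides the supplied animation with the spider death montage, while parameter setup and shooting pass straight through to the parent.
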(event EventBeginPlay
  (|CallParentFunction)
  (CallFunction|SetNPCParameters "NPC_SmallSpiderDroid" 1.0))

(event Collision|EventActorBeginOverlap
  (params (OtherActor :type Actor%20Object%20Reference))
  (|CallParentFunction OtherActor) ; This node is disabled and will not be called.\nDrag off pins to build functionality.
)

(event EventTick
  (params (DeltaSeconds :type Float%20%28single-precision%29))
  (|CallParentFunction DeltaSeconds) ; This node is disabled and will not be called.\nDrag off pins to build functionality.
)

(fn ConstructionScript
  (|CallParentFunction))

(fn SetNPCParameters
  (params (ID :type Name :default "None") (ScaleFactor :type Float%20%28double-precision%29))
  (|CallParentFunction ID ScaleFactor))

(fn Death
  (params (DeathAnim :type Anim%20Montage%20Object%20Reference))
  (|CallParentFunction "/Game/Ironsphere/3D/Animations/Spider/SpiderDeath_Montage.SpiderDeath_Montage"))

(fn NPCShot
  (|CallParentFunction))