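; Final boss spider droid NPC, scaled by difficulty, that marks its BP_MissionBoss20 mission as killed on death.
; Incoming damage can trigger a temporary shield boost, more likely for bigger hits relative to max HP and gated by a cooldown.
; Tick periodically spawns small blow or spider droids nearby and grants speed bursts when its first enemy is out of close range.
; Shots extend the parent attack with an occasional Chimera explosive missile.
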(event EventBeginPlay
  (|CallParentFunction)
  (CallFunction|SetNPCParameters "NPC_FinalBoss" (+ 0.9 (* (Variables|/Game/Ironsphere/Core/Framework/GI_Main.GI_Main_C|GetDifficultyLevel (Variables|Default|GetGI_Main_ref)) 0.1))))

(event Collision|EventActorBeginOverlap
  (params (OtherActor :type Actor%20Object%20Reference))
  (|CallParentFunction OtherActor) ; This node is disabled and will not be called.\nDrag off pins to build functionality.
)

(event EventTick
  (params (DeltaSeconds :type Float%20%28single-precision%29))
  (|CallParentFunction DeltaSeconds)
  (Utilities|FlowControl|Sequence
    (:then_0
      (if (> (Variables|Default|GetSpawnDroidCooldown) 0.0)
        (Variables|Default|SetSpawnDroidCooldown (- (Variables|Default|GetSpawnDroidCooldown) DeltaSeconds))
        (else
          (bind _randomlocation (Class|NavigationSystemV1|GetRandomLocationinNavigableRadius (Transformation|GetActorLocation) 2e+02 0 0))
          (if (== (Math|Random|RandomIntegerinRange 1 3) 3)
            (bind _returnvalue (AI|SpawnAIFromClass "/Game/Ironsphere/Feature/NPC/SpiderDroid/BP_SmallBlowDroid.BP_SmallBlowDroid_C" 0 (Math|Vector|MakeVector (.X (Math|Vector|BreakVector _randomlocation)) (.Y (Math|Vector|BreakVector _randomlocation)) 122.0) "0, 0, 0" false 0))
            (if (Utilities|IsValid _returnvalue)
              (Variables|Default|SetSpawnDroidCooldown 9.0))
            (else
              (bind _returnvalue_2 (AI|SpawnAIFromClass "/Game/Ironsphere/Feature/NPC/SpiderDroid/BP_SmallSpiderDroid.BP_SmallSpiderDroid_C" 0 (Math|Vector|MakeVector (.X (Math|Vector|BreakVector _randomlocation)) (.Y (Math|Vector|BreakVector _randomlocation)) 122.0) "0, 0, 0" false 0))
              (if (Utilities|IsValid _returnvalue_2)
                (Variables|Default|SetSpawnDroidCooldown 9.0)))))))
    (:then_1
      (if (> (Variables|Default|GetSpawnShieldCooldown) 0.0)
        (Variables|Default|SetSpawnShieldCooldown (- (Variables|Default|GetSpawnShieldCooldown) DeltaSeconds))))
    (:then_2
      (Variables|Default|SetSpeedBuffCD (- (Variables|Default|GetSpeedBuffCD) DeltaSeconds))
      (if (and (<= (Variables|Default|GetSpeedBuffCD) 0.0) (> (Math|Vector|VectorLength (- (Transformation|GetActorLocation) (Transformation|GetActorLocation (Utilities|Array|Get(acopy) (Variables|Default|GetEnemy))))) 2.5e+02))
        (CallFunction|AddBuff (Utilities|Struct|MakeST_buff "NewEnumerator0" 0.3 2.0 false "None" 0))
        (Variables|Default|SetSpeedBuffCD 2.0)))))

(event Game|Damage|EventAnyDamage
  (params (Damage :type Float%20%28single-precision%29) (DamageType :type Damage%20Type%20Object%20Reference) (InstigatedBy :type Controller%20Object%20Reference) (DamageCauser :type Actor%20Object%20Reference))
  (|CallParentFunction Damage DamageType InstigatedBy DamageCauser)
  (if (and (> (* Damage 15.0) (Math|Random|RandomFloatinRange 0.0 (Variables|Default|GetMaxHP))) (<= (Variables|Default|GetSpawnShieldCooldown) 0.0))
    (CallFunction|AddBuff (Utilities|Struct|MakeST_buff "NewEnumerator4" 2.5e+02 1e+01 false "DarkWidowShield" 0))
    (Variables|Default|SetCurrentShield (+ (Variables|Default|GetCurrentShield) 2.5e+02))
    (Audio|SpawnSoundatLocation "/Game/Ironsphere/Sound/Devices/shield_boost.shield_boost" (Transformation|GetActorLocation) "0, 0, 0" 0.15 1.0 0.0 0 0)
    (Variables|Default|SetSpawnShieldCooldown 15.0)))

(fn ConstructionScript
  (|CallParentFunction))

(fn SetNPCParameters
  (params (ID :type Name :default "None") (ScaleFactor :type Float%20%28double-precision%29))
  (|CallParentFunction ID ScaleFactor))

(fn Death
  (params (DeathAnim :type Anim%20Montage%20Object%20Reference))
  (bind _outactors (Actor|GetAllActorsOfClass "/Game/Ironsphere/Missions/Boss/BP_MissionBoss20.BP_MissionBoss20_C"))
  (Variables|/Game/Ironsphere/Missions/Boss/BP_MissionBoss20.BP_MissionBoss20_C|SetBossKilled (Utilities|Array|Get(acopy) _outactors) true)
  (|CallParentFunction "/Game/Ironsphere/3D/Animations/Spider/SpiderDeath_Montage.SpiderDeath_Montage"))

(fn NPCShot
  (bind _self self)
  (bind _damage (Variables|Default|GetDamage))
  (bind _returnvalue (* _damage 5.0))
  (Utilities|FlowControl|Sequence
    (:then_1
      (|CallParentFunction)
      (switch int (Math|Random|RandomIntegerinRange 0 5)
        (:0
          (Game|SpawnActorfromClass :Class "/Game/Ironsphere/Feature/Consumable/Ammo/Chimera.Chimera_C" :SpawnTransform (Transformation|GetActorTransform _self) :CollisionHandlingOverride "AlwaysSpawn" :TransformScaleMethod "MultiplyWithRoot" :Owner _self :ProjectileVelocity 3e+02 :ProjectileRange (Variables|Default|GetAttackRange) :ProjectileDamage _returnvalue :ProjectileExplosionDamge (/ _returnvalue 2.0) :ProjectileExplosionRadius 5e+01 :ProjectileArmorPenetration 0.4 :MissileAccuracy 0.1 :Instigator _self)
          (Audio|PlaySound2D "/Game/Ironsphere/Sound/Shot/Missle1.Missle1" 1.0 1.0 0.0 0 0))))))