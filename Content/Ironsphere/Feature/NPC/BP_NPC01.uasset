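; BP_NPC01 is an armed NPC pawn that tracks enemies and fires a child-actor laser weapon through NPCShot.
; SensorIn overlaps and damage dealers add pawns to an Enemy list, and leaving SensorOut removes them after a random delay.
; AttackRange overlaps with the first enemy toggle TargetInRange on BP_AIController_Old.
; The health widget is only initialized, as health update, panic and explosion-death logic is disconnected.
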(event OnComponentBeginOverlap(sensorIn)
  (params (OverlappedComponent :type Primitive%20Component%20Object%20Reference) (OtherActor :type Actor%20Object%20Reference) (OtherComp :type Primitive%20Component%20Object%20Reference) (OtherBodyIndex :type Integer) (bFromSweep :type Boolean) (SweepResult :type Hit%20Result%20Structure%20%28by%20ref%29))
  (bind _aspawn (Utilities|Casting|CastToPawn OtherActor))
  (if (!= OtherActor self)
    (Utilities|Array|AddUnique (Variables|Default|GetEnemy) _aspawn)))

(event OnComponentEndOverlap(sensorOut)
  (params (OverlappedComponent :type Primitive%20Component%20Object%20Reference) (OtherActor :type Actor%20Object%20Reference) (OtherComp :type Primitive%20Component%20Object%20Reference) (OtherBodyIndex :type Integer))
  (bind _aspawn (Utilities|Casting|CastToPawn OtherActor)
    (:then
      (if (Utilities|Array|ContainsItem (Variables|Default|GetEnemy) _aspawn)
        (Utilities|FlowControl|Delay (Math|Random|RandomFloatinRange 2.0 5.0))
        (Utilities|Array|RemoveItem (Variables|Default|GetEnemy) _aspawn)))
    (:CastFailed
      (Development|PrintString "Enemy Fail"))))

(event OnComponentBeginOverlap(AttackRange)
  (params (OverlappedComponent :type Primitive%20Component%20Object%20Reference) (OtherActor :type Actor%20Object%20Reference) (OtherComp :type Primitive%20Component%20Object%20Reference) (OtherBodyIndex :type Integer) (bFromSweep :type Boolean) (SweepResult :type Hit%20Result%20Structure%20%28by%20ref%29))
  (if (!= OtherActor self)
    (if (== OtherActor (Utilities|Array|Get(acopy) (Variables|Default|GetEnemy)))
      (bind _asbp_aicontroller_old (Utilities|Casting|CastToBP_AIController_Old (AI|GetAIController self)))
      (Variables|/Game/Ironsphere/Feature/NPC/BP_AIController_Old.BP_AIController_Old_C|SetTargetInRange _asbp_aicontroller_old true))))

(event OnComponentEndOverlap(AttackRange)
  (params (OverlappedComponent :type Primitive%20Component%20Object%20Reference) (OtherActor :type Actor%20Object%20Reference) (OtherComp :type Primitive%20Component%20Object%20Reference) (OtherBodyIndex :type Integer))
  (if (!= OtherActor self)
    (if (== OtherActor (Utilities|Array|Get(acopy) (Variables|Default|GetEnemy)))
      (bind _asbp_aicontroller_old (Utilities|Casting|CastToBP_AIController_Old (AI|GetAIController self)))
      (Variables|/Game/Ironsphere/Feature/NPC/BP_AIController_Old.BP_AIController_Old_C|SetTargetInRange _asbp_aicontroller_old false))))

(event EventBeginPlay
  (CallFunction|InitNPCWeapon)
  (bind _aswbc_hehth_bar (Utilities|Casting|CastToWBC_HehthBar (UserInterface|GetWidget (Variables|Default|Getwidget_HPbar))))
  (bind _output_get (Variables|Default|SetAIInfoWidget _aswbc_hehth_bar))
  (Default|UpdateHP _output_get 1.0)
  (Default|UpdateText _output_get (Utilities|Text|ToText(Float) 0.0 "HalfToEven")))

(event Collision|EventActorBeginOverlap
  (params (OtherActor :type Actor%20Object%20Reference)))

(event EventTick
  (params (DeltaSeconds :type Float%20%28single-precision%29)))

(event Game|Damage|EventAnyDamage
  (params (Damage :type Float%20%28single-precision%29) (DamageType :type Damage%20Type%20Object%20Reference) (InstigatedBy :type Controller%20Object%20Reference) (DamageCauser :type Actor%20Object%20Reference))
  (bind _aspawn (Utilities|Casting|CastToPawn DamageCauser))
  (Variables|Default|SetLastDamageDealer _aspawn)
  (Utilities|Array|AddUnique (Variables|Default|GetEnemy) _aspawn))

(fn ConstructionScript)

(fn InitNPCWeapon
  (bind _asbp_weapon_base (Utilities|Casting|CastToBP_WeaponBase (Variables|/Script/Engine.ChildActorComponent|GetChildActor (Variables|Default|GetBP_SmallLaser))))
  (bind _output_get (Variables|Default|SetWeaponNPCReference _asbp_weapon_base))
  (Actor|SetOwner _output_get self))

(fn NPCShot
  (params (Active :type Boolean))
  (Default|WeaponShot (Variables|Default|GetWeaponNPCReference) Active))