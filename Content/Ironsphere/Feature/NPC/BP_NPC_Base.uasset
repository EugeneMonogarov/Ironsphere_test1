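; Base enemy NPC for Ironsphere that targets the player's mech and shows a minimap icon.
; Stats load from DT_NPC, with size, range, HP, damage and kill reward adjusted by a scale factor.
; Tick runs cooldown and wind-up timers that halt movement and play a montage before NPCShot applies melee damage or spawns a projectile.
; Death pays money and experience through GI_Main and drains a crate accumulator that gates random crate or buff drops.
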(event OnComponentBeginOverlap(sensorDetect)
  (params (OverlappedComponent :type Primitive%20Component%20Object%20Reference) (OtherActor :type Actor%20Object%20Reference) (OtherComp :type Primitive%20Component%20Object%20Reference) (OtherBodyIndex :type Integer) (bFromSweep :type Boolean) (SweepResult :type Hit%20Result%20Structure%20%28by%20ref%29))
  (bind _aspawn (Utilities|Casting|CastToPawn OtherActor))
  (if (!= OtherActor self)
    (Utilities|Array|AddUnique (Variables|Default|GetEnemy) _aspawn)))

(event OnComponentEndOverlap(sensorDetect)
  (params (OverlappedComponent :type Primitive%20Component%20Object%20Reference) (OtherActor :type Actor%20Object%20Reference) (OtherComp :type Primitive%20Component%20Object%20Reference) (OtherBodyIndex :type Integer)))

(event Custom|PlayMontage
  (params (AnimMontage :type Anim%20Montage%20Object%20Reference))
  (Animation|Montage|PlayMontage (Variables|Default|GetSkeletalMesh) AnimMontage))

(event EventBeginPlay
  (bind _asgi_main (Utilities|Casting|CastToGI_Main (Game|GetGameInstance))
    (:then
      (Variables|Default|SetGI_Main_ref _asgi_main)
      (Components|Sphere|SetSphereRadius (Variables|Default|GetsensorDetect) 2e+04 true)
      (Transformation|AttachComponentToComponent 0 "None" "SnapToTarget" "SnapToTarget" "SnapToTarget" true)
      (bind _aspc_ingame (Utilities|Casting|CastToPC_Ingame (Game|GetPlayerController 0))
        (:then
          (Variables|Default|SetControlledMech_ref (Variables|/Game/Ironsphere/Core/Framework/Battle/PC_Ingame.PC_Ingame_C|GetControlledMech _aspc_ingame))
          (if (Utilities|IsValid (Variables|/Game/Ironsphere/Core/Framework/Battle/PC_Ingame.PC_Ingame_C|GetControlledMech _aspc_ingame)) :!label _label
            (bind _output_get (Variables|Default|SetEnemy (Utilities|Array|MakeArray (Variables|/Game/Ironsphere/Core/Framework/Battle/PC_Ingame.PC_Ingame_C|GetControlledMech _aspc_ingame))))
            (bind _returnvalue (UserInterface|CreateWidget "/Game/Ironsphere/UI/Ingame/Map/WBS_MinimapObject.WBS_MinimapObject_C" 0 "/Game/Ironsphere/UI/Ingame/Map/Spider.Spider"))
            (Class|UserWidget|SetDesiredSizeinViewport _returnvalue "(X=22.000000,Y=22.000000)")
            (UserInterface|Viewport|AddtoViewport _returnvalue 0)
            (Variables|Default|SetMinimapObject _returnvalue)
            (else
              (Utilities|FlowControl|Delay 0.2)
              (Audio|SpawnSound2D 0 1.0 1.0 0.0 0)
              (goto _label))))
        (:CastFailed
          (Audio|SpawnSound2D "/Game/Ironsphere/Sound/Shot/179222__mixedupmoviestuff__knife-stab.179222__mixedupmoviestuff__knife-stab" 1.0 1.0 0.0 0))))
    (:CastFailed
      (Audio|SpawnSound2D "/Engine/EditorSounds/Notifications/CompileFailed.CompileFailed" 1.0 1.0 0.0 0))))

(event Collision|EventActorBeginOverlap
  (params (OtherActor :type Actor%20Object%20Reference)))

(event EventTick
  (params (DeltaSeconds :type Float%20%28single-precision%29))
  (bind _returnvalue (Transformation|GetActorLocation))
  (bind _returnvalue_2 (Transformation|GetActorLocation))
  (bind (_x _y _z) (Math|Vector|BreakVector _returnvalue))
  (bind (_x_2 _y_2) (Math|Vector|BreakVector _returnvalue_2))
  (Utilities|FlowControl|Sequence
    (:then_0
      (|CallParentFunction DeltaSeconds))
    (:then_1
      ;[1 1 1] Объект на миникарте
      (if (Utilities|IsValid (stale EventBeginPlay _returnvalue))
        (Class|UserWidget|SetPositioninViewport (stale EventBeginPlay _returnvalue) (Math|Vector2D|MakeVector2D (+ (* _x_2 -0.1) 2e+02) (+ (* _y_2 -0.1) 2e+02)) true)
        (else
          (Development|PrintString "invalidMapObject" true true "(R=0.000000,G=0.660000,B=1.000000,A=1.000000)" 0.0))))
    (:then_2
      ;[1 1 1] Таймер КД оружия и продолжительности атаки
      (if (Variables|Default|GetAlive)
        (if (<= (Variables|Default|GetWeaponCooldownTimer) 0.0)
          (Variables|Default|SetWeaponCooldownTimer 0.0)
          (else
            (Variables|Default|SetWeaponCooldownTimer (- (Variables|Default|GetWeaponCooldownTimer) DeltaSeconds))))
        (if (or (Variables|Default|GetNPCShooting) (Variables|Default|GetAttackAnimationOn))
          (if (Variables|Default|GetAttackAnimationOn)
            (bind _output_get (Variables|Default|SetAttackDurationTimer (- (Variables|Default|GetAttackDurationTimer) DeltaSeconds)))
            (Development|PrintString (Utilities|String|ToString(Float) _output_get) true true "(R=0.000000,G=0.660000,B=1.000000,A=1.000000)" 0.0)))))
    (:then_3
      ;[1 1 1] Атака по КД
      (if (Variables|Default|GetAlive)
        (if (Variables|Default|GetAttackAnimationOn)
          (if (<= (Variables|Default|GetWeaponCooldownTimer) 0.0) :!label _label
            (if (Variables|Default|GetAttackAnimationOn)
              (if (<= (Variables|Default|GetAttackDurationTimer) 0.0)
                (CallFunction|NPCShot)
                (Variables|Default|SetWeaponCooldownTimer (/ 1.0 (Variables|Default|GetFireRate)))
                (Variables|Default|SetNPCShooting false)
                (Variables|Default|SetAttackAnimationOn false)
                (Variables|Default|SetAttackDurationTimer (Variables|Default|GetAttackDuration)))
              (else
                (Variables|Default|SetAttackDurationTimer (Variables|Default|GetAttackDuration))
                (Variables|Default|SetAttackAnimationOn true)
                (CallFunction|PlayMontage (Variables|Default|GetAttackAnimation))
                (Variables|/Script/Engine.CharacterMovementComponent|SetMaxWalkSpeed (Variables|Character|GetCharacterMovement) 0.0))))
          (elif (Variables|Default|GetNPCShooting)
            (goto _label)))))
    (:then_5
      (if (< _z 0.0)
        (Transformation|SetActorLocation (Math|Vector|MakeVector _x _y 0.0) false false)))))

(event Game|Damage|EventAnyDamage
  (params (Damage :type Float%20%28single-precision%29) (DamageType :type Damage%20Type%20Object%20Reference) (InstigatedBy :type Controller%20Object%20Reference) (DamageCauser :type Actor%20Object%20Reference))
  (bind _returnvalue (Math|Random|RandomFloatinRange 0.3 1.0))
  (bind _returnvalue_2 (Math|Random|RandomFloatinRange 0.7 1.3))
  (bind _returnvalue_3 (* _returnvalue Damage))
  (bind _returnvalue_4 (/ _returnvalue_3 111.0))
  (bind _returnvalue_5 (Math|Float|Sqrt _returnvalue_4))
  (|CallParentFunction Damage DamageType InstigatedBy DamageCauser)
  (if (> Damage 2.0)
    (switch int (Math|Random|RandomIntegerinRange 0 3)
      (:Default
        (Audio|PlaySound2D "/Game/Ironsphere/Sound/NPC/Damaged/impact_projectile_006.impact_projectile_006" _returnvalue_5 _returnvalue_2 0.0 0 0 :!label _label))
      (:0
        (goto _label))
      (:1
        (Audio|PlaySound2D "/Game/Ironsphere/Sound/NPC/Damaged/impact_projectile_007.impact_projectile_007" _returnvalue_5 _returnvalue_2 0.0 0 0))
      (:2
        (Audio|PlaySound2D "/Game/Ironsphere/Sound/NPC/Damaged/impact_projectile_005.impact_projectile_005" _returnvalue_5 _returnvalue_2 0.0 0 0))
      (:3
        (Audio|PlaySound2D "/Game/Ironsphere/Sound/NPC/Damaged/impact_projectile_metal_007.impact_projectile_metal_007" _returnvalue_5 _returnvalue_2 0.0 0 0)))))

(fn ConstructionScript)

(fn InitNPCWeapon)

(fn NPCShot
  (bind _returnvalue (Transformation|GetActorLocation))
  (bind _returnvalue_2 (Math|Random|RandomFloatinRange 0.75 1.0))
  (bind _returnvalue_3 (Math|Random|RandomFloatinRange 0.5 1.5))
  (bind _returnvalue_4 (Math|Random|RandomFloatinRange 0.1 0.8))
  (bind _returnvalue_5 (Transformation|GetActorLocation))
  (bind _damage (Variables|Default|GetDamage))
  (Utilities|FlowControl|Sequence
    (:then_0
      (if (Variables|Default|GetAlive)
        (if (Variables|Default|GetMelee)
          (switch Utilities|FlowControl|Switch|SwitchonE_DamageTypes (Variables|Default|GetDamageType)
            (:NewEnumerator0
              (Game|Damage|ApplyDamage (Utilities|Array|Get(acopy) (Variables|Default|GetEnemy)) _damage 0 self "/Game/Ironsphere/Feature/Consumable/DamageTypes/BP_PhysicalDamage.BP_PhysicalDamage_C"))
            (:NewEnumerator1
              (Game|Damage|ApplyDamage 0 _damage 0 0 "/Game/Ironsphere/Feature/Consumable/DamageTypes/BP_LaserDamage.BP_LaserDamage_C"))
            (:NewEnumerator2
              (Game|Damage|ApplyDamage 0 0.0 0 0 "/Game/Ironsphere/Feature/Consumable/DamageTypes/BP_LaserDamage.BP_LaserDamage_C")))
          (else
            (Game|SpawnActorfromClass :Class (Variables|Default|GetProjectile) :SpawnTransform (Transformation|GetActorTransform) :CollisionHandlingOverride "AlwaysSpawn" :TransformScaleMethod "MultiplyWithRoot" :Owner self :ProjectileVelocity 2e+02 :ProjectileRange (Variables|Default|GetAttackRange) :ProjectileDamage (Variables|Default|GetDamage) :Instigator self)))))
    (:then_1
      (switch int (Math|Random|RandomInteger 3)
        (:Default
          (Audio|SpawnSoundatLocation "/Game/Ironsphere/Sound/NPC/SpyderAttack3.SpyderAttack3" _returnvalue "0, 0, 0" 0.5 _returnvalue_2 0.0 0 0 :!label _label))
        (:0
          (Audio|SpawnSoundatLocation "/Game/Ironsphere/Sound/NPC/SpyderAttack1.SpyderAttack1" _returnvalue "0, 0, 0" 0.5 _returnvalue_2 0.0 0 0))
        (:1
          (Audio|SpawnSoundatLocation "/Game/Ironsphere/Sound/NPC/SpyderAttack2.SpyderAttack2" _returnvalue "0, 0, 0" 0.5 _returnvalue_2 0.0 0 0))
        (:2
          (goto _label)))
      (switch int (Math|Random|RandomInteger 3)
        (:0
          (Audio|SpawnSoundatLocation "/Game/Ironsphere/Sound/NPC/gui_006.gui_006" _returnvalue_5 "0, 0, 0" _returnvalue_4 _returnvalue_3 0.0 0 0))
        (:1
          (Audio|SpawnSoundatLocation "/Game/Ironsphere/Sound/NPC/gui_005.gui_005" _returnvalue_5 "0, 0, 0" _returnvalue_4 _returnvalue_3 0.0 0 0))))))

(fn Death
  (params (DeathAnim :type Anim%20Montage%20Object%20Reference))
  (bind _returnvalue (Transformation|GetActorTransform))
  (bind _gi_main_ref (Variables|Default|GetGI_Main_ref))
  (bind _gi_main_ref_2 (Variables|Default|GetGI_Main_ref))
  (bind _killmoneyreward (Variables|Default|GetKillMoneyReward))
  (bind _gi_main_ref_3 (Variables|Default|GetGI_Main_ref))
  (bind _minimapobject (Variables|Default|GetMinimapObject))
  (bind _location (Math|Transform|BreakTransform _returnvalue))
  (bind _currentlevelindex (Variables|/Game/Ironsphere/Core/Framework/GI_Main.GI_Main_C|GetCurrentLevelIndex _gi_main_ref))
  (bind _inflation (Variables|/Game/Ironsphere/Core/Framework/GI_Main.GI_Main_C|GetInflation _gi_main_ref_2))
  (bind _minutes (Variables|/Game/Ironsphere/Core/Framework/GI_Main.GI_Main_C|GetMinutes _gi_main_ref_2))
  (bind _progress (Variables|/Game/Ironsphere/Core/Framework/GI_Main.GI_Main_C|GetProgress _gi_main_ref))
  (bind (_x _y) (Math|Vector|BreakVector _location))
  (bind _returnvalue_2 (Math|Conversions|ToFloat(Integer) _minutes))
  (bind _output (Utilities|Array|Get(acopy) _progress _currentlevelindex))
  (bind (_open _passed _bonusreceived _killreward) (Utilities|Struct|BreakST_Progress _output))
  (bind _returnvalue_3 (Math|Vector|MakeVector _x _y 0.0))
  (bind _returnvalue_4 (Math|Float|Power _inflation _returnvalue_2))
  (bind _returnvalue_5 (Math|Transform|MakeTransform _returnvalue_3))
  (bind _returnvalue_6 (* _killmoneyreward _killreward))
  (bind _returnvalue_7 (* _returnvalue_4 3e+01))
  (Utilities|FlowControl|Sequence
    (:then_0
      (Variables|Default|SetAlive false)
      (Audio|SpawnSound2D "/Game/Ironsphere/Sound/NPC/SyderDeath.SyderDeath" 1.0 1.0 0.0 0)
      (Collision|SetCollisionEnabled (Variables|Default|GetsensorDetect) "NoCollision")
      (CallFunction|PlayMontage DeathAnim)
      (Utilities|Array|SetArrayElem (Variables|/Game/Ironsphere/Core/Framework/GI_Main.GI_Main_C|GetProgress (Variables|Default|GetGI_Main_ref)) _currentlevelindex (Utilities|Struct|MakeST_Progress _open _passed _bonusreceived (- _killreward (/ _returnvalue_6 (* (.MoneyReward (Utilities|Struct|BreakST_Level (Utilities|Array|Get(acopy) (Variables|/Game/Ironsphere/Core/Framework/GI_Main.GI_Main_C|GetLevels _gi_main_ref) _currentlevelindex))) 2.0)))))
      (Variables|/Game/Ironsphere/Core/Framework/GI_Main.GI_Main_C|SetMoney _gi_main_ref (+ (Variables|/Game/Ironsphere/Core/Framework/GI_Main.GI_Main_C|GetMoney _gi_main_ref) (* (Variables|/Game/Ironsphere/Core/Character/BP_CharacterBase.BP_CharacterBase_C|GetKillRewardMultiplier (Variables|Default|GetControlledMech_ref)) _returnvalue_6)))
      (Variables|/Game/Ironsphere/Core/Framework/GI_Main.GI_Main_C|SetExperience _gi_main_ref_3 (+ (Variables|/Game/Ironsphere/Core/Framework/GI_Main.GI_Main_C|GetExperience _gi_main_ref_3) (* (Variables|/Game/Ironsphere/Core/Character/BP_CharacterBase.BP_CharacterBase_C|GetExperienceMultiplier (Variables|Default|GetControlledMech_ref)) (Variables|Default|GetKillMoneyReward))))
      (bind _output_get (Variables|/Game/Ironsphere/Core/Framework/GI_Main.GI_Main_C|SetCrateAccumulating _gi_main_ref_3 (- (Variables|/Game/Ironsphere/Core/Framework/GI_Main.GI_Main_C|GetCrateAccumulating _gi_main_ref_3) (* _returnvalue_6 (.Value (Utilities|Struct|BreakST_Skills (Utilities|Array|Get(acopy) (Variables|/Game/Ironsphere/Core/Framework/GI_Main.GI_Main_C|GetSkills _gi_main_ref_3) 3)))))))
      (if (< _output_get 0.0)
        (Variables|/Game/Ironsphere/Core/Framework/GI_Main.GI_Main_C|SetCrateAccumulating _gi_main_ref_3 0.0)
        (if (Utilities|IsValid _minimapobject)
          (Widget|SetVisibility _minimapobject "Hidden"))
        (if (> _returnvalue_6 (Math|Random|RandomFloatinRange 0.0 (Variables|/Game/Ironsphere/Core/Framework/GI_Main.GI_Main_C|GetCrateAccumulating _gi_main_ref_2)))
          (Variables|/Game/Ironsphere/Core/Framework/GI_Main.GI_Main_C|SetCrateAccumulating (Variables|Default|GetGI_Main_ref) _returnvalue_7)
          (switch int (Math|Random|RandomIntegerinRange 0 2)
            (:0
              (Game|SpawnActorfromClass "/Game/Ironsphere/Feature/World/Crates/AmmoCrate.AmmoCrate_C" _returnvalue_5 "Undefined" "MultiplyWithRoot" 0 0))
            (:1
              (Game|SpawnActorfromClass "/Game/Ironsphere/Feature/World/Crates/MoneyCrate.MoneyCrate_C" _returnvalue_5 "Undefined" "MultiplyWithRoot" 0 0))
            (:2
              (Game|SpawnActorfromClass "/Game/Ironsphere/Feature/World/Crates/RepairCrate.RepairCrate_C" _returnvalue_5 "Undefined" "MultiplyWithRoot" 0 0)))
          (elif (> (Variables|Default|GetKillMoneyReward) (Math|Random|RandomFloatinRange 0.0 _returnvalue_7))
            (switch int (Math|Random|RandomIntegerinRange 0 4)
              (:0
                (Game|SpawnActorfromClass "/Game/Ironsphere/Feature/World/Crates/Buff_Damage.Buff_Damage_C" _returnvalue_5 "Undefined" "MultiplyWithRoot" 0 0))
              (:1
                (Game|SpawnActorfromClass "/Game/Ironsphere/Feature/World/Crates/Buff_Expereince.Buff_Expereince_C" _returnvalue_5 "Undefined" "MultiplyWithRoot" 0 0))
              (:2
                (Game|SpawnActorfromClass "/Game/Ironsphere/Feature/World/Crates/Buff_KillReward.Buff_KillReward_C" _returnvalue_5 "Undefined" "MultiplyWithRoot" 0 0))
              (:3
                (Game|SpawnActorfromClass "/Game/Ironsphere/Feature/World/Crates/Buff_Shield.Buff_Shield_C" _returnvalue_5 "Undefined" "MultiplyWithRoot" 0 0))
              (:4
                (Game|SpawnActorfromClass "/Game/Ironsphere/Feature/World/Crates/Buff_Speed.Buff_Speed_C" _returnvalue_5 "Undefined" "MultiplyWithRoot" 0 0)))))))
    (:then_1
      (|CallParentFunction 0))))

(fn SetNPCParameters
  (params (ID :type Name) (ScaleFactor :type Float%20%28double-precision%29))
  (bind _capsulecomponent (Variables|Default|GetCapsuleComponent))
  (bind _skeletalmesh (Variables|Default|GetSkeletalMesh))
  (bind _capsuletakingdamage (Variables|Default|GetCapsuleTakingDamage))
  (Variables|Default|SetScaleFactor ScaleFactor)
  (bind _returnvalue (Utilities|GetDataTableRow "/Game/Ironsphere/Feature/NPC/DT_NPC.DT_NPC" ID)
    (:then
      (Variables|Default|SetAttackRange (* (Variables|Default|GetScaleFactor) (.Range (Utilities|Struct|BreakST_NPC _returnvalue))))
      (bind _output_get (Variables|Default|SetMaxHP (* (* (Variables|Default|GetScaleFactor) (Variables|Default|GetScaleFactor) (Variables|Default|GetScaleFactor)) (.HP (Utilities|Struct|BreakST_NPC _returnvalue)))))
      (Variables|Default|SetCurrentHP _output_get)
      (bind _output_get_2 (Variables|Default|SetPhysicalArmor (.PhysicalArmor (Utilities|Struct|BreakST_NPC _returnvalue))))
      (Variables|Default|SetBasePhysicalArmor _output_get_2)
      (Variables|Default|SetFireRate (.FireRate (Utilities|Struct|BreakST_NPC _returnvalue)))
      (bind _output_get_3 (Variables|Default|SetLaserArmor (.LaserArmor (Utilities|Struct|BreakST_NPC _returnvalue))))
      (Variables|Default|SetBaseLaserArmor _output_get_3)
      (Variables|/Script/Engine.CharacterMovementComponent|SetMaxWalkSpeed (Variables|Character|GetCharacterMovement) (.Speed (Utilities|Struct|BreakST_NPC _returnvalue)))
      (Variables|Default|SetDamage (* (.Damage (Utilities|Struct|BreakST_NPC _returnvalue)) (* (Variables|Default|GetScaleFactor) (Variables|Default|GetScaleFactor) (Variables|Default|GetScaleFactor))))
      (bind _output_get_4 (Variables|Default|SetBaseCharacterSpeed (.Speed (Utilities|Struct|BreakST_NPC _returnvalue))))
      (Variables|Default|SetCharacterSpeed _output_get_4)
      (Variables|Default|SetKillMoneyReward (* (.MoneyReward (Utilities|Struct|BreakST_NPC _returnvalue)) (* (Variables|Default|GetScaleFactor) (Variables|Default|GetScaleFactor) (Variables|Default|GetScaleFactor))))
      (Components|Capsule|SetCapsuleRadius _capsulecomponent (* (Variables|/Script/Engine.CapsuleComponent|GetCapsuleRadius _capsulecomponent) (Variables|Default|GetScaleFactor)) true)
      (Components|Capsule|SetCapsuleRadius _capsuletakingdamage (* (Class|CapsuleComponent|GetUnscaledCapsuleRadius _capsuletakingdamage) (Variables|Default|GetScaleFactor)) true)
      (Variables|Default|SetAttackDuration (.AttackDuration (Utilities|Struct|BreakST_NPC _returnvalue)))
      (Variables|Default|SetDamageType (.DamageType (Utilities|Struct|BreakST_NPC _returnvalue)))
      (Transformation|SetWorldScale3D _skeletalmesh (* (Transformation|GetWorldScale _skeletalmesh) (Math|Vector|MakeVector (Variables|Default|GetScaleFactor) (Variables|Default|GetScaleFactor) (Variables|Default|GetScaleFactor))))
      (Variables|Default|SetAttackAnimation (.AttackAnimation (Utilities|Struct|BreakST_NPC _returnvalue)))
      (Variables|Default|SetMelee (.Melee (Utilities|Struct|BreakST_NPC _returnvalue)))
      (Variables|Default|SetProjectile (.Projectile (Utilities|Struct|BreakST_NPC _returnvalue))))
    (:RowNotFound
      (Audio|SpawnSound2D "/Engine/EditorSounds/Notifications/CompileStart_Cue.CompileStart_Cue" 1.0 1.0 0.0 0))))