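; Allied small missile turret NPC that builds on a parent character class, initialized with the allied turret parameters.
; After a few warm-up ticks, it re-picks its target every tick by swapping a randomized, distance-biased choice to the front of the Enemy array.
; A dead front enemy is removed, triggering an immediate re-pick.
; Death passes a spider death montage to the parent and destroys BaseT, whose spawn code here is disconnected.
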(event EventBeginPlay
  (Variables|Default|SetAllied true)
  (|CallParentFunction)
  (CallFunction|SetNPCParameters "NPC_AlliedTurret" 1.0))

(event Collision|EventActorBeginOverlap
  (params (OtherActor :type Actor%20Object%20Reference))
  (|CallParentFunction OtherActor) ; This node is disabled and will not be called.\nDrag off pins to build functionality.
)

(event EventTick
  (params (DeltaSeconds :type Float%20%28single-precision%29))
  (bind _enemy (Variables|Default|GetEnemy))
  (bind _tickcount (Variables|Default|GetTickCount))
  (|CallParentFunction DeltaSeconds)
  (Math|Integer|IncrementInt _tickcount
    (:%20%20
      (bind _asbp_character_base (Utilities|Casting|CastToBP_CharacterBase (Utilities|Array|Get(acopy) (Variables|Default|GetEnemy))))
      (if (Variables|/Game/Ironsphere/Core/Character/BP_CharacterBase.BP_CharacterBase_C|GetAlive _asbp_character_base)
        (if (> _tickcount 5)
          (Utilities|Array|Clear (Variables|Default|GetLenghtToEnemiesTurret) :!label _label)
          (Variables|Default|SetNearestDistanceTurret 1e+05)
          (for (_array_element _array_index) _enemy
            (if (Utilities|IsValid _array_element)
              (if (< (Math|Vector|VectorLength (- (Transformation|GetActorLocation (Utilities|Array|Get(acopy) _enemy _array_index)) (Transformation|GetActorLocation))) (Variables|Default|GetNearestDistanceTurret))
                (Variables|Default|SetNearestDistanceTurret (Math|Random|RandomFloatinRange 0.0 (Math|Vector|VectorLength (- (Transformation|GetActorLocation (Utilities|Array|Get(acopy) _enemy _array_index)) (Transformation|GetActorLocation)))))
                (Variables|Default|SetNearestIndexTurret _array_index))
              (else
                (Utilities|Array|RemoveItem _enemy (Utilities|Array|Get(acopy) _enemy _array_index)))))
          (if (> (Variables|Default|GetNearestIndexTurret) 0)
            (Utilities|Array|Swap (Variables|Default|GetEnemy) (Variables|Default|GetNearestIndexTurret))))
        (else
          (Utilities|Array|RemoveIndex (Variables|Default|GetEnemy))
          (goto _label))))))

(fn ConstructionScript
  (|CallParentFunction))

(fn SetNPCParameters
  (params (ID :type Name :default "None") (ScaleFactor :type Float%20%28double-precision%29))
  (|CallParentFunction ID ScaleFactor))

(fn Death
  (params (DeathAnim :type Anim%20Montage%20Object%20Reference))
  (|CallParentFunction "/Game/Ironsphere/3D/Animations/Spider/SpiderDeath_Montage.SpiderDeath_Montage")
  (Actor|DestroyActor (Variables|Default|GetBaseT)))

(fn NPCShot
  (|CallParentFunction))