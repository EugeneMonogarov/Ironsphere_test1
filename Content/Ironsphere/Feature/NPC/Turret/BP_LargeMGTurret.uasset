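; Large machine-gun turret NPC, a child Blueprint that leaves shooting and death logic to its parent.
; On BeginPlay it sets its parameters by NPC ID and scale factor, then spawns and stores a scaled-down BP_TurretBase beneath it at world Z zero.
; Death always passes a spider death montage to the parent, and leftover nodes that flag a mission boss as killed never run.
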(event EventBeginPlay
  (bind _returnvalue (Transformation|GetActorTransform))
  (bind (_location _rotation) (Math|Transform|BreakTransform _returnvalue))
  (bind (_x _y) (Math|Vector|BreakVector _location))
  (|CallParentFunction)
  (CallFunction|SetNPCParameters "NPC_LargeMGTurret" (Variables|Default|GetScaleFactor))
  (bind _returnvalue_2 (Game|SpawnActorfromClass "/Game/Ironsphere/Feature/NPC/Turret/BP_TurretBase.BP_TurretBase_C" (Math|Transform|MakeTransform (Math|Vector|MakeVector _x _y 0.0) _rotation "0.700000,0.700000,0.700000") "Undefined" "MultiplyWithRoot" 0 0))
  (Variables|Default|SetBase _returnvalue_2))

(event Collision|EventActorBeginOverlap
  (params (OtherActor :type Actor%20Object%20Reference))
  (|CallParentFunction OtherActor) ; This node is disabled and will not be called.\nDrag off pins to build functionality.
)

(event EventTick
  (params (DeltaSeconds :type Float%20%28single-precision%29))
  (|CallParentFunction DeltaSeconds) ; This node is disabled and will not be called.\nDrag off pins to build functionality.
)

(fn ConstructionScript
  (|CallParentFunction))

(fn SetNPCParameters
  (params (ID :type Name :default "None") (ScaleFactor :type Float%20%28double-precision%29))
  (|CallParentFunction ID ScaleFactor))

(fn Death
  (params (DeathAnim :type Anim%20Montage%20Object%20Reference))
  (|CallParentFunction "/Game/Ironsphere/3D/Animations/Spider/SpiderDeath_Montage.SpiderDeath_Montage"))

(fn NPCShot
  (|CallParentFunction))