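; Worm enemy NPC, a child of a shared NPC base that registers as NPC_Worm with a randomized scale on BeginPlay.
; Its shot override plays the worm attack montage and a random spider attack sound, then fires the referenced NPC weapon with its damage.
; The random pick only reaches two of the three wired sounds.
; A custom event plays any supplied montage on the skeletal mesh.
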(event Custom|CustomEvent
  (params (AnimMontage :type Anim%20Montage%20Object%20Reference))
  (Animation|Montage|PlayMontage (Variables|Default|GetSkeletalMesh) AnimMontage))

(event EventBeginPlay
  (|CallParentFunction)
  (CallFunction|SetNPCParameters "NPC_Worm" (Math|Random|RandomFloatinRange 0.7 1.2)))

(event Collision|EventActorBeginOverlap
  (params (OtherActor :type Actor%20Object%20Reference))
  (|CallParentFunction OtherActor) ; This node is disabled and will not be called.\nDrag off pins to build functionality.
)

(event EventTick
  (params (DeltaSeconds :type Float%20%28single-precision%29))
  (|CallParentFunction DeltaSeconds) ; This node is disabled and will not be called.\nDrag off pins to build functionality.
)

(fn ConstructionScript
  (|CallParentFunction))

(fn NPCShot
  (params (Active :type Boolean))
  (bind _returnvalue (Transformation|GetActorLocation))
  (CallFunction|PlayMontage "/Game/Ironsphere/3D/Animations/Worm/WormAttackMontage.WormAttackMontage")
  (switch int (Math|Random|RandomInteger 2)
    (:0
      (Audio|SpawnSoundatLocation "/Game/Ironsphere/Sound/NPC/SpyderAttack1.SpyderAttack1" _returnvalue "0, 0, 0" 1.0 1.0 0.0 0 0))
    (:1
      (Audio|SpawnSoundatLocation "/Game/Ironsphere/Sound/NPC/SpyderAttack2.SpyderAttack2" _returnvalue "0, 0, 0" 1.0 1.0 0.0 0 0))
    (:2
      (Audio|SpawnSoundatLocation "/Game/Ironsphere/Sound/NPC/SpyderAttack3.SpyderAttack3" _returnvalue "0, 0, 0" 1.0 1.0 0.0 0 0)))
  (Default|NPCWeaponShot (Variables|Default|GetWeaponNPCReference) (Variables|Default|GetDamage)))

(fn SetNPCParameters
  (params (ID :type Name :default "None") (ScaleFactor :type Float%20%28double-precision%29))
  (|CallParentFunction ID ScaleFactor))