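; BP_Plant is a plant NPC child Blueprint that sets itself up as "NPC_Plant" with a slight random scale variation.
; On BeginPlay it spawns a scaled-down BP_PlantBase at its XY position on Z=0 and keeps a reference.
; Death forwards HornetDeathMontage to the parent, while the node destroying the plant base is unconnected.
; A custom event plays a given montage, and NPC_Shot only calls the parent.
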(event Custom|CustomEvent
  (params (AnimMontage :type Anim%20Montage%20Object%20Reference))
  (Animation|Montage|PlayMontage (Variables|Default|GetSkeletalMesh) AnimMontage))

(event EventBeginPlay
  (bind _returnvalue (Transformation|GetActorTransform))
  (bind (_location _rotation) (Math|Transform|BreakTransform _returnvalue))
  (bind (_x _y) (Math|Vector|BreakVector _location))
  (|CallParentFunction)
  (CallFunction|SetNPCParameters "NPC_Plant" (Math|Random|RandomFloatinRange 0.9 1.1))
  (bind _returnvalue_2 (Game|SpawnActorfromClass "/Game/Ironsphere/Feature/NPC/Plant/BP_PlantBase.BP_PlantBase_C" (Math|Transform|MakeTransform (Math|Vector|MakeVector _x _y 0.0) _rotation "0.700000,0.700000,0.700000") "Undefined" "MultiplyWithRoot" 0 0))
  (Variables|Default|SetPlantBase _returnvalue_2))

(event Collision|EventActorBeginOverlap
  (params (OtherActor :type Actor%20Object%20Reference))
  (|CallParentFunction OtherActor) ; This node is disabled and will not be called.\nDrag off pins to build functionality.
)

(event EventTick
  (params (DeltaSeconds :type Float%20%28single-precision%29))
  (|CallParentFunction DeltaSeconds) ; This node is disabled and will not be called.\nDrag off pins to build functionality.
)

(fn ConstructionScript
  (|CallParentFunction))

(fn SetNPCParameters
  (params (ID :type Name :default "None") (ScaleFactor :type Float%20%28double-precision%29))
  (|CallParentFunction ID ScaleFactor))

(fn Death
  (params (DeathAnim :type Anim%20Montage%20Object%20Reference))
  (|CallParentFunction "/Game/Ironsphere/3D/Animations/Hornet/HornetDeathMontage.HornetDeathMontage"))

(fn NPCShot
  (|CallParentFunction))