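; Spider NPC "Dark Widow Mother", a child Blueprint that spawns Dark Widow minions and can shield itself when hurt.
; Shortly after BeginPlay it rolls a limited brood count, which Tick spends one widow at a time beside it on a randomized countdown.
; AnyDamage may grant a temporary shield buff, with odds rising with damage relative to max HP, gated by a random cooldown.
; Death passes the spider death montage to the parent.
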(event EventBeginPlay
  (|CallParentFunction)
  (CallFunction|SetNPCParameters "NPC_DarkWidowMother" 1.0)
  (Utilities|FlowControl|Delay 2.0)
  (Variables|Default|SetNumberOfWidows (Math|Random|RandomIntegerinRange 5 8)))

(event Collision|EventActorBeginOverlap
  (params (OtherActor :type Actor%20Object%20Reference))
  (|CallParentFunction OtherActor) ; This node is disabled and will not be called.\nDrag off pins to build functionality.
)

(event EventTick
  (params (DeltaSeconds :type Float%20%28single-precision%29))
  (bind _returnvalue (Transformation|GetActorLocation))
  (bind (_x _y _z) (Math|Vector|BreakVector _returnvalue))
  (|CallParentFunction DeltaSeconds)
  (if (> (Variables|Default|GetNumberOfWidows) 0)
    (Variables|Default|SetSpawnWidows (- (Variables|Default|GetSpawnWidows) DeltaSeconds))
    (if (<= (Variables|Default|GetSpawnWidows) 0.0)
      (AI|SpawnAIFromClass "/Game/Ironsphere/Feature/NPC/Spider/BP_DarkWidow.BP_DarkWidow_C" 0 (Math|Vector|MakeVector (+ _x -5e+01) _y _z) "0, 0, 0" false 0)
      (Variables|Default|SetSpawnWidows (Math|Random|RandomFloatinRange 22.0 25.0))
      (Math|Integer|DecrementInt (Variables|Default|GetNumberOfWidows)))))

(event Game|Damage|EventAnyDamage
  (params (Damage :type Float%20%28single-precision%29) (DamageType :type Damage%20Type%20Object%20Reference) (InstigatedBy :type Controller%20Object%20Reference) (DamageCauser :type Actor%20Object%20Reference))
  (|CallParentFunction Damage DamageType InstigatedBy DamageCauser)
  (if (and (<= (Variables|Default|GetShieldCD) 0.0) (> (* Damage 9.0) (Math|Random|RandomFloatinRange 0.0 (Variables|Default|GetMaxHP))))
    (CallFunction|AddBuff (Utilities|Struct|MakeST_buff "NewEnumerator4" 5e+02 7.0 false "DarkWidowShield" 0))
    (Variables|Default|SetCurrentShield 5e+02)
    (Variables|Default|SetShieldCD (Math|Random|RandomFloatinRange 1e+01 16.0))))

(fn ConstructionScript
  (|CallParentFunction))

(fn SetNPCParameters
  (params (ID :type Name :default "None") (ScaleFactor :type Float%20%28double-precision%29))
  (|CallParentFunction ID ScaleFactor))

(fn Death
  (params (DeathAnim :type Anim%20Montage%20Object%20Reference))
  (|CallParentFunction "/Game/Ironsphere/3D/Animations/Spider/SpiderDeath_Montage.SpiderDeath_Montage"))

(fn NPCShot
  (|CallParentFunction))