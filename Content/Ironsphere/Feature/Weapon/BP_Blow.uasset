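; BP_Blow is a weapon explosion actor that detonates after a configurable delay from BeginPlay.
; It plays an explosion sound with concurrency settings, applies falloff radial physical damage using configurable damage and radius, and spawns a particle effect.
; The damage origin keeps the actor's X and Y but uses a fixed low world height.
; It also shakes the first player's camera, then destroys itself shortly afterward.
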(event EventBeginPlay
  (bind _returnvalue (Transformation|GetActorLocation))
  (bind (_x _y) (Math|Vector|BreakVector _returnvalue))
  (Utilities|FlowControl|Delay (Variables|Default|GetDelay))
  (Audio|SpawnSoundatLocation "/Game/Ironsphere/Sound/Explosion/explosion_1.explosion_1" (Transformation|GetActorLocation) "0, 0, 0" 1.0 1.0 0.0 0 "/Game/Ironsphere/Feature/World/CnC_DestroySound.CnC_DestroySound")
  (Class|GameplayStatics|ApplyRadialDamagewithFalloff (Variables|Default|GetDamage) 0.0 (Math|Vector|MakeVector _x _y 1e+01) 0.0 (Variables|Default|GetRadius) 0.2 "/Game/Ironsphere/Feature/Consumable/DamageTypes/BP_PhysicalDamage.BP_PhysicalDamage_C" 0 self 0 "ECC_Visibility")
  (Effects|SpawnEmitteratLocation "/Game/StarterContent/Particles/P_Explosion.P_Explosion" _returnvalue)
  (Class|LegacyCameraShake|StartLegacyCameraShake (Game|GetPlayerCameraManager 0) "/Game/Ironsphere/Core/Player/CamShakeBlow.CamShakeBlow_C" 1.0 "CameraLocal" "0, 0, 0")
  (Utilities|FlowControl|Delay 0.2)
  (Actor|DestroyActor))

(event Collision|EventActorBeginOverlap
  (params (OtherActor :type Actor%20Object%20Reference)))

(event EventTick
  (params (DeltaSeconds :type Float%20%28single-precision%29)))

(fn ConstructionScript)