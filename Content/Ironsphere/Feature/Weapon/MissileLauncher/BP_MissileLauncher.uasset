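; BP_MissileLauncher is a weapon actor that fires missile projectiles while its trigger is held.
; WeaponShot sets a firing flag, and Tick counts down a reload timer, launching a missile and restarting the cooldown whenever it reaches zero during firing.
; MissileLaunch spawns the projectile class mapped to the current ammo type at the arrow, passing weapon stats and the owning pawn, with launch sound and explosion effect.
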(event EventBeginPlay
  (|CallParentFunction) ; This node is disabled and will not be called.\nDrag off pins to build functionality.
)

(event Collision|EventActorBeginOverlap
  (params (OtherActor :type Actor%20Object%20Reference))
  (|CallParentFunction OtherActor) ; This node is disabled and will not be called.\nDrag off pins to build functionality.
)

(event EventTick
  (params (DeltaSeconds :type Float%20%28single-precision%29))
  (|CallParentFunction DeltaSeconds)
  (if (> (Variables|Default|GetReloadingTimer) 0.0)
    (Variables|Default|SetReloadingTimer (- (Variables|Default|GetReloadingTimer) DeltaSeconds))
    (else
      (Variables|Default|SetReloadingTimer 0.0)))
  (if (== (Variables|Default|GetReloadingTimer) 0.0)
    (if (Variables|Default|GetOnMissileLaunching)
      (CallFunction|MissileLaunch)
      (Variables|Default|SetReloadingTimer (Variables|Default|GetWeaponCooldown)))))

(fn ConstructionScript
  (|CallParentFunction))

(fn MissileLaunch
  (bind _ammotype (Variables|Default|GetAmmoType))
  (bind _ammotypelist (Variables|Default|GetAmmoTypeList))
  (bind _arrow (Variables|Default|GetArrow))
  (bind (_value _returnvalue) (Utilities|Map|Find _ammotypelist _ammotype))
  (bind _returnvalue_2 (Transformation|GetWorldTransform _arrow))
  (Audio|SpawnSoundatLocation "/Game/StarterContent/Audio/Bluezone_BC0245_064_hit_metal.Bluezone_BC0245_064_hit_metal" (.Location (Math|Transform|BreakTransform (Transformation|GetActorTransform))) "0, 0, 0" 0.1 1.0 0.0 0 0)
  (bind _aspawn (Utilities|Casting|CastToPawn (Components|GetOwner)))
  (if _returnvalue
    (Game|SpawnActorfromClass _value _returnvalue_2 "AlwaysSpawn" "MultiplyWithRoot" _aspawn (Variables|Default|GetProjectileVelocity) (Variables|Default|GetWeaponRange) (Variables|Default|GetWeaponDamage) (Variables|Default|GetWeaponExplosionDamage) (Variables|Default|GetWeaponExplosionRadius) _aspawn)
    (Effects|SpawnEmitteratLocation "/Game/StarterContent/Particles/P_Explosion.P_Explosion" (.Location (Math|Transform|BreakTransform _returnvalue_2)) "0, 0, 0" "0.100000,0.100000,0.100000")
    (else
      (Development|PrintString "AmmoNotFound"))))

(fn WeaponShot
  (params (Active :type Boolean))
  (Variables|Default|SetOnMissileLaunching Active))