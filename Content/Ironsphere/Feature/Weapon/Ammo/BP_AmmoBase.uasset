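; Base ammo projectile actor that damages the actor it overlaps, ignoring its owner, then explodes and destroys itself.
; Damage is full within ProjectileRange of the spawn point and falls off linearly to zero at twice that range, where Tick destroys the projectile.
; Explosion particle scale, sound volume and inverse pitch derive from the square root of damage dealt.
; The construction script sets the projectile movement's initial and max speed from ProjectileVelocity.
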(event EventBeginPlay
  (Variables|Default|SetStartPosition (Transformation|GetActorLocation)))

(event Collision|EventActorBeginOverlap
  (params (OtherActor :type Actor%20Object%20Reference))
  (bind _returnvalue (Transformation|GetActorLocation))
  (bind _returnvalue_2 (Components|GetOwner))
  (if (!= OtherActor _returnvalue_2)
    (if (<= (Math|Vector|Distance(Vector) (Variables|Default|GetStartPosition) (Transformation|GetActorLocation)) (Variables|Default|GetProjectileRange))
      (Variables|Default|SetIncomingDamage (Variables|Default|GetProjectileDamage))
      (else
        (Variables|Default|SetIncomingDamage (* (Variables|Default|GetProjectileDamage) (- 1.0 (/ (- (Math|Vector|Distance(Vector) (Variables|Default|GetStartPosition) (Transformation|GetActorLocation)) (Variables|Default|GetProjectileRange)) (Variables|Default|GetProjectileRange)))))))
    (Game|Damage|ApplyDamage OtherActor (Variables|Default|GetIncomingDamage) 0 _returnvalue_2)
    (Development|PrintString (Utilities|String|ToString(Float) (Variables|Default|GetIncomingDamage)))
    (Effects|SpawnEmitteratLocation "/Game/StarterContent/Particles/P_Explosion.P_Explosion" _returnvalue "0, 0, 0" (Math|Conversions|ToVector(Float) (/ (Math|Float|Sqrt (Variables|Default|GetIncomingDamage)) 3e+01)))
    (Audio|SpawnSoundatLocation "/Game/StarterContent/Audio/Explosion01.Explosion01" _returnvalue "0, 0, 0" (/ (Math|Float|Sqrt (Variables|Default|GetIncomingDamage)) 3e+01) (/ 1.0 (/ (Math|Float|Sqrt (Variables|Default|GetIncomingDamage)) 3e+01)) 0.0 0 0)
    (Actor|DestroyActor)))

(event EventTick
  (params (DeltaSeconds :type Float%20%28single-precision%29))
  (if (>= (Math|Vector|Distance(Vector) (Variables|Default|GetStartPosition) (Transformation|GetActorLocation)) (* (Variables|Default|GetProjectileRange) 2.0))
    (Actor|DestroyActor)))

(fn ConstructionScript
  (bind _projectilemovement (Variables|Default|GetProjectileMovement))
  (bind _output_get (Variables|/Script/Engine.ProjectileMovementComponent|SetInitialSpeed _projectilemovement (Variables|Default|GetProjectileVelocity)))
  (Variables|/Script/Engine.ProjectileMovementComponent|SetMaxSpeed _projectilemovement _output_get))