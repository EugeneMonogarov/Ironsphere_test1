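; BP_Laser is a weapon Blueprint that fires repeated hitscan laser shots while its shooting flag is on.
; WeaponShot sets the flag, and Tick counts down a cooldown, calling TraceBeam whenever it reaches zero with the flag on.
; TraceBeam sphere-traces forward to twice Range against selected object types, ignoring the owner, then applies damage and plays a sound.
; The only beam visual here is the trace's brief debug draw.
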(event EventBeginPlay
  (|CallParentFunction) ; This node is disabled and will not be called.\nDrag off pins to build functionality.
)

(event Collision|EventActorBeginOverlap
  (params (OtherActor :type Actor%20Object%20Reference))
  (|CallParentFunction OtherActor) ; This node is disabled and will not be called.\nDrag off pins to build functionality.
)

(event EventTick
  (params (DeltaSeconds :type Float%20%28single-precision%29))
  (|CallParentFunction DeltaSeconds)
  (if (> (Variables|Default|GetReloadingTimer) 0.0)
    (Variables|Default|SetReloadingTimer (- (Variables|Default|GetReloadingTimer) DeltaSeconds))
    (else
      (Variables|Default|SetReloadingTimer 0.0)))
  (if (== (Variables|Default|GetReloadingTimer) 0.0)
    (if (Variables|Default|GetOnLaserShooting)
      (CallFunction|TraceBeam)
      (Variables|Default|SetReloadingTimer (Variables|Default|GetWeaponCooldown)))))

(fn ConstructionScript
  (|CallParentFunction))

(fn TraceBeam
  (bind _returnvalue (Transformation|GetActorTransform))
  (bind (_location _rotation) (Math|Transform|BreakTransform _returnvalue))
  (bind _outhit (Collision|SphereTraceForObjects _location (+ (* (Math|Rotator|GetRotationXVector _rotation) (* (Variables|Default|GetRange) 2.0)) _location) 1.0 (Utilities|Array|MakeArray "ObjectTypeQuery7" "ObjectTypeQuery8" "ObjectTypeQuery6") false (Utilities|Array|MakeArray (Components|GetOwner)) "ForDuration" true "(R=1.000000,G=0.000000,B=0.000000,A=1.000000)" "(R=0.000000,G=1.000000,B=0.000000,A=1.000000)" 0.1))
  (Game|Damage|ApplyDamage (.HitActor (Collision|BreakHitResult _outhit)) (Variables|Default|GetDamage) 0 (Components|GetOwner))
  (Audio|SpawnSoundatLocation "/Engine/VREditor/Sounds/UI/Laser_Pull.Laser_Pull" (Transformation|GetActorLocation) "0, 0, 0" 1.0 1.0 0.0 0 0))

(fn WeaponShot
  (params (Active :type Boolean))
  (Variables|Default|SetOnLaserShooting Active))