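; BP_UltraBolster is a shotgun-style ballistic weapon that overrides the parent's projectile launch to fire a burst of pellets.
; It looks up the projectile class by ammo type, offsets aim by player Shake, then scatters each pellet by Accuracy with randomized velocity.
; Direct damage is divided per pellet, while explosion damage is not.
; Each shot plays camera shake, muzzle effect and sound, and increases player Shake, widening later shots.
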(event EventBeginPlay
  (|CallParentFunction) ; This node is disabled and will not be called.\nDrag off pins to build functionality.
)

(event Collision|EventActorBeginOverlap
  (params (OtherActor :type Actor%20Object%20Reference))
  (|CallParentFunction OtherActor) ; This node is disabled and will not be called.\nDrag off pins to build functionality.
)

(event EventTick
  (params (DeltaSeconds :type Float%20%28single-precision%29))
  (|CallParentFunction DeltaSeconds) ; This node is disabled and will not be called.\nDrag off pins to build functionality.
)

(fn ConstructionScript
  (|CallParentFunction))

(fn WeaponShot
  (params (Active :type Boolean))
  (|CallParentFunction Active))

(fn ProjectileLaunch
  (params (Buff :type ST%20Buff%20Structure))
  (bind _ammotype (Variables|Default|GetAmmoType))
  (bind _ammotypelist (Variables|Default|GetAmmoTypeList))
  (bind _characterplayer_ref (Variables|Default|GetCharacterPlayer_ref))
  (bind _weapondamage (Variables|Default|GetWeaponDamage))
  (bind _accuracy (Variables|Default|GetAccuracy))
  (bind _characterplayer_ref_2 (Variables|Default|GetCharacterPlayer_ref))
  (bind _arrow (Variables|Default|GetArrow))
  (bind (_value _returnvalue) (Utilities|Map|Find _ammotypelist _ammotype))
  (bind _returnvalue_2 (Transformation|GetWorldTransform _arrow))
  (bind _returnvalue_3 (- 1.0 _accuracy))
  (bind _damagemultiplier (Variables|/Game/Ironsphere/Core/Character/BP_CharacterBase.BP_CharacterBase_C|GetDamageMultiplier _characterplayer_ref_2))
  (bind _location (Math|Transform|BreakTransform _returnvalue_2))
  (bind (_location_2 _rotation) (Math|Transform|BreakTransform _returnvalue_2))
  (bind _returnvalue_4 (* _returnvalue_3 45.0))
  (bind (_roll _pitch _yaw) (Math|Rotator|BreakRotator _rotation))
  (bind _aspawn (Utilities|Casting|CastToPawn (Components|GetOwner)))
  (if _returnvalue
    (bind _output_get (LocalVariables|SetSpawnTransform (Math|Transform|MakeTransform _location_2 (Math|Rotator|MakeRotator _roll _pitch (+ _yaw (Math|Random|RandomFloatinRange (* (/ (* (Variables|/Game/Ironsphere/Core/Player/BP_CharacterPlayer.BP_CharacterPlayer_C|GetShake (Variables|Default|GetCharacterPlayer_ref)) 8.0) 1e+01) -1.0) (/ (* (Variables|/Game/Ironsphere/Core/Player/BP_CharacterPlayer.BP_CharacterPlayer_C|GetShake (Variables|Default|GetCharacterPlayer_ref)) 8.0) 1e+01)))))))
    (for _index (range 0 10)
      (Game|SpawnActorfromClass _value (Math|Transform|MakeTransform (.Location (Math|Transform|BreakTransform _output_get)) (Math|Rotator|MakeRotator (.Roll (Math|Rotator|BreakRotator (.Rotation (Math|Transform|BreakTransform _output_get)))) (.Pitch (Math|Rotator|BreakRotator (.Rotation (Math|Transform|BreakTransform _output_get)))) (+ (.Yaw (Math|Rotator|BreakRotator (.Rotation (Math|Transform|BreakTransform _output_get)))) (Math|Random|RandomFloatinRange (* _returnvalue_4 -1.0) _returnvalue_4))) (.Scale (Math|Transform|BreakTransform _output_get))) "AlwaysSpawn" "MultiplyWithRoot" (Components|GetOwner) (* (Variables|Default|GetProjectileVelocity) (Math|Random|RandomFloatinRange 0.9 1.1)) (Variables|Default|GetWeaponRange) (/ (* _damagemultiplier _weapondamage) 1e+01) (* _damagemultiplier (Variables|Default|GetWeaponExplosionDamage)) (Variables|Default|GetWeaponExplosionRadius) (Utilities|Enum|Equal(Enum) (Variables|Default|GetWeaponType) "NewEnumerator2") (Variables|Default|GetWeaponBuff) (Variables|Default|GetArmorPenetration) (Variables|Default|GetAccuracy) _aspawn))
    (Class|LegacyCameraShake|StartLegacyCameraShake (Game|GetPlayerCameraManager 0) "/Game/Ironsphere/Core/Player/CamShakeBlow.CamShakeBlow_C" (/ _weapondamage 1e+01) "CameraLocal" "0, 0, 0")
    (Effects|SpawnEmitteratLocation "/Game/StarterContent/Particles/P_Explosion.P_Explosion" _location "0, 0, 0" "0.100000,0.100000,0.100000")
    (Audio|SpawnSoundatLocation (Variables|Default|GetShotSound) _location "0, 0, 0" 1.0 (Math|Random|RandomFloatinRange 0.9 1.1) 0.0 0 0)
    (Variables|/Game/Ironsphere/Core/Player/BP_CharacterPlayer.BP_CharacterPlayer_C|SetShake _characterplayer_ref (+ (Variables|/Game/Ironsphere/Core/Player/BP_CharacterPlayer.BP_CharacterPlayer_C|GetShake _characterplayer_ref) (/ (Variables|Default|GetWeaponDamage) 1e+02)))
    (else
      (Development|PrintString "AmmoNotFound"))))