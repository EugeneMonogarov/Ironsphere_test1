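; Ballistic weapon actor that fires ammo-type projectiles from the player's mech, inactive in the Hangar level.
; WeaponShot sets the firing flag; Tick runs reload, fire-rate and low-energy sound timers, spending ammo and energy per shot or triggering reloads.
; ProjectileLaunch spawns the projectile along the tower's rotation, with yaw spread from accuracy and accumulated shake, plus effects.
; Randomized cooldown scales with a skill and mech bonus.
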(event EventBeginPlay
  (bind _returnvalue (Game|GetCurrentLevelName true))
  (if (not (Utilities|Enum|Equal(Enum) _returnvalue "Hangar"))
    (|CallParentFunction)
    (Variables|Default|SetOutOfAmmoInventory false)))

(event Collision|EventActorBeginOverlap
  (params (OtherActor :type Actor%20Object%20Reference))
  (|CallParentFunction 0))

(event EventTick
  (params (DeltaSeconds :type Float%20%28single-precision%29))
  (bind _returnvalue (Math|Random|RandomFloatinRange 0.7 1.3))
  (bind _gi_main_ref (Variables|Default|GetGI_main_ref))
  (bind _characterplayer_ref (Variables|Default|GetCharacterPlayer_ref))
  (bind _characterplayer_ref_2 (Variables|Default|GetCharacterPlayer_ref))
  (bind _weaponcooldown (Variables|Default|GetWeaponCooldown))
  (bind _returnvalue_2 (* _weaponcooldown _returnvalue))
  (bind _skills (Variables|/Game/Ironsphere/Core/Framework/GI_Main.GI_Main_C|GetSkills _gi_main_ref))
  (bind _output (Utilities|Array|Get(acopy) _skills 6))
  (bind _value (Utilities|Struct|BreakST_Skills _output))
  (bind _returnvalue_3 (/ _returnvalue_2 _value))
  (bind _returnvalue_4 (Game|GetCurrentLevelName true))
  (if (not (Utilities|Enum|Equal(Enum) _returnvalue_4 "Hangar"))
    (Utilities|FlowControl|Sequence
      (:then_0
        (|CallParentFunction DeltaSeconds)
        (Utilities|FlowControl|Sequence
          (:then_0
            (if (> (Variables|Default|GetReloadingTimer) 0.0)
              (Variables|Default|SetReloadingTimer (- (Variables|Default|GetReloadingTimer) DeltaSeconds))
              (else
                (Variables|Default|SetReloadingTimer 0.0)))
            (if (> (Variables|Default|GetFireRateTimer) 0.0)
              (Variables|Default|SetFireRateTimer (- (Variables|Default|GetFireRateTimer) DeltaSeconds))
              (else
                (Variables|Default|SetFireRateTimer 0.0)))
            (if (and (== (Variables|Default|GetReloadingTimer) 0.0) (== (Variables|Default|GetFireRateTimer) 0.0))
              (if (Variables|Default|GetReloading)
                (Variables|Default|SetCurrentAmmoInMag (+ (Variables|Default|GetAmmoFromInventory) (Variables|Default|GetCurrentAmmoInMag)))
                (Variables|Default|SetReloading false)
                (Variables|Default|SetAmmoFromInventory 0)
                (Audio|SpawnSoundatLocation "/Game/Ironsphere/Sound/Reload/reload_1.reload_1" (Transformation|GetActorLocation) "0, 0, 0" 0.3 1.0 0.0 0 0)
                (else
                  (Variables|Default|SetAmmoFromInventory 0)))
              (if (== (Variables|Default|GetReloadingTimer) 0.0)
                (if (> (Variables|Default|GetCurrentAmmoInMag) 0)
                  (if (< (Variables|Default|GetPowerConsumption) (Variables|/Game/Ironsphere/Core/Character/BP_CharacterBase.BP_CharacterBase_C|GetCurrentEnergy (Variables|Default|GetCharacterPlayer_ref)))
                    (if (== (Variables|Default|GetFireRateTimer) 0.0)
                      (if (Variables|Default|GetOnBallisticShooting)
                        (Variables|Default|SetCurrentAmmoInMag (- (Variables|Default|GetCurrentAmmoInMag) 1))
                        (Variables|/Game/Ironsphere/Core/Character/BP_CharacterBase.BP_CharacterBase_C|SetCurrentEnergy _characterplayer_ref (- (Variables|/Game/Ironsphere/Core/Character/BP_CharacterBase.BP_CharacterBase_C|GetCurrentEnergy _characterplayer_ref) (Variables|Default|GetPowerConsumption)))
                        (CallFunction|ProjectileLaunch)
                        (if (Utilities|Enum|Equal(Enum) (Variables|/Game/Ironsphere/Core/Player/BP_CharacterPlayer.BP_CharacterPlayer_C|GetMechBonus _characterplayer_ref_2) "NewEnumerator9")
                          (Variables|Default|SetFireRateTimer (/ _returnvalue_3 (Variables|/Game/Ironsphere/Core/Player/BP_CharacterPlayer.BP_CharacterPlayer_C|GetMechBonusValue _characterplayer_ref_2)))
                          (else
                            (Variables|Default|SetFireRateTimer _returnvalue_3)))))
                    (elif (<= (Variables|Default|GetLowEnergySoundTimer) 0.0)
                      (Audio|SpawnSound2D "/Engine/VREditor/Sounds/UI/Dockable_Window_Close.Dockable_Window_Close" 1.0 1.0 0.0 0)
                      (Variables|Default|SetLowEnergySoundTimer 1.0)))
                  (elif (not (Variables|Default|GetOutOfAmmoInventory))
                    (CallFunction|WeaponReload))))))))
      (:then_1
        (if (> (Variables|Default|GetLowEnergySoundTimer) 0.0)
          (Variables|Default|SetLowEnergySoundTimer (- (Variables|Default|GetLowEnergySoundTimer) DeltaSeconds)))))))

(fn ConstructionScript
  (|CallParentFunction))

(fn WeaponShot
  (params (Active :type Boolean))
  (Variables|Default|SetOnBallisticShooting Active)
  (|CallParentFunction Active))

(fn ProjectileLaunch
  (params (Buff :type ST%20Buff%20Structure))
  (bind _ammotype (Variables|Default|GetAmmoType))
  (bind _ammotypelist (Variables|Default|GetAmmoTypeList))
  (bind _characterplayer_ref (Variables|Default|GetCharacterPlayer_ref))
  (bind _weapondamage (Variables|Default|GetWeaponDamage))
  (bind _accuracy (Variables|Default|GetAccuracy))
  (bind _characterplayer_ref_2 (Variables|Default|GetCharacterPlayer_ref))
  (bind _arrow (Variables|Default|GetArrow))
  (bind _characterplayer_ref_3 (Variables|Default|GetCharacterPlayer_ref))
  (bind (_value _returnvalue) (Utilities|Map|Find _ammotypelist _ammotype))
  (bind _returnvalue_2 (Transformation|GetWorldTransform _arrow))
  (bind _returnvalue_3 (- 1.0 _accuracy))
  (bind _damagemultiplier (Variables|/Game/Ironsphere/Core/Character/BP_CharacterBase.BP_CharacterBase_C|GetDamageMultiplier _characterplayer_ref_3))
  (bind _towerroot1 (Variables|/Game/Ironsphere/Core/Player/BP_CharacterPlayer.BP_CharacterPlayer_C|GetTowerRoot1 _characterplayer_ref_2))
  (bind _location (Math|Transform|BreakTransform _returnvalue_2))
  (bind _returnvalue_4 (Transformation|GetWorldRotation _towerroot1))
  (bind _returnvalue_5 (* _damagemultiplier _weapondamage))
  (bind _returnvalue_6 (* _returnvalue_3 3e+01))
  (bind (_roll _pitch _yaw) (Math|Rotator|BreakRotator _returnvalue_4))
  (bind _aspawn (Utilities|Casting|CastToPawn (Components|GetOwner)))
  (if _returnvalue
    (Game|SpawnActorfromClass _value (Math|Transform|MakeTransform (.Location (Math|Transform|BreakTransform _returnvalue_2)) (Math|Rotator|MakeRotator _roll _pitch (+ _yaw (Math|Random|RandomFloatinRange (* (* (Variables|/Game/Ironsphere/Core/Player/BP_CharacterPlayer.BP_CharacterPlayer_C|GetShake (Variables|Default|GetCharacterPlayer_ref)) 6.0) -1.0) (* (Variables|/Game/Ironsphere/Core/Player/BP_CharacterPlayer.BP_CharacterPlayer_C|GetShake (Variables|Default|GetCharacterPlayer_ref)) 6.0)) (Math|Random|RandomFloatinRange (* _returnvalue_6 -1.0) _returnvalue_6)))) "AlwaysSpawn" "MultiplyWithRoot" (Components|GetOwner) (Variables|Default|GetProjectileVelocity) (Variables|Default|GetWeaponRange) _returnvalue_5 (* _damagemultiplier (Variables|Default|GetWeaponExplosionDamage)) (Variables|Default|GetWeaponExplosionRadius) (Utilities|Enum|Equal(Enum) (Variables|Default|GetWeaponType) "NewEnumerator2") (Variables|Default|GetWeaponBuff) (Variables|Default|GetArmorPenetration) (Variables|Default|GetAccuracy) _aspawn)
    (Class|LegacyCameraShake|StartLegacyCameraShake (Game|GetPlayerCameraManager 0) "/Game/Ironsphere/Core/Player/CamShakeBlow.CamShakeBlow_C" (* _weapondamage 0.06) "CameraLocal" "0, 0, 0")
    (Effects|SpawnEmitteratLocation "/Game/StarterContent/Particles/P_Explosion.P_Explosion" _location "0, 0, 0" (Math|Conversions|ToVector(Float) (* (Math|Float|Sqrt _returnvalue_5) 0.02)))
    (Audio|SpawnSoundatLocation (Variables|Default|GetShotSound) _location "0, 0, 0" 1.0 (Math|Random|RandomFloatinRange 0.9 1.1) 0.0 "/Game/Ironsphere/Sound/SA_Default3d.SA_Default3d" 0)
    (Variables|/Game/Ironsphere/Core/Player/BP_CharacterPlayer.BP_CharacterPlayer_C|SetShake _characterplayer_ref (+ (Variables|/Game/Ironsphere/Core/Player/BP_CharacterPlayer.BP_CharacterPlayer_C|GetShake _characterplayer_ref) (/ (Variables|Default|GetWeaponDamage) 1e+02)))
    (else
      (Development|PrintString "AmmoNotFound"))))