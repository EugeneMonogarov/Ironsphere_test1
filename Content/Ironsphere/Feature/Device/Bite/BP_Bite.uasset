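; BP_Bite is a device actor that registers itself as an enemy of every NPC in the level, apparently serving as a damageable decoy.
; On BeginPlay it plays a pitched-up reload sound, then adds itself to the Enemy array of each existing BP_NPC_Base actor.
; The same loop makes its HP bar widget visible, so this happens only if NPCs are present.
; Destruction simply defers to the parent class.
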(event EventBeginPlay
  (|CallParentFunction)
  (Audio|SpawnSoundatLocation "/Game/Ironsphere/Sound/Reload/reload_3.reload_3" (Transformation|GetActorLocation) "0, 0, 0" 0.4 1.4 0.5 0 0)
  (bind _outactors (Actor|GetAllActorsOfClass "/Game/Ironsphere/Feature/NPC/BP_NPC_Base.BP_NPC_Base_C"))
  (for _array_element _outactors
    (Utilities|Array|AddUnique (Variables|/Game/Ironsphere/Feature/NPC/BP_NPC_Base.BP_NPC_Base_C|GetEnemy _array_element) self)
    (Rendering|SetVisibility (Variables|Default|Getwidget_HPbar) true false)))

(event Collision|EventActorBeginOverlap
  (params (OtherActor :type Actor%20Object%20Reference))
  (|CallParentFunction OtherActor) ; This node is disabled and will not be called.\nDrag off pins to build functionality.
)

(event EventTick
  (params (DeltaSeconds :type Float%20%28single-precision%29))
  (|CallParentFunction DeltaSeconds) ; This node is disabled and will not be called.\nDrag off pins to build functionality.
)

(fn ConstructionScript
  (|CallParentFunction))

(fn Destruction
  (params (IsBlow :type Boolean) (Damage :type Float%20%28double-precision%29) (Radius :type Float%20%28double-precision%29) (Sound :type SoundDestroy%20Enum :default "NewEnumerator0"))
  (|CallParentFunction IsBlow Damage Radius Sound))