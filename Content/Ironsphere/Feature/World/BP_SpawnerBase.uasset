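; Spawner actor that endlessly spawns BP_DesertSpider AI at its SpawnPoint, at an accelerating rate.
; BeginPlay spawns the first spider after a short delay, then enters a looping Delay driven by SpawnCooldown.
; Each pass shrinks the cooldown by a fixed factor while it is above SpawnCooldownMinimal, then spawns another spider.
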(event Collision|EventActorBeginOverlap
  (params (OtherActor :type Actor%20Object%20Reference))
  (|CallParentFunction OtherActor) ; This node is disabled and will not be called.\nDrag off pins to build functionality.
)

(event EventTick
  (params (DeltaSeconds :type Float%20%28single-precision%29)))

(event EventBeginPlay
  (bind _spawnpoint (Variables|Default|GetSpawnPoint))
  (bind _returnvalue (Transformation|GetWorldTransform _spawnpoint))
  (bind _location (Math|Transform|BreakTransform _returnvalue))
  (bind _returnvalue_2 (+ _location "0.000000,0.000000,-0.000000"))
  (bind _returnvalue_3 (* _returnvalue_2 "1.000000,1.000000,1.000000"))
  (Utilities|FlowControl|Delay 1.0)
  (AI|SpawnAIFromClass "/Game/Ironsphere/Feature/NPC/BP_DesertSpider.BP_DesertSpider_C" 0 _returnvalue_3 "0, 0, 0" false 0)
  (Utilities|FlowControl|Delay (Variables|Default|GetSpawnCooldown) :!label _label)
  (if (< (Variables|Default|GetSpawnCooldownMinimal) (Variables|Default|GetSpawnCooldown))
    (Variables|Default|SetSpawnCooldown (* (Variables|Default|GetSpawnCooldown) 0.8)))
  (AI|SpawnAIFromClass "/Game/Ironsphere/Feature/NPC/BP_DesertSpider.BP_DesertSpider_C" 0 _returnvalue_3 "0, 0, 0" false 0)
  (goto _label))

(fn ConstructionScript
  (|CallParentFunction))