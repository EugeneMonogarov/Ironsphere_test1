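; BP_Shield1 is a world shield actor in Ironsphere that decays over time, building on logic from its parent class.
; On BeginPlay it plays a spawn sound at its location and shows its HP bar widget.
; Each tick it drains CurrentHP at a fixed rate, then calls Destruction with a sound type and destroys itself once HP runs out.
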(event EventBeginPlay
  (|CallParentFunction)
  (Audio|SpawnSoundatLocation "/Engine/VREditor/Sounds/UI/Teleport_Mode_Entered.Teleport_Mode_Entered" (Transformation|GetActorLocation) "0, 0, 0" 1.0 1.0 0.0 0 0)
  (Rendering|SetVisibility (Variables|Default|Getwidget_HPbar) true false))

(event Collision|EventActorBeginOverlap
  (params (OtherActor :type Actor%20Object%20Reference))
  (|CallParentFunction OtherActor) ; This node is disabled and will not be called.\nDrag off pins to build functionality.
)

(event EventTick
  (params (DeltaSeconds :type Float%20%28single-precision%29))
  (|CallParentFunction DeltaSeconds)
  (bind _output_get (Variables|Default|SetCurrentHP (- (Variables|Default|GetCurrentHP) (* DeltaSeconds 3.0))))
  (if (<= _output_get 0.0)
    (CallFunction|Destruction false 0.0 0.0 "NewEnumerator4")
    (Actor|DestroyActor)))

(fn ConstructionScript
  (|CallParentFunction))