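; World prop actor that dresses itself as a randomized dead worm skeleton on BeginPlay.
; It picks one of 17 meshes (the last two switch cases are unreachable), then randomizes mesh scale and rotation.
; It usually spawns another actor, class not shown, at a random horizontal offset with jittered scale.
; A downward sphere trace from a fixed world height snaps it onto WorldStatic geometry, or destroys it when nothing is hit.
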(event EventBeginPlay
  (bind _returnvalue (Transformation|GetActorTransform))
  (bind _returnvalue_2 (Math|Random|RandomFloatinRange 0.9 1.1))
  (bind _returnvalue_3 (Math|Random|RandomFloatinRange 1.9 2.2))
  (bind _self self)
  (bind _skel (Variables|Default|GetSkel))
  (bind _skel_2 (Variables|Default|GetSkel))
  (bind _skel_3 (Variables|Default|GetSkel))
  (bind _skel_4 (Variables|Default|GetSkel))
  (bind (_location _rotation _scale) (Math|Transform|BreakTransform _returnvalue))
  (bind _returnvalue_4 (Transformation|GetActorTransform _self))
  (bind _returnvalue_5 (Transformation|GetActorLocation _self))
  (bind (_x _y) (Math|Vector|BreakVector _returnvalue_5))
  (bind (_x_2 _y_2 _z) (Math|Vector|BreakVector _returnvalue_5))
  (bind (_location_2 _rotation_2 _scale_2) (Math|Transform|BreakTransform _returnvalue_4))
  (Utilities|FlowControl|Sequence
    (:then_0
      (switch int (Math|Random|RandomIntegerinRange 1 17)
        (:1
          (Components|StaticMesh|SetStaticMesh _skel_3 "/Game/Ironsphere/3D/Meshes/Props/DeadWormSkeletons/DeadWormSkeletons_DeadwormSkel000.DeadWormSkeletons_DeadwormSkel000"))
        (:2
          (Components|StaticMesh|SetStaticMesh _skel_3 "/Game/Ironsphere/3D/Meshes/Props/DeadWormSkeletons/DeadWormSkeletons_DeadwormSkel001.DeadWormSkeletons_DeadwormSkel001"))
        (:3
          (Components|StaticMesh|SetStaticMesh _skel_3 "/Game/Ironsphere/3D/Meshes/Props/DeadWormSkeletons/DeadWormSkeletons_DeadwormSkel002.DeadWormSkeletons_DeadwormSkel002"))
        (:4
          (Components|StaticMesh|SetStaticMesh _skel_3 "/Game/Ironsphere/3D/Meshes/Props/DeadWormSkeletons/DeadWormSkeletons_DeadwormSkel003.DeadWormSkeletons_DeadwormSkel003"))
        (:5
          (Components|StaticMesh|SetStaticMesh _skel_3 "/Game/Ironsphere/3D/Meshes/Props/DeadWormSkeletons/DeadWormSkeletons_DeadwormSkel004.DeadWormSkeletons_DeadwormSkel004"))
        (:6
          (Components|StaticMesh|SetStaticMesh _skel_3 "/Game/Ironsphere/3D/Meshes/Props/DeadWormSkeletons/DeadWormSkeletons_DeadwormSkel005.DeadWormSkeletons_DeadwormSkel005"))
        (:7
          (Components|StaticMesh|SetStaticMesh _skel_4 "/Game/Ironsphere/3D/Meshes/Props/DeadWormSkeletons/DeadWormSkeletons_DeadwormSkel006.DeadWormSkeletons_DeadwormSkel006"))
        (:8
          (Components|StaticMesh|SetStaticMesh _skel_4 "/Game/Ironsphere/3D/Meshes/Props/DeadWormSkeletons/DeadWormSkeletons_DeadwormSkel007.DeadWormSkeletons_DeadwormSkel007"))
        (:9
          (Components|StaticMesh|SetStaticMesh _skel_4 "/Game/Ironsphere/3D/Meshes/Props/DeadWormSkeletons/DeadWormSkeletons_DeadwormSkel008.DeadWormSkeletons_DeadwormSkel008"))
        (:10
          (Components|StaticMesh|SetStaticMesh _skel_4 "/Game/Ironsphere/3D/Meshes/Props/DeadWormSkeletons/DeadWormSkeletons_DeadwormSkel009.DeadWormSkeletons_DeadwormSkel009"))
        (:11
          (Components|StaticMesh|SetStaticMesh _skel_4 "/Game/Ironsphere/3D/Meshes/Props/DeadWormSkeletons/DeadWormSkeletons_DeadwormSkel010.DeadWormSkeletons_DeadwormSkel010"))
        (:12
          (Components|StaticMesh|SetStaticMesh _skel_4 "/Game/Ironsphere/3D/Meshes/Props/DeadWormSkeletons/DeadWormSkeletons_DeadwormSkel011.DeadWormSkeletons_DeadwormSkel011"))
        (:13
          (Components|StaticMesh|SetStaticMesh _skel_2 "/Game/Ironsphere/3D/Meshes/Props/DeadWormSkeletons/DeadWormSkeletons_DeadwormSkel012.DeadWormSkeletons_DeadwormSkel012"))
        (:14
          (Components|StaticMesh|SetStaticMesh _skel_2 "/Game/Ironsphere/3D/Meshes/Props/DeadWormSkeletons/DeadWormSkeletons_DeadwormSkel013.DeadWormSkeletons_DeadwormSkel013"))
        (:15
          (Components|StaticMesh|SetStaticMesh _skel_2 "/Game/Ironsphere/3D/Meshes/Props/DeadWormSkeletons/DeadWormSkeletons_DeadwormSkel014.DeadWormSkeletons_DeadwormSkel014"))
        (:16
          (Components|StaticMesh|SetStaticMesh _skel_2 "/Game/Ironsphere/3D/Meshes/Props/DeadWormSkeletons/DeadWormSkeletons_DeadwormSkel015.DeadWormSkeletons_DeadwormSkel015"))
        (:17
          (Components|StaticMesh|SetStaticMesh _skel_2 "/Game/Ironsphere/3D/Meshes/Props/DeadWormSkeletons/DeadWormSkeletons_DeadwormSkel016.DeadWormSkeletons_DeadwormSkel016"))
        (:18
          (Components|StaticMesh|SetStaticMesh _skel_2 "/Game/Ironsphere/3D/Meshes/Props/DeadWormSkeletons/DeadWormSkeletons_DeadwormSkel017.DeadWormSkeletons_DeadwormSkel017"))
        (:19
          (Components|StaticMesh|SetStaticMesh _skel_2 "/Game/Ironsphere/3D/Meshes/Props/DeadWormSkeletons/DeadWormSkeletons_DeadwormSkel018.DeadWormSkeletons_DeadwormSkel018"))))
    (:then_1
      (Transformation|SetRelativeScale3D _skel (Math|Vector|MakeVector _returnvalue_3 _returnvalue_3 _returnvalue_3))
      (Transformation|SetRelativeRotation _skel (Math|Random|RandomRotator false) false false))
    (:then_2
      (if (> (Math|Random|RandomIntegerinRange 0 12) 2)
        (Game|SpawnActorfromClass "BP_Skeletons_C" (Math|Transform|MakeTransform (+ _location (* (Math|Random|RandomUnitVector) "222.000000,222.000000,0.000000")) "0, 0, 0" (* _scale (Math|Vector|MakeVector _returnvalue_2 _returnvalue_2 _returnvalue_2))) "Undefined" "MultiplyWithRoot" 0 0)))
    (:then_3
      (bind (_outhit _returnvalue_6) (Collision|SphereTraceForObjects (Math|Vector|MakeVector _x _y 5.0) (Math|Vector|MakeVector _x_2 _y_2 (- _z 3e+02)) 0.0 (Utilities|Array|MakeArray "ObjectTypeQuery1") false (Utilities|Array|MakeArray _self) "None"))
      (if _returnvalue_6
        (Transformation|SetActorTransform (Math|Transform|MakeTransform (.Location (Collision|BreakHitResult _outhit)) _rotation_2 _scale_2))
        (else
          (Actor|DestroyActor))))))

(event Collision|EventActorBeginOverlap
  (params (OtherActor :type Actor%20Object%20Reference)))

(event EventTick
  (params (DeltaSeconds :type Float%20%28single-precision%29)))

(fn ConstructionScript)