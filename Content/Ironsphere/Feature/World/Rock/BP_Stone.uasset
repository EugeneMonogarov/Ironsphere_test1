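; BP_Stone is a damageable world rock that randomizes its appearance and durability on BeginPlay.
; It picks a mesh through random branches (Rock4 is unreachable behind a constant-true branch), then applies random yaw and horizontal actor scale.
; CurrentHP and MaxHP get separate random multipliers, and the Rock component's world scale is finally set uniformly from Scale.
; Damage calls the parent and SoundDamage, while Destruction defers to the parent.
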(event EventBeginPlay
  (bind _returnvalue (Math|Random|RandomFloatinRange 0.8 1.2))
  (bind _returnvalue_2 (Math|Random|RandomFloatinRange 0.8 1.2))
  (bind _rock (Variables|Default|GetRock))
  (|CallParentFunction)
  (Utilities|FlowControl|Sequence
    (:then_0
      (if (Math|Random|RandomBool)
        (if (Math|Random|RandomBool)
          (Components|StaticMesh|SetStaticMesh _rock "/Game/Ironsphere/3D/Meshes/Props/Rock/Rock1.Rock1")
          (else
            (Components|StaticMesh|SetStaticMesh _rock "/Game/Ironsphere/3D/Meshes/Props/Rock/Rock2.Rock2")))
        (elif true
          (Components|StaticMesh|SetStaticMesh _rock "/Game/Ironsphere/3D/Meshes/Props/Rock/Rock3.Rock3")
          (else
            (Components|StaticMesh|SetStaticMesh _rock "/Game/Ironsphere/3D/Meshes/Props/Rock/Rock4.Rock4")))))
    (:then_1
      (Transformation|SetActorRotation (Math|Rotator|MakeRotator 0.0 0.0 (.Yaw (Math|Rotator|BreakRotator (Math|Random|RandomRotator false)))))
      (Transformation|SetActorScale3D (Math|Vector|MakeVector _returnvalue_2 _returnvalue 1.0))
      (Variables|Default|SetCurrentHP (* (Variables|Default|GetMaxHP) (* _returnvalue_2 _returnvalue)))
      (Variables|Default|SetMaxHP (* (Variables|Default|GetMaxHP) (* _returnvalue_2 _returnvalue))))
    (:then_2
      (Transformation|SetWorldScale3D (Variables|Default|GetRock) (Math|Conversions|ToVector(Float) (* (Variables|Default|Getscale) 2.0))))))

(event Collision|EventActorBeginOverlap
  (params (OtherActor :type Actor%20Object%20Reference))
  (|CallParentFunction OtherActor) ; This node is disabled and will not be called.\nDrag off pins to build functionality.
)

(event EventTick
  (params (DeltaSeconds :type Float%20%28single-precision%29))
  (|CallParentFunction DeltaSeconds) ; This node is disabled and will not be called.\nDrag off pins to build functionality.
)

(event EventAnyDamage
  (params (Damage :type Float%20%28single-precision%29) (DamageType :type Damage%20Type%20Object%20Reference) (InstigatedBy :type Controller%20Object%20Reference) (DamageCauser :type Actor%20Object%20Reference))
  (|CallParentFunction Damage DamageType InstigatedBy DamageCauser)
  (CallFunction|SoundDamage "NewEnumerator1"))

(fn ConstructionScript
  (|CallParentFunction))

(fn Destruction
  (params (IsBlow :type Boolean) (Damage :type Float%20%28double-precision%29) (Radius :type Float%20%28double-precision%29) (Sound :type SoundDestroy%20Enum :default "NewEnumerator0"))
  (|CallParentFunction false 0.0 0.0 "NewEnumerator0"))