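; Den objective that acts as an enemy spawner with an HP bar and minimap markers.
; On BeginPlay it places a spawner icon on the minimap by scaling its world location to screen space, plus an objective icon if flagged.
; It then endlessly spawns staggered NPC packs at random points within a radius, multiplying the cooldown by a falloff each wave down to a minimum.
; KillWidgets hides the minimap markers.
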(event Collision|EventActorBeginOverlap
  (params (OtherActor :type Actor%20Object%20Reference))
  (|CallParentFunction OtherActor) ; This node is disabled and will not be called.\nDrag off pins to build functionality.
)

(event EventTick
  (params (DeltaSeconds :type Float%20%28single-precision%29)))

(event EventBeginPlay
  (bind _returnvalue (Transformation|GetActorLocation))
  (bind _spawnradius (Variables|Default|GetSpawnRadius))
  (bind (_x _y) (Math|Vector|BreakVector _returnvalue))
  (bind _returnvalue_2 (* _x -0.1))
  (bind _returnvalue_3 (* _y -0.1))
  (bind _returnvalue_4 (+ _returnvalue_2 2e+02))
  (bind _returnvalue_5 (+ _returnvalue_3 2e+02))
  (bind _returnvalue_6 (Math|Vector2D|MakeVector2D _returnvalue_4 _returnvalue_5))
  (Utilities|FlowControl|Delay 0.2)
  (|CallParentFunction)
  (Rendering|SetVisibility (Variables|Default|Getwidget_HPbar) true false)
  (bind _returnvalue_7 (UserInterface|CreateWidget "/Game/Ironsphere/UI/Ingame/Map/WBS_MinimapObject.WBS_MinimapObject_C" 0 "/Game/Ironsphere/UI/Ingame/Spawner.Spawner"))
  (Variables|Default|SetMarker _returnvalue_7)
  (UserInterface|Viewport|AddtoViewport _returnvalue_7 0)
  (Class|UserWidget|SetPositioninViewport _returnvalue_7 _returnvalue_6 true)
  (if (Variables|Default|GetObjective)
    (bind _returnvalue_8 (UserInterface|CreateWidget "/Game/Ironsphere/UI/Ingame/Map/WBS_MinimapObject.WBS_MinimapObject_C" 0 "/Game/Ironsphere/UI/Ingame/Map/Objective.Objective"))
    (Variables|Default|SetObjectiveMarker _returnvalue_8)
    (UserInterface|Viewport|AddtoViewport _returnvalue_8 0)
    (Class|UserWidget|SetPositioninViewport _returnvalue_8 _returnvalue_6 true))
  (Utilities|FlowControl|Delay 1.0)
  (Utilities|FlowControl|Delay (Variables|Default|GetSpawnCooldown) :!label _label)
  (if (< (Variables|Default|GetSpawnCooldownMinimal) (Variables|Default|GetSpawnCooldown))
    (Variables|Default|SetSpawnCooldown (* (Variables|Default|GetSpawnCooldown) (Variables|Default|GetSpawnFalloff)))
    (else
      (Variables|Default|SetSpawnCooldown (Variables|Default|GetSpawnCooldownMinimal))))
  (Variables|Default|SetCount (Variables|Default|GetPack))
  (if (> (Variables|Default|GetCount) 0) :!label _label_2
    (AI|SpawnAIFromClass (Variables|Default|GetNPC) 0 (.Location (Math|Transform|BreakTransform (Math|Conversions|ToTransform(Vector) (+ (+ (* (Math|Random|RandomUnitVector) (Math|Vector|MakeVector _spawnradius _spawnradius 0.0)) "0.000000,0.000000,10.000000") (Transformation|GetActorLocation))))) "0, 0, 0" true 0)
    (Utilities|FlowControl|Delay (Math|Random|RandomFloatinRange 0.1 0.4))
    (Variables|Default|SetCount (- (Variables|Default|GetCount) 1))
    (goto _label_2)
    (else
      (goto _label))))

(fn ConstructionScript
  (|CallParentFunction))

(fn KillWidgets
  (if (Variables|Default|GetObjective)
    (Widget|SetVisibility (Variables|Default|GetObjectiveMarker) "Hidden"))
  (Widget|SetVisibility (Variables|Default|GetMarker) "Hidden"))