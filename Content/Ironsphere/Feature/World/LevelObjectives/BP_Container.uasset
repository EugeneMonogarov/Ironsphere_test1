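; BP_Container is a crate pickup in a level that grants the player money when their controlled mech overlaps it.
; On BeginPlay it hides its HP bar and adds a Crate minimap widget, positioned from its world location.
; Pickup adds a bonus scaled from the level's reward to GI_Main, rewrites Progress unchanged, hides the icon and destroys the actor.
; Its Destruction override only clears IsAlive, skipping the parent logic.
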(event OnComponentBeginOverlap(PickUp)
  (params (OverlappedComponent :type Primitive%20Component%20Object%20Reference) (OtherActor :type Actor%20Object%20Reference) (OtherComp :type Primitive%20Component%20Object%20Reference) (OtherBodyIndex :type Integer) (bFromSweep :type Boolean) (SweepResult :type Hit%20Result%20Structure%20%28by%20ref%29))
  (bind _aspc_ingame (Utilities|Casting|CastToPC_Ingame (Game|GetPlayerController 0))
    (:then
      (if (== (Variables|/Game/Ironsphere/Core/Framework/Battle/PC_Ingame.PC_Ingame_C|GetControlledMech _aspc_ingame) OtherActor)
        (Audio|SpawnSound2D "/Game/Ironsphere/Sound/Reload/reload_1.reload_1" 1.0 0.8 0.0 0)
        (bind _asgi_main (Utilities|Casting|CastToGI_Main (Game|GetGameInstance)))
        (Variables|/Game/Ironsphere/Core/Framework/GI_Main.GI_Main_C|SetMoney _asgi_main (+ (Variables|/Game/Ironsphere/Core/Framework/GI_Main.GI_Main_C|GetMoney _asgi_main) (+ (/ (.MoneyReward (Utilities|Struct|BreakST_Level (Utilities|Array|Get(acopy) (Variables|/Game/Ironsphere/Core/Framework/GI_Main.GI_Main_C|GetLevels _asgi_main) (Variables|/Game/Ironsphere/Core/Framework/GI_Main.GI_Main_C|GetCurrentLevelIndex _asgi_main)))) 5.0) 5e+01)))
        (Utilities|Array|SetArrayElem (Variables|/Game/Ironsphere/Core/Framework/GI_Main.GI_Main_C|GetProgress _asgi_main) (Variables|/Game/Ironsphere/Core/Framework/GI_Main.GI_Main_C|GetCurrentLevelIndex _asgi_main) (Utilities|Struct|MakeST_Progress (.Open (Utilities|Struct|BreakST_Progress (Utilities|Array|Get(acopy) (Variables|/Game/Ironsphere/Core/Framework/GI_Main.GI_Main_C|GetProgress _asgi_main) (Variables|/Game/Ironsphere/Core/Framework/GI_Main.GI_Main_C|GetCurrentLevelIndex _asgi_main)))) (.Passed (Utilities|Struct|BreakST_Progress (Utilities|Array|Get(acopy) (Variables|/Game/Ironsphere/Core/Framework/GI_Main.GI_Main_C|GetProgress _asgi_main) (Variables|/Game/Ironsphere/Core/Framework/GI_Main.GI_Main_C|GetCurrentLevelIndex _asgi_main)))) (.BonusReceived (Utilities|Struct|BreakST_Progress (Utilities|Array|Get(acopy) (Variables|/Game/Ironsphere/Core/Framework/GI_Main.GI_Main_C|GetProgress _asgi_main) (Variables|/Game/Ironsphere/Core/Framework/GI_Main.GI_Main_C|GetCurrentLevelIndex _asgi_main)))) (.KillReward (Utilities|Struct|BreakST_Progress (Utilities|Array|Get(acopy) (Variables|/Game/Ironsphere/Core/Framework/GI_Main.GI_Main_C|GetProgress _asgi_main) (Variables|/Game/Ironsphere/Core/Framework/GI_Main.GI_Main_C|GetCurrentLevelIndex _asgi_main))))))
        (Widget|SetVisibility (Variables|Default|GetObject%20Map) "Hidden")
        (Actor|DestroyActor)))
    (:CastFailed
      (Audio|SpawnSound2D "/Engine/EditorSounds/Notifications/CompileFailed_Cue.CompileFailed_Cue" 1.0 1.0 0.0 0))))

(event EventBeginPlay
  (bind _returnvalue (Transformation|GetActorLocation))
  (bind (_x _y) (Math|Vector|BreakVector _returnvalue))
  (|CallParentFunction)
  (Rendering|SetVisibility (Variables|Default|Getwidget_HPbar) false false)
  (bind _returnvalue_2 (UserInterface|CreateWidget "/Game/Ironsphere/UI/Ingame/Map/WBS_MinimapObject.WBS_MinimapObject_C" 0 "/Game/Ironsphere/UI/Ingame/Map/Crate.Crate"))
  (Variables|Default|SetObject%20Map _returnvalue_2)
  (UserInterface|Viewport|AddtoViewport _returnvalue_2 1)
  (Class|UserWidget|SetPositioninViewport _returnvalue_2 (Math|Vector2D|MakeVector2D (+ (* _x -0.1) 2e+02) (+ (* _y -0.1) 2e+02)) true))

(event Collision|EventActorBeginOverlap
  (params (OtherActor :type Actor%20Object%20Reference)))

(event EventTick
  (params (DeltaSeconds :type Float%20%28single-precision%29))
  (|CallParentFunction DeltaSeconds)
  (CallFunction|UpdateHPbar))

(fn ConstructionScript)

(fn UpdateHPbar
  (|CallParentFunction))

(fn Destruction
  (params (IsBlow :type Boolean) (Damage :type Float%20%28double-precision%29) (Radius :type Float%20%28double-precision%29))
  (Variables|Default|SetIsAlive false))