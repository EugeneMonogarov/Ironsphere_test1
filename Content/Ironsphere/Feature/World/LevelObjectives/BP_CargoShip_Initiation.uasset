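; BP_CargoShip_Initiation is a cargo ship level objective that becomes active once no fuel barrel objectives remain in the level.
; Tick updates the inherited HP bar and polls for remaining BP_FuelBarrel_objective actors until it sets IsObjective.
; Once active, it creates a minimap objective widget a single time, positioned from its scaled world location.
; Its Destruction override only clears IsAlive, leaving the parent's destruction logic uncalled.
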(event EventBeginPlay
  (|CallParentFunction)
  (Rendering|SetVisibility (Variables|Default|Getwidget_HPbar) true false))

(event Collision|EventActorBeginOverlap
  (params (OtherActor :type Actor%20Object%20Reference)))

(event EventTick
  (params (DeltaSeconds :type Float%20%28single-precision%29))
  (bind _returnvalue (Transformation|GetActorLocation))
  (bind (_x _y) (Math|Vector|BreakVector _returnvalue))
  (|CallParentFunction DeltaSeconds)
  (CallFunction|UpdateHPbar)
  (if (Variables|Default|GetIsObjective)
    (Utilities|FlowControl|DoOnce false
      (:Completed
        (bind _returnvalue_2 (UserInterface|CreateWidget "/Game/Ironsphere/UI/Ingame/Map/WBS_MinimapObject.WBS_MinimapObject_C" 0 "/Game/Ironsphere/UI/Ingame/Map/Objective.Objective"))
        (Variables|Default|SetObjectMap _returnvalue_2)
        (UserInterface|Viewport|AddtoViewport _returnvalue_2 1)
        (Class|UserWidget|SetPositioninViewport _returnvalue_2 (Math|Vector2D|MakeVector2D (+ (* _x -0.1) 2e+02) (+ (* _y -0.1) 2e+02)) true)))
    (else
      (bind _outactors (Actor|GetAllActorsOfClass "/Game/Ironsphere/Feature/World/LevelObjectives/BP_FuelBarrel_objective.BP_FuelBarrel_objective_C"))
      (if (not (> (Utilities|Array|Length _outactors) 0))
        (Variables|Default|SetIsObjective true)))))

(fn ConstructionScript)

(fn UpdateHPbar
  (|CallParentFunction))

(fn Destruction
  (params (IsBlow :type Boolean) (Damage :type Float%20%28double-precision%29) (Radius :type Float%20%28double-precision%29) (Sound :type Boolean))
  (Variables|Default|SetIsAlive false))