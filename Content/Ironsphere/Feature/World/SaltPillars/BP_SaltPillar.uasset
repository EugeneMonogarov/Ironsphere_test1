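; Salt pillar world prop that grows itself into a randomized cluster at BeginPlay.
; Each pillar picks one of eight meshes with random scale and yaw, then very likely spawns another copy at its position, chaining recursively.
; Only afterward does it shift a short random distance, so the chain scatters around the origin.
; A vertical sphere trace snaps it onto low WorldStatic surfaces, destroying it on a miss or higher hit.
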(event EventBeginPlay
  (bind _returnvalue (Math|Random|RandomFloatinRange 0.6 1.5))
  (bind _returnvalue_2 (Math|Random|RandomFloatinRange 0.9 1.2))
  (bind _self self)
  (bind _smallstone1 (Variables|Default|GetSmallStone1))
  (bind _smallstone1_2 (Variables|Default|GetSmallStone1))
  (bind _returnvalue_3 (Math|Float|Power _returnvalue_2 5.0))
  (bind _returnvalue_4 (Transformation|GetActorTransform _self))
  (bind (_location _rotation _scale) (Math|Transform|BreakTransform _returnvalue_4))
  (Utilities|FlowControl|Sequence
    (:then_0
      (switch int (Math|Random|RandomIntegerinRange 1 8)
        (:1
          (Components|StaticMesh|SetStaticMesh _smallstone1_2 "/Game/Ironsphere/3D/Meshes/Props/SaltPillars/SaltPillars_Cylinder017.SaltPillars_Cylinder017"))
        (:2
          (Components|StaticMesh|SetStaticMesh _smallstone1_2 "/Game/Ironsphere/3D/Meshes/Props/SaltPillars/SaltPillars_Cylinder018.SaltPillars_Cylinder018"))
        (:3
          (Components|StaticMesh|SetStaticMesh _smallstone1_2 "/Game/Ironsphere/3D/Meshes/Props/SaltPillars/SaltPillars_Cylinder019.SaltPillars_Cylinder019"))
        (:4
          (Components|StaticMesh|SetStaticMesh _smallstone1_2 "/Game/Ironsphere/3D/Meshes/Props/SaltPillars/SaltPillars_Cylinder020.SaltPillars_Cylinder020"))
        (:5
          (Components|StaticMesh|SetStaticMesh _smallstone1_2 "/Game/Ironsphere/3D/Meshes/Props/SaltPillars/SaltPillars_Cylinder021.SaltPillars_Cylinder021"))
        (:6
          (Components|StaticMesh|SetStaticMesh _smallstone1_2 "/Game/Ironsphere/3D/Meshes/Props/SaltPillars/SaltPillars_Cylinder022.SaltPillars_Cylinder022"))
        (:7
          (Components|StaticMesh|SetStaticMesh _smallstone1_2 "/Game/Ironsphere/3D/Meshes/Props/SaltPillars/SaltPillars_Cylinder023.SaltPillars_Cylinder023"))
        (:8
          (Components|StaticMesh|SetStaticMesh _smallstone1_2 "/Game/Ironsphere/3D/Meshes/Props/SaltPillars/SaltPillars_Cylinder024.SaltPillars_Cylinder024"))))
    (:then_1
      (Transformation|SetRelativeScale3D _smallstone1 (Math|Vector|MakeVector _returnvalue_3 _returnvalue_3 _returnvalue_3))
      (Transformation|SetRelativeRotation _smallstone1 (Math|Rotator|MakeRotator 0.0 0.0 (Math|Random|RandomFloatinRange 0.0 3.6e+02)) false false))
    (:then_2
      (if (> (Math|Random|RandomIntegerinRange 0 33) 2)
        (Game|SpawnActorfromClass "BP_SaltPillar_C" (Math|Transform|MakeTransform (.Location (Math|Transform|BreakTransform (Transformation|GetActorTransform))) "0, 0, 0" (Math|Vector|MakeVector _returnvalue _returnvalue (Math|Random|RandomFloatinRange 0.6 1.8))) "Undefined" "MultiplyWithRoot" 0 0)))
    (:then_3
      (Transformation|SetActorTransform (Math|Transform|MakeTransform (+ (* (Math|Random|RandomUnitVector) (Math|Random|RandomFloatinRange 15.0 55.0)) _location) _rotation _scale))
      (bind (_outhit _returnvalue_5) (Collision|SphereTraceForObjects (+ (Transformation|GetActorLocation) "0.000000,0.000000,300.000000") (+ (Transformation|GetActorLocation) "0.000000,0.000000,-300.000000") 0.0 (Utilities|Array|MakeArray "ObjectTypeQuery1") false (Utilities|Array|MakeArray _self) "None"))
      (if _returnvalue_5
        (if (< (.Z (Math|Vector|BreakVector (.Location (Collision|BreakHitResult _outhit)))) 2.0)
          (Transformation|SetActorLocation (.Location (Collision|BreakHitResult _outhit)) false false)
          (else
            (Actor|DestroyActor :!label _label)))
        (else
          (goto _label))))))

(event Collision|EventActorBeginOverlap
  (params (OtherActor :type Actor%20Object%20Reference)))

(event EventTick
  (params (DeltaSeconds :type Float%20%28single-precision%29)))

(fn ConstructionScript)