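; Spawner actor that scatters salt pillars around the world origin when play begins.
; BeginPlay runs a fixed-count loop, picking random X and Y within a square area at a fixed height and spawning BP_SaltPillar there.
; Positions are world-space, not relative to the spawner, and colliding spawns are skipped, so the pillar count varies.
; The non-zero check on X and Y rejects only exact zeros.
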(event EventBeginPlay
  (for _index (range 0 33)
    (bind _output_get (Variables|Default|SetRand1 (Math|Random|RandomFloatinRange -1.2e+03 1.2e+03)))
    (bind _output_get_2 (Variables|Default|SetRand2 (Math|Random|RandomFloatinRange -1.2e+03 1.2e+03)))
    (if (and (> (Math|Float|Absolute(Float) _output_get_2) 0.0) (> (Math|Float|Absolute(Float) _output_get) 0.0))
      (Game|SpawnActorfromClass "/Game/Ironsphere/Feature/World/SaltPillars/BP_SaltPillar.BP_SaltPillar_C" (Math|Transform|MakeTransform (Math|Vector|MakeVector _output_get _output_get_2 1e+02)) "DontSpawnIfColliding" "MultiplyWithRoot" 0 0))))

(event Collision|EventActorBeginOverlap
  (params (OtherActor :type Actor%20Object%20Reference)))

(event EventTick
  (params (DeltaSeconds :type Float%20%28single-precision%29)))

(fn ConstructionScript)