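; BP_Hide is a damageable world spawner that releases a batch of worms once, after a randomized hiding time.
; On BeginPlay it hides its HP bar, waits for the ingame player controller, then delays around UnhideTime.
; It holds spawning until the player's mech is clear of the capsule, then spawns NumberOfWorms AI at staggered intervals, scattered nearby at world Z zero.
; Damage and destruction defer to the parent class.
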(event Game|Damage|EventAnyDamage
  (params (Damage :type Float%20%28single-precision%29) (DamageType :type Damage%20Type%20Object%20Reference) (InstigatedBy :type Controller%20Object%20Reference) (DamageCauser :type Actor%20Object%20Reference))
  (|CallParentFunction Damage DamageType InstigatedBy DamageCauser))

(event Collision|EventActorBeginOverlap
  (params (OtherActor :type Actor%20Object%20Reference))
  (|CallParentFunction OtherActor) ; This node is disabled and will not be called.\nDrag off pins to build functionality.
)

(event EventTick
  (params (DeltaSeconds :type Float%20%28single-precision%29)))

(event EventBeginPlay
  (bind _capsule (Variables|Default|GetCapsule))
  (bind _returnvalue (Transformation|GetWorldTransform _capsule))
  (bind _location (Math|Transform|BreakTransform _returnvalue))
  (bind (_x _y) (Math|Vector|BreakVector _location))
  (Rendering|SetVisibility (Variables|Default|Getwidget_HPbar) false false)
  (Utilities|FlowControl|Delay 3.0)
  (bind _aspc_ingame (Utilities|Casting|CastToPC_Ingame (Game|GetPlayerController 0) :!label _label)
    (:then
      (Utilities|FlowControl|Delay (+ (Variables|Default|GetUnhideTime) (Math|Random|RandomFloatinRange -3.0 3.0)))
      (if (> (Math|Vector|VectorLength (- (Transformation|GetActorLocation (Variables|/Game/Ironsphere/Core/Framework/Battle/PC_Ingame.PC_Ingame_C|GetControlledMech _aspc_ingame)) _location)) 3e+02) :!label _label_2
        (if (> (Variables|Default|GetNumberOfWorms) 0) :!label _label_3
          (AI|SpawnAIFromClass (Variables|Default|GetClass) 0 (Math|Vector|MakeVector (+ _x (Math|Random|RandomFloatinRange -1e+02 1e+02)) (+ _y (Math|Random|RandomFloatinRange -1e+02 1e+02)) 0.0) "0, 0, 0" true 0)
          (Variables|Default|SetNumberOfWorms (- (Variables|Default|GetNumberOfWorms) 1))
          (Utilities|FlowControl|Delay (Math|Random|RandomFloatinRange 0.0 1.0))
          (goto _label_3))
        (else
          (Utilities|FlowControl|Delay 1.0)
          (goto _label_2))))
    (:CastFailed
      (Utilities|FlowControl|Delay 1.0)
      (goto _label))))

(fn ConstructionScript
  (|CallParentFunction))

(fn Destruction
  (params (IsBlow :type Boolean) (Damage :type Float%20%28double-precision%29) (Radius :type Float%20%28double-precision%29))
  (|CallParentFunction false 0.0 0.0))