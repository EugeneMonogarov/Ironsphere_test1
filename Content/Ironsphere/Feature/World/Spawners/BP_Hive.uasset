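; BP_Hive is a damageable enemy spawner that releases a limited stock of NPCs around itself.
; Tick spawns them at randomized intervals while GS_Battle's enemy count is below its cap.
; Dropping below 85% health triggers a one-time switch to the minimal cooldown, with a sound.
; BeginPlay adds minimap spawner and optional objective icons, hidden by KillWidgets, and swaps the den mesh to an airfield after mission 10.
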(event Game|Damage|EventAnyDamage
  (params (Damage :type Float%20%28single-precision%29) (DamageType :type Damage%20Type%20Object%20Reference) (InstigatedBy :type Controller%20Object%20Reference) (DamageCauser :type Actor%20Object%20Reference))
  (|CallParentFunction Damage DamageType InstigatedBy DamageCauser))

(event Collision|EventActorBeginOverlap
  (params (OtherActor :type Actor%20Object%20Reference))
  (|CallParentFunction OtherActor) ; This node is disabled and will not be called.\nDrag off pins to build functionality.
)

(event EventTick
  (params (DeltaSeconds :type Float%20%28single-precision%29))
  (bind _as_gs_battle (Variables|Default|GetAs%20GS%20Battle))
  (bind _spawnradius (Variables|Default|GetSpawnRadius))
  (Utilities|FlowControl|Sequence
    (:then_0
      (|CallParentFunction DeltaSeconds)
      (Variables|Default|SetSpawnTimer (- (Variables|Default|GetSpawnTimer) DeltaSeconds))
      (if (< (Variables|Default|GetCurrentHP) (* (Variables|Default|GetMaxHP) 0.85))
        (if (Variables|Default|GetExtraSpawn)
          _
          (else
            (Variables|Default|SetSpawnCooldown (Variables|Default|GetSpawnCooldownMinimal))
            (Variables|Default|SetSpawnTimer (Variables|Default|GetSpawnCooldownMinimal))
            (Variables|Default|SetExtraSpawn true)
            (Audio|SpawnSound2D "/Engine/VREditor/Sounds/UI/Foliage_Placed.Foliage_Placed" 1.0 1.0 0.0 0))))
      (if (> (Variables|Default|GetNumberOfNPC) 0)
        (if (and (<= (Variables|Default|GetSpawnTimer) 0.0) (< (Variables|/Game/Ironsphere/Core/Framework/Battle/GS_Battle.GS_Battle_C|GetNumberOfEnemies _as_gs_battle) (Variables|/Game/Ironsphere/Core/Framework/Battle/GS_Battle.GS_Battle_C|GetMaximalNumberOfEnemies _as_gs_battle)))
          (bind _returnvalue (AI|SpawnAIFromClass (Variables|Default|GetNPC) 0 (+ (+ (* (Math|Random|RandomUnitVector) (Math|Vector|MakeVector _spawnradius _spawnradius 0.0)) "0.000000,0.000000,40.000000") (Transformation|GetActorLocation)) "0, 0, 0" true 0))
          (Variables|Default|SetNumberOfNPC (- (Variables|Default|GetNumberOfNPC) 1))
          (Variables|Default|SetSpawnTimer (Math|Random|RandomFloatinRange 1.0 (* (Variables|Default|GetSpawnCooldown) 2.0))))))))

(event EventBeginPlay
  (bind _returnvalue (Transformation|GetActorLocation))
  (bind (_x _y) (Math|Vector|BreakVector _returnvalue))
  (bind _returnvalue_2 (* _x -0.1))
  (bind _returnvalue_3 (* _y -0.1))
  (bind _returnvalue_4 (+ _returnvalue_2 2e+02))
  (bind _returnvalue_5 (+ _returnvalue_3 2e+02))
  (bind _returnvalue_6 (Math|Vector2D|MakeVector2D _returnvalue_4 _returnvalue_5))
  (Utilities|FlowControl|Sequence
    (:then_0
      (bind _asgs_battle (Utilities|Casting|CastToGS_Battle (Game|GetGameState)))
      (Variables|Default|SetAs%20GS%20Battle _asgs_battle))
    (:then_1
      (Utilities|FlowControl|Delay 0.2)
      (|CallParentFunction)
      (bind _returnvalue_7 (UserInterface|CreateWidget "/Game/Ironsphere/UI/Ingame/Map/WBS_MinimapObject.WBS_MinimapObject_C" 0 "/Game/Ironsphere/UI/Ingame/Spawner.Spawner"))
      (Variables|Default|SetObjectMap _returnvalue_7)
      (UserInterface|Viewport|AddtoViewport _returnvalue_7 0)
      (Class|UserWidget|SetPositioninViewport _returnvalue_7 _returnvalue_6 true)
      (if (Variables|Default|GetIsLevelObjectiveMarker)
        (bind _returnvalue_8 (UserInterface|CreateWidget "/Game/Ironsphere/UI/Ingame/Map/WBS_MinimapObject.WBS_MinimapObject_C" 0 "/Game/Ironsphere/UI/Ingame/Map/Objective.Objective"))
        (Variables|Default|SetObjectiveMap _returnvalue_8)
        (UserInterface|Viewport|AddtoViewport _returnvalue_8 0)
        (Class|UserWidget|SetPositioninViewport _returnvalue_8 _returnvalue_6 true)))
    (:then_2
      (bind _outactors (Actor|GetAllActorsOfClass "/Game/Ironsphere/Feature/NPC/Hornet/BP_DesertWasp.BP_DesertWasp_C"))
      (Variables|Default|SetNumberOfWasps (Utilities|Array|Length _outactors)))
    (:then_3
      (bind _asgi_main (Utilities|Casting|CastToGI_Main (Game|GetGameInstance)))
      (if (> (Variables|/Game/Ironsphere/Core/Framework/GI_Main.GI_Main_C|GetCurrentMission _asgi_main) 10)
        (Components|StaticMesh|SetStaticMesh (Variables|Default|GetSpiderDen) "/Game/Ironsphere/3D/Meshes/NPCs/Airfield.Airfield")))))

(fn ConstructionScript
  (|CallParentFunction))

(fn Destruction
  (params (IsBlow :type Boolean) (Damage :type Float%20%28double-precision%29) (Radius :type Float%20%28double-precision%29) (Sound :type SoundDestroy%20Enum :default "NewEnumerator0"))
  (|CallParentFunction false 0.0 0.0 "NewEnumerator0"))

(fn KillWidgets
  (if (Variables|Default|GetIsLevelObjectiveMarker)
    (Widget|SetVisibility (Variables|Default|GetObjectiveMap) "Hidden"))
  (Widget|SetVisibility (Variables|Default|GetObjectMap) "Hidden"))