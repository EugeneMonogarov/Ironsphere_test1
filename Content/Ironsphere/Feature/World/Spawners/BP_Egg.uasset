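; BP_Egg is a world spawner egg that hatches into an AI NPC after a randomized cooldown, then removes itself.
; BeginPlay adds a position-mapped minimap marker and waits out a cooldown built from 15-second steps plus jitter.
; Hatching removes the mesh, spawns the NPC with pitch-varied sounds and calls Destruction.
; Destruction hides the marker, pays the money reward only when HP is depleted, and plays the destroy sound.
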(event Collision|EventActorBeginOverlap
  (params (OtherActor :type Actor%20Object%20Reference))
  (|CallParentFunction OtherActor) ; This node is disabled and will not be called.\nDrag off pins to build functionality.
)

(event EventTick
  (params (DeltaSeconds :type Float%20%28single-precision%29)))

(event EventBeginPlay
  (bind _returnvalue (Transformation|GetActorLocation))
  (bind _returnvalue_2 (Math|Random|RandomFloatinRange 0.5 1.5))
  (bind _returnvalue_3 (Transformation|GetActorLocation))
  (bind _returnvalue_4 (Transformation|GetActorLocation))
  (bind _spawncooldownmin (Variables|Default|GetSpawnCooldownMin))
  (bind _spawncooldownmax (Variables|Default|GetSpawnCooldownMax))
  (bind _returnvalue_5 (Math|Random|RandomFloatinRange _spawncooldownmin _spawncooldownmax))
  (bind (_x _y) (Math|Vector|BreakVector _returnvalue))
  (bind (_x_2 _y_2) (Math|Vector|BreakVector _returnvalue_3))
  (Utilities|FlowControl|Delay 0.2)
  (|CallParentFunction)
  (Rendering|SetVisibility (Variables|Default|Getwidget_HPbar) true false)
  (bind _returnvalue_6 (UserInterface|CreateWidget "/Game/Ironsphere/UI/Ingame/Map/WBS_MinimapObject.WBS_MinimapObject_C" 0 "/Game/Ironsphere/UI/Ingame/Spawner.Spawner"))
  (Variables|Default|SetMarker _returnvalue_6)
  (UserInterface|Viewport|AddtoViewport _returnvalue_6 0)
  (Class|UserWidget|SetPositioninViewport _returnvalue_6 (Math|Vector2D|MakeVector2D (+ (* _x -0.1) 2e+02) (+ (* _y -0.1) 2e+02)) true)
  (Utilities|FlowControl|Delay 1.0)
  (Utilities|FlowControl|Delay (+ (- _returnvalue_5 (Math|Float|%(Float) _returnvalue_5 15.0)) (Math|Random|RandomFloatinRange 0.0 2.0)))
  (Components|DestroyComponent (Variables|Default|GetEggMesh))
  (Components|Activation|SetActive (Variables|Default|GetCapsule1) false false)
  (AI|SpawnAIFromClass (Variables|Default|GetNPC) 0 (Math|Vector|MakeVector _x_2 _y_2 5.0) (Math|Random|RandomRotator true) true 0)
  (Audio|SpawnSoundatLocation "/Engine/VREditor/Sounds/UI/Foliage_Placed.Foliage_Placed" _returnvalue_4 "0, 0, 0" 0.8 _returnvalue_2 0.0 0 0)
  (Audio|SpawnSoundatLocation "/Game/Ironsphere/Sound/Impact/Rock/rock_impact_6.rock_impact_6" _returnvalue_4 "0, 0, 0" 0.4 _returnvalue_2 0.0 0 0)
  (CallFunction|Destruction false 0.0 0.0 "NewEnumerator0")
  (Actor|DestroyActor))

(fn ConstructionScript
  (|CallParentFunction))

(fn KillWidgets
  (bind _marker (Variables|Default|GetMarker))
  (bind _objectivemarker (Variables|Default|GetObjectiveMarker))
  (if (Utilities|IsValid _objectivemarker)
    (Widget|SetVisibility _objectivemarker "Hidden"))
  (if (Utilities|IsValid _marker)
    (Widget|SetVisibility _marker "Hidden")))

(fn Destruction
  (params (IsBlow :type Boolean) (Damage :type Float%20%28double-precision%29) (Radius :type Float%20%28double-precision%29) (Sound :type SoundDestroy%20Enum :default "NewEnumerator0"))
  (Widget|SetVisibility (Variables|Default|GetMarker) "Hidden")
  (if (<= (Variables|Default|GetCurrentHP) 0.0)
    (bind _asgi_main (Utilities|Casting|CastToGI_Main (Game|GetGameInstance)))
    (Variables|/Game/Ironsphere/Core/Framework/GI_Main.GI_Main_C|SetMoney _asgi_main (+ (Variables|/Game/Ironsphere/Core/Framework/GI_Main.GI_Main_C|GetMoney _asgi_main) (Variables|Default|GetReward))))
  (CallFunction|SoundDestroy "NewEnumerator3"))