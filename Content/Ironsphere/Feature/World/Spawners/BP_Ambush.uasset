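; BP_Ambush is a world spawner that releases a limited batch of NPCs (counted as worms) when the player's mech comes within range.
; BeginPlay hides the HP bar and retries until it gets the controlled mech from PC_Ingame.
; After an initial timer, Tick checks distance to the capsule and runs a Delay-driven loop spawning NPCs at random nearby XY offsets and zero Z, retrying failed spawns.
; Damage and destruction defer to the parent class.
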(event Game|Damage|EventAnyDamage
  (params (Damage :type Float%20%28single-precision%29) (DamageType :type Damage%20Type%20Object%20Reference) (InstigatedBy :type Controller%20Object%20Reference) (DamageCauser :type Actor%20Object%20Reference))
  (|CallParentFunction Damage DamageType InstigatedBy DamageCauser))

(event Collision|EventActorBeginOverlap
  (params (OtherActor :type Actor%20Object%20Reference))
  (|CallParentFunction OtherActor) ; This node is disabled and will not be called.\nDrag off pins to build functionality.
)

(event EventTick
  (params (DeltaSeconds :type Float%20%28single-precision%29))
  (bind _capsule (Variables|Default|GetCapsule))
  (bind _returnvalue (Transformation|GetWorldTransform _capsule))
  (bind _location (Math|Transform|BreakTransform _returnvalue))
  (bind (_x _y) (Math|Vector|BreakVector _location))
  (if (> (Variables|Default|GetTimerDelay) (Variables|Default|GetDelayTime))
    (Utilities|FlowControl|Delay 1.0)
    (if (> (Variables|Default|GetLenght) (Math|Vector|VectorLength (- (Transformation|GetActorLocation (Variables|Default|GetControlledMech_ref)) _location)))
      (if (> (Variables|Default|GetNumberOfWorms) 0) :!label _label
        (bind _returnvalue_2 (AI|SpawnAIFromClass (Variables|Default|GetNPC) 0 (Math|Vector|MakeVector (+ _x (Math|Random|RandomFloatinRange -1e+02 1e+02)) (+ _y (Math|Random|RandomFloatinRange -1e+02 1e+02)) 0.0) "0, 0, 0" true 0 :!label _label_2))
        (if (Utilities|IsValid _returnvalue_2)
          (Variables|Default|SetNumberOfWorms (- (Variables|Default|GetNumberOfWorms) 1))
          (Utilities|FlowControl|Delay (Math|Random|RandomFloatinRange 0.0 1.0))
          (goto _label)
          (else
            (Utilities|FlowControl|Delay 0.2)
            (goto _label_2)))))
    (else
      (Variables|Default|SetTimerDelay (+ DeltaSeconds (Variables|Default|GetTimerDelay))))))

(event EventBeginPlay
  (Rendering|SetVisibility (Variables|Default|Getwidget_HPbar) false false)
  (Utilities|FlowControl|Delay 0.5)
  (bind _aspc_ingame (Utilities|Casting|CastToPC_Ingame (Game|GetPlayerController 0) :!label _label)
    (:then
      (Variables|Default|SetControlledMech_ref (Variables|/Game/Ironsphere/Core/Framework/Battle/PC_Ingame.PC_Ingame_C|GetControlledMech _aspc_ingame)))
    (:CastFailed
      (Utilities|FlowControl|Delay 1.0)
      (goto _label))))

(fn ConstructionScript
  (|CallParentFunction))

(fn Destruction
  (params (IsBlow :type Boolean) (Damage :type Float%20%28double-precision%29) (Radius :type Float%20%28double-precision%29))
  (|CallParentFunction false 0.0 0.0))