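; BP_NearPlayerHide is a spawner that brings a limited number of AI "worms" out near the player's mech.
; On BeginPlay it waits briefly, retries until it finds the PC_Ingame controller, then waits a randomized UnhideTime.
; It then spawns the configured pawn class one by one at short random intervals until NumberOfWorms runs out.
; Each spawn uses the mech's current location plus a jittered random offset scaled by SpawnRadius, at world Z zero.
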(event Collision|EventActorBeginOverlap
  (params (OtherActor :type Actor%20Object%20Reference))
  (|CallParentFunction OtherActor) ; This node is disabled and will not be called.\nDrag off pins to build functionality.
)

(event EventTick
  (params (DeltaSeconds :type Float%20%28single-precision%29)))

(event EventBeginPlay
  (bind _spawnradius (Variables|Default|GetSpawnRadius))
  (Utilities|FlowControl|Delay 3.0)
  (bind _aspc_ingame (Utilities|Casting|CastToPC_Ingame (Game|GetPlayerController 0) :!label _label)
    (:then
      (Utilities|FlowControl|Delay (+ (Variables|Default|GetUnhideTime) (Math|Random|RandomFloatinRange -3.0 3.0)))
      (if (> (Variables|Default|GetNumberOfWorms) 0) :!label _label_2
        (AI|SpawnAIFromClass (Variables|Default|GetClass) 0 (Math|Vector|MakeVector (+ (.X (Math|Vector|BreakVector (+ (* (Math|Random|RandomUnitVector) (Math|Vector|MakeVector _spawnradius _spawnradius 0.0)) (Transformation|GetActorLocation (Variables|/Game/Ironsphere/Core/Framework/Battle/PC_Ingame.PC_Ingame_C|GetControlledMech _aspc_ingame))))) (Math|Random|RandomFloatinRange -1e+02 1e+02)) (+ (.Y (Math|Vector|BreakVector (+ (* (Math|Random|RandomUnitVector) (Math|Vector|MakeVector _spawnradius _spawnradius 0.0)) (Transformation|GetActorLocation (Variables|/Game/Ironsphere/Core/Framework/Battle/PC_Ingame.PC_Ingame_C|GetControlledMech _aspc_ingame))))) (Math|Random|RandomFloatinRange -1e+02 1e+02)) 0.0) "0, 0, 0" false 0)
        (Variables|Default|SetNumberOfWorms (- (Variables|Default|GetNumberOfWorms) 1))
        (Utilities|FlowControl|Delay (Math|Random|RandomFloatinRange 0.0 1.0))
        (goto _label_2)))
    (:CastFailed
      (Utilities|FlowControl|Delay 1.0)
      (goto _label))))

(fn ConstructionScript
  (|CallParentFunction))

(fn Destruction
  (|CallParentFunction))