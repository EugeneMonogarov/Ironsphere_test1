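; BP_EggsSpawner is a destructible world spawner that scatters a set number of BP_Egg actors around itself at game start.
; Once PC_Ingame is available, it spawns eggs at random nearby points, passing each its NPC class, cooldown range, HP and reward.
; Spawns blocked by collision retry with a gradually widening radius until the count runs out.
; Its destruction adds the egg reward to GI_Main's money, then runs the parent's destruction.
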(event Game|Damage|EventAnyDamage
  (params (Damage :type Float%20%28single-precision%29) (DamageType :type Damage%20Type%20Object%20Reference) (InstigatedBy :type Controller%20Object%20Reference) (DamageCauser :type Actor%20Object%20Reference))
  (|CallParentFunction Damage DamageType InstigatedBy DamageCauser))

(event Collision|EventActorBeginOverlap
  (params (OtherActor :type Actor%20Object%20Reference))
  (|CallParentFunction OtherActor) ; This node is disabled and will not be called.\nDrag off pins to build functionality.
)

(event EventTick
  (params (DeltaSeconds :type Float%20%28single-precision%29)))

(event EventBeginPlay
  (bind _eggshp (Variables|Default|GetEggsHP))
  (bind _capsule (Variables|Default|GetCapsule))
  (bind _returnvalue (Transformation|GetWorldTransform _capsule))
  (bind _location (Math|Transform|BreakTransform _returnvalue))
  (bind (_x _y) (Math|Vector|BreakVector _location))
  (Rendering|SetVisibility (Variables|Default|Getwidget_HPbar) false false)
  (Utilities|FlowControl|Delay 1.0)
  (bind _aspc_ingame (Utilities|Casting|CastToPC_Ingame (Game|GetPlayerController 0) :!label _label)
    (:then
      (if (> (Variables|Default|GetNumberOfEggs) 0) :!label _label_2
        (bind _returnvalue_2 (Game|SpawnActorfromClass "/Game/Ironsphere/Feature/World/Spawners/BP_Egg.BP_Egg_C" (Math|Conversions|ToTransform(Vector) (Math|Vector|MakeVector (+ _x (Math|Random|RandomFloatinRange (* (Variables|Default|GetSpawnRadiusEncrease) -1.0) (Variables|Default|GetSpawnRadiusEncrease))) (+ _y (Math|Random|RandomFloatinRange (* (Variables|Default|GetSpawnRadiusEncrease) -1.0) (Variables|Default|GetSpawnRadiusEncrease))) 15.0)) "DontSpawnIfColliding" "MultiplyWithRoot" 0 (Variables|Default|GetSpawnCooldownMin) (Variables|Default|GetNPC) (Variables|Default|GetSpawnCooldownMax) _eggshp _eggshp (Variables|Default|GetRewardForEggs) 0 :!label _label_3))
        (if (Utilities|IsValid _returnvalue_2)
          (Variables|Default|SetNumberOfEggs (- (Variables|Default|GetNumberOfEggs) 1))
          (Utilities|FlowControl|Delay (Math|Random|RandomFloatinRange 0.01 0.03))
          (goto _label_2)
          (else
            (Utilities|FlowControl|Delay 0.05)
            (Variables|Default|SetSpawnRadiusEncrease (+ (Variables|Default|GetSpawnRadiusEncrease) 1.0))
            (goto _label_3)))))
    (:CastFailed
      (Utilities|FlowControl|Delay 1.0)
      (goto _label))))

(fn ConstructionScript
  (|CallParentFunction))

(fn Destruction
  (params (IsBlow :type Boolean) (Damage :type Float%20%28double-precision%29) (Radius :type Float%20%28double-precision%29) (Sound :type SoundDestroy%20Enum :default "NewEnumerator0"))
  (bind _asgi_main (Utilities|Casting|CastToGI_Main (Game|GetGameInstance)))
  (Variables|/Game/Ironsphere/Core/Framework/GI_Main.GI_Main_C|SetMoney _asgi_main (+ (Variables|Default|GetRewardForEggs) (Variables|/Game/Ironsphere/Core/Framework/GI_Main.GI_Main_C|GetMoney _asgi_main)))
  (|CallParentFunction false 0.0 0.0 "NewEnumerator3"))