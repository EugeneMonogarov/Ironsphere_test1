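; Green fuel barrel Blueprint, a damageable world prop that can explode and irradiates nearby characters when destroyed.
; Health bar updates and damage handling defer to the parent, with a sound on spawn and on each hit.
; Its Destruction override skips the parent's: a blow adds radial falloff damage, a radius-scaled explosion and camera shake.
; Either way it removes widgets and gives characters within close range a timed negative Radiation buff.
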(event EventBeginPlay
  (|CallParentFunction)
  (Rendering|SetVisibility (Variables|Default|Getwidget_HPbar) true false)
  (Audio|PlaySound2D "/Game/Ironsphere/Sound/Devices/mechanical_002.mechanical_002" 1.0 2.0 0.0 0 0))

(event Collision|EventActorBeginOverlap
  (params (OtherActor :type Actor%20Object%20Reference)))

(event EventTick
  (params (DeltaSeconds :type Float%20%28single-precision%29))
  (|CallParentFunction DeltaSeconds)
  (CallFunction|UpdateHPbar))

(event Game|Damage|EventAnyDamage
  (params (Damage :type Float%20%28single-precision%29) (DamageType :type Damage%20Type%20Object%20Reference) (InstigatedBy :type Controller%20Object%20Reference) (DamageCauser :type Actor%20Object%20Reference))
  (|CallParentFunction Damage DamageType InstigatedBy DamageCauser)
  (CallFunction|SoundDamage "NewEnumerator0"))

(fn ConstructionScript)

(fn UpdateHPbar
  (|CallParentFunction))

(fn SoundDamage
  (params (SoundDamage :type SoundDamage%20Enum :default "NewEnumerator0"))
  (|CallParentFunction "NewEnumerator0"))

(fn Destruction
  (params (IsBlow :type Boolean) (Damage :type Float%20%28double-precision%29) (Radius :type Float%20%28double-precision%29) (Sound :type SoundDestroy%20Enum :default "NewEnumerator0"))
  (bind _returnvalue (Transformation|GetActorLocation))
  (bind (_x _y) (Math|Vector|BreakVector _returnvalue))
  (if IsBlow
    (CallFunction|SoundDestroy "NewEnumerator2")
    (Class|GameplayStatics|ApplyRadialDamagewithFalloff Damage 0.0 (Math|Vector|MakeVector _x _y 1e+01) 0.0 Radius 0.2 "/Game/Ironsphere/Feature/Consumable/DamageTypes/BP_PhysicalDamage.BP_PhysicalDamage_C" 0 self 0 "ECC_Visibility")
    (Effects|SpawnEmitteratLocation "/Game/StarterContent/Particles/P_Explosion.P_Explosion" _returnvalue "0, 0, 0" (Math|Conversions|ToVector(Float) (/ (Math|Float|Sqrt (Math|Float|Sqrt Radius)) 3.0)))
    (Class|LegacyCameraShake|StartLegacyCameraShake (Game|GetPlayerCameraManager 0) "/Game/Ironsphere/Core/Player/CamShakeBlow.CamShakeBlow_C" (/ Damage 1e+01) "CameraLocal" "0, 0, 0")
    (else
      (CallFunction|SoundDestroy "NewEnumerator0")))
  (CallFunction|KillWidgets)
  (bind _outactors (Actor|GetAllActorsOfClass "/Game/Ironsphere/Core/Character/BP_CharacterBase.BP_CharacterBase_C"))
  (for _array_element _outactors
    (if (< (Math|Vector|VectorLength (- (Transformation|GetActorLocation _array_element) (Transformation|GetActorLocation))) 1.3e+02)
      (Default|AddBuff _array_element (Utilities|Struct|MakeST_buff "NewEnumerator7" -4.0 12.0 false "Radiation" "/Game/Ironsphere/UI/Icons/Buffs/Fire.Fire")))))