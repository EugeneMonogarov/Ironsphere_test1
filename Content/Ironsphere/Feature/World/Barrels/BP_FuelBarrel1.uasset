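; BP_FuelBarrel1 is a fuel barrel world object that inherits its health bar and damage behavior from a parent Blueprint.
; It makes the HP bar widget visible at BeginPlay and updates it every Tick through the parent's UpdateHPbar.
; On any damage it calls the parent handler, then triggers a damage sound through a SoundDamage override that always passes the same enum value to the parent.
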(event EventBeginPlay
  (|CallParentFunction)
  (Rendering|SetVisibility (Variables|Default|Getwidget_HPbar) true false))

(event Collision|EventActorBeginOverlap
  (params (OtherActor :type Actor%20Object%20Reference)))

(event EventTick
  (params (DeltaSeconds :type Float%20%28single-precision%29))
  (|CallParentFunction DeltaSeconds)
  (CallFunction|UpdateHPbar))

(event Game|Damage|EventAnyDamage
  (params (Damage :type Float%20%28single-precision%29) (DamageType :type Damage%20Type%20Object%20Reference) (InstigatedBy :type Controller%20Object%20Reference) (DamageCauser :type Actor%20Object%20Reference))
  (|CallParentFunction Damage DamageType InstigatedBy DamageCauser)
  (CallFunction|SoundDamage "NewEnumerator0"))

(fn ConstructionScript)

(fn UpdateHPbar
  (|CallParentFunction))

(fn SoundDamage
  (params (SoundDamage :type SoundDamage%20Enum :default "NewEnumerator0"))
  (|CallParentFunction "NewEnumerator0"))