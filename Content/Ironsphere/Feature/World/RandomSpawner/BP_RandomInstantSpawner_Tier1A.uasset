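; Tier 1A random enemy spawner that places one hidden group or egg nest at its own location as soon as play begins.
; BeginPlay removes the placeholder cube, then a weighted random roll picks a BP_Hide ambush of grey worms, flying eyes, sand spiders or tiger leeches, or a BP_EggsSpawner of grey worm eggs.
; Group sizes are randomized per type, and the Delay variable drives unhide time and egg spawn cooldown.
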(event EventBeginPlay
  (bind _delay (Variables|Default|GetDelay))
  (Components|DestroyComponent (Variables|Default|GetCube))
  (Variables|Default|Setrandom (Math|Random|RandomFloatinRange 0.0 1e+02))
  (if (< (Variables|Default|Getrandom) 25.0)
    (Game|SpawnActorfromClass "/Game/Ironsphere/Feature/World/Spawners/BP_Hide.BP_Hide_C" (Transformation|GetActorTransform) "AlwaysSpawn" "MultiplyWithRoot" 0 (Variables|Default|GetDelay) (Math|Random|RandomIntegerinRange 5 7) "/Game/Ironsphere/Feature/NPC/Worm/BP_GreyWorm.BP_GreyWorm_C" 2.5e+02 2.5e+02 0)
    (elif (< (Variables|Default|Getrandom) 5e+01)
      (Game|SpawnActorfromClass "/Game/Ironsphere/Feature/World/Spawners/BP_EggsSpawner.BP_EggsSpawner_C" (Transformation|GetActorTransform) "AlwaysSpawn" "MultiplyWithRoot" 0 _delay (+ _delay 3.0) (Math|Random|RandomIntegerinRange 5 7) "/Game/Ironsphere/Feature/NPC/Worm/BP_GreyWorm.BP_GreyWorm_C" 2e+01 2.5e+02 2.5e+02 0)
      (elif (< (Variables|Default|Getrandom) 75.0)
        (Game|SpawnActorfromClass "/Game/Ironsphere/Feature/World/Spawners/BP_Hide.BP_Hide_C" (Transformation|GetActorTransform) "AlwaysSpawn" "MultiplyWithRoot" 0 (Variables|Default|GetDelay) (Math|Random|RandomIntegerinRange 3 4) "/Game/Ironsphere/Feature/NPC/Hornet/BP_FlyingEye.BP_FlyingEye_C" 2.5e+02 2.5e+02 0)
        (elif (< (Variables|Default|Getrandom) 87.0)
          (Game|SpawnActorfromClass "/Game/Ironsphere/Feature/World/Spawners/BP_Hide.BP_Hide_C" (Transformation|GetActorTransform) "AlwaysSpawn" "MultiplyWithRoot" 0 (Variables|Default|GetDelay) (Math|Random|RandomIntegerinRange 1 2) "/Game/Ironsphere/Feature/NPC/Spider/BP_SandSpider.BP_SandSpider_C" 2.5e+02 2.5e+02 0)
          (else
            (Game|SpawnActorfromClass "/Game/Ironsphere/Feature/World/Spawners/BP_Hide.BP_Hide_C" (Transformation|GetActorTransform) "AlwaysSpawn" "MultiplyWithRoot" 0 (Variables|Default|GetDelay) (Math|Random|RandomIntegerinRange 3 5) "/Game/Ironsphere/Feature/NPC/Worm/BP_TigerLeech.BP_TigerLeech_C" 2.5e+02 2.5e+02 0)))))))

(event Collision|EventActorBeginOverlap
  (params (OtherActor :type Actor%20Object%20Reference)))

(event EventTick
  (params (DeltaSeconds :type Float%20%28single-precision%29)))

(fn ConstructionScript)