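; Tier 1 random world spawner that replaces its placeholder cube with one randomly chosen enemy encounter or fuel barrel at its transform.
; On BeginPlay, nested percentage rolls mostly pick hides or ambushes of worms, wasps, spiders or leeches.
; Less often they pick a den, hive or barrel.
; Each spawn receives its NPC class and tuning, with counts, unhide times and den cooldowns often randomized.
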(event EventBeginPlay
  (Components|DestroyComponent (Variables|Default|GetCube))
  (if (> (Math|Random|RandomFloatinRange 0.0 1e+02) 22.0)
    (if (> (Math|Random|RandomFloatinRange 0.0 1e+02) 6e+01)
      (if (> (Math|Random|RandomFloatinRange 0.0 1e+02) 5e+01)
        (Game|SpawnActorfromClass "/Game/Ironsphere/Feature/World/Spawners/BP_Hide.BP_Hide_C" (Transformation|GetActorTransform) "Undefined" "MultiplyWithRoot" 0 (Math|Random|RandomFloatinRange 0.0 1.6e+02) (Math|Random|RandomIntegerinRange 4 8) "/Game/Ironsphere/Feature/NPC/Worm/BP_GreyWorm.BP_GreyWorm_C" 2.5e+02 2.5e+02 0)
        (else
          (Game|SpawnActorfromClass "/Game/Ironsphere/Feature/World/Spawners/BP_Ambush.BP_Ambush_C" (Transformation|GetActorTransform) "Undefined" "MultiplyWithRoot" 0 (Math|Random|RandomIntegerinRange 3 5) "/Game/Ironsphere/Feature/NPC/Worm/BP_GreyWorm.BP_GreyWorm_C" 2.5e+02 2.5e+02 0)))
      (elif (> (Math|Random|RandomFloatinRange 0.0 1e+02) 66.0)
        (Game|SpawnActorfromClass "/Game/Ironsphere/Feature/World/Spawners/BP_Hide.BP_Hide_C" (Transformation|GetActorTransform) "Undefined" "MultiplyWithRoot" 0 (Math|Random|RandomFloatinRange 0.0 1.6e+02) (Math|Random|RandomIntegerinRange 2 5) "/Game/Ironsphere/Feature/NPC/Hornet/BP_DesertWasp.BP_DesertWasp_C" 2.5e+02 2.5e+02 0)
        (elif (> (Math|Random|RandomFloatinRange 0.0 1e+02) 66.0)
          (if (> (Math|Random|RandomFloatinRange 0.0 1e+02) 5e+01)
            (Game|SpawnActorfromClass "/Game/Ironsphere/Feature/World/Spawners/BP_Hide.BP_Hide_C" (Transformation|GetActorTransform) "Undefined" "MultiplyWithRoot" 0 (Math|Random|RandomFloatinRange 0.0 1.6e+02) (Math|Random|RandomIntegerinRange 2 4) "/Game/Ironsphere/Feature/NPC/Worm/BP_TigerLeech.BP_TigerLeech_C" 2.5e+02 2.5e+02 0)
            (else
              (Game|SpawnActorfromClass "/Game/Ironsphere/Feature/World/Spawners/BP_Ambush.BP_Ambush_C" (Transformation|GetActorTransform) "Undefined" "MultiplyWithRoot" 0 (Math|Random|RandomIntegerinRange 2 4) "/Game/Ironsphere/Feature/NPC/Worm/BP_GreyWorm.BP_GreyWorm_C" 2.5e+02 2.5e+02 0)))
          (else
            (Game|SpawnActorfromClass "/Game/Ironsphere/Feature/World/Spawners/BP_Hide.BP_Hide_C" (Transformation|GetActorTransform) "Undefined" "MultiplyWithRoot" 0 (Math|Random|RandomFloatinRange 0.0 1.6e+02) (Math|Random|RandomIntegerinRange 2 4) "/Game/Ironsphere/Feature/NPC/Spider/BP_DesertSpider.BP_DesertSpider_C" 2.5e+02 2.5e+02 0)))))
    (elif (> (Math|Random|RandomFloatinRange 0.0 1e+02) 66.0)
      (Game|SpawnActorfromClass "/Game/Ironsphere/Feature/World/Spawners/BP_Den.BP_Den_C" (Transformation|GetActorTransform) "Undefined" "MultiplyWithRoot" 0 (Math|Random|RandomFloatinRange 2e+01 35.0) 15.0 "/Game/Ironsphere/Feature/NPC/Spider/BP_DesertSpider.BP_DesertSpider_C" 5e+01 3 2 0.9 false 1.2e+02 1.2e+02 0)
      (elif (> (Math|Random|RandomFloatinRange 0.0 1e+02) 66.0)
        (if (> (Math|Random|RandomFloatinRange 0.0 1e+02) 5e+01)
          (Game|SpawnActorfromClass "/Game/Ironsphere/Feature/World/Spawners/BP_Hive.BP_Hive_C" (Transformation|GetActorTransform) "Undefined" "MultiplyWithRoot" 0 15.0 1.5 "/Game/Ironsphere/Feature/NPC/Hornet/BP_DesertWasp.BP_DesertWasp_C" 5e+01 15 1 0.9 false 8e+01 8e+01 0)
          (else
            (Game|SpawnActorfromClass "/Game/Ironsphere/Feature/World/Spawners/BP_Den.BP_Den_C" (Transformation|GetActorTransform) "Undefined" "MultiplyWithRoot" 0 (Math|Random|RandomFloatinRange 3e+01 4e+01) 15.0 "/Game/Ironsphere/Feature/NPC/Spider/BP_SandSpider.BP_SandSpider_C" 5e+01 (Math|Random|RandomIntegerinRange 1 2) 1 0.9 false 1.5e+02 1.5e+02 0)))
        (else
          (Game|SpawnActorfromClass "/Game/Ironsphere/Feature/World/Barrels/BP_FuelBarrel1.BP_FuelBarrel1_C" (Transformation|GetActorTransform) "Undefined" "MultiplyWithRoot" 0 12.0 12.0 0))))))

(event Collision|EventActorBeginOverlap
  (params (OtherActor :type Actor%20Object%20Reference)))

(event EventTick
  (params (DeltaSeconds :type Float%20%28single-precision%29)))

(fn ConstructionScript)