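; Tier 2 random world spawner that places one enemy spawner at its own transform on BeginPlay, after removing its placeholder Cube.
; Nested random rolls pick either a BP_Den of giant, red or dark widow spiders, or a BP_Hive of hornets or flying eyes.
; Each spawned actor receives its NPC class and tuning, with some cooldowns and pack sizes randomized.
; Disconnected Hide, Ambush and fuel barrel branches never run.
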(event EventBeginPlay
  (Components|DestroyComponent (Variables|Default|GetCube))
  (if (> (Math|Random|RandomFloatinRange 0.0 1e+02) 75.0)
    (Game|SpawnActorfromClass "/Game/Ironsphere/Feature/World/Spawners/BP_Den.BP_Den_C" (Transformation|GetActorTransform) "Undefined" "MultiplyWithRoot" 0 (Math|Random|RandomFloatinRange 3e+01 33.0) 18.0 "/Game/Ironsphere/Feature/NPC/Spider/BP_GiantSpider.BP_GiantSpider_C" 5e+01 1 1 0.9 false 1.2e+02 1.2e+02 0)
    (elif (> (Math|Random|RandomFloatinRange 0.0 1e+02) 66.0)
      (if (> (Math|Random|RandomFloatinRange 0.0 1e+02) 4e+01)
        (if (> (Math|Random|RandomFloatinRange 0.0 1e+02) 5e+01)
          (Game|SpawnActorfromClass "/Game/Ironsphere/Feature/World/Spawners/BP_Hive.BP_Hive_C" (Transformation|GetActorTransform) "Undefined" "MultiplyWithRoot" 0 15.0 1.5 "/Game/Ironsphere/Feature/NPC/Hornet/BP_Hornet.BP_Hornet_C" 5e+01 25 1 0.9 false 1.2e+02 1.2e+02 0)
          (else
            (Game|SpawnActorfromClass "/Game/Ironsphere/Feature/World/Spawners/BP_Hive.BP_Hive_C" (Transformation|GetActorTransform) "Undefined" "MultiplyWithRoot" 0 8.0 1.0 "/Game/Ironsphere/Feature/NPC/Hornet/BP_FlyingEye.BP_FlyingEye_C" 5e+01 45 1 0.9 false 1.2e+02 1.2e+02 0)))
        (else
          (Game|SpawnActorfromClass "/Game/Ironsphere/Feature/World/Spawners/BP_Den.BP_Den_C" (Transformation|GetActorTransform) "Undefined" "MultiplyWithRoot" 0 (Math|Random|RandomFloatinRange 34.0 4e+01) 19.0 "/Game/Ironsphere/Feature/NPC/Spider/BP_DarkWidow.BP_DarkWidow_C" 5e+01 (Math|Random|RandomIntegerinRange 1 2) 1 0.9 false 1.2e+02 1.2e+02 0)))
      (else
        (Game|SpawnActorfromClass "/Game/Ironsphere/Feature/World/Spawners/BP_Den.BP_Den_C" (Transformation|GetActorTransform) "Undefined" "MultiplyWithRoot" 0 (Math|Random|RandomFloatinRange 34.0 4e+01) 19.0 "/Game/Ironsphere/Feature/NPC/Spider/BP_RedSpider.BP_RedSpider_C" 5e+01 3 1 0.9 false 1.2e+02 1.2e+02 0)))))

(event Collision|EventActorBeginOverlap
  (params (OtherActor :type Actor%20Object%20Reference)))

(event EventTick
  (params (DeltaSeconds :type Float%20%28single-precision%29)))

(fn ConstructionScript)