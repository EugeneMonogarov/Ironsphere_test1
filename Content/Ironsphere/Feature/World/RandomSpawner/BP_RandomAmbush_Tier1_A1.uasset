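; Tier 1 random ambush spawner that places one randomly chosen enemy encounter at its location when play begins.
; On BeginPlay it destroys its Cube component, waits a delay, then runs a chain of weighted random rolls.
; The rolls spawn either a randomly rotated plant at fixed height, a flying eye, or a BP_Ambush configured with spider, leech, needle worm or grey worm NPCs and a count.
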(event EventBeginPlay
  (bind _returnvalue (Transformation|GetActorTransform))
  (bind _location (Math|Transform|BreakTransform _returnvalue))
  (bind (_x _y) (Math|Vector|BreakVector _location))
  (Components|DestroyComponent (Variables|Default|GetCube))
  (Utilities|FlowControl|Delay (Variables|Default|GetDelay))
  (if (> (Math|Random|RandomFloatinRange 0.0 1e+02) 8e+01)
    (AI|SpawnAIFromClass "/Game/Ironsphere/Feature/NPC/Plant/BP_Plant.BP_Plant_C" 0 (Math|Vector|MakeVector _x _y 22.0) (Math|Rotator|MakeRotator 0.0 0.0 (Math|Random|RandomFloatinRange 0.0 3.6e+02)) false 0)
    (elif (> (Math|Random|RandomFloatinRange 0.0 1e+02) 85.0)
      (Game|SpawnActorfromClass "/Game/Ironsphere/Feature/World/Spawners/BP_Ambush.BP_Ambush_C" _returnvalue "Undefined" "MultiplyWithRoot" 0 1 "/Game/Ironsphere/Feature/NPC/Spider/BP_SandSpider.BP_SandSpider_C" 0.0 3e+02 2.5e+02 2.5e+02 0)
      (elif (> (Math|Random|RandomFloatinRange 0.0 1e+02) 5e+01)
        (if (> (Math|Random|RandomFloatinRange 0.0 1e+02) 5e+01)
          (if (> (Math|Random|RandomFloatinRange 0.0 1e+02) 5e+01)
            (Game|SpawnActorfromClass "/Game/Ironsphere/Feature/World/Spawners/BP_Ambush.BP_Ambush_C" (Transformation|GetActorTransform) "Undefined" "MultiplyWithRoot" 0 (Math|Random|RandomIntegerinRange 2 3) "/Game/Ironsphere/Feature/NPC/Worm/BP_TigerLeech.BP_TigerLeech_C" 0.0 3e+02 2.5e+02 2.5e+02 0)
            (else
              (Game|SpawnActorfromClass "/Game/Ironsphere/Feature/World/Spawners/BP_Ambush.BP_Ambush_C" (Transformation|GetActorTransform) "Undefined" "MultiplyWithRoot" 0 (Math|Random|RandomIntegerinRange 1 2) "/Game/Ironsphere/Feature/NPC/Worm/BP_NeedleWorm.BP_NeedleWorm_C" 0.0 3e+02 2.5e+02 2.5e+02 0)))
          (else
            (AI|SpawnAIFromClass "/Game/Ironsphere/Feature/NPC/Hornet/BP_FlyingEye.BP_FlyingEye_C" 0 (.Location (Math|Transform|BreakTransform (Transformation|GetActorTransform))) "0, 0, 0" false 0)))
        (else
          (Game|SpawnActorfromClass "/Game/Ironsphere/Feature/World/Spawners/BP_Ambush.BP_Ambush_C" (Transformation|GetActorTransform) "Undefined" "MultiplyWithRoot" 0 (Math|Random|RandomIntegerinRange 4 5) "/Game/Ironsphere/Feature/NPC/Worm/BP_GreyWorm.BP_GreyWorm_C" 0.0 3e+02 2.5e+02 2.5e+02 0))))))

(event Collision|EventActorBeginOverlap
  (params (OtherActor :type Actor%20Object%20Reference)))

(event EventTick
  (params (DeltaSeconds :type Float%20%28single-precision%29)))

(fn ConstructionScript)