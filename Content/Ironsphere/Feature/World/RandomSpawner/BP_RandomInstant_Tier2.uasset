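; BP_RandomInstant_Tier2 is a placeable Tier 2 random spawner that creates one group of hostile-creature NPCs at its location.
; On BeginPlay it removes its Cube component, waits a random delay, then spawns a BP_Hide configured with zero UnhideTime, an NPC class and a randomized count.
; Cascading percentage rolls give roughly equal odds to SandSpider, NeedleWorm, Hornet, RedSpider and TigerLeech, each with its own count range.
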(event EventBeginPlay
  (Components|DestroyComponent (Variables|Default|GetCube))
  (Utilities|FlowControl|Delay (Math|Random|RandomFloatinRange (Variables|Default|GetDelayMin) (Variables|Default|GetDelayMax)))
  (if (> (Math|Random|RandomFloatinRange 0.0 1e+02) 2e+01)
    (if (> (Math|Random|RandomFloatinRange 0.0 1e+02) 25.0)
      (if (> (Math|Random|RandomFloatinRange 0.0 1e+02) 33.0)
        (if (> (Math|Random|RandomFloatinRange 0.0 1e+02) 5e+01)
          (Game|SpawnActorfromClass "/Game/Ironsphere/Feature/World/Spawners/BP_Hide.BP_Hide_C" (Transformation|GetActorTransform) "Undefined" "MultiplyWithRoot" 0 0.0 (Math|Random|RandomIntegerinRange 5 9) "/Game/Ironsphere/Feature/NPC/Worm/BP_TigerLeech.BP_TigerLeech_C" 2.5e+02 2.5e+02 0)
          (else
            (Game|SpawnActorfromClass "/Game/Ironsphere/Feature/World/Spawners/BP_Hide.BP_Hide_C" (Transformation|GetActorTransform) "Undefined" "MultiplyWithRoot" 0 0.0 (Math|Random|RandomIntegerinRange 3 4) "/Game/Ironsphere/Feature/NPC/Spider/BP_RedSpider.BP_RedSpider_C" 2.5e+02 2.5e+02 0)))
        (else
          (Game|SpawnActorfromClass "/Game/Ironsphere/Feature/World/Spawners/BP_Hide.BP_Hide_C" (Transformation|GetActorTransform) "Undefined" "MultiplyWithRoot" 0 0.0 (Math|Random|RandomIntegerinRange 3 6) "/Game/Ironsphere/Feature/NPC/Hornet/BP_Hornet.BP_Hornet_C" 2.5e+02 2.5e+02 0)))
      (else
        (Game|SpawnActorfromClass "/Game/Ironsphere/Feature/World/Spawners/BP_Hide.BP_Hide_C" (Transformation|GetActorTransform) "Undefined" "MultiplyWithRoot" 0 0.0 (Math|Random|RandomIntegerinRange 4 6) "/Game/Ironsphere/Feature/NPC/Worm/BP_NeedleWorm.BP_NeedleWorm_C" 2.5e+02 2.5e+02 0)))
    (else
      (Game|SpawnActorfromClass "/Game/Ironsphere/Feature/World/Spawners/BP_Hide.BP_Hide_C" (Transformation|GetActorTransform) "Undefined" "MultiplyWithRoot" 0 0.0 (Math|Random|RandomIntegerinRange 7 10) "/Game/Ironsphere/Feature/NPC/Spider/BP_SandSpider.BP_SandSpider_C" 2.5e+02 2.5e+02 0))))

(event Collision|EventActorBeginOverlap
  (params (OtherActor :type Actor%20Object%20Reference)))

(event EventTick
  (params (DeltaSeconds :type Float%20%28single-precision%29)))

(fn ConstructionScript)