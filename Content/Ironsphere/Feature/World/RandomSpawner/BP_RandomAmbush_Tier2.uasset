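; Tier 2 random spawner that places either plants or an enemy ambush at its location in the world.
; On BeginPlay it removes its Cube component, waits a delay, then rolls nested random chances.
; The likeliest branch spawns BP_Plant AI at jittered positions with random yaw, retrying failed spawns after a short delay.
; Otherwise it spawns BP_Ambush configured with a random count of sand spiders, tiger leeches, red spiders or needle worms.
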(event EventBeginPlay
  (bind _returnvalue (Transformation|GetActorTransform))
  (bind _location (Math|Transform|BreakTransform _returnvalue))
  (bind (_x _y) (Math|Vector|BreakVector _location))
  (Components|DestroyComponent (Variables|Default|GetCube))
  (Utilities|FlowControl|Delay (Variables|Default|GetDelay))
  (if (> (Math|Random|RandomFloatinRange 0.0 1e+02) 4e+01)
    (for _index (range 0 2)
      (Variables|Default|SetCount 0)
      (bind _returnvalue_2 (AI|SpawnAIFromClass "/Game/Ironsphere/Feature/NPC/Plant/BP_Plant.BP_Plant_C" 0 (Math|Vector|MakeVector (+ _x (Math|Random|RandomFloatinRange -1e+02 1e+02)) (+ _y (Math|Random|RandomFloatinRange -1e+02 1e+02)) 55.0) (Math|Rotator|MakeRotator 0.0 0.0 (Math|Random|RandomFloatinRange -1.8e+02 1.8e+02)) false 0 :!label _label))
      (bind _result (Math|Integer|IncrementInt (Variables|Default|GetCount))
        (:%20%20
          (if (not (and (< _result 4) (Utilities|IsValid _returnvalue_2)))
            (Utilities|FlowControl|Delay 0.2)
            (goto _label)))))
    (elif (> (Math|Random|RandomFloatinRange 0.0 1e+02) 75.0)
      (Game|SpawnActorfromClass "/Game/Ironsphere/Feature/World/Spawners/BP_Ambush.BP_Ambush_C" (Transformation|GetActorTransform) "Undefined" "MultiplyWithRoot" 0 (Math|Random|RandomIntegerinRange 3 5) "/Game/Ironsphere/Feature/NPC/Spider/BP_SandSpider.BP_SandSpider_C" 0.0 3e+02 2.5e+02 2.5e+02 0)
      (elif (> (Math|Random|RandomFloatinRange 0.0 1e+02) 33.0)
        (if (> (Math|Random|RandomFloatinRange 0.0 1e+02) 5e+01)
          (Game|SpawnActorfromClass "/Game/Ironsphere/Feature/World/Spawners/BP_Ambush.BP_Ambush_C" (Transformation|GetActorTransform) "Undefined" "MultiplyWithRoot" 0 (Math|Random|RandomIntegerinRange 4 7) "/Game/Ironsphere/Feature/NPC/Worm/BP_TigerLeech.BP_TigerLeech_C" 0.0 3e+02 2.5e+02 2.5e+02 0)
          (else
            (Game|SpawnActorfromClass "/Game/Ironsphere/Feature/World/Spawners/BP_Ambush.BP_Ambush_C" (Transformation|GetActorTransform) "Undefined" "MultiplyWithRoot" 0 (Math|Random|RandomIntegerinRange 3 5) "/Game/Ironsphere/Feature/NPC/Spider/BP_RedSpider.BP_RedSpider_C" 0.0 3e+02 2.5e+02 2.5e+02 0)))
        (else
          (Game|SpawnActorfromClass "/Game/Ironsphere/Feature/World/Spawners/BP_Ambush.BP_Ambush_C" (Transformation|GetActorTransform) "Undefined" "MultiplyWithRoot" 0 (Math|Random|RandomIntegerinRange 3 5) "/Game/Ironsphere/Feature/NPC/Worm/BP_NeedleWorm.BP_NeedleWorm_C" 0.0 3e+02 2.5e+02 2.5e+02 0))))))

(event Collision|EventActorBeginOverlap
  (params (OtherActor :type Actor%20Object%20Reference)))

(event EventTick
  (params (DeltaSeconds :type Float%20%28single-precision%29)))

(fn ConstructionScript)