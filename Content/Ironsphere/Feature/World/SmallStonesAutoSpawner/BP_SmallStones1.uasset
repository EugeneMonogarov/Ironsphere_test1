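; BP_SmallStones1 is a self-propagating scatter actor that places randomized small stones on world geometry.
; On BeginPlay it picks one of three meshes (cases 4–6 are unreachable), then randomizes its scale and rotation.
; It usually spawns a smaller copy of itself nearby, forming recursive chains with no depth limit.
; It then jitters its horizontal position and snaps to a WorldStatic sphere-trace hit, destroying itself on a miss.
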(event EventBeginPlay
  (bind _returnvalue (Transformation|GetActorTransform))
  (bind _returnvalue_2 (Math|Random|RandomFloatinRange 0.12 0.4))
  (bind _returnvalue_3 (Math|Random|RandomFloatinRange 0.8 1.2))
  (bind _self self)
  (bind _smallstone1 (Variables|Default|GetSmallStone1))
  (bind _smallstone1_2 (Variables|Default|GetSmallStone1))
  (bind _returnvalue_4 (Math|Float|Power _returnvalue_3 4.0))
  (bind (_location _rotation _scale) (Math|Transform|BreakTransform _returnvalue))
  (bind _returnvalue_5 (Transformation|GetActorTransform _self))
  (bind (_location_2 _rotation_2 _scale_2) (Math|Transform|BreakTransform _returnvalue_5))
  (Utilities|FlowControl|Sequence
    (:then_0
      (switch int (Math|Random|RandomIntegerinRange 1 3)
        (:1
          (Components|StaticMesh|SetStaticMesh _smallstone1_2 "/Game/Ironsphere/3D/Meshes/Props/SmallStones/SmallStone1.SmallStone1"))
        (:2
          (Components|StaticMesh|SetStaticMesh _smallstone1_2 "/Game/Ironsphere/3D/Meshes/Props/SmallStones/SmallStone2.SmallStone2"))
        (:3
          (Components|StaticMesh|SetStaticMesh _smallstone1_2 "/Game/Ironsphere/3D/Meshes/Props/SmallStones/SmallStone3.SmallStone3"))
        (:4
          (Components|StaticMesh|SetStaticMesh _smallstone1_2 "/Game/Ironsphere/3D/Meshes/Props/SmallStones/SmallStone4.SmallStone4"))
        (:5
          (Components|StaticMesh|SetStaticMesh _smallstone1_2 "/Game/Ironsphere/3D/Meshes/Props/SmallStones/SmallStone5.SmallStone5"))
        (:6
          (Components|StaticMesh|SetStaticMesh _smallstone1_2 "/Game/Ironsphere/3D/Meshes/Props/SmallStones/SmallStone6.SmallStone6"))))
    (:then_1
      (Transformation|SetRelativeScale3D _smallstone1 (Math|Vector|MakeVector _returnvalue_4 _returnvalue_4 _returnvalue_4))
      (Transformation|SetRelativeRotation _smallstone1 (Math|Random|RandomRotator false) false false))
    (:then_2
      (if (> (Math|Random|RandomIntegerinRange 0 12) 2)
        (Game|SpawnActorfromClass "BP_SmallStones1_C" (Math|Transform|MakeTransform (+ _location (* (Math|Random|RandomUnitVector) "33.000000,33.000000,0.000000")) "0, 0, 0" (* _scale (Math|Vector|MakeVector _returnvalue_2 _returnvalue_2 _returnvalue_2))) "Undefined" "MultiplyWithRoot" 0 0)))
    (:then_3
      (Transformation|SetActorTransform (Math|Transform|MakeTransform (+ (* (Math|Random|RandomUnitVector) (Math|Vector|MakeVector (Math|Float|Power (Math|Random|RandomFloatinRange 0.0 3.0) 3.0) (Math|Float|Power (Math|Random|RandomFloatinRange 0.0 3.0) 3.0) 0.0)) _location_2) _rotation_2 _scale_2))
      (bind (_outhit _returnvalue_6) (Collision|SphereTraceForObjects (+ (Transformation|GetActorLocation) "0.000000,0.000000,300.000000") (+ (Transformation|GetActorLocation) "0.000000,0.000000,-300.000000") 0.0 (Utilities|Array|MakeArray "ObjectTypeQuery1") false (Utilities|Array|MakeArray _self) "None"))
      (if _returnvalue_6
        (Transformation|SetActorLocation (.Location (Collision|BreakHitResult _outhit)) false false)
        (else
          (Actor|DestroyActor))))))

(event Collision|EventActorBeginOverlap
  (params (OtherActor :type Actor%20Object%20Reference)))

(event EventTick
  (params (DeltaSeconds :type Float%20%28single-precision%29)))

(fn ConstructionScript)