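; Self-replicating ruin stone that scatters random clusters of debris across the world on BeginPlay.
; Each instance randomizes its mesh, stretch and 45-degree yaw, then usually spawns another BP_RuinsSpawner nearby, forming a probabilistic chain.
; It jitters its position, occasionally jumps farther, then sphere-traces vertically against WorldStatic to snap to the hit point.
; It destroys itself when the trace misses, hits above zero height or lands too close to actors from a class query.
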(event EventBeginPlay
  (bind _returnvalue (Math|Random|RandomFloatinRange 0.9 1.2))
  (bind _self self)
  (bind _smallstone1 (Variables|Default|GetSmallStone1))
  (bind _smallstone1_2 (Variables|Default|GetSmallStone1))
  (bind _returnvalue_2 (Math|Float|Power _returnvalue 5.0))
  (bind _returnvalue_3 (Transformation|GetActorTransform _self))
  (bind (_location _rotation _scale) (Math|Transform|BreakTransform _returnvalue_3))
  (Utilities|FlowControl|Sequence
    (:then_0
      (switch int (Math|Random|RandomIntegerinRange 1 6)
        (:1
          (Components|StaticMesh|SetStaticMesh _smallstone1_2 "/Game/Ironsphere/3D/Meshes/Props/Ruins/Ruins_Ruins000.Ruins_Ruins000"))
        (:2
          (Components|StaticMesh|SetStaticMesh _smallstone1_2 "/Game/Ironsphere/3D/Meshes/Props/Ruins/Ruins_Ruins001.Ruins_Ruins001"))
        (:3
          (Components|StaticMesh|SetStaticMesh _smallstone1_2 "/Game/Ironsphere/3D/Meshes/Props/Ruins/Ruins_Ruins002.Ruins_Ruins002"))
        (:4
          (Components|StaticMesh|SetStaticMesh _smallstone1_2 "/Game/Ironsphere/3D/Meshes/Props/Ruins/Ruins_Ruins003.Ruins_Ruins003"))
        (:5
          (Components|StaticMesh|SetStaticMesh _smallstone1_2 "/Game/Ironsphere/3D/Meshes/Props/SmallStones/SmallStone5.SmallStone5"))
        (:6
          (Components|StaticMesh|SetStaticMesh _smallstone1_2 "/Game/Ironsphere/3D/Meshes/Props/Ruins/Ruins_Ruins005.Ruins_Ruins005"))))
    (:then_1
      (Transformation|SetRelativeScale3D _smallstone1 (Math|Vector|MakeVector _returnvalue_2 _returnvalue_2 1.0))
      (Transformation|SetRelativeRotation _smallstone1 (Math|Rotator|MakeRotator 0.0 0.0 (Math|Conversions|ToFloat(Integer) (* (Math|Random|RandomIntegerinRange 0 7) 45))) false false))
    (:then_2
      (if (> (Math|Random|RandomIntegerinRange 0 22) 1)
        (Game|SpawnActorfromClass "BP_RuinsSpawner_C" (Math|Transform|MakeTransform (+ (.Location (Math|Transform|BreakTransform (Transformation|GetActorTransform))) (* (Math|Random|RandomUnitVector) "33.000000,33.000000,0.000000"))) "Undefined" "MultiplyWithRoot" 0 0)))
    (:then_3
      (Transformation|SetActorTransform (Math|Transform|MakeTransform (+ (* (Math|Random|RandomUnitVector) (Math|Random|RandomFloatinRange 15.0 255.0)) _location) _rotation _scale))
      (if (> (Math|Random|RandomIntegerinRange 0 12) 11)
        (Transformation|SetActorLocation (+ (Math|Vector|MakeVector (Math|Random|RandomFloatinRange 33.0 444.0) (Math|Random|RandomFloatinRange 33.0 444.0) 0.0) (Transformation|GetActorLocation)) false false))
      (bind (_outhit _returnvalue_4) (Collision|SphereTraceForObjects (+ (Transformation|GetActorLocation) "0.000000,0.000000,300.000000") (+ (Transformation|GetActorLocation) "0.000000,0.000000,-300.000000") 0.0 (Utilities|Array|MakeArray "ObjectTypeQuery1") false (Utilities|Array|MakeArray _self) "None"))
      (if (<= (.Z (Math|Vector|BreakVector (.Location (Collision|BreakHitResult _outhit)))) 0.0)
        (if _returnvalue_4
          (bind _outactors (Actor|GetAllActorsOfClass 0))
          (for _array_element _outactors
            (if (not (> (Math|Vector|VectorLength (- (.Location (Collision|BreakHitResult _outhit)) (Transformation|GetActorLocation _array_element))) 35.0))
              (Actor|DestroyActor)))
          (Transformation|SetActorLocation (.Location (Collision|BreakHitResult _outhit)) false false)
          (else
            (Actor|DestroyActor :!label _label)))
        (else
          (goto _label))))))

(event Collision|EventActorBeginOverlap
  (params (OtherActor :type Actor%20Object%20Reference)))

(event EventTick
  (params (DeltaSeconds :type Float%20%28single-precision%29)))

(fn ConstructionScript)