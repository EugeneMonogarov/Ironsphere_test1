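; Base ammo projectile actor that serves as either a straight shot or a self-propelled missile.
; Shots use ProjectileMovement and lose damage linearly beyond range, vanishing at double range; missiles move on Tick with accuracy-based yaw wobble around launch heading, exploding at randomized range.
; Overlapping non-owners deals randomized damage, buffs characters, and triggers ricochet sounds, impact effects and optional radial explosion.
; Missiles ignore overlaps within blast radius of their owner.
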(event EventBeginPlay
  (Variables|/Game/Ironsphere/Feature/Consumable/DamageTypes/BP_DamageComponent.BP_DamageComponent_C|SetComponentArmorPenetration (Variables|Default|GetBP_ArmorPenetration) (Variables|Default|GetProjectileArmorPenetration))
  (Variables|/Game/Ironsphere/Feature/Consumable/DamageTypes/BP_Buffs.BP_Buffs_C|SetComponent_Buff (Variables|Default|GetBP_Buffs) "")
  (if (Variables|Default|GetMissile)
    (Variables|Default|SetRangeMultyplier 1)
    (else
      (Variables|Default|SetRangeMultyplier 2)))
  (Variables|Default|SetStartPosition (Transformation|GetActorLocation)))

(event Collision|EventActorBeginOverlap
  (params (OtherActor :type Actor%20Object%20Reference))
  (bind _returnvalue (Transformation|GetActorLocation))
  (bind _returnvalue_2 (Math|Random|RandomFloatinRange 0.0 0.1))
  (bind _returnvalue_3 (Transformation|GetActorLocation))
  (bind _returnvalue_4 (Components|GetOwner))
  (bind _returnvalue_5 (Math|Random|RandomFloatinRange 0.8 1.2))
  (bind _returnvalue_6 (Math|Random|RandomFloatinRange 0.8 1.2))
  (bind _returnvalue_7 (Math|Random|RandomFloatinRange 0.8 1.2))
  (bind _returnvalue_8 (Math|Random|RandomFloatinRange 0.8 1.2))
  (bind _projectileexplosionradius (Variables|Default|GetProjectileExplosionRadius))
  (bind _projectileexplosionradius_2 (Variables|Default|GetProjectileExplosionRadius))
  (bind _returnvalue_9 (* _returnvalue_8 _returnvalue_6 _returnvalue_5 _returnvalue_7))
  (if (!= OtherActor _returnvalue_4)
    (if (Variables|Default|GetMissile)
      (if (> (Math|Vector|VectorLength (- (Transformation|GetActorLocation _returnvalue_4) (Transformation|GetActorLocation))) (Variables|Default|GetProjectileExplosionRadius))
        (if (not (Variables|Default|Getunable)) :!label _label
          (if (<= (Math|Vector|Distance(Vector) (Variables|Default|GetStartPosition) (Transformation|GetActorLocation)) (Variables|Default|GetProjectileRange))
            (Variables|Default|SetIncomingDamage (* (Variables|Default|GetProjectileDamage) _returnvalue_9))
            (else
              (Variables|Default|SetIncomingDamage (* (* (Variables|Default|GetProjectileDamage) (- 1.0 (/ (- (Math|Vector|Distance(Vector) (Variables|Default|GetStartPosition) (Transformation|GetActorLocation)) (Variables|Default|GetProjectileRange)) (Variables|Default|GetProjectileRange)))) _returnvalue_9))))
          (bind _asbp_character_base (Utilities|Casting|CastToBP_CharacterBase OtherActor)
            (:then
              (if (not (Utilities|Enum|Equal(Enum) (.Parameter (Utilities|Struct|BreakST_buff (Variables|Default|GetProjectileBuff))) "NewEnumerator6"))
                (Default|AddBuff _asbp_character_base (Variables|Default|GetProjectileBuff))))
            (:CastFailed
              _))
          (Game|Damage|ApplyDamage OtherActor (Variables|Default|GetIncomingDamage) 0 self "/Game/Ironsphere/Feature/Consumable/DamageTypes/BP_PhysicalDamage.BP_PhysicalDamage_C")
          (switch int (Math|Random|RandomInteger 7)
            (:Default
              (Audio|SpawnSoundatLocation "/Game/Ironsphere/Sound/Shot/Ricoshet/Ricochet1.Ricochet1" _returnvalue "0, 0, 0" _returnvalue_2 1.0 0.0 0 0 :!label _label_2))
            (:0
              (goto _label_2))
            (:1
              (Audio|SpawnSoundatLocation "/Game/Ironsphere/Sound/Shot/Ricoshet/Ricochet2.Ricochet2" _returnvalue "0, 0, 0" _returnvalue_2 1.0 0.0 0 0))
            (:2
              (Audio|SpawnSoundatLocation "/Game/Ironsphere/Sound/Shot/Ricoshet/Ricochet3.Ricochet3" _returnvalue "0, 0, 0" _returnvalue_2 1.0 0.2 0 0))
            (:3
              (goto _label_2)))
          (if (and (> (Variables|Default|GetProjectileExplosionDamge) 0.0) (> (Variables|Default|GetProjectileExplosionRadius) 0.0))
            (Class|GameplayStatics|ApplyRadialDamagewithFalloff (Variables|Default|GetProjectileExplosionDamge) 0.0 (Transformation|GetActorLocation) (/ _projectileexplosionradius_2 5.0) _projectileexplosionradius_2 0.5 "/Game/Ironsphere/Feature/Consumable/DamageTypes/BP_PhysicalDamage.BP_PhysicalDamage_C" 0 self 0 "ECC_Camera")
            (Effects|SpawnEmitteratLocation "/Game/StarterContent/Particles/P_Explosion.P_Explosion" (Transformation|GetActorLocation) "0, 0, 0" (Math|Conversions|ToVector(Float) (/ _projectileexplosionradius 1e+02)))
            (Audio|SpawnSoundatLocation "/Game/StarterContent/Audio/Explosion01.Explosion01" "0, 0, 0" "0, 0, 0" (/ _projectileexplosionradius 2e+02) 12.0 0.2 0 0))
          (Effects|SpawnEmitteratLocation "/Game/StarterContent/Particles/P_Explosion.P_Explosion" _returnvalue_3 "0, 0, 0" (Math|Conversions|ToVector(Float) (/ (Math|Float|Sqrt (Variables|Default|GetIncomingDamage)) 4e+01)))
          (Audio|SpawnSoundatLocation "/Game/Ironsphere/Sound/Impact/metal_impact_3.metal_impact_3" _returnvalue_3 "0, 0, 0" (/ (Math|Float|Sqrt (Variables|Default|GetIncomingDamage)) 4e+01) (/ 1.0 (/ (Math|Float|Sqrt (Variables|Default|GetIncomingDamage)) 4e+01)) 0.0 0 0)
          (Variables|Default|Setunable true)
          (Utilities|FlowControl|Delay 0.1)
          (Actor|DestroyActor)))
      (else
        (goto _label)))))

(event EventTick
  (params (DeltaSeconds :type Float%20%28single-precision%29))
  (bind _returnvalue (Transformation|GetActorLocation))
  (bind _projectileexplosionradius (Variables|Default|GetProjectileExplosionRadius))
  (bind _incomingdamage (Variables|Default|GetIncomingDamage))
  (bind _projectileexplosionradius_2 (Variables|Default|GetProjectileExplosionRadius))
  (bind _returnvalue_2 (Math|Float|Sqrt _incomingdamage))
  (bind _returnvalue_3 (/ _returnvalue_2 4e+01))
  (if (not (Variables|Default|Getunable))
    (if (Variables|Default|GetMissile)
      (Utilities|FlowControl|Sequence
        (:then_0
          (Transformation|AddActorLocalOffset self (Math|Vector|MakeVector (* DeltaSeconds (Variables|Default|GetProjectileVelocity)) 0.0 0.0) false false))
        (:then_1
          (if (> (Variables|Default|GetMissileRandomTimer) 0.0)
            (Variables|Default|SetMissileRandomTimer (- (Variables|Default|GetMissileRandomTimer) DeltaSeconds))
            (else
              (Variables|Default|SetMissileRandomTimer (Math|Random|RandomFloatinRange 0.05 0.1))
              (Transformation|AddRelativeRotation (Variables|Default|GetDefaultSceneRoot) (Math|Rotator|MakeRotator 0.0 0.0 (+ (* (.Yaw (Math|Rotator|BreakRotator (Math|Rotator|Delta(Rotator) (Math|Rotator|MakeRotator 0.0 0.0 (.Yaw (Math|Rotator|BreakRotator (Transformation|GetActorRotation)))) (Math|Rotator|MakeRotator 0.0 0.0 (Variables|Default|GetMissileRotationOnStart))))) -0.3) (* (Math|Random|RandomFloatinRange -13.0 13.0) (- 1.0 (Variables|Default|GetMissileAccuracy))))) false false))))
        (:then_2
          (if (>= (Math|Vector|Distance(Vector) (Variables|Default|GetStartPosition) (Transformation|GetActorLocation)) (* (Variables|Default|GetProjectileRange) (Variables|Default|GetRangeMultyplier))) :!label _label
            (if (Variables|Default|GetMissile)
              (Class|GameplayStatics|ApplyRadialDamagewithFalloff (Variables|Default|GetProjectileExplosionDamge) 0.0 (Transformation|GetActorLocation) (/ _projectileexplosionradius_2 5.0) _projectileexplosionradius_2 0.5 "/Game/Ironsphere/Feature/Consumable/DamageTypes/BP_PhysicalDamage.BP_PhysicalDamage_C" 0 self 0 "ECC_Camera")
              (Effects|SpawnEmitteratLocation "/Game/StarterContent/Particles/P_Explosion.P_Explosion" (Transformation|GetActorLocation) "0, 0, 0" (Math|Conversions|ToVector(Float) (/ _projectileexplosionradius 1e+02)))
              (Audio|SpawnSoundatLocation "/Game/StarterContent/Audio/Explosion01.Explosion01" "0, 0, 0" "0, 0, 0" (/ _projectileexplosionradius 2e+02) 12.0 0.2 0 0)
              (Effects|SpawnEmitteratLocation "/Game/StarterContent/Particles/P_Explosion.P_Explosion" _returnvalue "0, 0, 0" (Math|Conversions|ToVector(Float) _returnvalue_3))
              (Audio|SpawnSoundatLocation "/Game/Ironsphere/Sound/Impact/metal_impact_3.metal_impact_3" _returnvalue "0, 0, 0" _returnvalue_3 (/ 1.0 _returnvalue_3) 0.0 0 0)
              (Variables|Default|Setunable true)
              (Utilities|FlowControl|Delay 0.1)
              (Actor|DestroyActor)
              (else
                (Actor|DestroyActor))))))
      (else
        (goto _label)))))

(fn ConstructionScript
  (bind _projectilemovement (Variables|Default|GetProjectileMovement))
  (if (Variables|Default|GetMissile)
    (Variables|/Script/Engine.ProjectileMovementComponent|SetbSimulationEnabled (Variables|Default|GetProjectileMovement) false)
    (Variables|Default|SetMissileRotationOnStart (.Yaw (Math|Rotator|BreakRotator (Transformation|GetActorRotation self))))
    (Variables|Default|SetProjectileRange (* (Variables|Default|GetProjectileRange) (Math|Random|RandomFloatinRange 0.7 1.3)))
    (else
      (bind _output_get (Variables|/Script/Engine.ProjectileMovementComponent|SetInitialSpeed _projectilemovement (Variables|Default|GetProjectileVelocity)))
      (Variables|/Script/Engine.ProjectileMovementComponent|SetMaxSpeed _projectilemovement _output_get))))