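; BP_NPC01 is an AI-controlled NPC with health, a widget HP bar and a list of enemy pawns.
; Damage records the attacker as an enemy, updates the bar, may randomly set panic on its BP_AI_controller, and at zero health triggers an explosion and destroys the NPC.
; Sensor overlaps add pawns to the enemy list or remove them after a random delay.
; AttackRange overlaps tell the controller whether the first enemy is in range.
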(event OnComponentBeginOverlap(sensorIn)
  (params (OverlappedComponent :type Primitive%20Component%20Object%20Reference) (OtherActor :type Actor%20Object%20Reference) (OtherComp :type Primitive%20Component%20Object%20Reference) (OtherBodyIndex :type Integer) (bFromSweep :type Boolean) (SweepResult :type Hit%20Result%20Structure%20%28by%20ref%29))
  (bind _aspawn (Utilities|Casting|CastToPawn OtherActor))
  (if (!= OtherActor self)
    (Utilities|Array|AddUnique (Variables|Default|GetEnemy) _aspawn)))

(event OnComponentEndOverlap(sensorOut)
  (params (OverlappedComponent :type Primitive%20Component%20Object%20Reference) (OtherActor :type Actor%20Object%20Reference) (OtherComp :type Primitive%20Component%20Object%20Reference) (OtherBodyIndex :type Integer))
  (bind _aspawn (Utilities|Casting|CastToPawn OtherActor)
    (:then
      (if (Utilities|Array|ContainsItem (Variables|Default|GetEnemy) _aspawn)
        (Utilities|FlowControl|Delay (Math|Random|RandomFloatinRange 2.0 5.0))
        (Utilities|Array|RemoveItem (Variables|Default|GetEnemy) _aspawn)))
    (:CastFailed
      (Development|PrintString "Enemy Fail"))))

(event OnComponentBeginOverlap(AttackRange)
  (params (OverlappedComponent :type Primitive%20Component%20Object%20Reference) (OtherActor :type Actor%20Object%20Reference) (OtherComp :type Primitive%20Component%20Object%20Reference) (OtherBodyIndex :type Integer) (bFromSweep :type Boolean) (SweepResult :type Hit%20Result%20Structure%20%28by%20ref%29))
  (if (!= OtherActor self)
    (if (== OtherActor (Utilities|Array|Get(acopy) (Variables|Default|GetEnemy)))
      (bind _asbp_ai_controller (Utilities|Casting|CastToBP_AI_controller (AI|GetAIController self)))
      (Variables|/Game/NPC/BP_AI_controller.BP_AI_controller_C|SetTargetInRange _asbp_ai_controller true))))

(event OnComponentEndOverlap(AttackRange)
  (params (OverlappedComponent :type Primitive%20Component%20Object%20Reference) (OtherActor :type Actor%20Object%20Reference) (OtherComp :type Primitive%20Component%20Object%20Reference) (OtherBodyIndex :type Integer))
  (if (!= OtherActor self)
    (if (== OtherActor (Utilities|Array|Get(acopy) (Variables|Default|GetEnemy)))
      (bind _asbp_ai_controller (Utilities|Casting|CastToBP_AI_controller (AI|GetAIController self)))
      (Variables|/Game/NPC/BP_AI_controller.BP_AI_controller_C|SetTargetInRange _asbp_ai_controller false))))

(event EventBeginPlay
  (bind _aswbc_hehth_bar (Utilities|Casting|CastToWBC_HehthBar (UserInterface|GetWidget (Variables|Default|Getwidget_HPbar))))
  (bind _output_get (Variables|Default|SetAIInfoWidget _aswbc_hehth_bar))
  (Default|UpdateHP _output_get 1.0)
  (Default|UpdateText _output_get (Utilities|Text|ToText(Float) (Variables|Default|GetCurrentHP) "HalfToEven"))
  (Variables|Default|SetCurrentHP (Variables|Default|GetMaxHP))
  (bind _asbp_ai_controller (Utilities|Casting|CastToBP_AI_controller (AI|GetAIController self))
    (:then
      (Variables|Default|SetAI_controller_var _asbp_ai_controller))
    (:CastFailed
      (Development|PrintString "AIC_fail"))))

(event Collision|EventActorBeginOverlap
  (params (OtherActor :type Actor%20Object%20Reference)))

(event EventTick
  (params (DeltaSeconds :type Float%20%28single-precision%29)))

(event Game|Damage|EventAnyDamage
  (params (Damage :type Float%20%28single-precision%29) (DamageType :type Damage%20Type%20Object%20Reference) (InstigatedBy :type Controller%20Object%20Reference) (DamageCauser :type Actor%20Object%20Reference))
  (bind _aiinfowidget (Variables|Default|GetAIInfoWidget))
  (bind _aspawn (Utilities|Casting|CastToPawn DamageCauser))
  (Variables|Default|SetLastDamageDealer _aspawn)
  (Development|PrintString "Hello" true true "(R=0.000000,G=0.660000,B=1.000000,A=1.000000)" 1.0)
  (Utilities|Array|AddUnique (Variables|Default|GetEnemy) _aspawn)
  (Variables|Default|SetCurrentHP (- (Variables|Default|GetCurrentHP) Damage))
  (Default|UpdateHP _aiinfowidget (/ (Variables|Default|GetCurrentHP) (Variables|Default|GetMaxHP)))
  (Default|UpdateText _aiinfowidget (Utilities|Text|ToText(Float) (Variables|Default|GetCurrentHP) "HalfToEven" false true 1 324 0 0))
  (if (<= (Math|Random|RandomFloatinRange 0.0 5.0) (/ Damage (Variables|Default|GetCurrentHP)))
    (Variables|/Game/NPC/BP_AI_controller.BP_AI_controller_C|SetIsPanic (Variables|Default|GetAI_controller_var) true)
    (Development|PrintString "AAAAAAAAAAAAAAAA"))
  (if (<= (Variables|Default|GetCurrentHP) 0.0)
    (Effects|SpawnEmitteratLocation "/Game/StarterContent/Particles/P_Explosion.P_Explosion" (Transformation|GetActorLocation) "0, 0, 0" "3.000000,3.000000,3.000000")
    (Actor|DestroyActor)))

(fn ConstructionScript)