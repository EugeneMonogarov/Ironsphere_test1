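; AI controller for BP_NPC01 that wanders between random nearby points and chases the NPC's Enemy whenever one is set.
; Tick advances timers, checks for an enemy, and alternates random idle pauses with moves toward a target.
; Steering sets Move and Turn, applied as unswept local offsets and yaw steps, without navigation or a running behavior tree.
; Panic, Possess, Attack and MoveTo are empty stubs, and debug prints remain.
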(event Custom|MoveTo
  (params (NewParam :type Float%20%28double-precision%29)))

(event Custom|Attack)

(event Custom|Panic)

(event EventBeginPlay
  (Variables|Default|SetIdle true)
  (bind _asbp_npc01 (Utilities|Casting|CastToBP_NPC01 (Pawn|GetControlledPawn))
    (:then
      (Variables|Default|SetNPC01_var _asbp_npc01))
    (:CastFailed
      (Development|PrintString "AI fail"))))

(event EventTick
  (params (DeltaSeconds :type Float%20%28single-precision%29))
  (CallFunction|Timers DeltaSeconds)
  (CallFunction|MovementControl DeltaSeconds)
  (CallFunction|UpdateStates)
  (CallFunction|UpdateDirection "0, 0, 0")
  (Development|PrintString (Utilities|String|Append "Move:" (Utilities|String|ToString(Float) (Variables|Default|GetMove)) "Turn:" (Utilities|String|ToString(Float) (Variables|Default|GetTurn))) true true "(R=0.000000,G=0.660000,B=1.000000,A=1.000000)" 0.0)
  (if (Variables|Default|GetHasEnemy)
    (Variables|Default|SetMove 1.0)
    (bind _output_get (Variables|Default|SetMoveTargetLocation (Transformation|GetActorLocation (Variables|/Game/NPC/BP_NPC01.BP_NPC01_C|GetEnemy (Variables|Default|GetNPC01_var)))))
    (CallFunction|UpdateDirection _output_get)
    (elif (Variables|Default|GetIdle)
      (if (> (Variables|Default|GetTimerIdle) (Variables|Default|GetIdleRandomDelay))
        (Variables|Default|SetIdle false)
        (CallFunction|UpdateMoveTargetLoc)
        (Development|PrintString "MoveTargetLoc updated")
        (Variables|Default|SetMove (Math|Random|RandomFloatinRange 0.2 0.9))
        (else
          (Variables|Default|SetTurn 0.0)
          (Variables|Default|SetMove 0.0)
          (Development|PrintString "Idle" true true "(R=0.000000,G=0.660000,B=1.000000,A=1.000000)" 0.0)))
      (elif (> (Math|Vector|Distance(Vector) (Transformation|GetActorLocation (Pawn|GetControlledPawn)) (Variables|Default|GetMoveTargetLocation)) 3e+01)
        (CallFunction|UpdateDirection (Variables|Default|GetMoveTargetLocation))
        (else
          (Variables|Default|SetIdle true)
          (Variables|Default|SetIdleRandomDelay (+ (Math|Random|RandomFloatinRange 0.0 3.0) (Math|Random|RandomFloatinRange 0.0 3.0) (Math|Random|RandomFloatinRange 0.0 3.0)))
          (Variables|Default|SetTimerIdle 0.0))))))

(event EventPossess
  (params (PossessedPawn :type Pawn%20Object%20Reference)))

(fn ConstructionScript)

(fn MovementControl
  (params (B :type Float%20%28double-precision%29))
  (bind _returnvalue (Pawn|GetControlledPawn))
  (Transformation|AddActorLocalOffset _returnvalue (Math|Vector|MakeVector (* (Variables|Default|GetMove) B (Variables|Default|GetMaxVelocity)) 0.0 0.0) false false)
  (Transformation|AddRelativeRotation (Variables|/Script/Engine.Actor|GetRootComponent _returnvalue) (Math|Rotator|MakeRotator 0.0 0.0 (Variables|Default|GetTurn)) false false))

(fn UpdateStates
  (bind _npc01_var (Variables|Default|GetNPC01_var))
  (bind _enemy (Variables|/Game/NPC/BP_NPC01.BP_NPC01_C|GetEnemy _npc01_var))
  (if true
    (bind _output_get (Variables|Default|SetHasEnemy (Utilities|IsValid _enemy)))
    (Development|PrintString (Utilities|GetDisplayName _enemy) true true "(R=0.000000,G=0.660000,B=1.000000,A=1.000000)" 0.0)))

(fn Timers
  (params (dT :type Float%20%28double-precision%29))
  (bind _output_get (Variables|Default|SetTimerIdle (+ (Variables|Default|GetTimerIdle) dT)))
  (bind _output_get_2 (Variables|Default|SetTimeAgressiveCooldown (+ (Variables|Default|GetTimeAgressiveCooldown) dT)))
  (bind _output_get_3 (Variables|Default|SetTimePanic (+ (Variables|Default|GetTimePanic) dT))))

(fn UpdateDirection
  (params (A :type Vector))
  (bind _returnvalue (Pawn|GetControlledPawn))
  (bind _npc01_var (Variables|Default|GetNPC01_var))
  (bind _returnvalue_2 (Transformation|GetActorLocation _returnvalue))
  (bind _rootcomponent (Variables|/Script/Engine.Actor|GetRootComponent _npc01_var))
  (bind _returnvalue_3 (Transformation|GetWorldRotation _rootcomponent))
  (bind _returnvalue_4 (- A _returnvalue_2))
  (bind _returnvalue_5 (Math|Vector|Normalize _returnvalue_4))
  (bind _returnvalue_6 (Math|Conversions|RotationFromXVector _returnvalue_5))
  (bind _yaw (Math|Rotator|BreakRotator _returnvalue_6))
  (bind _returnvalue_7 (Math|Rotator|MakeRotator 0.0 0.0 _yaw))
  (bind _returnvalue_8 (Math|Rotator|Delta(Rotator) _returnvalue_3 _returnvalue_7))
  (bind _yaw_2 (Math|Rotator|BreakRotator _returnvalue_8))
  (if (> (Math|Float|Absolute(Float) _yaw_2) 2.0)
    (bind _output_get (Variables|Default|SetTurn (* (Math|Float|Sign(Float) _yaw_2) -1.0)))
    (else
      (Variables|Default|SetTurn 0.0))))

(fn UpdateMoveTargetLoc
  (bind _returnvalue (Pawn|GetControlledPawn))
  (bind _returnvalue_2 (Transformation|GetActorLocation _returnvalue))
  (bind (_x _y) (Math|Vector|BreakVector _returnvalue_2))
  (bind _output_get (Variables|Default|SetMoveTargetLocation (Math|Vector|MakeVector (+ _x (Math|Random|RandomFloatinRange -2.5e+02 2.5e+02)) (+ _y (Math|Random|RandomFloatinRange -2.5e+02 2.5e+02)) 0.0) :!label _label))
  (if (not (< (Math|Vector|Distance(Vector) _returnvalue_2 _output_get) 1.5e+02))
    (goto _label)))